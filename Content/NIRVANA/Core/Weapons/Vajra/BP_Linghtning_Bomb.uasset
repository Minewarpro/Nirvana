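; Lightning bomb projectile for the Vajra weapon that flies along an initial direction and zaps targets around it.
; A looping timer sphere-overlaps enemies, or bosses if the Boss flag is set, dealing tick damage with Niagara electric beams and setting a fixed speed when targets are in range.
; On hit it explodes, damaging nearby BP_Enemy pawns in both modes, then destroys itself.
; The construction script scales the ring effect to the tick radius.
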(event `LaunchTickBoss`
  (bind _is_slowing (`self.Is Slowing`))
  (bind (_outactors _returnvalue) (`KismetSystemLibrary.SphereOverlapActors` (`self.K2_GetActorLocation`) (`self.Tick Radius`) (`|MakeArray` "ObjectTypeQuery2" :!type "EObjectTypeQuery Enum") "/Game/NIRVANA/Core/Characters/Enemies/Boss/BP_Boss.BP_Boss_C"))
  (if _returnvalue
    (if (not _is_slowing)
      (`self.Set Velocity` (select `bool` _returnvalue :`false` (`self.Velocity Power`) :`true` 500.0 :!type "Float (single-precision)") :!label _label))
    (elif _is_slowing
      (goto _label)
      (else
        _)))
  (for _array_element _outactors
    (message `/Game/NIRVANA/Core/Characters/FirstPerson/BPI_Hit.Hit` _array_element (`self.Tick Damage`))
    (`self.Spawn ElectricBeam` _array_element)))

(event `self.ReceiveBeginPlay`
  (`PrimitiveComponent.SetPhysicsLinearVelocity` (`self.Collision`) (* (`self.Init Velocity Direction`) (`self.Velocity Power`)) false "None")
  (if (`self.boss`)
    (`KismetSystemLibrary.K2_SetTimerDelegate` (delegate `LaunchTickBoss`) 0.4 true -0.2)
    (else
      (`KismetSystemLibrary.K2_SetTimerDelegate` (delegate `Laucnh Tick`) 0.4 true -0.2))))

(event `Laucnh Tick`
  (bind _is_slowing (`self.Is Slowing`))
  (bind (_outactors _returnvalue) (`KismetSystemLibrary.SphereOverlapActors` (`self.K2_GetActorLocation`) (`self.Tick Radius`) (`|MakeArray` "ObjectTypeQuery3" :!type "EObjectTypeQuery Enum") "/Game/NIRVANA/Core/Characters/Enemies/Common/BP_Enemy.BP_Enemy_C"))
  (if _returnvalue
    (if (not _is_slowing)
      (`self.Set Velocity` (select `bool` _returnvalue :`false` (`self.Velocity Power`) :`true` 500.0 :!type "Float (single-precision)") :!label _label_2))
    (elif _is_slowing
      (goto _label_2)
      (else
        _)))
  (for _array_element _outactors
    (message `/Game/NIRVANA/Core/Characters/FirstPerson/BPI_Hit.Hit` _array_element (`self.Tick Damage`))
    (`self.Spawn ElectricBeam` _array_element)))

(event `/Game/NIRVANA/Core/Characters/FirstPerson/BPI_Hit.Hit`
  (params (Damages :type "Float (double-precision)"))
  (`self.Explode`))

(event `Explode`
  (bind _outactors (`KismetSystemLibrary.SphereOverlapActors` (`self.K2_GetActorLocation`) 1000.0 (`|MakeArray` "ObjectTypeQuery3" :!type "EObjectTypeQuery Enum") "/Game/NIRVANA/Core/Characters/Enemies/Common/BP_Enemy.BP_Enemy_C"))
  (`NiagaraFunctionLibrary.SpawnSystemAtLocation` "/Game/NIRVANA/Core/Weapons/Vajra/FX_Vajra/NS_LightningBallExplode.NS_LightningBallExplode" (`self.K2_GetActorLocation`))
  (for _array_element _outactors
    (message `/Game/NIRVANA/Core/Characters/FirstPerson/BPI_Hit.Hit` _array_element (`self.ExplodeDamage`)))
  (`self.K2_DestroyActor`))

(fn `Set Velocity`
  (params (`New Velocity Power` :type "Float (single-precision)"))
  (bind _collision (`self.Collision`))
  (bind _returnvalue (`PrimitiveComponent.GetPhysicsLinearVelocity` _collision "None"))
  (`PrimitiveComponent.SetPhysicsLinearVelocity` _collision (* (`KismetMathLibrary.Normal` _returnvalue) (`local.New Velocity Power`)) false "None")
  (return))

(fn `Spawn ElectricBeam`
  (params (Target :type "Actor Object Reference"))
  (bind _returnvalue (`NiagaraFunctionLibrary.SpawnSystemAtLocation` "/Game/NIRVANA/Core/Weapons/Vajra/FX_Vajra/NS_EletricBeam.NS_EletricBeam"))
  (`FXSystemComponent.SetVectorParameter` _returnvalue "BeamStart" (`SceneComponent.K2_GetComponentLocation` (`self.Bomb`)))
  (`FXSystemComponent.SetVectorParameter` _returnvalue "BeamEnd" (`self.K2_GetActorLocation` Target)))

(fn `UserConstructionScript`
  (bind _returnvalue (`KismetMathLibrary.Conv_IntToDouble` (`KismetMathLibrary.FTrunc` (/ (`self.Tick Radius`) 56.66))))
  (`FXSystemComponent.SetVectorParameter` (`self.NS_LightningBall`) "Ring Scale" (`KismetMathLibrary.MakeVector` _returnvalue _returnvalue 5.0)))
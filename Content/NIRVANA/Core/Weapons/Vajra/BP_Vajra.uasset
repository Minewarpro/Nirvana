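; First-person Vajra weapon that fires lightning projectiles as primary fire and throws a lightning bomb on a timed cooldown as secondary.
; Each shot builds overheat (Surchauffe), which drives the HUD bar, sound pitch and lightning VFX, blocks firing when high, and decays after a retriggerable delay.
; Timelines drive weapon recoil, overheat blink, dissolve and the secondary recharge bar.
; The laser beam's start logic and the impulse dash's trigger are left unwired.
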(event `self.ReceiveBeginPlay`
  ;[1 1 1] Begin Play
  (`parent.ReceiveBeginPlay`)
  (`TimelineComponent.SetPlayRate` (`self.Secondary Fill TL`) (/ 1.0 (`self.Secondary Shoot Delay`)))
  (`TimelineComponent.SetPlayRate` (`self.Clignotement main emissive`) (/ 1.0 2.5)))

(event `ShootAnimation`
  (bind _mesh_1p (`/Game/NIRVANA/Core/Characters/FirstPerson/BP_FirstPersonCharacter.Mesh_1P` (`self.Player Ref`)))
  ;[0.4444 1 0.4482] shoot anim
  (`self.VajraShootAnimation`)
  (bind _notifyname (`|PlayMontage` (`/Game/NIRVANA/Core/Characters/FirstPerson/BP_FirstPersonCharacter.Mesh_1P` (`self.Player Ref`)) "/Game/NIRVANA/Core/Characters/FirstPerson/Animation/Vajra/Vajra_Shoot_Montage.Vajra_Shoot_Montage" 1.5)
    (:`then`
      (`AudioComponent.Play` (`self.MS_VajraFire`) 0.0))
    (:`OnNotifyBegin`
      (if (== _notifyname "Reload")
        (if (`self.InSurchauffe`)
          (`|PlayMontage` _mesh_1p "/Game/NIRVANA/Core/Characters/FirstPerson/Animation/Vajra/Vajara_Surchauffe_Montage.Vajara_Surchauffe_Montage" 3.0
            (:`then`
              (`PlayerCameraManager.StartCameraShake` :`self` (`GameplayStatics.GetPlayerCameraManager` 0) :`ShakeClass` "/Game/NIRVANA/Core/Characters/FirstPerson/Camera/CamShake/CamShake_VajraShoot.CamShake_VajraShoot_C")
              (bind (_direction _newtrack_0) (`Timeline|Clignotement main emissive` :!via `PlayFromStart`)
                (:`Update`
                  (`MaterialInstanceDynamic.SetVectorParameterValue` (`/Game/NIRVANA/Core/Characters/FirstPerson/BP_FirstPersonCharacter.MaterialInstance` (`self.Player Ref`)) "Emissive" (`KismetMathLibrary.LinearColorLerp` (struct :`R` 0.027451 :`G` 0.576471 :`B` 1.0 :`A` 1.0) (struct :`R` 1.0 :`A` 1.0) (`KismetMathLibrary.Lerp` 0.0 1.0 _newtrack_0)))))))
          (else
            (`|PlayMontage` _mesh_1p "/Game/NIRVANA/Core/Characters/FirstPerson/Animation/Vajra/Vajra_Reload_Montage.Vajra_Reload_Montage")))))))

(event `self.Fire Start`
  (bind _player_ref (`self.Player Ref`))
  ;[0.3958 0.112 0.1072] Primary Shoot
  (if (and (`self.CanShoot`) (<= (`self.Surchauffe Value`) 0.8) (not (`self.InSurchauffe`))) :!label _label
    (`PlayerCameraManager.StartCameraShake` :`self` (`GameplayStatics.GetPlayerCameraManager` 0) :`ShakeClass` "/Game/NIRVANA/Core/Characters/FirstPerson/Camera/CamShake/CamShake_VajraShoot.CamShake_VajraShoot_C" :`Scale` 3.0)
    (`|ExecutionSequence`
      (:`then_0`
        (set `self.CanShoot` false)
        (`KismetSystemLibrary.Delay` (`self.Shoot Delay`))
        (set `self.CanShoot` true))
      (:`then_1`
        (`self.Add Surchauffe` (`self.Surchauffe to add`))
        (`ActorComponent.Activate` (`self.NS_VajraShoot`) true)
        (set `self.HasTouch` false)
        (`self.ShootAnimation`)
        (`|SpawnActorFromClass` "/Game/NIRVANA/Core/Weapons/Vajra/BP_ProjectileVajra.BP_ProjectileVajra_C" (`KismetMathLibrary.MakeTransform` (`KismetMathLibrary.MakeVector` (.x (`SceneComponent.GetSocketLocation` (`self.Vajra`) "Muzzle")) (.y (`SceneComponent.GetSocketLocation` (`self.Vajra`) "Muzzle")) (- (.z (`SceneComponent.GetSocketLocation` (`self.Vajra`) "Muzzle")) 50.0)) (`SceneComponent.K2_GetComponentRotation` (`/Game/NIRVANA/Core/Characters/FirstPerson/BP_FirstPersonCharacter.FirstPersonCamera` _player_ref))) "AlwaysSpawn" "MultiplyWithRoot" null _player_ref 250.0 null)
        (`self.Lightning Shoot Effect`)))))

(event `VajraShootAnimation`
  ;[0.4444 1 0.4482] shoot anim
  (bind (_direction _location _rotation_x) (`Timeline|VajraShoot_TL` :!via `PlayFromStart`)
    (:`Update`
      (`SceneComponent.K2_SetRelativeLocation` (`self.VajraOffset`) _location false false)
      (`SceneComponent.K2_SetRelativeRotation` (`self.VajraOffset`) (`KismetMathLibrary.MakeRotator` 0.0 _rotation_x) false false))))

(event `self.Fire Hold`
  ;[0.3958 0.112 0.1072] Primary Shoot
  (goto _label))

(event `Secondary vajra shoot anim`
  ;[0.4444 1 0.4482] shoot anim
  (bind (_direction _location _rotation_x) (`Timeline|VajraSecondaryShoot_TL` :!via `PlayFromStart`)
    (:`Update`
      (`SceneComponent.K2_SetRelativeLocation` (`self.VajraOffset`) (`KismetMathLibrary.MakeVector` (.x _location) (`KismetMathLibrary.Lerp` 0.0 30.0 (.y _location)) (.z _location)) false false)
      (`SceneComponent.K2_SetRelativeRotation` (`self.VajraOffset`) (`KismetMathLibrary.MakeRotator` 0.0 (`KismetMathLibrary.Lerp` 0.0 180.0 _rotation_x)) false false))))

(event `self.Dissolve`
  ;[1 1 1] Dissolve
  (`TimelineComponent.SetPlayRate` (`self.Dissolve TL`) (/ 1.0 1.0))
  (bind (_direction _alpha_dissolve) (`Timeline|Dissolve TL` :!via `PlayFromStart` :!label _label_2)
    (:`Update`
      (`MeshComponent.SetScalarParameterValueOnMaterials` (`self.Vajra`) "Alpha" (`KismetMathLibrary.Lerp` 0.0 1.0 _alpha_dissolve)))
    (:`Finished`
      (`/Game/NIRVANA/Core/Characters/FirstPerson/BP_FirstPersonCharacter.Set Weapon Visibility` (`self.Player Ref`)))))

(event `Lightning Shoot Effect`
  ;[1 1 1] Linghting Shoot Effect
  (`TimelineComponent.SetPlayRate` (`self.Lightning Spawn Rate TL`) (/ 1.0 0.5))
  (bind (_direction _spawn_rate) (`Timeline|Lightning Spawn Rate TL` :!via `PlayFromStart`)
    (:`Update`
      (`NiagaraComponent.SetVariableFloat` (`/Game/NIRVANA/Core/Characters/FirstPerson/BP_FirstPersonCharacter.NS_Lightning` (`self.Player Ref`)) "SpawnRate" (`KismetMathLibrary.Lerp` 200.0 (`self.Current Spawn Rate Lightning`) _spawn_rate)))))

(event `Secondary Shoot`
  ;[1 0.5531 0.09423] Secondary Shoot
)

(event `self.Resolve`
  ;[1 1 1] Dissolve
  (`TimelineComponent.SetPlayRate` (`self.Dissolve TL`) (/ 1.0 0.2))
  (goto _label_2 :!via `ReverseFromEnd`))

(event `Impulse Player`
  (bind _player_ref (`self.Player Ref`))
  (bind _charactermovement (`Character.CharacterMovement` _player_ref))
  (bind _returnvalue (`KismetMathLibrary.GetForwardVector` (`SceneComponent.K2_GetComponentRotation` (`/Game/NIRVANA/Core/Characters/FirstPerson/BP_FirstPersonCharacter.FirstPersonCamera` _player_ref))))
  ;[1 0.5531 0.09423] Secondary Shoot
  ;;[0.3594 0.3594 0.3594] Impulse
  (set `MovementComponent.Velocity` (0.0 0.0 0.0) _charactermovement)
  (`CharacterMovementComponent.AddImpulse` _charactermovement (* (* _returnvalue -1.0) 2000.0) true)
  (if (> (.z _returnvalue) 0.0)
    (`CharacterMovementComponent.AddImpulse` _charactermovement (0.0 0.0 1000.0) true)))

(event `Refresh Niagara`
  (bind _returnvalue (`self.K2_GetActorLocation`))
  (bind _laserlightning (`self.LaserLightning`))
  ;[1 1 1] Laser Lightning
  (`NiagaraComponent.SetVariableVec3` (`self.LaserLightning`) "Beam Start" (`SceneComponent.K2_GetComponentLocation` (`self.Vajra`)))
  (bind _outhit (`KismetSystemLibrary.LineTraceSingle` _returnvalue (+ _returnvalue (* (`KismetMathLibrary.GetForwardVector` (`SceneComponent.K2_GetComponentRotation` (`/Game/NIRVANA/Core/Characters/FirstPerson/BP_FirstPersonCharacter.FirstPersonCamera` (`self.Player Ref`)))) (`self.LaserDistance`))) "TraceTypeQuery1"))
  (bind (_bblockinghit _binitialoverlap _time _distance _location _impactpoint _normal _impactnormal _physmat _hitactor _hitcomponent _hitbonename _bonename _hititem _elementindex _faceindex _tracestart _traceend) (`GameplayStatics.BreakHitResult` _outhit))
  (if _bblockinghit
    (`NiagaraComponent.SetVariableVec3` _laserlightning "Beam End" _location)
    (else
      (`NiagaraComponent.SetVariableVec3` _laserlightning "Beam End" _traceend))))

(event `Hit Loop`
  (bind _returnvalue (`self.K2_GetActorLocation`))
  ;[1 1 1] Laser Lightning
  (`|ExecutionSequence`
    (:`then_0`
      (`self.Add Surchauffe` -0.05)
      (bind _outhit (`KismetSystemLibrary.SphereTraceSingle` _returnvalue (+ _returnvalue (* (`KismetMathLibrary.GetForwardVector` (`SceneComponent.K2_GetComponentRotation` (`/Game/NIRVANA/Core/Characters/FirstPerson/BP_FirstPersonCharacter.FirstPersonCamera` (`self.Player Ref`)))) (`self.LaserDistance`))) 150.0 "TraceTypeQuery3"))
      (bind (_bblockinghit _binitialoverlap _time _distance _location _impactpoint _normal _impactnormal _physmat _hitactor) (`GameplayStatics.BreakHitResult` _outhit))
      (if _bblockinghit
        (message `/Game/NIRVANA/Core/Characters/FirstPerson/BPI_Hit.Hit` _hitactor 100.0)))
    (:`then_1`
      (if (<= (`self.Surchauffe Value`) 0.0)
        (`self.Stop Laser Lightning`)
        (`KismetSystemLibrary.PrintString` "Hello")))))

(event `Stop Laser Lightning`
  ;[1 1 1] Laser Lightning
  (set `self.CanShoot` true)
  (`SceneComponent.SetHiddenInGame` (`self.LaserLightning`) true false)
  (`KismetSystemLibrary.K2_ClearAndInvalidateTimerHandle` (`self.Hit Loop Event`))
  (`KismetSystemLibrary.K2_ClearAndInvalidateTimerHandle` (`self.Refresh Niagara Event`))
  (bind _output_get (set `self.Current Spawn Rate Lightning` 50.0))
  (`NiagaraComponent.SetVariableFloat` (`/Game/NIRVANA/Core/Characters/FirstPerson/BP_FirstPersonCharacter.NS_Lightning` (`self.Player Ref`)) "SpawnRate" _output_get))

(event `self.Secondary Fire Release`
  ;[1 1 1] Laser Lightning
)

(event `Add Surchauffe`
  (params (`surchauffe to add` :type "Float (double-precision)"))
  ;[1 1 1] Surchauffe
  (`|ExecutionSequence`
    (:`then_0`
      (bind _output_get (set `self.Surchauffe Value` (+ (`self.Surchauffe Value`) `surchauffe to add`)))
      (set `self.Current Spawn Rate Lightning` (`KismetMathLibrary.Lerp` 5.0 50.0 _output_get))
      (set `self.Surchauffe Pitch Mult` (* (`KismetMathLibrary.Lerp` 0.0 3.0 _output_get) (`KismetMathLibrary.MapRangeClamped` _output_get 0.65 1.0 1.0 2.0)))
      (`AudioParameterControllerInterface.SetFloatParameter` (`self.MS_VajraFire`) "SurchauffePitchMod" (`self.Surchauffe Pitch Mult`))
      (`ProgressBar.SetPercent` (`/Game/NIRVANA/UI/Player/WB_Base.ProgressBar_SecondaryShootCjara` (`self.WB Base`)) _output_get)
      (if (>= _output_get 0.9)
        (set `self.InSurchauffe` true)
        (`AudioComponent.Play` (`self.MS_OverheatWeapon`) 0.0))
      (`KismetSystemLibrary.RetriggerableDelay` 1.5)
      (`self.Start Dechauffe`))
    (:`then_1`
      (bind (_direction _chauffe_value) (`Timeline|Dechauffe_TL` :!via `Stop` :!label _label_3)
        (:`Update`
          (bind _output_get_2 (set `self.Surchauffe Value` (`KismetMathLibrary.Lerp` (`self.Temp Chauffe Value`) 0.0 _chauffe_value)))
          (`ProgressBar.SetPercent` (`/Game/NIRVANA/UI/Player/WB_Base.ProgressBar_SecondaryShootCjara` (`self.WB Base`)) _output_get_2)
          (bind _output_get_3 (set `self.Current Spawn Rate Lightning` (`KismetMathLibrary.Lerp` 50.0 5.0 _output_get_2)))
          (`NiagaraComponent.SetVariableFloat` (`/Game/NIRVANA/Core/Characters/FirstPerson/BP_FirstPersonCharacter.NS_Lightning` (`self.Player Ref`)) "SpawnRate" _output_get_3))
        (:`Finished`
          (set `self.InSurchauffe` false)
          (`AudioParameterControllerInterface.SetTriggerParameter` (`self.MS_OverheatWeapon`) "IsCoolingDown"))))))

(event `Start Dechauffe`
  (bind _surchauffe_value (`self.Surchauffe Value`))
  ;[1 1 1] Surchauffe
  (set `self.Temp Chauffe Value` _surchauffe_value)
  (`TimelineComponent.SetPlayRate` (`self.Dechauffe_TL`) (/ 1.0 (* _surchauffe_value (`self.Déchauffe Time`))))
  (goto _label_3 :!via `PlayFromStart`))

(event `self.Secondary Fire Start`
  (bind _player_ref (`self.Player Ref`))
  (bind _wb_base (`self.WB Base`))
  (bind _returnvalue (`KismetMathLibrary.GetForwardVector` (`SceneComponent.K2_GetComponentRotation` (`/Game/NIRVANA/Core/Characters/FirstPerson/BP_FirstPersonCharacter.FirstPersonCamera` _player_ref))))
  ;[1 1 1] Secondary Shoot
  (if (`self.Can Secondary Shoot`)
    (set `self.Can Secondary Shoot` false)
    (`Widget.SetVisibility` (`/Game/NIRVANA/UI/Player/WB_Base.SecondaryShootVajraIMG` _wb_base) (`/Game/NIRVANA/UI/Player/WB_Base.Get Secondary Shoot Vajra IMG` _wb_base))
    (`Widget.SetVisibility` (`/Game/NIRVANA/UI/Player/WB_Base.ProgressBar_Vajra` _wb_base) "Visible")
    (`|PlayMontage` (`/Game/NIRVANA/Core/Characters/FirstPerson/BP_FirstPersonCharacter.Mesh_1P` (`self.Player Ref`)) "/Game/NIRVANA/Core/Characters/FirstPerson/Animation/Vajra/Vajara_Atq_Secondaire_Montage.Vajara_Atq_Secondaire_Montage" 1.3 0.04
      (:`then`
        (`|SpawnActorFromClass` "/Game/NIRVANA/Core/Weapons/Vajra/BP_Linghtning_Bomb.BP_Linghtning_Bomb_C" (`KismetMathLibrary.MakeTransform` (+ (`self.K2_GetActorLocation` _player_ref) (* _returnvalue 150.0))) "AlwaysSpawn" "MultiplyWithRoot" null _returnvalue (`self.boss`) null)
        (`self.Secondary vajra shoot anim`)
        (bind (_direction _alpha_delay) (`Timeline|Secondary Fill TL` :!via `PlayFromStart`)
          (:`Update`
            (`ProgressBar.SetPercent` (`/Game/NIRVANA/UI/Player/WB_Base.ProgressBar_Vajra` (`self.WB Base`)) (`KismetMathLibrary.Lerp` 0.0 1.0 _alpha_delay)))
          (:`Finished`
            (`self.Reset Vajra Ball`)))))))

(event `Reset Vajra Ball`
  (bind _wb_base (`self.WB Base`))
  (bind _secondary_fill_tl (`self.Secondary Fill TL`))
  (bind _progressbar_vajra (`/Game/NIRVANA/UI/Player/WB_Base.ProgressBar_Vajra` _wb_base))
  ;[1 1 1] Secondary Shoot
  (`|ExecutionSequence`
    (:`then_0`
      (if (`TimelineComponent.IsPlaying` _secondary_fill_tl)
        (`TimelineComponent.Stop` _secondary_fill_tl)))
    (:`then_1`
      (set `self.Can Secondary Shoot` true)
      (`ProgressBar.SetPercent` _progressbar_vajra 1.0)
      (`Widget.SetVisibility` (`/Game/NIRVANA/UI/Player/WB_Base.SecondaryShootVajraIMG` _wb_base) (`/Game/NIRVANA/UI/Player/WB_Base.Get Secondary Shoot Vajra IMG` _wb_base))
      (`Widget.SetVisibility` _progressbar_vajra "Hidden"))))

(fn `Get Actor Angle`
  (params (`Target Actor` :type "Actor Object Reference"))
  (returns (Angle :type "Float (double-precision)"))
  (bind _player_ref (`self.Player Ref`))
  (return (- 90.0 (* (`KismetMathLibrary.Abs` (`KismetMathLibrary.Dot_VectorVector` (`SceneComponent.GetForwardVector` (`Character.CapsuleComponent` _player_ref)) (`KismetMathLibrary.GetDirectionUnitVector` (`self.K2_GetActorLocation` _player_ref) (`self.K2_GetActorLocation` `Target Actor`)))) 90.0))))

(fn `Get Damage With Distance`
  (params (`Target Actor` :type "Actor Object Reference"))
  (returns (Damages :type "Float (double-precision)"))
  (bind _max_distance (`self.Max DIstance`))
  (bind _returnvalue (`self.GetDistanceTo` `Target Actor` (`self.Player Ref`)))
  (if (not (> _returnvalue _max_distance))
    (return (* (`CurveFloat.GetFloatValue` (`self.Curve`) (`KismetMathLibrary.NormalizeToRange` (`KismetMathLibrary.FClamp` _returnvalue 0.0 _max_distance) 0.0 _max_distance)) (`self.Max Damage`)))))

(fn `UserConstructionScript`
  (`parent.UserConstructionScript`))
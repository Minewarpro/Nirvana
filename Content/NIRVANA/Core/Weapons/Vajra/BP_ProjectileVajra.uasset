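; BP_ProjectileVajra is the projectile fired by the Vajra weapon, travelling along the direction of the player's first-person camera.
; A timeline scaled to a set duration lerps it, without sweep, from its spawn point to a target at a set distance, then destroys it.
; SlashVajra overlaps send a damage hit message to actors other than the player, while a hit on MiddleCollision destroys the projectile.
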(event `self.ReceiveBeginPlay`
  (bind _initlocation (`self.InitLocation`))
  ;[1 1 1] Comment
  (set `self.InitLocation` (`self.K2_GetActorLocation`))
  (set `self.Target Location` (+ _initlocation (* (`KismetMathLibrary.GetForwardVector` (`SceneComponent.K2_GetComponentRotation` (`/Game/NIRVANA/Core/Characters/FirstPerson/BP_FirstPersonCharacter.FirstPersonCamera` (`self.PlayerRef`)))) (`self.Distance`))))
  (`TimelineComponent.SetPlayRate` (`self.Trajectoire TL`) (/ 1.0 (`self.Trajectoire Duration`)))
  (bind (_direction _location) (`Timeline|Trajectoire TL` :!via `PlayFromStart`)
    (:`Update`
      (`self.K2_SetActorLocation` (`KismetMathLibrary.VLerp` _initlocation (`self.Target Location`) _location)))
    (:`Finished`
      (`self.Destroy`))))

(event `self.SlashVajra.OnComponentBeginOverlap`
  (params (OverlappedComponent :type "PrimitiveComponent Object Reference") (OtherActor :type "Actor Object Reference") (OtherComp :type "PrimitiveComponent Object Reference") (OtherBodyIndex :type Integer) (bFromSweep :type Boolean) (SweepResult :type "HitResult Structure (by ref)"))
  ;[1 1 1] Overlap
  (if (not (== OtherActor (`self.PlayerRef`)))
    (message `/Game/NIRVANA/Core/Characters/FirstPerson/BPI_Hit.Hit` OtherActor (`self.Damages`))))

(event `Destroy`
  ;[1 1 1] Destroy
  (`self.K2_DestroyActor`))

(event `self.MiddleCollision.OnComponentHit`
  (params (HitComponent :type "PrimitiveComponent Object Reference") (OtherActor :type "Actor Object Reference") (OtherComp :type "PrimitiveComponent Object Reference") (NormalImpulse :type "Vector Structure") (Hit :type "HitResult Structure (by ref)"))
  (`self.K2_DestroyActor`))

(fn `UserConstructionScript`)
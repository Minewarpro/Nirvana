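; Player shotgun weapon with a pellet-spread primary fire and a gauge-powered secondary blast.
; Primary fire checks ammo and cooldown, line-traces random pellets in a camera cone, applies distance-reduced damage with a floor, and spawns beam projectiles.
; Pellets hitting components that block GameTraceChannel2 charge the player's gauge, once per shot.
; At full gauge, secondary fire multi-traces for heavy damage, spawns VFX, launches the player backward and resets the gauge.
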(event `self.ReceiveBeginPlay`
  (`parent.ReceiveBeginPlay`))

(event `self.Fire Start`
  (bind _shotgun_damage (`self.Shotgun Damage`))
  (bind _min_shotgun_damage (`self.Min Shotgun Damage`))
  (bind _firstpersoncamera (`/Game/NIRVANA/Core/Characters/FirstPerson/BP_FirstPersonCharacter.FirstPersonCamera` (`self.Player Ref`)))
  (bind _returnvalue (`SceneComponent.K2_GetComponentLocation` _firstpersoncamera))
  ;[0.3958 0.112 0.1072] Primary Shoot
  (if (`self.CanShoot`) :!label _label
    (if (> (`/Game/NIRVANA/Core/Characters/FirstPerson/BP_FirstPersonCharacter.Shotgun Munitions` (`self.Player Ref`)) 0)
      (`|ExecutionSequence`
        (:`then_0`
          (set `self.CanShoot` false)
          (`KismetSystemLibrary.Delay` (`self.Shoot Delay`))
          (set `self.CanShoot` true))
        (:`then_1`
          (`GameplayStatics.PlaySound2D` "/Game/NIRVANA/Core/Weapons/ShotGun/Sound/ShotGun_Fire.ShotGun_Fire" 1.0 1.0 0.0 null null)
          (set `self.HasTouch` false)
          (`self.ShootAnimation`)
          (for _ (range (`self.Nb Bullet Shotgun`))
            (bind _outhit (`KismetSystemLibrary.LineTraceSingle` _returnvalue (+ _returnvalue (* (`KismetMathLibrary.RandomUnitVectorInConeInDegrees` (`KismetMathLibrary.GetForwardVector` (`SceneComponent.K2_GetComponentRotation` _firstpersoncamera)) (`self.Cone Half Angle in Degrees`)) (`self.Max DIstance`))) "TraceTypeQuery4"))
            (bind (_bblockinghit _binitialoverlap _time _distance _location _impactpoint _normal _impactnormal _physmat _hitactor _hitcomponent _hitbonename _bonename _hititem _elementindex _faceindex _tracestart _traceend) (`GameplayStatics.BreakHitResult` _outhit))
            (`KismetSystemLibrary.PrintString` (`KismetSystemLibrary.GetDisplayName` _hitactor))
            (if _bblockinghit
              (set `self.Shotgun Damage` (`self.Max one bullet Shotgun Damage`))
              (for _ (range (`KismetMathLibrary.FTrunc` (/ _distance (`self.Distance to reduce damage`))))
                (set `self.Shotgun Damage` (/ (`self.Shotgun Damage`) (`self.Coef Reduction Damage (>=1)`))))
              (`|ExecutionSequence`
                (:`then_0`
                  (message `/Game/NIRVANA/Core/Characters/FirstPerson/BPI_Hit.Hit` _hitactor (`KismetMathLibrary.SelectFloat` _min_shotgun_damage _shotgun_damage (< _shotgun_damage _min_shotgun_damage)))
                  (bind _output_get (set `self.Impact Point` _impactpoint))
                  (`|SpawnActorFromClass` "/Game/NIRVANA/Core/Weapons/Test_Gun/Gun/BP_Projectile.BP_Projectile_C" (`KismetMathLibrary.MakeTransform` (`SceneComponent.GetSocketLocation` (`self.Weapon_Mesh`) "Muzzle")) "Undefined" "OverrideRootScale" null _output_get null :!label _label_2))
                (:`then_1`
                  (`/Engine/EditorBlueprintResources/StandardMacros.IsValid` _hitcomponent
                    (:`Is Valid`
                      (if (`KismetStringLibrary.EqualEqual_StrStr` (`|GetEnumeratorNameAsString` (`PrimitiveComponent.GetCollisionResponseToChannel` _hitcomponent "ECC_GameTraceChannel2")) "Block")
                        (set `self.HasTouch` true))))))
              (else
                (set `self.Impact Point` _traceend)
                (goto _label_2))))
          (if (`self.HasTouch`)
            (`/Game/NIRVANA/Core/Characters/FirstPerson/BP_FirstPersonCharacter.Set Jauge Pass Weapon` (`self.Player Ref`) 0.06)))))))

(event `self.Fire Hold`
  ;[0.3958 0.112 0.1072] Primary Shoot
  (goto _label))

(event `ShootAnimation`
  ;[0.4444 1 0.4482] shoot anim
  (bind _notifyname (`|PlayMontage` (`/Game/NIRVANA/Core/Characters/FirstPerson/BP_FirstPersonCharacter.Mesh_1P` (`self.Player Ref`)) "/Game/DevelopersContent/Core/Characters/FirstPerson/Animations/Shotguns/A_FP_PCH_Shotgun_01_Fire_Montage.A_FP_PCH_Shotgun_01_Fire_Montage")
    (:`OnNotifyBegin`
      (if (== _notifyname "Bolt")
        (`|PlayMontage` (`/Game/NIRVANA/Core/Characters/FirstPerson/BP_FirstPersonCharacter.Mesh_1P` (`self.Player Ref`)) "/Game/DevelopersContent/Core/Characters/FirstPerson/Animations/Shotguns/A_FP_PCH_Shotgun_01_Reload_Bolt_Montage.A_FP_PCH_Shotgun_01_Reload_Bolt_Montage"
          (:`then`
            (`GameplayStatics.PlaySound2D` "/Game/NIRVANA/Core/Weapons/ShotGun/Sound/Shotgun_Bolt.Shotgun_Bolt" 1.0 1.0 0.0 null null)))))))

(event `Secondary Shoot`
  (bind _firstpersoncamera (`/Game/NIRVANA/Core/Characters/FirstPerson/BP_FirstPersonCharacter.FirstPersonCamera` (`self.Player Ref`)))
  (bind _returnvalue (`SceneComponent.K2_GetComponentRotation` _firstpersoncamera))
  (bind _returnvalue_2 (`SceneComponent.K2_GetComponentLocation` _firstpersoncamera))
  ;[1 0.5531 0.09423] Secondary Shoot
  (bind _outhits (`KismetSystemLibrary.LineTraceMulti` _returnvalue_2 (+ _returnvalue_2 (* (`KismetMathLibrary.GetForwardVector` _returnvalue) (`self.Max DIstance`))) "TraceTypeQuery4"))
  (`|SpawnActorFromClass` "/Game/NIRVANA/Core/Weapons/ShotGun/Vfx/BP_Shotgun_VFX.BP_Shotgun_VFX_C" (`KismetMathLibrary.MakeTransform` (`SceneComponent.GetSocketLocation` (`self.Weapon_Mesh`) "Muzzle")) "Undefined" "MultiplyWithRoot" null _returnvalue 0.0 null)
  (for _array_element _outhits
    (bind (_bblockinghit _binitialoverlap _time _distance _location _impactpoint _normal _impactnormal _physmat _hitactor) (`GameplayStatics.BreakHitResult` _array_element))
    (if _bblockinghit
      (message `/Game/NIRVANA/Core/Characters/FirstPerson/BPI_Hit.Hit` _hitactor 600.0))))

(event `Impulse Player`
  (bind _player_ref (`self.Player Ref`))
  (bind _charactermovement (`Character.CharacterMovement` _player_ref))
  (bind _returnvalue (`KismetMathLibrary.GetForwardVector` (`SceneComponent.K2_GetComponentRotation` (`/Game/NIRVANA/Core/Characters/FirstPerson/BP_FirstPersonCharacter.FirstPersonCamera` _player_ref))))
  ;[1 0.5531 0.09423] Secondary Shoot
  ;;[0.3594 0.3594 0.3594] Impulse
  (set `MovementComponent.Velocity` (0.0 0.0 0.0) _charactermovement)
  (`CharacterMovementComponent.AddImpulse` _charactermovement (* (* _returnvalue -1.0) 2000.0) true)
  (if (> (.z _returnvalue) 0.0)
    (`CharacterMovementComponent.AddImpulse` _charactermovement (0.0 0.0 1000.0) true)))

(event `self.Secondary Fire Start`
  ;[1 0.5531 0.09423] Secondary Shoot
  ;;[1 0.7414 0.4479] Input
  (if (>= (`/Game/NIRVANA/Core/Characters/FirstPerson/BP_FirstPersonCharacter.JaugePassWeapon` (`self.Player Ref`)) 1.0)
    (`self.Secondary Shoot`)
    (`self.Impulse Player`)
    (`/Game/NIRVANA/Core/Characters/FirstPerson/BP_FirstPersonCharacter.Reset Jauge Pass` (`self.Player Ref`))))

(fn `UserConstructionScript`
  (`parent.UserConstructionScript`))
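; First-person dual chakram weapon that alternately throws left and right projectiles, briefly hiding the thrown mesh.
; Secondary fire plays a swirl, damages through a forward sphere trace and briefly blocks primary fire.
; Both modes add overheat (Surchauffe), which raises fire-sound pitch, locks firing when full and cools by timeline after a retriggerable delay.
; Timelines also drive material dissolve and resolve, while the idle-spin logic is unconnected.
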(event `Secondary Shoot Animation`
  (bind _mesh_1p (`/Game/NIRVANA/Core/Characters/FirstPerson/BP_FirstPersonCharacter.Mesh_1P` (`self.Player Ref`)))
  ;[1 1 1] Secondary Shoot Animation
  (`|PlayMontage` _mesh_1p "/Game/NIRVANA/Core/Characters/FirstPerson/Animation/Chakram/Y_2h_Swirl_End_Montage.Y_2h_Swirl_End_Montage" -1.0 0.6
    (:`OnNotifyBegin`
      (`|PlayMontage` _mesh_1p "/Game/NIRVANA/Core/Characters/FirstPerson/Animation/Chakram/Y_2h_Swirl_Loop_Montage.Y_2h_Swirl_Loop_Montage" 1.5 0.75))))

(event `SetVisibility`
  (params (Visibility :type Boolean))
  ;[1 1 1] Set Visibility
  (bind _output_get (set `self.CanBeVisible` Visibility))
  (`SceneComponent.SetVisibility` (`self.Weapon_Mesh_2`) _output_get true)
  (`SceneComponent.SetVisibility` (`self.Weapon_Mesh`) _output_get true))

(event `Shoot animation`
  (bind _mesh_1p (`/Game/NIRVANA/Core/Characters/FirstPerson/BP_FirstPersonCharacter.Mesh_1P` (`self.Player Ref`)))
  ;[1 1 1] Shoot Animation
  (if (`self.InverseDeg`)
    (`|PlayMontage` _mesh_1p "/Game/DevelopersContent/Core/Characters/FirstPerson/Animations/Mage/Y_L_Projectile_End_Montage.Y_L_Projectile_End_Montage")
    (else
      (`|PlayMontage` _mesh_1p "/Game/DevelopersContent/Core/Characters/FirstPerson/Animations/Mage/Y_R_Projectile_End_Montage.Y_R_Projectile_End_Montage"))))

(event `self.Dissolve`
  ;[1 1 1] Dissolve
  (`TimelineComponent.SetPlayRate` (`self.Dissolve TL`) (/ 1.0 1.2))
  (bind (_direction _alpha) (`Timeline|Dissolve TL` :!via `PlayFromStart` :!label _label)
    (:`Update`
      (`MeshComponent.SetScalarParameterValueOnMaterials` (`self.Weapon_Mesh_2`) "Alpha" (`KismetMathLibrary.Lerp` 0.0 1.0 _alpha))
      (`MeshComponent.SetScalarParameterValueOnMaterials` (`self.Weapon_Mesh`) "Alpha" (`KismetMathLibrary.Lerp` 0.0 1.0 _alpha)))))

(event `self.ReceiveBeginPlay`
  ;[1 1 1] Begin Play
  (`parent.ReceiveBeginPlay`)
  ;[1 1 1] Attach Second Chakram to Socket
  (`SceneComponent.K2_AttachToComponent` (`self.Weapon_Mesh_2`) (`/Game/NIRVANA/Core/Characters/FirstPerson/BP_FirstPersonCharacter.Mesh_1P` (`self.Player Ref`)) "GripPointChakram_2" "KeepRelative" "KeepRelative" "KeepRelative" true)
  (`TimelineComponent.SetPlayRate` (`self.Idle Chakram`) (/ 1.0 0.5)))

(event `self.Resolve`
  ;[1 1 1] Dissolve
  (`TimelineComponent.SetPlayRate` (`self.Dissolve TL`) (/ 1.0 0.2))
  (goto _label :!via `ReverseFromEnd`))

(event `self.Fire Hold`
  (bind _player_ref (`self.Player Ref`))
  (bind _weapon_mesh_2 (`self.Weapon_Mesh_2`))
  (bind _weapon_mesh (`self.Weapon_Mesh`))
  (bind _returnvalue (`SceneComponent.K2_GetComponentRotation` (`/Game/NIRVANA/Core/Characters/FirstPerson/BP_FirstPersonCharacter.FirstPersonCamera` _player_ref)))
  ;[1 1 1] Shoot
  (if (`self.Can Shot`)
    (if (not (`self.IsAfter Secondary Shoot`))
      (if (not (`self.InSurchauffe`))
        (`|ExecutionSequence`
          (:`then_0`
            (`KismetSystemLibrary.Delay` (`self.delay shoot`))
            (set `self.Can Shot` true))
          (:`then_1`
            (`self.Shoot animation`)
            (bind _isa (`/Engine/EditorBlueprintResources/StandardMacros.FlipFlop`)
              (:`A`
                (`SceneComponent.SetVisibility` _weapon_mesh false false)
                (`|ExecutionSequence`
                  (:`then_0`
                    (`PlayerCameraManager.StartCameraShake` :`self` (`GameplayStatics.GetPlayerCameraManager` 0) :`ShakeClass` (select `bool` _isa :`false` "/Game/NIRVANA/Core/Characters/FirstPerson/Camera/CamShake/CamShake_ChakramShoot2.CamShake_ChakramShoot2_C" :`true` "/Game/NIRVANA/Core/Characters/FirstPerson/Camera/CamShake/CamShake_ChakramShoot.CamShake_ChakramShoot_C" :!type "CameraShakeBase Class Reference") :!label _label_2)
                    (bind _output_get (set `self.InverseDeg` _isa))
                    (`|SpawnActorFromClass` "/Game/NIRVANA/Core/Weapons/Chakram/BP_Chakram_Projectile.BP_Chakram_Projectile_C" (`KismetMathLibrary.MakeTransform` (`SceneComponent.GetSocketLocation` (select `bool` _output_get :`false` (`self.Weapon_Mesh_2`) :`true` (`self.Weapon_Mesh`) :!type "SceneComponent Object Reference") "Muzzle") _returnvalue) "AlwaysSpawn" "MultiplyWithRoot" null (+ (`KismetMathLibrary.MakeVector` (.x (`self.K2_GetActorLocation` _player_ref)) (.y (`self.K2_GetActorLocation` _player_ref)) (+ (.z (`self.K2_GetActorLocation` _player_ref)) 65.0)) (* (`KismetMathLibrary.GetForwardVector` _returnvalue) (`self.Distance`))) (`self.Damage`) self _output_get _returnvalue null)
                    (set `self.Can Shot` false)
                    (`self.Add Surchauffe` (`self.Surchauffe to add`)))
                  (:`then_1`
                    (`KismetSystemLibrary.Delay` 0.3)
                    (if (`self.CanBeVisible`)
                      (`SceneComponent.SetVisibility` _weapon_mesh true false)))))
              (:`B`
                (`SceneComponent.SetVisibility` _weapon_mesh_2 false false)
                (`|ExecutionSequence`
                  (:`then_0`
                    (goto _label_2))
                  (:`then_1`
                    (`KismetSystemLibrary.Delay` 0.3)
                    (if (`self.CanBeVisible`)
                      (`SceneComponent.SetVisibility` _weapon_mesh_2 true false))))))))))))

(event `Add Surchauffe`
  (params (`Surchauffe to Add` :type "Float (double-precision)"))
  ;[1 1 1] Surchauffe
  (`|ExecutionSequence`
    (:`then_0`
      (bind _output_get (set `self.Surchauffe Value` (+ (`self.Surchauffe Value`) `Surchauffe to Add`)))
      ;;[1 0.6067 0.2543] Gestion du son en fonction de la surchauffe
      (set `self.SurchauffePitchMult` (* (`KismetMathLibrary.Lerp` 0.0 2.0 _output_get) (`KismetMathLibrary.MapRangeClamped` _output_get 0.65 1.0 1.0 2.0)))
      (bind _returnvalue (`GameplayStatics.SpawnSoundAtLocation` "/Game/NIRVANA/Core/Weapons/Chakram/SFX/MS_ChakramFire.MS_ChakramFire" (`self.K2_GetActorLocation`) (struct) 1.0 1.0 0.0 null null))
      (`AudioParameterControllerInterface.SetFloatParameter` _returnvalue "SurchauffePitchMod" (`self.SurchauffePitchMult`))
      (`AudioComponent.Play` _returnvalue 0.0)
      (if (>= _output_get 1.0)
        (set `self.InSurchauffe` true)
        (`AudioComponent.Play` (`self.MS_OverheatWeapon`) 0.0)
        (set `self.SurchauffePitchMult` 0.0))
      (`KismetSystemLibrary.RetriggerableDelay` 1.0)
      (`self.Start Dechauffe`))
    (:`then_1`
      (bind (_direction _chauffe_value) (`Timeline|Dechauffe TL` :!via `Stop` :!label _label_3)
        (:`Update`
          (set `self.Surchauffe Value` (`KismetMathLibrary.Lerp` (`self.Temp Chauffe Value`) 0.0 _chauffe_value)))
        (:`Finished`
          (if (>= (`self.Temp Chauffe Value`) 1.0)
            (set `self.InSurchauffe` false)
            (`AudioParameterControllerInterface.SetTriggerParameter` (`self.MS_OverheatWeapon`) "IsCoolingDown")))))))

(event `self.Secondary Fire Start`
  (bind _player_ref (`self.Player Ref`))
  (bind _returnvalue (`self.K2_GetActorLocation` _player_ref))
  ;[1 1 1] Secondary Shoot
  (if (`self.Can Secondary Shot`)
    (if (not (`self.InSurchauffe`))
      (`|ExecutionSequence`
        (:`then_0`
          (set `self.IsAfter Secondary Shoot` true)
          (set `self.Can Secondary Shot` false)
          (`self.Add Surchauffe` 0.15)
          (`self.Secondary Shoot Animation`)
          (bind _outhit (`KismetSystemLibrary.SphereTraceSingle` :`Start` _returnvalue :`End` (+ _returnvalue (* (`KismetMathLibrary.GetForwardVector` (`SceneComponent.K2_GetComponentRotation` (`/Game/NIRVANA/Core/Characters/FirstPerson/BP_FirstPersonCharacter.FirstPersonCamera` _player_ref))) (`self.Distance`))) :`Radius` 100.0 :`TraceChannel` "TraceTypeQuery3" :`DrawDebugType` "ForDuration"))
          (bind (_bblockinghit _binitialoverlap _time _distance _location _impactpoint _normal _impactnormal _physmat _hitactor) (`GameplayStatics.BreakHitResult` _outhit))
          (if _bblockinghit
            (message `/Game/NIRVANA/Core/Characters/FirstPerson/BPI_Hit.Hit` _hitactor (`self.Secondary Damages`) (0.0 0.0 0.0) (0.0 0.0 0.0) "None")))
        (:`then_1`
          (`KismetSystemLibrary.Delay` (`self.delay secondary shoot`))
          (set `self.Can Secondary Shot` true))
        (:`then_2`
          (`KismetSystemLibrary.Delay` 1.0)
          (set `self.IsAfter Secondary Shoot` false))))))

(event `Start Dechauffe`
  (bind _surchauffe_value (`self.Surchauffe Value`))
  ;[1 1 1] Surchauffe
  (set `self.Temp Chauffe Value` _surchauffe_value)
  (`TimelineComponent.SetPlayRate` (`self.Dechauffe TL`) (/ 1.0 (* (`self.Déchauffe Time`) _surchauffe_value)))
  (goto _label_3 :!via `PlayFromStart`))

(fn `UserConstructionScript`
  (`parent.UserConstructionScript`))
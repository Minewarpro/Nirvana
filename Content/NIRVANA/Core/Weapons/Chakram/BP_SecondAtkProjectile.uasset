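; Chakram secondary attack projectile: a slash that flies along the player's camera aim and damages what it overlaps.
; A timeline lerps it over Distance in TrajectoireDuration, then destroys it.
; SlashVajra overlaps damage each enemy once via an ignore list, damage bosses without that check, and send zero-damage hits to lightning bombs.
; A MiddleCollision hit disables that collider, spawns impact VFX and destroys the actor after a brief delay.
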(event `self.ReceiveBeginPlay`
  (bind _initlocation (`self.InitLocation`))
  ;[1 1 1] Comment
  (set `self.InitLocation` (`self.K2_GetActorLocation`))
  (set `self.Target Location` (+ _initlocation (* (`KismetMathLibrary.GetForwardVector` (`SceneComponent.K2_GetComponentRotation` (`/Game/NIRVANA/Core/Characters/FirstPerson/BP_FirstPersonCharacter.FirstPersonCamera` (`self.PlayerRef`)))) (`self.Distance`))))
  (`TimelineComponent.SetPlayRate` (`self.Trajectoire TL`) (/ 1.0 (`self.Trajectoire Duration`)))
  (bind (_direction _location) (`Timeline|Trajectoire TL` :!via `PlayFromStart`)
    (:`Update`
      (`self.K2_SetActorLocation` (`KismetMathLibrary.VLerp` _initlocation (`self.Target Location`) _location)))
    (:`Finished`
      (`self.Destroy`))))

(event `self.SlashVajra.OnComponentBeginOverlap`
  (params (OverlappedComponent :type "PrimitiveComponent Object Reference") (OtherActor :type "Actor Object Reference") (OtherComp :type "PrimitiveComponent Object Reference") (OtherBodyIndex :type Integer) (bFromSweep :type Boolean) (SweepResult :type "HitResult Structure (by ref)"))
  (bind _returnvalue (`self.K2_GetActorLocation` OtherActor))
  ;[1 1 1] Overlap
  (set `self.EnemyAlreadyTouched` false)
  (if (not (== OtherActor (`self.PlayerRef`)))
    (bind _asbp_enemy (cast `/Game/NIRVANA/Core/Characters/Enemies/Common/BP_Enemy` OtherActor)
      (:`then`
        (bind _output_get (set `self.Enemy Touched` _asbp_enemy))
        (for _array_element (`self.EnemiesToIgnore`)
          (if (== _array_element _output_get)
            (set `self.EnemyAlreadyTouched` true)))
        (if (not (`self.EnemyAlreadyTouched`))
          (`KismetArrayLibrary.Array_Add` (`self.EnemiesToIgnore`) (`self.Enemy Touched`))
          (`NiagaraFunctionLibrary.SpawnSystemAtLocation` "/Game/NIRVANA/Core/Weapons/Chakram/FX/Hit_RightClick/NS_RC_Hit.NS_RC_Hit" _returnvalue (`KismetMathLibrary.FindLookAtRotation` _returnvalue (`self.K2_GetActorLocation` (`self.PlayerRef`))) (* (1.0 1.0 1.0) 1.0))
          (message `/Game/NIRVANA/Core/Characters/FirstPerson/BPI_Hit.Hit` OtherActor (`self.Damages`))))
      (:`CastFailed`
        (bind _asbp_boss (cast `/Game/NIRVANA/Core/Characters/Enemies/Boss/BP_Boss` OtherActor)
          (:`then`
            (message `/Game/NIRVANA/Core/Characters/FirstPerson/BPI_Hit.Hit` _asbp_boss (`self.Damages`)))
          (:`CastFailed`
            (bind _asbp_linghtning_bomb (cast `/Game/NIRVANA/Core/Weapons/Vajra/BP_Linghtning_Bomb` OtherActor))
            (message `/Game/NIRVANA/Core/Characters/FirstPerson/BPI_Hit.Hit` _asbp_linghtning_bomb 0.0)))))))

(event `Destroy`
  ;[1 1 1] Destroy
  (`self.K2_DestroyActor`))

(event `self.MiddleCollision.OnComponentHit`
  (params (HitComponent :type "PrimitiveComponent Object Reference") (OtherActor :type "Actor Object Reference") (OtherComp :type "PrimitiveComponent Object Reference") (NormalImpulse :type "Vector Structure") (Hit :type "HitResult Structure (by ref)"))
  (bind _slashvajra (`self.SlashVajra`))
  (bind _middlecollision (`self.MiddleCollision`))
  ;[1 1 1] Hit
  (`PrimitiveComponent.SetSimulatePhysics` _middlecollision false)
  (`PrimitiveComponent.SetCollisionEnabled` _middlecollision "NoCollision")
  (`NiagaraFunctionLibrary.SpawnSystemAtLocation` "/Game/NIRVANA/Core/Weapons/Chakram/FX/Hit_RightClick/NS_RC_Hit.NS_RC_Hit" (`SceneComponent.K2_GetComponentLocation` _slashvajra) (`SceneComponent.K2_GetComponentRotation` _slashvajra) (* (1.0 1.0 1.0) 3.0))
  (`KismetSystemLibrary.Delay` 0.1)
  (`self.K2_DestroyActor`))

(fn `UserConstructionScript`)
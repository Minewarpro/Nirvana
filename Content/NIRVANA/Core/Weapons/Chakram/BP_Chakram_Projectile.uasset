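; Thrown chakram projectile that flies to a target on a curved path, then returns to the player.
; BeginPlay sets a randomized, side-offset control point, which Tick interpolates toward the target while the actor chases it, bending the path.
; Overlaps send damage through HitMessage; overlaps, hits or arrival trigger a timeline lerp back to the player.
; On return, it toggles the weapon's left/right state, reveals that hand's mesh and destroys itself.
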(event `self.Sphere Collider.OnComponentHit`
  (params (HitComponent :type "PrimitiveComponent Object Reference") (OtherActor :type "Actor Object Reference") (OtherComp :type "PrimitiveComponent Object Reference") (NormalImpulse :type "Vector Structure") (Hit :type "HitResult Structure (by ref)"))
  (if (and (!= OtherActor self) (!= OtherActor (`self.Player Ref`)))
    (`self.Come Back` :!label _label)))

(event `self.Sphere Collider.OnComponentBeginOverlap`
  (params (OverlappedComponent :type "PrimitiveComponent Object Reference") (OtherActor :type "Actor Object Reference") (OtherComp :type "PrimitiveComponent Object Reference") (OtherBodyIndex :type Integer) (bFromSweep :type Boolean) (SweepResult :type "HitResult Structure (by ref)"))
  (if (not (== OtherActor (`self.Player Ref`)))
    (message `/Game/NIRVANA/Core/Characters/FirstPerson/BPI_Hit.Hit` OtherActor (`self.Damage`))
    (goto _label)))

(event `self.ReceiveTick`
  (params (DeltaSeconds :type "Float (single-precision)"))
  (`/Engine/EditorBlueprintResources/StandardMacros.Gate` true :!label _label_2
    (:`Exit`
      (if (and (!= (`self.K2_GetActorLocation`) (`self.TargetLocation`) :`ErrorTolerance` 10.0) (not (`self.Comming Back`)))
        (set `self.Curved Point` (`KismetMathLibrary.VInterpTo_Constant` (`self.Curved Point`) (`self.TargetLocation`) (`GameplayStatics.GetWorldDeltaSeconds`) (`self.Projectile Speed`)))
        (`self.K2_SetActorLocation` (`KismetMathLibrary.VInterpTo_Constant` (`self.K2_GetActorLocation`) (`self.Curved Point`) (`GameplayStatics.GetWorldDeltaSeconds`) (`self.Projectile Speed`)) true)
        (else
          (`/Engine/EditorBlueprintResources/StandardMacros.DoOnce` false
            (:`Completed`
              (`self.Come Back`))))))))

(event `self.ReceiveBeginPlay`
  (`SceneComponent.K2_SetRelativeRotation` (`self.Chakram`) (`self.Init Rotation`) false false)
  (bind _asbp_first_person_character (cast `/Game/NIRVANA/Core/Characters/FirstPerson/BP_FirstPersonCharacter` (`GameplayStatics.GetPlayerCharacter` 0))
    (:`then`
      (set `self.Player Ref` _asbp_first_person_character))
    (:`CastFailed`
      _))
  (set `self.Angle Deg` (select `bool` (`self.Inerverse Deg`) :`false` 180.0 :`true` 0.0 :!type "Float (single-precision)"))
  (`KismetSystemLibrary.Delay` 0.01)
  (`self.Mid Point Calculator`)
  (`self.Curve Control Point`)
  (goto _label_2 :!via `Open`))

(event `Come Back`
  (set `self.Comming Back` true)
  (set `self.Init Actor Location` (`self.K2_GetActorLocation`))
  (bind (_direction _location_) (`Timeline|ComeBack`)
    (:`Update`
      (`self.K2_SetActorLocation` (`KismetMathLibrary.VLerp` (`self.Init Actor Location`) (`self.K2_GetActorLocation` (`self.Player Ref`)) _location_)))
    (:`Finished`
      (bind _chakram_ref (`self.Chakram Ref`)
        (:`then`
          (if (`/Game/NIRVANA/Core/Weapons/Chakram/BP_Chakram.IsNextRight` _chakram_ref)
            (set `/Game/NIRVANA/Core/Weapons/Chakram/BP_Chakram.IsNextRight` false _chakram_ref)
            (`SceneComponent.SetVisibility` (`/Game/NIRVANA/Core/Weapons/Common/BP_Weapon.Weapon_Mesh` _chakram_ref) true false)
            (else
              (set `/Game/NIRVANA/Core/Weapons/Chakram/BP_Chakram.IsNextRight` true _chakram_ref)
              (`SceneComponent.SetVisibility` (`/Game/NIRVANA/Core/Weapons/Chakram/BP_Chakram.Weapon_Mesh_2` _chakram_ref) true false)))
          (`self.K2_DestroyActor`))
        (:`else`)))))

(fn `Curve Control Point`
  (bind (_x _y) (`KismetMathLibrary.BreakRotIntoAxes` (`KismetMathLibrary.FindLookAtRotation` (`self.Mid Point`) (`self.TargetLocation`))))
  (set `self.Curved Point` (+ (`self.Mid Point`) (`KismetMathLibrary.RotateAngleAxis` (* (`KismetMathLibrary.RandomFloatInRange` (`self.Min Curve Radius`) (`self.Max Curve Radius`)) _y) (`self.Angle Deg`) _x))))

(fn `Mid Point Calculator`
  (set `self.Mid Point` (+ (* (- (`self.TargetLocation`) (`self.K2_GetActorLocation`)) (`KismetMathLibrary.RandomFloatInRange` (`self.Min Curve Point Disctance`) (`self.Max Curve Point Distance`))) (`self.K2_GetActorLocation`))))

(fn `UserConstructionScript`)
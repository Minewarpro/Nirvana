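; Uzi projectile actor that deals area damage through a small burst when it hits something other than the player or its lifetime runs out.
; On spawn it launches its collision component along Direction at Speed and starts a fallback timer.
; Destroy plays a flash ring particle and sound, sends HitMessage with Damage to sphere-overlapped actors of each filtered class, then removes itself after a short delay.
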(event `Destroy`
  (bind _par_flashring (`self.Par_FlashRing`))
  (`SceneComponent.SetVisibility` _par_flashring true false)
  (`ActorComponent.Activate` _par_flashring false)
  (`AddComponent|NODE_AddAudioComponent-1`)
  (for _array_element (`self.Actor Class Filter`)
    (bind _outactors (`KismetSystemLibrary.SphereOverlapActors` (`SceneComponent.K2_GetComponentLocation` (`self.Collision`)) 220.0 (`self.Object Types`) _array_element))
    (`|ExecutionSequence`
      (:`then_1`
        (for _array_element_2 _outactors
          (message `/Game/NIRVANA/Core/Characters/FirstPerson/BPI_Hit.Hit` _array_element_2 (`self.Damage`))))))
  (`ActorComponent.K2_DestroyComponent` (`self.Projectile`))
  (`ActorComponent.K2_DestroyComponent` (`self.Collision`))
  (`KismetSystemLibrary.Delay` 0.5)
  (`self.K2_DestroyActor`))

(event `self.Collision.OnComponentBeginOverlap`
  (params (OverlappedComponent :type "PrimitiveComponent Object Reference") (OtherActor :type "Actor Object Reference") (OtherComp :type "PrimitiveComponent Object Reference") (OtherBodyIndex :type Integer) (bFromSweep :type Boolean) (SweepResult :type "HitResult Structure (by ref)"))
  (if (!= OtherActor (`self.Player Ref`))
    (`self.Destroy` :!label _label)))

(event `self.Collision.OnComponentHit`
  (params (HitComponent :type "PrimitiveComponent Object Reference") (OtherActor :type "Actor Object Reference") (OtherComp :type "PrimitiveComponent Object Reference") (NormalImpulse :type "Vector Structure") (Hit :type "HitResult Structure (by ref)"))
  (if (!= OtherActor (`self.Player Ref`))
    (goto _label)))

(event `self.ReceiveBeginPlay`
  (`PrimitiveComponent.SetPhysicsLinearVelocity` (`self.Collision`) (* (`self.Direction`) (`self.Speed`)) false "None")
  (`KismetSystemLibrary.Delay` 10.0)
  (`self.Destroy`))

(fn `UserConstructionScript`)
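; Uzi weapon Blueprint with an automatic primary fire and a gauge-charged secondary shot.
; Held fire checks Uzi ammo and a delay-reset gate, then spawns muzzle projectiles randomized within a cone around camera aim.
; Secondary fire needs a full player JaugePassWeapon, launches a straight big projectile, then resets the gauge.
; Primary shots play the first-person montage, whose FireSMG notify triggers the weapon mesh montage.
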(event `self.Fire Hold`
  ;[0.4531 0.0708 0.086] Primary Shoot
  (if (> (`/Game/NIRVANA/Core/Characters/FirstPerson/BP_FirstPersonCharacter.Uzi Munitions` (`self.Player Ref`)) 0)
    (if (`self.CanShoot`)
      (`|ExecutionSequence`
        (:`then_0`
          (set `self.CanShoot` false)
          (`KismetSystemLibrary.Delay` (`self.Fire Delay`))
          (set `self.CanShoot` true))
        (:`then_1`
          (`self.ShootAnimation`)
          (`|SpawnActorFromClass` "/Game/NIRVANA/Core/Weapons/Uzi/Bp_UziProjectile.Bp_UziProjectile_C" (`KismetMathLibrary.MakeTransform` (`SceneComponent.GetSocketLocation` (`self.Weapon_Mesh`) "Muzzle")) "AlwaysSpawn" "MultiplyWithRoot" null (`KismetMathLibrary.RandomUnitVectorInConeInDegrees` (`KismetMathLibrary.GetForwardVector` (`SceneComponent.K2_GetComponentRotation` (`/Game/NIRVANA/Core/Characters/FirstPerson/BP_FirstPersonCharacter.FirstPersonCamera` (`self.Player Ref`)))) (`self.Cone Half Angle in Degrees`)) (`self.Speed Projectile`) (`self.Damage`) (`self.Player Ref`) null)
          (`GameplayStatics.PlaySound2D` "/Game/NIRVANA/Core/Weapons/Uzi/Sound/Uzi_Fire.Uzi_Fire" 1.0 1.0 0.0 null null))))))

(event `Secondary Shoot`
  (bind _firstpersoncamera (`/Game/NIRVANA/Core/Characters/FirstPerson/BP_FirstPersonCharacter.FirstPersonCamera` (`self.Player Ref`)))
  ;[0.7292 0.332 0.1367] Secondary Shoot
  (`|SpawnActorFromClass` "/Game/NIRVANA/Core/Weapons/Uzi/Bp_UziProjectile_Big.Bp_UziProjectile_Big_C" (`KismetMathLibrary.MakeTransform` (+ (`SceneComponent.GetSocketLocation` (`self.Weapon_Mesh`) "Muzzle") (* (`SceneComponent.GetForwardVector` _firstpersoncamera) 50.0))) "AlwaysSpawn" "MultiplyWithRoot" null (`KismetMathLibrary.GetForwardVector` (`SceneComponent.K2_GetComponentRotation` _firstpersoncamera)) (`self.Speed Projectile`) (`self.Damage_Big`) (`self.Player Ref`) null)
  (`GameplayStatics.PlaySound2D` "/Game/NIRVANA/Core/Weapons/Uzi/Sound/Uzi_Fire.Uzi_Fire" 1.0 1.0 0.0 null null))

(event `ShootAnimation`
  ;[0.375 1 0.6674] Anim
  (bind _notifyname (`|PlayMontage` (`/Game/NIRVANA/Core/Characters/FirstPerson/BP_FirstPersonCharacter.Mesh_1P` (`self.Player Ref`)) "/Game/DevelopersContent/Core/Characters/FirstPerson/Animations/SMGs/A_FP_PCH_SMG_Fire_Montage.A_FP_PCH_SMG_Fire_Montage")
    (:`OnNotifyBegin`
      (if (== _notifyname "FireSMG")
        (`|PlayMontage` (`self.Weapon_Mesh`) "/Game/DevelopersContent/Core/Weapons/SMGs/Animations/A_FP_WEP_SMG_03_Fire_Montage.A_FP_WEP_SMG_03_Fire_Montage")))))

(event `self.Secondary Fire Start`
  (bind _player_ref (`self.Player Ref`))
  ;[0.7292 0.332 0.1367] Secondary Shoot
  (if (>= (`/Game/NIRVANA/Core/Characters/FirstPerson/BP_FirstPersonCharacter.JaugePassWeapon` _player_ref) 1.0)
    (`self.Secondary Shoot`)
    (`/Game/NIRVANA/Core/Characters/FirstPerson/BP_FirstPersonCharacter.Reset Jauge Pass` _player_ref)))

(fn `UserConstructionScript`
  (`parent.UserConstructionScript`))
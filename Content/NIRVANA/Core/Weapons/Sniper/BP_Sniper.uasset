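; Sniper rifle weapon Blueprint for the player, with hitscan fire and a hold-to-aim scope.
; Firing spends ammo, sphere-traces from the camera within a random cone, sends damage to the hit actor and spawns a shot VFX sized to the distance.
; The fire montage's notify triggers the bolt animation, while a delay gates the next shot.
; Scoping shows a widget, hides arms, zooms, removes spread and adjusts camera shake and mouse sensitivity until release.
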(event `self.Fire Start`
  (bind _impact_point (`self.Impact Point`))
  (bind _player_ref (`self.Player Ref`))
  (bind _firstpersoncamera (`/Game/NIRVANA/Core/Characters/FirstPerson/BP_FirstPersonCharacter.FirstPersonCamera` _player_ref))
  (bind _returnvalue (`SceneComponent.K2_GetComponentLocation` _firstpersoncamera))
  ;[0.1771 0.04611 0.05078] Fire
  (if (> (`/Game/NIRVANA/Core/Characters/FirstPerson/BP_FirstPersonCharacter.Sniper Munitions` _player_ref) 0)
    (if (`self.CanShoot`)
      (set `self.CanShoot` false)
      (`self.ShootAnimation`)
      (`/Game/NIRVANA/Core/Characters/FirstPerson/BP_FirstPersonCharacter.Add Munition` (`self.Player Ref`) -1 "NewEnumerator7")
      (bind _outhit (`KismetSystemLibrary.SphereTraceSingle` _returnvalue (+ _returnvalue (* (`KismetMathLibrary.RandomUnitVectorInConeInDegrees` (`KismetMathLibrary.GetForwardVector` (`SceneComponent.K2_GetComponentRotation` _firstpersoncamera)) (`self.Cone Half Angle in Degrees`)) 99999999.0)) 45.0 "TraceTypeQuery4"))
      (bind (_bblockinghit _binitialoverlap _time _distance _location _impactpoint _normal _impactnormal _physmat _hitactor _hitcomponent _hitbonename _bonename _hititem _elementindex _faceindex _tracestart _traceend) (`GameplayStatics.BreakHitResult` _outhit))
      (if _bblockinghit
        (message `/Game/NIRVANA/Core/Characters/FirstPerson/BPI_Hit.Hit` _hitactor (`self.Damages`))
        (set `self.Impact Point` _impactpoint)
        (else
          (set `self.Impact Point` _traceend)))
      (`|SpawnActorFromClass` "/Game/NIRVANA/Core/Weapons/Sniper/VFX/BP_Sniper_VFX.BP_Sniper_VFX_C" (`KismetMathLibrary.MakeTransform` (`SceneComponent.GetSocketLocation` (`self.Weapon_Mesh`) "Muzzle")) "Undefined" "MultiplyWithRoot" null (`KismetMathLibrary.FindLookAtRotation` _returnvalue _impact_point) (`KismetMathLibrary.Vector_Distance` _returnvalue _impact_point) null)
      (`GameplayStatics.PlaySound2D` "/Game/NIRVANA/Core/Weapons/Sniper/Sniper_Shot.Sniper_Shot" 1.0 1.0 0.0 null null))))

(event `ShootAnimation`
  ;[0.4583 1 0.8771] Animaton
  (bind _notifyname (`|PlayMontage` (`/Game/NIRVANA/Core/Characters/FirstPerson/BP_FirstPersonCharacter.Mesh_1P` (`self.Player Ref`)) "/Game/DevelopersContent/Core/Characters/FirstPerson/Animations/Snipers/A_FP_PCH_Sniper_Fire_Montage.A_FP_PCH_Sniper_Fire_Montage")
    (:`then`
      (`KismetSystemLibrary.Delay` (`self.Delay Shoot`))
      (set `self.CanShoot` true))
    (:`OnNotifyBegin`
      (if (== _notifyname "Bolt")
        (`|PlayMontage` (`/Game/NIRVANA/Core/Characters/FirstPerson/BP_FirstPersonCharacter.Mesh_1P` (`self.Player Ref`)) "/Game/DevelopersContent/Core/Characters/FirstPerson/Animations/Snipers/A_FP_PCH_Sniper_01_Reload_Bolt_Montage.A_FP_PCH_Sniper_01_Reload_Bolt_Montage"
          (:`then`
            (`GameplayStatics.PlaySound2D` "/Game/NIRVANA/Core/Weapons/Sniper/Sniper_Bolt.Sniper_Bolt" 1.0 1.0 0.0 null null)))))))

(event `Scope`
  (bind _player_ref (`self.Player Ref`))
  (bind _firstpersoncamera (`/Game/NIRVANA/Core/Characters/FirstPerson/BP_FirstPersonCharacter.FirstPersonCamera` (`self.Player Ref`)))
  (bind _fieldofview (`CameraComponent.FieldOfView` _firstpersoncamera))
  ;[1 0.7453 0.3802] Scope
  (if (not (`self.Scope?`))
    (set `self.Scope?` true)
    ;;[1 1 1] Create Scope Widget
    (bind _returnvalue (`|CreateWidget` "/Game/NIRVANA/Core/Weapons/Sniper/WB_Sniper_Scope.WB_Sniper_Scope_C"))
    (bind _output_get (set `self.Widget Scope` _returnvalue))
    (`UserWidget.AddToViewport` _output_get 0)
    ;;[1 1 1] Hidde 1P Mesh
    (`SceneComponent.SetHiddenInGame` (`/Game/NIRVANA/Core/Characters/FirstPerson/BP_FirstPersonCharacter.Mesh_1P` (`self.Player Ref`)) true true)
    ;;[1 1 1] Zoom
    (set `self.Init Field Of View` _fieldofview)
    (`CameraComponent.SetFieldOfView` _firstpersoncamera (/ _fieldofview (`self.Zoom rate`)))
    ;;[1 1 1] Set random cone
    (set `self.Cone Half Angle in Degrees` 0.0)
    ;;[1 1 1] Set Cam Shake Vars
    (set `self.Init Cam Strenght` (`/Game/NIRVANA/Core/Characters/FirstPerson/BP_FirstPersonCharacter.CamStrenght` _player_ref))
    (set `/Game/NIRVANA/Core/Characters/FirstPerson/BP_FirstPersonCharacter.CamStrenght` 300.0 _player_ref)
    (set `self.Init Max Cam Offset` (`/Game/NIRVANA/Core/Characters/FirstPerson/BP_FirstPersonCharacter.Max Cam Offset` _player_ref))
    (set `/Game/NIRVANA/Core/Characters/FirstPerson/BP_FirstPersonCharacter.Max Cam Offset` 100.0 _player_ref)
    ;;[1 1 1] Set Mouse sensitivity
    (bind _output_get_2 (set `self.Init Mouse Sensitivity Rate` (`/Game/NIRVANA/Core/Characters/FirstPerson/BP_FirstPersonCharacter.Mouse Sensitivity Rate` _player_ref)))
    (set `/Game/NIRVANA/Core/Characters/FirstPerson/BP_FirstPersonCharacter.Mouse Sensitivity Rate` (* _output_get_2 (`self.Mouse Sensitivity Reduce Rate`)) _player_ref)))

(event `self.Secondary Fire Start`
  ;[1 0.7453 0.3802] Scope
  ;;[1 1 1] Inputs
  (`self.Scope`))

(event `self.Secondary Fire Release`
  ;[1 0.7453 0.3802] Scope
  ;;[1 1 1] Inputs
  (`self.Un Scope`))

(event `Un Scope`
  (bind _player_ref (`self.Player Ref`))
  ;[1 0.7453 0.3802] Scope
  (if (`self.Scope?`)
    (set `self.Scope?` false)
    ;;[1 1 1] Un-Scope
    (`Widget.RemoveFromParent` (`self.Widget Scope`))
    ;;[1 1 1] Un-Hidde 1P Mesh
    (`SceneComponent.SetHiddenInGame` (`/Game/NIRVANA/Core/Characters/FirstPerson/BP_FirstPersonCharacter.Mesh_1P` (`self.Player Ref`)) false true)
    ;;[1 1 1] Un-Zoom
    (`CameraComponent.SetFieldOfView` (`/Game/NIRVANA/Core/Characters/FirstPerson/BP_FirstPersonCharacter.FirstPersonCamera` (`self.Player Ref`)) (`self.Init Field Of View`))
    ;;[1 1 1] Set random cone
    (set `self.Cone Half Angle in Degrees` 20.0)
    ;;[1 1 1] Reset Cam Shake Vars
    (set `/Game/NIRVANA/Core/Characters/FirstPerson/BP_FirstPersonCharacter.CamStrenght` (`self.Init Cam Strenght`) _player_ref)
    (set `/Game/NIRVANA/Core/Characters/FirstPerson/BP_FirstPersonCharacter.Max Cam Offset` (`self.Init Max Cam Offset`) _player_ref)
    ;;[1 1 1] Reset Mouse Sensitivity
    (set `/Game/NIRVANA/Core/Characters/FirstPerson/BP_FirstPersonCharacter.Mouse Sensitivity Rate` (`self.Init Mouse Sensitivity Rate`) _player_ref)))

(fn `UserConstructionScript`
  (`parent.UserConstructionScript`))
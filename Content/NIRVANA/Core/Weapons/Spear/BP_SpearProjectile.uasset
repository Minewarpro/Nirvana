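; BP_SpearProjectile is the spear weapon's projectile, damaging what it passes through until it hits something or expires.
; On spawn it faces a distant point along the player camera's forward vector, launches via physics velocity on BoxDestruction, and self-destructs after a short delay.
; BoxEnemiesDetection overlaps send HitMessage with Damage, while BoxDestruction hits destroy the actor, both ignoring the player.
; The construction script applies a configurable uniform scale.
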(event `Destroy`
  (`self.K2_DestroyActor`))

(event `self.ReceiveBeginPlay`
  (`self.K2_SetActorRotation` (`KismetMathLibrary.FindLookAtRotation` (`self.K2_GetActorLocation`) (* (`KismetMathLibrary.GetForwardVector` (`SceneComponent.K2_GetComponentRotation` (`/Game/NIRVANA/Core/Characters/FirstPerson/BP_FirstPersonCharacter.FirstPersonCamera` (`self.Player Ref`)))) 10000000.0)))
  (`PrimitiveComponent.SetPhysicsLinearVelocity` (`self.Box Destruction`) (* (`self.Direction`) (`self.Speed`)) false "None")
  (`KismetSystemLibrary.Delay` 3.0)
  (`self.K2_DestroyActor`))

(event `self.Box Destruction.OnComponentHit`
  (params (HitComponent :type "PrimitiveComponent Object Reference") (OtherActor :type "Actor Object Reference") (OtherComp :type "PrimitiveComponent Object Reference") (NormalImpulse :type "Vector Structure") (Hit :type "HitResult Structure (by ref)"))
  (if (!= OtherActor (`self.Player Ref`))
    (`self.K2_DestroyActor`)))

(event `self.Box Enemies Detection.OnComponentBeginOverlap`
  (params (OverlappedComponent :type "PrimitiveComponent Object Reference") (OtherActor :type "Actor Object Reference") (OtherComp :type "PrimitiveComponent Object Reference") (OtherBodyIndex :type Integer) (bFromSweep :type Boolean) (SweepResult :type "HitResult Structure (by ref)"))
  (if (!= OtherActor (`self.Player Ref`))
    (message `/Game/NIRVANA/Core/Characters/FirstPerson/BPI_Hit.Hit` OtherActor (`self.Damage`))))

(fn `UserConstructionScript`
  (`self.SetActorScale3D` (`KismetMathLibrary.Conv_DoubleToVector` (`self.Scale`))))
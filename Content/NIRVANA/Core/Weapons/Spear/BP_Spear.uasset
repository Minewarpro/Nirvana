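; BP_Spear is a first-person spear weapon that throws BP_SpearProjectile actors, limited by a regenerating charge and a cooldown.
; Firing throws immediately or, with NeedHold, on release after a hold timeline pulls the trident back and activates a ready effect.
; The throw montage's notifies hide the mesh and spawn the projectile, then play a reload montage that shows it again.
; Each throw spends half a charge, which a timeline refills over RecuperationTime.
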(event `self.Fire Start`
  ;[1 1 1] Fire Event
  (if (`self.CanShot`)
    (if (>= (`self.Charge Value`) 0.5)
      (if (not (`self.NeedHold?`))
        (`self.Shoot Animation` :!label _label) ; Start shoot event in Animation
        (set `self.CanShot` false)
        (set `self.IsHoldTimeGood` false)
        (`SceneComponent.K2_SetRelativeLocation` (`self.Trident`) (0.0 0.0 0.0) false false)
        (`self.Use Charge`)
        (`KismetSystemLibrary.Delay` (`KismetMathLibrary.SelectFloat` 0.5 (`self.shootCouldown`) (`self.NeedHold?`)))
        (set `self.CanShot` true)
        (else
          (bind (_direction _spear_offset) (`Timeline|Hold_TL` :!via `PlayFromStart` :!label _label_2)
            (:`Update`
              (`SceneComponent.K2_SetRelativeLocation` (`self.Trident`) (`KismetMathLibrary.MakeVector` 0.0 0.0 (`KismetMathLibrary.Lerp` 0.0 -25.0 _spear_offset)) false false))
            (:`Finished`
              (set `self.IsHoldTimeGood` true)
              (`ActorComponent.Activate` (`self.NS_ReadySpear`) true))))))))

(event `self.Fire Release`
  ;[1 1 1] Fire Event
  (`|ExecutionSequence`
    (:`then_0`
      (goto _label_2 :!via `Stop`))
    (:`then_1`
      (if (`self.IsHoldTimeGood`)
        (goto _label)
        (else
          (`SceneComponent.K2_SetRelativeLocation` (`self.Trident`) (0.0 0.0 0.0) false false))))))

(event `Shoot`
  ;[1 1 1] Shoot Projectile
  (`|SpawnActorFromClass` "/Game/NIRVANA/Core/Weapons/Spear/BP_SpearProjectile.BP_SpearProjectile_C" (`KismetMathLibrary.MakeTransform` (`SceneComponent.GetSocketLocation` (`self.Weapon_Mesh`) "Muzzle")) "AlwaysSpawn" "MultiplyWithRoot" null (`self.Speed Projectile`) (`self.Damage`) (`self.Player Ref`) null))

(event `Shoot Animation`
  ;[1 1 1] Animation
  (bind _notifyname (`|PlayMontage` (`/Game/NIRVANA/Core/Characters/FirstPerson/BP_FirstPersonCharacter.Mesh_1P` (`self.Player Ref`))) ; Spear_ThrowThrow_Montage
    (:`OnNotifyBegin`
      (if (== _notifyname "Throw")
        (`SceneComponent.SetVisibility` (`self.Weapon_Mesh`) false true)
        (`self.Shoot`)
        (elif (== _notifyname "Reload")
          (`|PlayMontage` (`/Game/NIRVANA/Core/Characters/FirstPerson/BP_FirstPersonCharacter.Mesh_1P` (`self.Player Ref`)) ; Spear_ThrowStart_Montage
            (:`then`
              (`SceneComponent.SetVisibility` (`self.Weapon_Mesh`) true true))))))))

(event `Use Charge`
  ;[1 1 1] Charge System
  (set `self.Charge Value` (- (`self.Charge Value`) 0.5))
  (`self.Charge Recuperation`))

(event `Charge Recuperation`
  ;[1 1 1] Charge System
  (set `self.Temp Charge Value` (`self.Charge Value`))
  (`TimelineComponent.SetPlayRate` (`self.Charge Recuperation TL`) (/ 1.0 (`self.Recuperation Time`)))
  (bind (_direction _charge_alpha) (`Timeline|Charge Recuperation TL` :!via `PlayFromStart`)
    (:`Update`
      (set `self.Charge Value` (`KismetMathLibrary.Lerp` (`self.Temp Charge Value`) 1.0 _charge_alpha)))))

(fn `UserConstructionScript`
  (`parent.UserConstructionScript`))
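; BP_Munition is an ammo pickup for one weapon type, with its cube material chosen by that type in the construction script.
; On spawn, its projectile movement launches it upward with a random horizontal offset.
; A detection sphere sets the player capsule as homing target when that weapon's ammo is not full.
; A recovery sphere then grants a per-weapon, partly randomized amount under the same condition and destroys the pickup.
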(event `self.ReceiveBeginPlay`
  (bind _returnvalue (`KismetMathLibrary.RandomFloatInRange` 50.0 200.0))
  (`ProjectileMovementComponent.SetVelocityInLocalSpace` (`self.ProjectileMovement`) (`KismetMathLibrary.MakeVector` _returnvalue _returnvalue 600.0)))

(event `self.Sphere Recuperation.OnComponentBeginOverlap`
  (params (OverlappedComponent :type "PrimitiveComponent Object Reference") (OtherActor :type "Actor Object Reference") (OtherComp :type "PrimitiveComponent Object Reference") (OtherBodyIndex :type Integer) (bFromSweep :type Boolean) (SweepResult :type "HitResult Structure (by ref)"))
  (bind _returnvalue (`KismetMathLibrary.RandomIntegerInRange` 6 9))
  (bind _weapon_munition (`self.Weapon Munition`))
  (bind _weapon_munition_2 (`self.Weapon Munition`))
  (bind _asbp_first_person_character (cast `/Game/NIRVANA/Core/Characters/FirstPerson/BP_FirstPersonCharacter` OtherActor))
  (if (!= (`/Game/NIRVANA/Core/Characters/FirstPerson/BP_FirstPersonCharacter.Get Current Munition` _asbp_first_person_character _weapon_munition_2) (`/Game/NIRVANA/Core/Characters/FirstPerson/BP_FirstPersonCharacter.Get Max Munition` _asbp_first_person_character _weapon_munition_2))
    (`/Game/NIRVANA/Core/Characters/FirstPerson/BP_FirstPersonCharacter.Add Munition` _asbp_first_person_character (select `/Game/NIRVANA/Core/Characters/FirstPerson/Enum_Weapons` _weapon_munition :`NewEnumerator5` (`KismetMathLibrary.RandomIntegerInRange` 1 2) :`NewEnumerator6` _returnvalue :`NewEnumerator7` 1 :`NewEnumerator9` _returnvalue) _weapon_munition)
    (`self.K2_DestroyActor`)))

(event `self.Sphere Detection.OnComponentBeginOverlap`
  (params (OverlappedComponent :type "PrimitiveComponent Object Reference") (OtherActor :type "Actor Object Reference") (OtherComp :type "PrimitiveComponent Object Reference") (OtherBodyIndex :type Integer) (bFromSweep :type Boolean) (SweepResult :type "HitResult Structure (by ref)"))
  (bind _weapon_munition (`self.Weapon Munition`))
  (bind _asbp_first_person_character (cast `/Game/NIRVANA/Core/Characters/FirstPerson/BP_FirstPersonCharacter` OtherActor))
  (if (!= (`/Game/NIRVANA/Core/Characters/FirstPerson/BP_FirstPersonCharacter.Get Current Munition` _asbp_first_person_character _weapon_munition) (`/Game/NIRVANA/Core/Characters/FirstPerson/BP_FirstPersonCharacter.Get Max Munition` _asbp_first_person_character _weapon_munition))
    (set `ProjectileMovementComponent.HomingTargetComponent` (`Character.CapsuleComponent` _asbp_first_person_character) (`self.ProjectileMovement`))))

(fn `UserConstructionScript`
  (`PrimitiveComponent.SetMaterial` (`self.Cube`) 0 (select `/Game/NIRVANA/Core/Characters/FirstPerson/Enum_Weapons` (`self.Weapon Munition`) :`NewEnumerator5` "/Engine/VREditor/BasicMeshes/MI_Cube_03.MI_Cube_03" :`NewEnumerator6` "/Game/DevelopersContent/_GENERATED/Lucaslebeauf/LevelPrototyping/Materials/ProtoTools/Materials/M_ProtoTools_Blue.M_ProtoTools_Blue" :`NewEnumerator7` "/Game/DevelopersContent/_GENERATED/Lucaslebeauf/LevelPrototyping/Materials/Supergrid/M_SuperGrid_DoubleColor.M_SuperGrid_DoubleColor" :`NewEnumerator8` "/Game/DevelopersContent/_GENERATED/Lucaslebeauf/LevelPrototyping/Materials/Supergrid/M_SuperGrid_Default_3.M_SuperGrid_Default_3" :!type "MaterialInterface Object Reference")))
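; BP_Spear is a thrown spear weapon for the player.
; FireStart, gated by CanShot, plays the throw montage on the first-person arms.
; Its "Throw" notify hides the spear mesh and spawns BP_SpearProjectile at the Muzzle socket, passing camera forward direction, speed, damage and the player.
; The "Reload" notify plays the throw-start montage; mesh visibility is not restored in this graph.
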(event `self.Fire Start`
  (if (`self.CanShot`)
    (`self.Shoot Animation`)))

(event `Shoot`
  (`|SpawnActorFromClass` "/Game/NIRVANA/Core/Weapons/Spear/BP_SpearProjectile.BP_SpearProjectile_C" (`KismetMathLibrary.MakeTransform` (`SceneComponent.GetSocketLocation` (`self.Weapon_Mesh`) "Muzzle") (struct)) "AlwaysSpawn" "MultiplyWithRoot" null (`KismetMathLibrary.GetForwardVector` (`SceneComponent.K2_GetComponentRotation` (`/Game/NIRVANA/Core/Characters/FirstPerson/BP_FirstPersonCharacter.FirstPersonCamera` (`self.Player Ref`)))) (`self.Speed Projectile`) (`self.Damage`) (`self.Player Ref`) null))

(event `Shoot Animation`
  ;[1 1 1] Animation
  (bind _notifyname (`|PlayMontage` (`/Game/NIRVANA/Core/Characters/FirstPerson/BP_FirstPersonCharacter.Mesh_1P` (`self.Player Ref`)) "/Game/DevelopersContent/Core/Characters/FirstPerson/Animations/Spear/Spear_ThrowThrow_Montage.Spear_ThrowThrow_Montage")
    (:`OnNotifyBegin`
      (if (== _notifyname "Throw")
        (`SceneComponent.SetVisibility` (`self.Weapon_Mesh`) false false)
        (`self.Shoot`)
        (elif (== _notifyname "Reload")
          (`|PlayMontage` (`/Game/NIRVANA/Core/Characters/FirstPerson/BP_FirstPersonCharacter.Mesh_1P` (`self.Player Ref`)) "/Game/DevelopersContent/Core/Characters/FirstPerson/Animations/Spear/Spear_ThrowStart_Montage.Spear_ThrowStart_Montage"))))))

(fn `UserConstructionScript`
  (`parent.UserConstructionScript`))
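; BP_Hookable_Spike is a spike trap that thrusts a cone out when ActivateTrap fires, hurting whatever it hits.
; A single timeline drives the cone's position, playing fast outward, then reversing slowly after a delay by changing its play rate.
; Box overlaps are enabled for the thrust and disabled shortly after it finishes.
; Overlapping actors receive a hit message with enemy damage, while the player also takes separate player damage.
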(event `self.Activate Trap`
  (`|ExecutionSequence`
    (:`then_0`
      (`TimelineComponent.SetPlayRate` (`self.Spike TL`) (/ 1.0 0.2))
      (set `PrimitiveComponent.bGenerateOverlapEvents` true (`self.Box`))
      (bind (_direction _alpha_locatio) (`Timeline|Spike TL` :!via `PlayFromStart` :!label _label)
        (:`Update`
          (`SceneComponent.K2_SetRelativeLocation` (`self.Cone`) (`KismetMathLibrary.MakeVector` (`KismetMathLibrary.Lerp` -900.0 340.0 _alpha_locatio) 0.0 440.0) false false))
        (:`Finished`
          (`KismetSystemLibrary.Delay` 0.2)
          (set `PrimitiveComponent.bGenerateOverlapEvents` false (`self.Box`)))))
    (:`then_1`
      (`KismetSystemLibrary.Delay` 1.0)
      (`TimelineComponent.SetPlayRate` (`self.Spike TL`) (/ 1.0 6.0))
      (goto _label :!via `Reverse`))))

(event `self.Box.OnComponentBeginOverlap`
  (params (OverlappedComponent :type "PrimitiveComponent Object Reference") (OtherActor :type "Actor Object Reference") (OtherComp :type "PrimitiveComponent Object Reference") (OtherBodyIndex :type Integer) (bFromSweep :type Boolean) (SweepResult :type "HitResult Structure (by ref)"))
  (message `/Game/NIRVANA/Core/Characters/FirstPerson/BPI_Hit.Hit` OtherActor (`self.Damages To Ennemies`) (0.0 0.0 0.0) (0.0 0.0 0.0) "Bind_Pelvis")
  (if (== OtherActor (`self.Player Ref`))
    (`/Game/NIRVANA/Core/Characters/FirstPerson/BP_FirstPersonCharacter.Take Damage` (`self.Player Ref`) (`self.Damages To Player`) null)))

(fn `UserConstructionScript`
  (`parent.UserConstructionScript`))
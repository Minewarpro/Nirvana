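; Placeable double door that swings open or closed when the player enters its trigger or when an arena-cleared event fires.
; The trigger works only while Activable and disables itself after one use, whereas OnArenaCleaned always toggles the door.
; A timeline, rate-scaled by TimeToRotate, rotates both leaves and plays in reverse to close.
; The construction script previews the open state and applies configurable trigger placement and size.
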(event `self.ReceiveBeginPlay`
  ;[1 1 1] PlayerRef
  (bind _asbp_first_person_character (cast `/Game/NIRVANA/Core/Characters/FirstPerson/BP_FirstPersonCharacter` (`GameplayStatics.GetPlayerCharacter` 0)))
  (set `self.PlayerRef` _asbp_first_person_character)
  (`TimelineComponent.SetPlayRate` (`self.DoorRotation`) (/ 1.0 (`self.TimeToRotate`))))

(event `self.Trigger.OnComponentBeginOverlap`
  (params (OverlappedComponent :type "PrimitiveComponent Object Reference") (OtherActor :type "Actor Object Reference") (OtherComp :type "PrimitiveComponent Object Reference") (OtherBodyIndex :type Integer) (bFromSweep :type Boolean) (SweepResult :type "HitResult Structure (by ref)"))
  ;[1 1 1] TriggerBox activation manuelle
  (if (and (== OtherActor (`self.PlayerRef`)) (`self.Activable`))
    (set `self.Activable` false)
    (if (`self.IsOpen`)
      (`self.CloseDoor`)
      (else
        (`self.OpenDoor`)))))

(event `/Game/NIRVANA/Core/Placeables/Management/BPI_ArenaManager.OnArenaCleaned`
  (params (ArenaManager :type "/Game/NIRVANA/Core/Placeables/Management/BP_ArenaManager Object Reference"))
  ;[1 1 1] Interface pour scripting arena
  (if (`self.IsOpen`)
    (`self.CloseDoor`)
    (else
      (`self.OpenDoor`))))

(event `OpenDoor`
  ;[1 1 1] Timeline Overture/Fermeture
  (set `self.IsOpen` true)
  (bind (_direction _newtrack_0) (`Timeline|DoorRotation` :!via `PlayFromStart` :!label _label)
    (:`Update`
      (`SceneComponent.K2_SetRelativeRotation` (`self.DoorLeft`) (`KismetMathLibrary.MakeRotator` 0.0 0.0 (`KismetMathLibrary.Lerp` -180.0 -90.0 _newtrack_0)) false false)
      (`SceneComponent.K2_SetRelativeRotation` (`self.DoorRight`) (`KismetMathLibrary.MakeRotator` 0.0 0.0 (`KismetMathLibrary.Lerp` 0.0 -90.0 _newtrack_0)) false false))))

(event `CloseDoor`
  ;[1 1 1] Timeline Overture/Fermeture
  (set `self.IsOpen` false)
  (goto _label :!via `ReverseFromEnd`))

(fn `UserConstructionScript`
  (`|ExecutionSequence`
    (:`then_0`
      (if (`self.IsOpen`)
        (`SceneComponent.K2_SetRelativeRotation` (`self.DoorLeft`) (`KismetMathLibrary.MakeRotator` 0.0 0.0 -90.0) false false)
        (`SceneComponent.K2_SetRelativeRotation` (`self.DoorRight`) (`KismetMathLibrary.MakeRotator` 0.0 0.0 -90.0) false false)))
    (:`then_1`
      (`SceneComponent.K2_SetRelativeLocation` (`self.Trigger`) (`KismetMathLibrary.MakeVector` (`self.TriggerLocX`) (`self.TriggerLocY`) (`self.TriggerLocZ`)) false false)
      (`SceneComponent.SetRelativeScale3D` (`self.Trigger`) (`KismetMathLibrary.MakeVector` (`self.TriggerSizeX`) (`self.TriggerSizeY`) (`self.TriggerSizeZ`))))))
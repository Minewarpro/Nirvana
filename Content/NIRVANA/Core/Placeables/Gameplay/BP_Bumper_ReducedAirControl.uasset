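; Bumper placeable variant that temporarily limits the player's movement, including air control, after an overlap.
; It extends a parent bumper's overlap logic by disabling slide and jump and applying its own air control value to the player's CharacterMovement.
; After a delay it resolves slide, re-enables jump and restores the air control cached at BeginPlay.
; On destruction it restores only the air control.
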(event `self.ReceiveBeginPlay`
  (`parent.ReceiveBeginPlay`)
  (set `self.InitAirControl` (`CharacterMovementComponent.AirControl` (`Character.CharacterMovement` (`self.PlayerRef`)))))

(event `self.Overlap`
  (params (Actor :type "Actor Object Reference"))
  (bind _playerref (`self.PlayerRef`))
  (bind _playerref_2 (`self.PlayerRef`))
  (`parent.Overlap` Actor)
  (set `/Game/NIRVANA/Core/Characters/FirstPerson/BP_FirstPersonCharacter.CanSlide` false _playerref)
  (set `/Game/NIRVANA/Core/Characters/FirstPerson/BP_FirstPersonCharacter.Can Jump` false _playerref)
  (set `CharacterMovementComponent.AirControl` (`self.AirControl`) (`Character.CharacterMovement` _playerref))
  (`KismetSystemLibrary.Delay` (`self.AirControlDuration`))
  (`/Game/NIRVANA/Core/Characters/FirstPerson/BP_FirstPersonCharacter.Resolve Slide` _playerref_2)
  (set `/Game/NIRVANA/Core/Characters/FirstPerson/BP_FirstPersonCharacter.Can Jump` true _playerref_2)
  (set `CharacterMovementComponent.AirControl` (`self.InitAirControl`) (`Character.CharacterMovement` _playerref_2)))

(event `self.ReceiveDestroyed`
  (set `CharacterMovementComponent.AirControl` (`self.InitAirControl`) (`Character.CharacterMovement` (`self.PlayerRef`))))

(fn `UserConstructionScript`
  (`parent.UserConstructionScript`))
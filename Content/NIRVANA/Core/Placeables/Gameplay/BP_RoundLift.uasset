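; Placeable lift that carries the player from its origin to a set end offset, with voice lines during the ride.
; Player overlap on the Start trigger runs a lerp timeline scaled by TravelTime, then plays voices sequentially from last array entry to first.
; Overlapping the construction-script-placed ResetBox, meant for falls, stops the lift, returns it to origin and re-arms it.
; The OnArenaCleaned event also enables starting when the manager matches InitArena.
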(event `self.ReceiveBeginPlay`
  (bind _asbp_first_person_character (cast `/Game/NIRVANA/Core/Characters/FirstPerson/BP_FirstPersonCharacter` (`GameplayStatics.GetPlayerCharacter` 0)))
  (set `self.PlayerRef` _asbp_first_person_character)
  (`TimelineComponent.SetPlayRate` (`self.LiftTravel1`) (/ 1.0 (`self.TravelTime`)))
  (set `self.LiftOrigin` (`SceneComponent.K2_GetComponentLocation` (`self.Lift`))))

(event `self.Start.OnComponentBeginOverlap`
  (params (OverlappedComponent :type "PrimitiveComponent Object Reference") (OtherActor :type "Actor Object Reference") (OtherComp :type "PrimitiveComponent Object Reference") (OtherBodyIndex :type Integer) (bFromSweep :type Boolean) (SweepResult :type "HitResult Structure (by ref)"))
  ;[1 1 1] Start
  (`|ExecutionSequence`
    (:`then_0`
      (if (and (== OtherActor (`self.PlayerRef`)) (`self.CanStart`))
        (set `self.CanStart` false)
        (`self.StartLift`)
        (`KismetSystemLibrary.Delay` 1.0)
        (`self.PlayVoices`)))))

(event `self.ResetBox.OnComponentBeginOverlap`
  (params (OverlappedComponent :type "PrimitiveComponent Object Reference") (OtherActor :type "Actor Object Reference") (OtherComp :type "PrimitiveComponent Object Reference") (OtherBodyIndex :type Integer) (bFromSweep :type Boolean) (SweepResult :type "HitResult Structure (by ref)"))
  ;[1 1 1] Reset
  (if (== OtherActor (`self.PlayerRef`))
    (`self.Reset`)))

(event `StartLift`
  ;[1 1 1] Move lift
  (bind (_direction _newtrack_0) (`Timeline|LiftTravel1` :!via `PlayFromStart` :!label _label)
    (:`Update`
      (`SceneComponent.K2_SetRelativeLocation` (`self.Lift`) (`KismetMathLibrary.VLerp` (0.0 0.0 0.0) (`self.CoordsEnd`) _newtrack_0) false false))))

(event `Reset`
  ;[1 1 1] Reset en cas de chute
  (`|ExecutionSequence`
    (:`then_0`
      (goto _label :!via `Stop`))
    (:`then_1`
      (set `self.CanStart` true)
      (`SceneComponent.K2_SetWorldLocation` (`self.Lift`) (`self.LiftOrigin`) false false))))

(event `/Game/NIRVANA/Core/Placeables/Management/BPI_ArenaManager.OnArenaCleaned`
  (params (ArenaManager :type "/Game/NIRVANA/Core/Placeables/Management/BP_ArenaManager Object Reference"))
  ;[1 1 1] Interface on arena
  (if (== ArenaManager (`self.InitArena`))
    (set `self.CanStart` true)))

(event `PlayVoices`
  (bind _sizeofsequence (`self.SizeOfSequence`))
  (bind _output (`|GetArrayItem` (`self.VoicesInSequence`) (- (`self.SizeOfSequence`) 1)))
  ;[1 1 1] Play Voices
  (if (> (`self.SizeOfSequence`) 0)
    (set `self.DelayForSequence` (+ (`SoundBase.Duration` _output) 0.8))
    (`GameplayStatics.PlaySoundAtLocation` _output (`self.K2_GetActorLocation` (`self.PlayerRef`)) (struct) (`self.VolumeMultiplier`) 1.0 0.0 null null null null)
    (set `self.SizeOfSequence` (- _sizeofsequence 1))
    (`KismetSystemLibrary.Delay` (`self.DelayForSequence`))
    (if (> _sizeofsequence 0)
      (`self.PlayVoices`))))

(fn `UserConstructionScript`
  (bind _resetbox (`self.ResetBox`))
  (`SceneComponent.SetWorldScale3D` _resetbox (`self.ResetScale`))
  (`SceneComponent.K2_SetRelativeLocation` _resetbox (`self.ResetLocation`) false false))
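; BP_Bumper is a placeable gameplay bumper that flings the first-person player along the direction of its Arrow component.
; On BeginPlay it caches the player character, and its Box overlap responds only to that actor.
; On overlap it zeroes movement velocity, then applies a velocity-change impulse from Arrow forward XY scaled by Velocity, with ZVelocityFactor as vertical speed.
; An alternative LaunchCharacter call is left disconnected.
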(event `self.ReceiveBeginPlay`
  (bind _asbp_first_person_character (cast `/Game/NIRVANA/Core/Characters/FirstPerson/BP_FirstPersonCharacter` (`GameplayStatics.GetPlayerCharacter` 0)))
  (set `self.PlayerRef` _asbp_first_person_character))

(event `self.Box.OnComponentBeginOverlap`
  (params (OverlappedComponent :type "PrimitiveComponent Object Reference") (OtherActor :type "Actor Object Reference") (OtherComp :type "PrimitiveComponent Object Reference") (OtherBodyIndex :type Integer) (bFromSweep :type Boolean) (SweepResult :type "HitResult Structure (by ref)"))
  (bind (_returnvalue_x _returnvalue_y) (`KismetMathLibrary.BreakVector` (`SceneComponent.GetForwardVector` (`self.Arrow`))))
  (bind _charactermovement (`Character.CharacterMovement` (`self.PlayerRef`)))
  (if (== OtherActor (`self.PlayerRef`))
    (set `MovementComponent.Velocity` (0.0 0.0 0.0) _charactermovement)
    (`CharacterMovementComponent.AddImpulse` _charactermovement (`KismetMathLibrary.MakeVector` (* _returnvalue_x (`self.Velocity`)) (* _returnvalue_y (`self.Velocity`)) (`self.ZVelocityFactor`)) true)))

(fn `UserConstructionScript`)
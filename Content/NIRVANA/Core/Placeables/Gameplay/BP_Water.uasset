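; BP_Water is a placeable water volume that tells the first-person player character when it enters and leaves the water.
; It caches the player on BeginPlay, then calls InWater and OutWater from the Water component's begin and end overlaps, ignoring other actors.
; The construction script offsets the Collision box downward by its scaled Z extent plus Height, so its top sits Height below its parent's origin.
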(event `self.ReceiveBeginPlay`
  (bind _asbp_first_person_character (cast `/Game/NIRVANA/Core/Characters/FirstPerson/BP_FirstPersonCharacter` (`GameplayStatics.GetPlayerCharacter` 0)))
  (set `self.PlayerRef` _asbp_first_person_character))

(event `self.Water.OnComponentBeginOverlap`
  (params (OverlappedComponent :type "PrimitiveComponent Object Reference") (OtherActor :type "Actor Object Reference") (OtherComp :type "PrimitiveComponent Object Reference") (OtherBodyIndex :type Integer) (bFromSweep :type Boolean) (SweepResult :type "HitResult Structure (by ref)"))
  (bind _playerref (`self.PlayerRef`))
  (if (== OtherActor _playerref)
    (`/Game/NIRVANA/Core/Characters/FirstPerson/BP_FirstPersonCharacter.InWater` _playerref)))

(event `self.Water.OnComponentEndOverlap`
  (params (OverlappedComponent :type "PrimitiveComponent Object Reference") (OtherActor :type "Actor Object Reference") (OtherComp :type "PrimitiveComponent Object Reference") (OtherBodyIndex :type Integer))
  (bind _playerref (`self.PlayerRef`))
  (if (== OtherActor _playerref)
    (`/Game/NIRVANA/Core/Characters/FirstPerson/BP_FirstPersonCharacter.OutWater` _playerref)))

(fn `UserConstructionScript`
  (bind _collision (`self.Collision`))
  (bind (_returnvalue_x _returnvalue_y _returnvalue_z) (`KismetMathLibrary.BreakVector` (* (* (`SceneComponent.RelativeScale3D` _collision) (`BoxComponent.BoxExtent` _collision)) -1.0)))
  (`SceneComponent.K2_SetRelativeLocation` _collision (`KismetMathLibrary.MakeVector` 0.0 0.0 (- _returnvalue_z (`self.Height`))) false false))
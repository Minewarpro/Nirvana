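; Cinematic events Blueprint, named as a backup, that dissolves and resolves the referenced Vajra's skeletal mesh.
; BeginPlay creates and stores a dynamic material instance for the mesh's first material slot.
; DissolveVajra plays a timeline forward and ResolveVajra reverses it from the end.
; The timeline's update writes the Alpha scalar parameter directly on the mesh's materials, not through the stored instance.
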(event `self.ReceiveBeginPlay`
  (bind _skeletalmeshcomponent (`SkeletalMeshActor.SkeletalMeshComponent` (`self.Vajra`)))
  (bind _returnvalue (`PrimitiveComponent.CreateDynamicMaterialInstance` _skeletalmeshcomponent 0 (`PrimitiveComponent.GetMaterial` _skeletalmeshcomponent 0) "None"))
  (set `self.Material instance` _returnvalue))

(event `DissolveVajra`
  (`TimelineComponent.SetPlayRate` (`self.Timeline`) (/ 1.0 1.0))
  (bind (_direction _alpha_dissolve) (`Timeline|Timeline` :!via `PlayFromStart` :!label _label)
    (:`Update`
      (`MeshComponent.SetScalarParameterValueOnMaterials` (`SkeletalMeshActor.SkeletalMeshComponent` (`self.Vajra`)) "Alpha" (`KismetMathLibrary.Lerp` 0.0 1.0 _alpha_dissolve)))))

(event `ResolveVajra`
  (`TimelineComponent.SetPlayRate` (`self.Timeline`) (/ 1.0 1.0))
  (goto _label :!via `ReverseFromEnd`))

(fn `UserConstructionScript`)
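; Main menu camera actor that moves a cine camera between its origin, options and game-start views.
; BeginPlay caches origin and marker locations, then per-transition timelines lerp location and rotation, with options and return moves updating the current pose on finish.
; StartGame also plays a launch sequence alongside its move.
; A separate idle timeline drifts the root vertically and can be stopped, though this graph's calls to both are disconnected.
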(event `self.ReceiveBeginPlay`
  (bind _cinecamera (`self.CineCamera`))
  (bind _returnvalue (`SceneComponent.K2_GetComponentLocation` _cinecamera))
  (bind _returnvalue_2 (`SceneComponent.K2_GetComponentRotation` _cinecamera))
  (set `self.OriginLocation` _returnvalue)
  (set `self.currentLocation` _returnvalue)
  (set `self.OriginRotation` _returnvalue_2)
  (set `self.currentRotation` _returnvalue_2)
  (set `self.IsIdle` true)
  (`TimelineComponent.SetPlayRate` (`self.IdleMove`) (/ 1.0 10.0))
  (set `self.OptionsLocation` (`SceneComponent.K2_GetComponentLocation` (`self.optionloc`)))
  (set `self.StartLocation` (`SceneComponent.K2_GetComponentLocation` (`self.Start`))))

(event `Idle`
  (bind (_currentlocation_x _currentlocation_y _currentlocation_z) (`KismetMathLibrary.BreakVector` (`self.currentLocation`)))
  (bind (_direction _newtrack_0) (`Timeline|IdleMove` :!via `PlayFromStart` :!label _label)
    (:`Update`
      (`SceneComponent.K2_SetWorldLocation` (`self.DefaultSceneRoot`) (`KismetMathLibrary.VLerp` (`self.currentLocation`) (`KismetMathLibrary.MakeVector` _currentlocation_x _currentlocation_y (+ _currentlocation_z 150.0)) _newtrack_0) false false))))

(event `PauseIdle`
  (goto _label :!via `Stop`))

(event `Options`
  (`TimelineComponent.SetPlayRate` (`self.ToOptions`) (/ 1.0 2.0))
  (bind (_direction _newtrack_0) (`Timeline|ToOptions` :!via `PlayFromStart`)
    (:`Update`
      (`SceneComponent.K2_SetWorldLocationAndRotation` (`self.CineCamera`) (`KismetMathLibrary.VLerp` (`self.currentLocation`) (`self.OptionsLocation`) _newtrack_0) (`KismetMathLibrary.RLerp` (`self.currentRotation`) (`self.OptionsRotation`) _newtrack_0 true) false false))
    (:`Finished`
      (set `self.currentLocation` (`self.OptionsLocation`))
      (set `self.currentRotation` (`self.OptionsRotation`)))))

(event `BackToOrigin`
  (`TimelineComponent.SetPlayRate` (`self.MovaBack`) (/ 1.0 2.0))
  (bind (_direction _newtrack_0) (`Timeline|MovaBack` :!via `PlayFromStart`)
    (:`Update`
      (`SceneComponent.K2_SetWorldLocationAndRotation` (`self.CineCamera`) (`KismetMathLibrary.VLerp` (`self.currentLocation`) (`self.OriginLocation`) _newtrack_0) (`KismetMathLibrary.RLerp` (`self.currentRotation`) (`self.OriginRotation`) _newtrack_0 true) false false))
    (:`Finished`
      (set `self.currentLocation` (`self.OriginLocation`))
      (set `self.currentRotation` (`self.OriginRotation`)))))

(event `StartGame`
  (`|ExecutionSequence`
    (:`then_0`
      (`TimelineComponent.SetPlayRate` (`self.StartMove`) (/ 1.0 1.5))
      (bind (_direction _newtrack_0) (`Timeline|StartMove` :!via `PlayFromStart`)
        (:`Update`
          (`SceneComponent.K2_SetWorldLocationAndRotation` (`self.CineCamera`) (`KismetMathLibrary.VLerp` (`self.currentLocation`) (`self.StartLocation`) _newtrack_0) (`KismetMathLibrary.RLerp` (`self.currentRotation`) (`self.StartRotation`) _newtrack_0 true) false false))))
    (:`then_1`
      (`MovieSceneSequencePlayer.Play` (`LevelSequenceActor.SequencePlayer` (`self.SequencerToLaunch`))))))

(fn `UserConstructionScript`)
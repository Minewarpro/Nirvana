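; A placeable one-shot trigger that plays a Level Sequence cinematic for the first-person player and can grant the Chakram weapon.
; On overlap it fades out, hides the HUD, disables input and blends to a configured view target for the sequence's duration, then teleports the player, restores control and fades in.
; With CHAKRAM set, a delayed step overwrites the weapon loadout in the Game Instance and player, switches weapon and reveals the Chakram HUD.
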(event `self.ReceiveBeginPlay`
  ;[1 1 1] SetPlayerRef
  (bind _asbp_first_person_character (cast `/Game/NIRVANA/Core/Characters/FirstPerson/BP_FirstPersonCharacter` (`GameplayStatics.GetPlayerCharacter` 0)))
  (set `self.PlayerRef` _asbp_first_person_character))

(event `self.trigger.OnComponentBeginOverlap`
  (params (OverlappedComponent :type "PrimitiveComponent Object Reference") (OtherActor :type "Actor Object Reference") (OtherComp :type "PrimitiveComponent Object Reference") (OtherBodyIndex :type Integer) (bFromSweep :type Boolean) (SweepResult :type "HitResult Structure (by ref)"))
  (bind _playerref (`self.PlayerRef`))
  (bind _playerref_2 (`self.PlayerRef`))
  (bind _wb_base_ref (`/Game/NIRVANA/Core/Characters/FirstPerson/BP_FirstPersonCharacter.WB_Base_Ref` _playerref))
  ;[1 1 1] Trigger Detection player
  (if (and (== OtherActor (`self.PlayerRef`)) (`self.IsActive`))
    (set `self.IsActive` false)
    (`PlayerCameraManager.StartCameraFade` :`self` (`GameplayStatics.GetPlayerCameraManager` 0) :`ToAlpha` 1.0 :`Duration` 0.5)
    (`KismetSystemLibrary.Delay` 0.5)
    (`self.PlayCine`)
    (if (`self.CHAKRAM`)
      (`KismetSystemLibrary.Delay` 1.0)
      (bind _output_get (set `/Game/NIRVANA/Core/GameModes/Game_Instance.WeaponToEquip` (`|MakeArray` "NewEnumerator12" "NewEnumerator11" "NewEnumerator8" :!type "/Game/NIRVANA/Core/Characters/FirstPerson/Enum_Weapons Enum") (cast `/Game/NIRVANA/Core/GameModes/Game_Instance` (`GameplayStatics.GetGameInstance`) :!pure true)))
      (set `/Game/NIRVANA/Core/Characters/FirstPerson/BP_FirstPersonCharacter.MyWeapons` _output_get _playerref_2)
      (bind _output_get_2 (set `/Game/NIRVANA/Core/Characters/FirstPerson/BP_FirstPersonCharacter.Current Weapon` "NewEnumerator8" _playerref_2))
      (`/Game/NIRVANA/Core/Characters/FirstPerson/BP_FirstPersonCharacter.Change Weapon` _playerref_2 _output_get_2 2)
      (`Widget.SetVisibility` (`/Game/NIRVANA/UI/Player/WB_Base.ProgressBar_Chakram` _wb_base_ref) "Visible")
      (`Widget.SetVisibility` (`/Game/NIRVANA/UI/Player/WB_Base.SecondaryChakramCanva` _wb_base_ref) "Visible")
      (`/Game/NIRVANA/UI/Player/WB_Base.Play Animation Switch Weapon` _wb_base_ref "Forward")
      (`/Game/NIRVANA/Core/Characters/FirstPerson/BP_FirstPersonCharacter.Next Weapon` _playerref 1))))

(event `PlayCine`
  (bind _returnvalue (`GameplayStatics.GetPlayerController` 0))
  (bind _returnvalue_2 (`GameplayStatics.GetPlayerController` 0))
  (bind _sequenceplayer (`LevelSequenceActor.SequencePlayer` (`self.SequencerToPlay`)))
  ;[1 1 1] Play Sequencer
  (`Widget.SetVisibility` (`/Game/NIRVANA/Core/Characters/FirstPerson/BP_FirstPersonCharacter.WB_Base_Ref` (`self.PlayerRef`)) "Hidden")
  (`self.DisableInput` (`self.PlayerRef`) _returnvalue_2)
  (set `self.CamToReturn` (`Controller.GetViewTarget` _returnvalue_2))
  (`PlayerController.SetViewTargetWithBlend` _returnvalue_2 (`self.BPToBlend`) (`self.BlendTime`) "VTBlend_Linear" 0.0 false)
  (set `/Game/NIRVANA/Core/Characters/FirstPerson/BP_FirstPersonCharacter.inCinematic` true (`self.PlayerRef`))
  (`MovieSceneSequencePlayer.Play` _sequenceplayer)
  (`KismetSystemLibrary.Delay` (`TimeManagementBlueprintLibrary.Conv_QualifiedFrameTimeToSeconds` (`MovieSceneSequencePlayer.GetDuration` _sequenceplayer)))
  (set `/Game/NIRVANA/Core/Characters/FirstPerson/BP_FirstPersonCharacter.inCinematic` false (`self.PlayerRef`))
  (`self.K2_SetActorLocation` (`self.PlayerRef`) (`SceneComponent.K2_GetComponentLocation` (`self.TP`)) false false)
  (`Controller.SetControlRotation` _returnvalue (`self.RotationTP`))
  (`PlayerController.SetViewTargetWithBlend` _returnvalue (`self.CamToReturn`) (`self.BlendTime`) "VTBlend_EaseOut" 0.0 false)
  (`PlayerCameraManager.StartCameraFade` :`self` (`GameplayStatics.GetPlayerCameraManager` 0) :`FromAlpha` 1.0 :`Duration` 0.8)
  (`self.EnableInput` (`self.PlayerRef`) _returnvalue)
  (`Widget.SetVisibility` (`/Game/NIRVANA/Core/Characters/FirstPerson/BP_FirstPersonCharacter.WB_Base_Ref` (`self.PlayerRef`)) "Visible"))

(fn `UserConstructionScript`
  (`SceneComponent.SetRelativeScale3D` (`self.trigger`) (`self.TriggerSize`))
  (`SceneComponent.K2_SetRelativeLocation` (`self.TP`) (`self.CoordsTP`) false false))
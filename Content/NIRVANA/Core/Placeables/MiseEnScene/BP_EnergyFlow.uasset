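; BP_EnergyFlow is a placeable that animates an energy flow along a row of meshes.
; The construction script builds a configurable-length row of strip meshes and a matching set of cube meshes along X.
; At BeginPlay it creates dynamic materials for both sets.
; Timelines then animate each strip's Panner and matching cube's emissive in sequence, optionally inverted, looping after an end delay.
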(event `self.ReceiveBeginPlay`
  (`KismetArrayLibrary.Array_Clear` (`self.MatTab`))
  (`|ExecutionSequence`
    (:`then_0`
      (`self.SetLastIndex`)
      (for _array_element (`self.Tab`)
        (bind _returnvalue (`PrimitiveComponent.CreateDynamicMaterialInstance` _array_element 0 null "None"))
        (`KismetArrayLibrary.Array_Add` (`self.MatTab`) _returnvalue))
      (for _array_element_2 (`self.CubeTab`)
        (bind _returnvalue_2 (`PrimitiveComponent.CreateDynamicMaterialInstance` _array_element_2 0 null "None"))
        (`KismetArrayLibrary.Array_Add` (`self.CubeMatTab`) _returnvalue_2)))
    (:`then_1`
      (`KismetSystemLibrary.Delay` (`self.Delay`))
      (`self.CubeIntensity`)
      (`self.PlayPanner`))))

(event `SetLastIndex`
  (set `self.MaxIndex` (`KismetArrayLibrary.Array_LastIndex` (`self.Tab`))))

(event `PlayPanner`
  (bind _paninverted (`self.PanInverted`))
  (set `self.MatToPan` (`|GetArrayItem` (`self.MatTab`) (`self.IndexToPan`)))
  (`TimelineComponent.SetPlayRate` (`self.Panner`) (/ 1.0 (`self.PannerPlayRate`)))
  (bind (_direction _newtrack_0 _newtrack_1) (`Timeline|Panner` :!via `PlayFromStart`)
    (:`Update`
      (`MaterialInstanceDynamic.SetScalarParameterValue` (`self.MatToPan`) "Panner" (`KismetMathLibrary.Lerp` (`KismetMathLibrary.SelectFloat` 0.0 -0.35 _paninverted) (`KismetMathLibrary.SelectFloat` 1.35 1.0 _paninverted) (`KismetMathLibrary.SelectFloat` _newtrack_0 _newtrack_1 _paninverted))))
    (:`Finished`
      (bind _output_get (set `self.IndexToPan` (+ (`self.IndexToPan`) 1)))
      (if (> _output_get (`self.MaxIndex`))
        (set `self.IndexToPan` 0)
        (`KismetSystemLibrary.Delay` (`self.EndDelay`))
        (`self.CubeIntensity`)
        (`self.PlayPanner`)
        (else
          (`self.CubeIntensity`)
          (`self.PlayPanner`))))))

(event `CubeIntensity`
  (set `self.MatCube` (`|GetArrayItem` (`self.CubeMatTab`) (`self.IndexToPan`)))
  (`TimelineComponent.SetPlayRate` (`self.Intensity`) (/ 1.0 0.2))
  (bind (_direction _newtrack_0) (`Timeline|Intensity` :!via `PlayFromStart`)
    (:`Update`
      (`MaterialInstanceDynamic.SetScalarParameterValue` (`self.MatCube`) "Emissive Multiply" (`KismetMathLibrary.Lerp` 0.024 0.5 _newtrack_0)))))

(fn `UserConstructionScript`
  (`KismetArrayLibrary.Array_Clear` (`self.Tab`))
  (`KismetArrayLibrary.Array_Clear` (`self.CubeTab`))
  (for _index (range (`self.MeshNumber`))
    (bind _returnvalue (`AddComponent|NODE_AddStaticMeshComponent-1` :`RelativeTransform` (`KismetMathLibrary.MakeTransform` (`KismetMathLibrary.MakeVector` (`KismetMathLibrary.Conv_IntToDouble` (* _index (* 499 (`self.ScaleX`))))) (`KismetMathLibrary.MakeRotator` 0.0 0.0 (`KismetMathLibrary.SelectFloat` 180.0 0.0 (`self.IsRotated`))) (`KismetMathLibrary.MakeVector` (`self.ScaleX`) 1.0 1.0))))
    (`KismetArrayLibrary.Array_Add` (`self.Tab`) _returnvalue))
  (for _index_2 (range (`self.MeshNumber`))
    (bind _returnvalue_2 (`AddComponent|NODE_AddStaticMeshComponent-2` :`RelativeTransform` (`KismetMathLibrary.MakeTransform` (`KismetMathLibrary.MakeVector` (`KismetMathLibrary.Conv_IntToDouble` (* (- _index_2 1) (* 499 (`self.ScaleX`))))) (`KismetMathLibrary.MakeRotator` 0.0 0.0 (`KismetMathLibrary.SelectFloat` 180.0 0.0 (`self.IsRotated`))))))
    (`KismetArrayLibrary.Array_Add` (`self.CubeTab`) _returnvalue_2)))
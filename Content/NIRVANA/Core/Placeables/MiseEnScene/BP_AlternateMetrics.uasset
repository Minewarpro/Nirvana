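; BP_AlternateMetrics is a mise-en-scène placeable built to change the first-person player's walk speed while a sequence of voice lines plays.
; StartVoices plays the sounds at the player's location from last array index to first, re-calling itself after each clip's duration plus padding.
; When the sequence runs out, BackToNormal restores the saved walk speed.
; The logic that saves and overrides the speed and the initial StartVoices call are disconnected and never run.
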(event `self.ReceiveBeginPlay`)

(event `StartVoices`
  (bind _sizeofsequence (`self.SizeOfSequence`))
  (bind _output (`|GetArrayItem` (`self.VoicesInSequence`) (- (`self.SizeOfSequence`) 1)))
  (`KismetSystemLibrary.Delay` 0.5)
  (if (> (`self.SizeOfSequence`) 0)
    (set `self.DelayForSequence` (+ (`SoundBase.Duration` _output) 0.5))
    (`GameplayStatics.PlaySoundAtLocation` _output (`self.K2_GetActorLocation` (`self.PlayerRef`)) (struct) (`self.VolumeMultiplier`) 1.0 0.0 null null null null)
    (set `self.SizeOfSequence` (- _sizeofsequence 1))
    (`KismetSystemLibrary.Delay` (`self.DelayForSequence`))
    (if (> _sizeofsequence 0)
      (`self.StartVoices`)
      (else
        (`self.BackToNormal`)))))

(event `BackToNormal`
  (set `/Game/NIRVANA/Core/Characters/FirstPerson/BP_FirstPersonCharacter.WalkSpeed` (`self.SpeedToReturn`) (`self.PlayerRef`)))

(fn `UserConstructionScript`)
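; BP_UIManagerStart is a placeable actor that exposes events to control the player's HUD and subtitles.
; On BeginPlay it caches the player as BP_FirstPersonCharacter, then uses that reference to reach the character's base widget and subtitle widget.
; Separate events show or hide each widget, and the Subtiles event sets the subtitle text.
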(event `self.ReceiveBeginPlay`
  (bind _asbp_first_person_character (cast `/Game/NIRVANA/Core/Characters/FirstPerson/BP_FirstPersonCharacter` (`GameplayStatics.GetPlayerCharacter` 0)))
  (set `self.PlayerRef` _asbp_first_person_character))

(event `HideUI`
  (`Widget.SetVisibility` (`/Game/NIRVANA/Core/Characters/FirstPerson/BP_FirstPersonCharacter.WB_Base_Ref` (`self.PlayerRef`)) "Hidden"))

(event `RevealUI`
  (`Widget.SetVisibility` (`/Game/NIRVANA/Core/Characters/FirstPerson/BP_FirstPersonCharacter.WB_Base_Ref` (`self.PlayerRef`)) "Visible"))

(event `Subtiles`
  (params (Text :type Text))
  (set `TextBlock.Text` Text (`/Game/NIRVANA/UI/WB_Subtitles.Subtitle` (`/Game/NIRVANA/Core/Characters/FirstPerson/BP_FirstPersonCharacter.SubtitleRef` (`self.PlayerRef`)))))

(event `ActivateSubtitles`
  (`Widget.SetVisibility` (`/Game/NIRVANA/Core/Characters/FirstPerson/BP_FirstPersonCharacter.SubtitleRef` (`self.PlayerRef`)) "Visible"))

(event `CutSubtitles`
  (`Widget.SetVisibility` (`/Game/NIRVANA/Core/Characters/FirstPerson/BP_FirstPersonCharacter.SubtitleRef` (`self.PlayerRef`)) "Hidden"))

(fn `UserConstructionScript`)
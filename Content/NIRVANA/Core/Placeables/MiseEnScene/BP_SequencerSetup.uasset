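; BP_SequencerSetup is a placeable that plays a one-shot cinematic when its OnArenaCleaned event fires while active.
; After a short delay, it hides the player's HUD, disables input, blends to a chosen camera and plays the assigned sequence.
; Once the sequence's duration elapses, it blends back to the previous view target and restores input and HUD.
; The construction script sizes a Trigger and positions a TP component, neither used by the event logic.
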(event `self.ReceiveBeginPlay`
  ;[1 1 1] SetPlayerRef
  (bind _asbp_first_person_character (cast `/Game/NIRVANA/Core/Characters/FirstPerson/BP_FirstPersonCharacter` (`GameplayStatics.GetPlayerCharacter` 0)))
  (set `self.PlayerRef` _asbp_first_person_character))

(event `/Game/NIRVANA/Core/Placeables/Management/BPI_ArenaManager.OnArenaCleaned`
  (params (ArenaManager :type "/Game/NIRVANA/Core/Placeables/Management/BP_ArenaManager Object Reference"))
  ;[1 1 1] Trigger Detection player
  (if (`self.IsActive`)
    (set `self.IsActive` false)
    (`KismetSystemLibrary.Delay` 1.0)
    (`self.PlayCine`)))

(event `PlayCine`
  (bind _returnvalue (`GameplayStatics.GetPlayerController` 0))
  (bind _returnvalue_2 (`GameplayStatics.GetPlayerController` 0))
  (bind _sequenceplayer (`LevelSequenceActor.SequencePlayer` (`self.SequencerToPlay`)))
  ;[1 1 1] Play Sequencer
  (`Widget.SetVisibility` (`/Game/NIRVANA/Core/Characters/FirstPerson/BP_FirstPersonCharacter.WB_Base_Ref` (`self.PlayerRef`)) "Hidden")
  (`self.DisableInput` (`self.PlayerRef`) _returnvalue_2)
  (set `self.CamToReturn` (`Controller.GetViewTarget` _returnvalue_2))
  (`PlayerController.SetViewTargetWithBlend` _returnvalue_2 (`self.CamToBlend`) (`self.BlendTime`) "VTBlend_Linear" 0.0 false)
  (`MovieSceneSequencePlayer.Play` _sequenceplayer)
  (`KismetSystemLibrary.Delay` (`TimeManagementBlueprintLibrary.Conv_QualifiedFrameTimeToSeconds` (`MovieSceneSequencePlayer.GetDuration` _sequenceplayer)))
  (`PlayerController.SetViewTargetWithBlend` _returnvalue (`self.CamToReturn`) (`self.BlendTime`) "VTBlend_EaseOut" 0.0 false)
  (`self.EnableInput` (`self.PlayerRef`) _returnvalue)
  (`Widget.SetVisibility` (`/Game/NIRVANA/Core/Characters/FirstPerson/BP_FirstPersonCharacter.WB_Base_Ref` (`self.PlayerRef`)) "Visible"))

(fn `UserConstructionScript`
  (`SceneComponent.SetRelativeScale3D` (`self.trigger`) (`self.TriggerSize`))
  (`SceneComponent.K2_SetRelativeLocation` (`self.TP`) (`self.CoordsTP`) false false))
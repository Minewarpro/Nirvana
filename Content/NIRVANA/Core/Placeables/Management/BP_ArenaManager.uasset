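; Arena manager that paces combat by rationing attacks among the ranged and swarmer enemies inside its box.
; On BeginPlay, box traces collect spawn areas and enemies, then two self-rescheduling loops rotate attackers.
; On-screen shooters draw from a shared token pool, while swarmers punch when in range.
; A timed spawner, not started here, walks linked areas with caps, an emergency burst, and leader or kill-count stops.
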(event `self.ReceiveBeginPlay`
  (bind _box (`self.Box`))
  (bind _returnvalue (`SceneComponent.K2_GetComponentLocation` _box))
  (bind _returnvalue_2 (`SceneComponent.K2_GetComponentRotation` _box))
  (bind _returnvalue_3 (* (`BoxComponent.BoxExtent` _box) (`self.GetActorScale3D`)))
  (bind _outhits (`KismetSystemLibrary.BoxTraceMulti` _returnvalue _returnvalue _returnvalue_3 _returnvalue_2 "TraceTypeQuery5"))
  (for _array_element _outhits
    (bind _asbp_enemy_area (cast `/Game/NIRVANA/Core/Placeables/Management/BP_EnemyArea` (`.HitActor` (`GameplayStatics.BreakHitResult` _array_element))))
    (`KismetArrayLibrary.Array_Add` (`self.Areas`) _asbp_enemy_area))
  (bind _outhits_2 (`KismetSystemLibrary.BoxTraceMulti` _returnvalue _returnvalue _returnvalue_3 _returnvalue_2 "TraceTypeQuery3"))
  (for _array_element_2 _outhits_2
    (bind _asbp_enemy_range (cast `/Game/NIRVANA/Core/Characters/Enemies/Range/BP_EnemyRange` (`.HitActor` (`GameplayStatics.BreakHitResult` _array_element_2)))
      (:`then`
        (`KismetArrayLibrary.Array_Add` (`self.Total EnemiesRange`) _asbp_enemy_range)
        (set `/Game/NIRVANA/Core/Characters/Enemies/Range/BP_EnemyRange.ArenaManager` self _asbp_enemy_range))
      (:`CastFailed`
        (bind _asbp_enemy_swarmer (cast `/Game/NIRVANA/Core/Characters/Enemies/Swarmer/BP_EnemySwarmer` (`.HitActor` (`GameplayStatics.BreakHitResult` _array_element_2))))
        (`KismetArrayLibrary.Array_Add` (`self.Total EnemiesSwarmer`) _asbp_enemy_swarmer))))
  (set `self.CurrentArea` (`KismetArrayLibrary.Array_Random` (`self.Areas`)))
  (`self.TokenDistribution`)
  (`self.SwarmerAttack`))

(event `Spawn Loop`
  (bind _returnvalue (`KismetSystemLibrary.K2_SetTimerDelegate` (delegate `Testing Spawn`) (`self.Spawn Delay`) true -5.0))
  (set `self.Spawn loop event` _returnvalue))

(event `Testing Spawn`
  (bind _total_enemiesrange (`self.Total EnemiesRange`))
  (for (_array_element _array_index) _total_enemiesrange
    (`/Engine/EditorBlueprintResources/StandardMacros.IsValid` _array_element
      (:`Is Not Valid`
        (`KismetArrayLibrary.Array_Remove` _total_enemiesrange _array_index))))
  (if (`self.CanSpawn`)
    (if (<= (`KismetArrayLibrary.Array_Length` (`self.Total EnemiesRange`)) (`self.Nb Enemie Cas Urgence`))
      (for _ (range (+ (`self.Nb Spawn Enemie Urgence`) 1))
        (bind _spawned_npc (`/Game/NIRVANA/Core/Placeables/Management/BP_EnemyArea.SpawnNPC` (`self.Get Next Area`) self :!label _label))
        (`/Engine/EditorBlueprintResources/StandardMacros.IsValid` _spawned_npc
          (:`Is Valid`
            (`KismetArrayLibrary.Array_Add` (`self.Total EnemiesRange`) _spawned_npc))))
      (else
        (goto _label)))))

(event `TokenDistribution`
  (if (not (`self.IsEnemyAttacking`))
    (bind _shooter (`self.GetShooter`))
    (`/Engine/EditorBlueprintResources/StandardMacros.IsValid` _shooter
      (:`Is Valid`
        (`self.MartialArtRange`)
        (`self.GetToken` (- (`/Game/NIRVANA/Core/Characters/Enemies/Range/BP_EnemyRange.TokenToShoot` _shooter) (`/Game/NIRVANA/Core/Characters/Enemies/Range/BP_EnemyRange.Token` _shooter)) _shooter))
      (:`Is Not Valid`
        (`KismetSystemLibrary.K2_SetTimerDelegate` (delegate `TokenDistribution`) 0.13579)))))

(event `MartialArtRange`
  (set `self.IsEnemyAttacking` true)
  (`KismetSystemLibrary.Delay` (`self.MartialArtRangeDelay`))
  (set `self.IsEnemyAttacking` false)
  (`self.TokenDistribution`))

(event `SwarmerAttack`
  (bind _slacher (`self.GetSlasher`))
  (`/Engine/EditorBlueprintResources/StandardMacros.IsValid` _slacher
    (:`Is Valid`
      (`/Game/NIRVANA/Core/Characters/Enemies/Common/BP_Enemy.Punch` _slacher)
      (`self.MartialArtSwarmer`))
    (:`Is Not Valid`
      (`KismetSystemLibrary.K2_SetTimerDelegate` (delegate `SwarmerAttack`) 0.13579))))

(event `MartialArtSwarmer`
  (`KismetSystemLibrary.Delay` (`self.MartialArtSwarmerDelay`))
  (`self.SwarmerAttack`))

(fn `Add Nb Killed Enemy`
  (bind _output_get (set `self.Enemy Killed` (+ (`self.Enemy Killed`) 1)))
  (if (>= _output_get (`self.Nb Need To Kill`))
    (`KismetSystemLibrary.K2_ClearAndInvalidateTimerHandle` (`self.Spawn loop event`))))

(fn `CanSpawn`
  (returns (`Can Spawn` :type Boolean))
  (bind _leaders (`self.Leaders`))
  (if (`self.Need Leader`)
    (for _array_element _leaders
      (`/Engine/EditorBlueprintResources/StandardMacros.IsValid` _array_element
        (:`Is Not Valid`
          (`KismetArrayLibrary.Array_RemoveItem` _leaders _array_element))))
    (if (and (`KismetArrayLibrary.Array_IsEmpty` _leaders) (`self.Need Leader`))
      (`KismetSystemLibrary.K2_ClearAndInvalidateTimerHandle` (`self.Spawn loop event`))
      (return false)
      (else
        _)))
  (return (< (`KismetArrayLibrary.Array_Length` (`self.Total EnemiesRange`)) (`self.Nb Max Enemie`))))

(fn `Get Next Area`
  (returns (Area :type "/Game/NIRVANA/Core/Placeables/Management/BP_EnemyArea Object Reference"))
  (bind _output_get (set `self.CurrentArea` (`KismetArrayLibrary.Array_Random` (`/Game/NIRVANA/Core/Placeables/Management/BP_EnemyArea.Next Areas` (`self.CurrentArea`)))))
  (return _output_get))

(fn `GetShooter`
  (returns (Shooter :type "/Game/NIRVANA/Core/Characters/Enemies/Range/BP_EnemyRange Object Reference"))
  (locals (CurrentRange :type "/Game/NIRVANA/Core/Characters/Enemies/Range/BP_EnemyRange Object Reference"))
  (bind _currentrange (`local.CurrentRange`))
  (bind _total_enemiesrange (`self.Total EnemiesRange`))
  (for _array_element (`self.Total EnemiesRange`)
    (`/Engine/EditorBlueprintResources/StandardMacros.IsValid` _array_element
      (:`Is Valid`
        (if (`/Game/NIRVANA/Core/Characters/Enemies/Common/BP_Enemy.CanAttack` _array_element)
          (if (<= (`/Game/NIRVANA/Core/Characters/Enemies/Range/BP_EnemyRange.TokenToShoot` _array_element) (`/Game/NIRVANA/Core/Characters/Enemies/Range/BP_EnemyRange.Token` _array_element))
            _
            (elif (`/Game/NIRVANA/Core/Characters/Enemies/Common/BP_Enemy.IsOnScreen` _array_element 45.0)
              (bind _output_get (set `local.CurrentRange` _array_element))
              (`KismetArrayLibrary.Array_RemoveItem` _total_enemiesrange _output_get)
              (`KismetArrayLibrary.Array_Add` _total_enemiesrange _currentrange)
              (return _currentrange)))))
      (:`Is Not Valid`
        (`KismetSystemLibrary.PrintString` (`KismetSystemLibrary.GetDisplayName` _array_element) true true (struct :`R` 0.618751 :`B` 1.0 :`A` 1.0)))))
  (return null))

(fn `GetSlasher`
  (returns (Slacher :type "/Game/NIRVANA/Core/Characters/Enemies/Swarmer/BP_EnemySwarmer Object Reference"))
  (locals (CurrentSwarmer :type "/Game/NIRVANA/Core/Characters/Enemies/Swarmer/BP_EnemySwarmer Object Reference"))
  (bind _total_enemiesswarmer (`self.Total EnemiesSwarmer`))
  (bind _currentswarmer (`local.CurrentSwarmer`))
  (for _array_element (`self.Total EnemiesSwarmer`)
    (bind _returnvalue (`AIBlueprintHelperLibrary.GetBlackboard` (`AIBlueprintHelperLibrary.GetAIController` _array_element)))
    (`/Engine/EditorBlueprintResources/StandardMacros.IsValid` _returnvalue
      (:`Is Valid`
        (if (and (`/Game/NIRVANA/Core/Characters/Enemies/Common/BP_Enemy.CanAttack` _array_element) (`BlackboardComponent.GetValueAsBool` _returnvalue "PlayerInRange") (not (== (`SkeletalMeshComponent.GetAnimInstance` (`Character.Mesh` _array_element)) "/Game/DevelopersContent/Core/Characters/Enemies/Common/Mixamo_Test/AM_Taunt.AM_Taunt")) (not (`BlackboardComponent.GetValueAsBool` _returnvalue "IsJumping")))
          (bind _output_get (set `local.CurrentSwarmer` _array_element))
          (`KismetArrayLibrary.Array_RemoveItem` _total_enemiesswarmer _currentswarmer)
          (`KismetArrayLibrary.Array_Add` _total_enemiesswarmer _currentswarmer)
          (return _output_get)))))
  (return null))

(fn `GetToken`
  (params (Amount :type Integer) (Enemy :type "/Game/NIRVANA/Core/Characters/Enemies/Range/BP_EnemyRange Object Reference"))
  (locals (HasValid :type Boolean) (availableTokens :type Integer :default 0))
  (bind _tokens (`self.Tokens`))
  (bind _output_get (set `local.availableTokens` (`KismetMathLibrary.SelectInt` Amount _tokens (<= Amount _tokens))))
  (set `self.Tokens` (- (`self.Tokens`) _output_get))
  (set `/Game/NIRVANA/Core/Characters/Enemies/Range/BP_EnemyRange.Token` (+ (`/Game/NIRVANA/Core/Characters/Enemies/Range/BP_EnemyRange.Token` Enemy) _output_get) Enemy)
  (return))

(fn `ReleaseToken`
  (params (Enemy :type "/Game/NIRVANA/Core/Characters/Enemies/Range/BP_EnemyRange Object Reference"))
  (set `/Game/NIRVANA/Core/Characters/Enemies/Range/BP_EnemyRange.Token` 0 Enemy)
  (`|SpawnActorFromClass` "/Game/NIRVANA/Core/Characters/FirstPerson/BP_TokenReAb.BP_TokenReAb_C" (`KismetMathLibrary.MakeTransform` (0.0 0.0 0.0)) "Undefined" "MultiplyWithRoot" null self (`/Game/NIRVANA/Core/Characters/Enemies/Range/BP_EnemyRange.TokenToShoot` Enemy) null)
  (return))

(fn `UserConstructionScript`
  (`BoxComponent.SetBoxExtent` (`self.Box`) (`self.In Box Extent`) true)
  (set `self.Need Leader` (!= (`KismetArrayLibrary.Array_Length` (`self.Leaders`)) 0))
  (set `self.Tokens` (`self.TokensMax`)))
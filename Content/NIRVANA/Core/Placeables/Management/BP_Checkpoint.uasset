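; Checkpoint trigger that sets and saves the player's respawn point when the first-person character enters its box.
; On overlap it disables further overlaps, stores its location with the player's rotation and scale in Game_Instance, then saves.
; Checkpoints are identified by world location: if absent from the save's list, it prints a message and appends itself to the "SaveMain" slot, if that exists.
; The construction script orients an arrow from Rot, which does not affect the spawn transform.
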(event `self.ReceiveBeginPlay`)

(event `self.Box.OnComponentBeginOverlap`
  (params (OverlappedComponent :type "PrimitiveComponent Object Reference") (OtherActor :type "Actor Object Reference") (OtherComp :type "PrimitiveComponent Object Reference") (OtherBodyIndex :type Integer) (bFromSweep :type Boolean) (SweepResult :type "HitResult Structure (by ref)"))
  (bind _returnvalue_location (`KismetMathLibrary.BreakTransform` (`self.GetTransform`)))
  (bind _asgame_instance (cast `/Game/NIRVANA/Core/GameModes/Game_Instance` (`GameplayStatics.GetGameInstance`) :!pure true))
  (bind _asbp_first_person_character (cast `/Game/NIRVANA/Core/Characters/FirstPerson/BP_FirstPersonCharacter` OtherActor))
  (set `PrimitiveComponent.bGenerateOverlapEvents` false (`self.Box`))
  (bind (_returnvalue_location_2 _returnvalue_rotation _returnvalue_scale) (`KismetMathLibrary.BreakTransform` (`self.GetTransform` _asbp_first_person_character)))
  (set `/Game/NIRVANA/Core/GameModes/Game_Instance.Spawn Location` (`KismetMathLibrary.MakeTransform` _returnvalue_location _returnvalue_rotation _returnvalue_scale) _asgame_instance)
  (`/Game/NIRVANA/Core/GameModes/Game_Instance.Save` _asgame_instance)
  (bind _output_get (set `self.SaveGame` (`/Game/NIRVANA/Core/GameModes/Game_Instance.SaveGame` _asgame_instance)))
  (for _array_element (`/Game/NIRVANA/Core/GameModes/SaveGameMain.Checkpoint Location` _output_get)
    (if (== _array_element (`self.K2_GetActorLocation`))
      (set `self.Active` false)))
  (if (`self.Active`)
    (`KismetSystemLibrary.PrintString` "CHECKPOINT")
    (set `PrimitiveComponent.bGenerateOverlapEvents` false (`self.Box`))
    (bind _returnvalue (`GameplayStatics.DoesSaveGameExist` "SaveMain"))
    (if _returnvalue
      (`KismetArrayLibrary.Array_Add` (`/Game/NIRVANA/Core/GameModes/SaveGameMain.Checkpoint Location` (`self.SaveGame`)) (`self.K2_GetActorLocation`))
      (`GameplayStatics.SaveGameToSlot` (`self.SaveGame`) "SaveMain"))))

(fn `UserConstructionScript`
  (`SceneComponent.K2_SetRelativeRotation` (`self.Arrow`) (`self.rot`) false false))
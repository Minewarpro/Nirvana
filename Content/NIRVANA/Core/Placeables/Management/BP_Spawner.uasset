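; BP_Spawner is a placeable box volume that supplies random navigable points inside its bounds, with no spawning logic in this file.
; The construction script sizes the box from an extent variable.
; GetRandomPointInSpawner scales the bounds by actor scale and Precision, rotates the random offset by actor yaw, then projects it 300 units lower onto the navmesh.
; A zero projection result triggers an uncapped recursive retry.
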(fn `GetRandomPointInSpawner`
  (params (Precision :type "Float (double-precision)" :default 0.75))
  (returns (RandomPoint :type "Vector Structure"))
  (locals (ImpactPoint :type "Vector Structure"))
  (bind (_returnvalue_roll _returnvalue_pitch _returnvalue_yaw) (`KismetMathLibrary.BreakRotator` (`self.K2_GetActorRotation`)))
  (bind _box (`self.Box`))
  (bind _returnvalue (`SceneComponent.K2_GetComponentLocation` _box))
  (bind _returnvalue_2 (`KismetMathLibrary.RandomPointInBoundingBox` _returnvalue (* (`BoxComponent.BoxExtent` _box) (`self.GetActorScale3D`) (`local.Precision`))))
  (bind _output_get (set `local.ImpactPoint` (`NavigationSystemV1.K2_ProjectPointToNavigation` (- (+ (* (`KismetMathLibrary.RotateAngleAxis` (`KismetMathLibrary.GetDirectionUnitVector` _returnvalue _returnvalue_2) _returnvalue_yaw (0.0 0.0 1.0)) (`KismetMathLibrary.Vector_Distance` _returnvalue_2 _returnvalue)) _returnvalue) (0.0 0.0 300.0)) null null (10.0 10.0 300.0))))
  (if (== _output_get (0.0 0.0 0.0) :`ErrorTolerance` 0.0)
    (return (`self.GetRandomPointInSpawner` Precision))
    (else
      (return (`local.ImpactPoint`)))))

(fn `UserConstructionScript`
  (`BoxComponent.SetBoxExtent` (`self.Box`) (`self.InBoxExtent`) true))
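; BP_SpawnManager is a placeable trigger that spawns ranged enemies when the player enters its box.
; On begin play it caches the first-person player character, and it checks overlaps against that reference while it is activated.
; It asks the ArenaManager to spawn V1 enemies at each spawner in List1 and V2 enemies at those in List2.
; It then deactivates itself after triggering.
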(event `self.ReceiveBeginPlay`
  (bind _asbp_first_person_character (cast `/Game/NIRVANA/Core/Characters/FirstPerson/BP_FirstPersonCharacter` (`GameplayStatics.GetPlayerCharacter` 0)))
  (set `self.PlayerRef` _asbp_first_person_character))

(event `self.Box.OnComponentBeginOverlap`
  (params (OverlappedComponent :type "PrimitiveComponent Object Reference") (OtherActor :type "Actor Object Reference") (OtherComp :type "PrimitiveComponent Object Reference") (OtherBodyIndex :type Integer) (bFromSweep :type Boolean) (SweepResult :type "HitResult Structure (by ref)"))
  (bind _arenamanager (`self.ArenaManager`))
  (if (`self.Activated`)
    (if (== OtherActor (`self.PlayerRef`))
      (for _array_element (`self.List1`)
        (`/Game/NIRVANA/Core/Placeables/Management/BP_ArenaManager.SpawnEnemy` _arenamanager "/Game/NIRVANA/Core/Characters/Enemies/Range/BP_EnemyRange_V1.BP_EnemyRange_V1_C" _array_element))
      (for _array_element_2 (`self.List2`)
        (`/Game/NIRVANA/Core/Placeables/Management/BP_ArenaManager.SpawnEnemy` _arenamanager "/Game/NIRVANA/Core/Characters/Enemies/Range/BP_EnemyRange_V2.BP_EnemyRange_V2_C" _array_element_2))
      (set `self.Activated` false))))

(fn `UserConstructionScript`)
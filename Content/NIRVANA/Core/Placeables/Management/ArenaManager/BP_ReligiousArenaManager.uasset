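; BP_ReligiousArenaManager is an arena manager for the religious arena that picks shoot sequences and their difficulty.
; SetFirstShootSequence and SetNewSootSequence both draw a random entry from the Normal pool into CurrentSequence, but set different CurrentDifficulty values.
; A weighted Easy/Normal/Hard selection is left unconnected, so the random float rolled for new sequences has no effect.
; The event graph holds only disabled placeholder events.
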(fn `SetFirstShootSequence`
  (set `self.currentSequence` (`KismetArrayLibrary.Array_Random` (`self.Normal`)))
  (set `self.currentDifficulty` "NewEnumerator1")
  (return))

(fn `SetNewSootSequence`
  (locals (rand :type "Float (double-precision)"))
  (set `local.rand` (`KismetMathLibrary.RandomFloat`))
  (set `self.currentSequence` (`KismetArrayLibrary.Array_Random` (`self.Normal`)))
  (set `self.currentDifficulty` "NewEnumerator0")
  (return))

(fn `UserConstructionScript`
  (`parent.UserConstructionScript`))
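; Placeable box volume that supplies random navigable spawn points, presumably for swarmer enemies.
; The construction script sizes the box from an extent variable.
; GetRandomPointInSpawner picks a point in the scaled box, rotates it by actor yaw, lowers it and projects it onto the navmesh.
; Failed projections retry recursively with a tightened area up to a capped count, then fall back to the box center.
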(fn `GetRandomPointInSpawner`
  (params (Precision :type "Float (double-precision)" :default 0.75) (Iterations :type Integer :default 0))
  (returns (RandomPoint :type "Vector Structure"))
  (locals (ImpactPoint :type "Vector Structure"))
  (bind (_returnvalue_roll _returnvalue_pitch _returnvalue_yaw) (`KismetMathLibrary.BreakRotator` (`self.K2_GetActorRotation`)))
  (bind _returnvalue (+ Iterations 1))
  (bind _box (`self.Box`))
  (bind _returnvalue_2 (`SceneComponent.K2_GetComponentLocation` _box))
  (bind _returnvalue_3 (`KismetMathLibrary.RandomPointInBoundingBox` _returnvalue_2 (* (`BoxComponent.BoxExtent` _box) (`self.GetActorScale3D`) (`local.Precision`))))
  (bind _output_get (set `local.ImpactPoint` (`NavigationSystemV1.K2_ProjectPointToNavigation` (- (+ (* (`KismetMathLibrary.RotateAngleAxis` (`KismetMathLibrary.GetDirectionUnitVector` _returnvalue_2 _returnvalue_3) _returnvalue_yaw (0.0 0.0 1.0)) (`KismetMathLibrary.Vector_Distance` _returnvalue_3 _returnvalue_2)) _returnvalue_2) (0.0 0.0 100.0)) null null (10.0 10.0 100.0))))
  (if (== _output_get (0.0 0.0 0.0))
    (if (<= _returnvalue 30)
      (return (`self.GetRandomPointInSpawner` 0.75 _returnvalue))
      (else
        (return (`SceneComponent.K2_GetComponentLocation` (`self.Box`)))))
    (else
      (return (`local.ImpactPoint`)))))

(fn `UserConstructionScript`
  (`BoxComponent.SetBoxExtent` (`self.Box`) (`self.InBoxExtent`) true))
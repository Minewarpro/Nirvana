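; BP_HeavyZone is a placeable box zone that detects BP_Fake_Heavy actors standing in it when play begins.
; The construction script sizes the Zone box from the BoxExtent variable.
; On BeginPlay, a zero-length multi box trace matching the box's scaled extent and rotation marks the zone occupied and sets itself as each found heavy's CurrentZone.
; Occupancy is not updated afterwards in this Blueprint.
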(event `self.ReceiveBeginPlay`
  (bind _zone (`self.Zone`))
  (bind _returnvalue (`SceneComponent.K2_GetComponentLocation` _zone))
  (bind (_outhits _returnvalue_2) (`KismetSystemLibrary.BoxTraceMulti` _returnvalue _returnvalue (* (`BoxComponent.BoxExtent` _zone) (`self.GetActorScale3D`)) (`SceneComponent.K2_GetComponentRotation` _zone) "TraceTypeQuery3"))
  (if _returnvalue_2
    (for _array_element _outhits
      (bind _asbp_fake_heavy (cast `/Game/NIRVANA/Core/Characters/Enemies/Heavy/BP_Fake_Heavy` (`.HitActor` (`GameplayStatics.BreakHitResult` _array_element))))
      (set `self.IsOccupated` true)
      (set `/Game/NIRVANA/Core/Characters/Enemies/Heavy/BP_Fake_Heavy.CurrentZone` self _asbp_fake_heavy))))

(fn `UserConstructionScript`
  (`BoxComponent.SetBoxExtent` (`self.Zone`) (`self.Box Extent`) true))
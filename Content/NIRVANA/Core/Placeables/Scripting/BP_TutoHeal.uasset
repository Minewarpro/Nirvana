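; BP_TutoHeal is a placeable trigger that heals the player to full health, apparently for the tutorial.
; On BeginPlay it caches the player's BP_FirstPersonCharacter as PlayerRef.
; When that character overlaps the Box while Activated is set, it clears the flag and sets CurrentHealth to MaxHealth, with nothing in the Blueprint re-arming it.
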(event `self.ReceiveBeginPlay`
  (bind _asbp_first_person_character (cast `/Game/NIRVANA/Core/Characters/FirstPerson/BP_FirstPersonCharacter` (`GameplayStatics.GetPlayerCharacter` 0)))
  (set `self.PlayerRef` _asbp_first_person_character))

(event `self.Box.OnComponentBeginOverlap`
  (params (OverlappedComponent :type "PrimitiveComponent Object Reference") (OtherActor :type "Actor Object Reference") (OtherComp :type "PrimitiveComponent Object Reference") (OtherBodyIndex :type Integer) (bFromSweep :type Boolean) (SweepResult :type "HitResult Structure (by ref)"))
  (bind _playerref (`self.PlayerRef`))
  (if (and (== OtherActor (`self.PlayerRef`)) (`self.Activated`))
    (set `self.Activated` false)
    (set `/Game/NIRVANA/Core/Characters/FirstPerson/BP_FirstPersonCharacter.Current Health` (`/Game/NIRVANA/Core/Characters/FirstPerson/BP_FirstPersonCharacter.MaxHealth` _playerref) _playerref)))

(fn `UserConstructionScript`)
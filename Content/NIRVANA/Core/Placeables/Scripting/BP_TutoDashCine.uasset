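; Placeable trigger that runs a dash tutorial: when the player overlaps its box while Activated, it plays a one-time cinematic.
; It disables input, blends to a set camera, plays a level sequence, then blends back to the player.
; A timeline eases global time dilation into slow motion while a dash info widget shows.
; Pressing Dash removes the widget, reverses the slow motion and slides a wall aside along Y.
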(event `self.ReceiveBeginPlay`
  (bind _returnvalue (`GameplayStatics.GetPlayerCharacter` 0))
  (bind _asbp_first_person_character (cast `/Game/NIRVANA/Core/Characters/FirstPerson/BP_FirstPersonCharacter` _returnvalue))
  (set `self.PlayerRef` _asbp_first_person_character)
  (set `self.CamToReturn` _returnvalue))

(event `self.Box.OnComponentBeginOverlap`
  (params (OverlappedComponent :type "PrimitiveComponent Object Reference") (OtherActor :type "Actor Object Reference") (OtherComp :type "PrimitiveComponent Object Reference") (OtherBodyIndex :type Integer) (bFromSweep :type Boolean) (SweepResult :type "HitResult Structure (by ref)"))
  (if (and (== OtherActor (`self.PlayerRef`)) (`self.Activated`))
    (`self.StartSequencer`)
    (set `self.Activated` false)))

(event `StartSequencer`
  (bind _returnvalue (`GameplayStatics.GetPlayerController` 0))
  (bind _sequenceplayer (`LevelSequenceActor.SequencePlayer` (`self.SequenceToPlay`)))
  (bind (_returnvalue_x _returnvalue_y) (`KismetMathLibrary.BreakVector` (`SceneComponent.K2_GetComponentLocation` (`StaticMeshActor.StaticMeshComponent` (`self.WallToMove`)))))
  (`self.DisableInput` (`self.PlayerRef`) _returnvalue)
  (`PlayerController.SetViewTargetWithBlend` _returnvalue (`self.CamToBlend`) (`self.BlendTime`) "VTBlend_Linear" 0.0 false)
  (set `/Game/NIRVANA/Core/Characters/FirstPerson/BP_FirstPersonCharacter.inCinematic` true (`self.PlayerRef`))
  (`MovieSceneSequencePlayer.Play` _sequenceplayer)
  (`KismetSystemLibrary.Delay` (`TimeManagementBlueprintLibrary.Conv_QualifiedFrameTimeToSeconds` (`MovieSceneSequencePlayer.GetDuration` _sequenceplayer)))
  (set `/Game/NIRVANA/Core/Characters/FirstPerson/BP_FirstPersonCharacter.inCinematic` false (`self.PlayerRef`))
  (`PlayerController.SetViewTargetWithBlend` (`GameplayStatics.GetPlayerController` 0) (`self.CamToReturn`) (`self.BlendTime`) "VTBlend_Linear" 0.0 false)
  (`self.EnableInput` (`self.PlayerRef`) (`GameplayStatics.GetPlayerController` 0))
  (`self.StartTuto`)
  (set `self.OriginY` _returnvalue_y))

(event `StartTuto`
  (`self.SlowMoStart`)
  (bind _returnvalue (`|CreateWidget` "/Game/NIRVANA/UI/Player/WB_TutoInfos.WB_TutoInfos_C" null false false false true))
  (bind _output_get (set `self.TutoInfo` _returnvalue))
  (`UserWidget.AddToViewport` _output_get 0)
  (set `self.CanEndTuto` true))

(event `SlowMoStart`
  (bind (_direction _newtrack_0) (`Timeline|Timeline` :!via `PlayFromStart` :!label _label)
    (:`Update`
      (`GameplayStatics.SetGlobalTimeDilation` (`KismetMathLibrary.Lerp` 1.0 0.1 _newtrack_0)))))

(event `SlowMoEnd`
  (goto _label :!via `ReverseFromEnd`))

(event `EnhancedInput|/Game/NIRVANA/Core/Characters/FirstPerson/Input/Actions/IA_Dash`
  (params (ActionValue :type Boolean) (ElapsedSeconds :type "Float (double-precision)") (TriggeredSeconds :type "Float (double-precision)") (InputAction :type "InputAction Object Reference" :default "/Game/NIRVANA/Core/Characters/FirstPerson/Input/Actions/IA_Dash.IA_Dash"))
  (bind _originy (`self.OriginY`))
  (bind _staticmeshcomponent (`StaticMeshActor.StaticMeshComponent` (`self.WallToMove`)))
  (bind (_returnvalue_x _returnvalue_y _returnvalue_z) (`KismetMathLibrary.BreakVector` (`SceneComponent.K2_GetComponentLocation` _staticmeshcomponent)))
  (:`Started`
    (if (`self.CanEndTuto`)
      (`Widget.RemoveFromParent` (`self.TutoInfo`))
      (`self.SlowMoEnd`)
      (set `self.CanEndTuto` false)
      (bind (_direction _newtrack_0) (`Timeline|WallMove` :!via `PlayFromStart`)
        (:`Update`
          (`SceneComponent.K2_SetWorldLocation` _staticmeshcomponent (`KismetMathLibrary.MakeVector` _returnvalue_x (`KismetMathLibrary.Lerp` _originy (- _originy 750.0) _newtrack_0) _returnvalue_z) false false))))))

(fn `UserConstructionScript`)
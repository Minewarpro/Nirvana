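; Tutorial trigger volume that closes a referenced partition (cloison) mesh when the player enters its box.
; On BeginPlay it caches the first-person character and the partition's starting height.
; A player overlap clears the Activated flag, so it fires only once if armed, then plays a Timeline.
; The Timeline lerps the partition straight down by a fixed distance, leaving X and Y unchanged.
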(event `self.ReceiveBeginPlay`
  (bind (_returnvalue_x _returnvalue_y _returnvalue_z) (`KismetMathLibrary.BreakVector` (`SceneComponent.K2_GetComponentLocation` (`StaticMeshActor.StaticMeshComponent` (`self.CloisonToClose`)))))
  (bind _asbp_first_person_character (cast `/Game/NIRVANA/Core/Characters/FirstPerson/BP_FirstPersonCharacter` (`GameplayStatics.GetPlayerCharacter` 0)))
  (set `self.PlayerRef` _asbp_first_person_character)
  (set `self.StartZ` _returnvalue_z))

(event `self.Box.OnComponentBeginOverlap`
  (params (OverlappedComponent :type "PrimitiveComponent Object Reference") (OtherActor :type "Actor Object Reference") (OtherComp :type "PrimitiveComponent Object Reference") (OtherBodyIndex :type Integer) (bFromSweep :type Boolean) (SweepResult :type "HitResult Structure (by ref)"))
  (bind _startz (`self.StartZ`))
  (bind _staticmeshcomponent (`StaticMeshActor.StaticMeshComponent` (`self.CloisonToClose`)))
  (bind (_returnvalue_x _returnvalue_y) (`KismetMathLibrary.BreakVector` (`SceneComponent.K2_GetComponentLocation` _staticmeshcomponent)))
  (if (== OtherActor (`self.PlayerRef`))
    (if (`self.Activated`)
      (set `self.Activated` false)
      (bind (_direction _newtrack_0) (`Timeline|Timeline` :!via `PlayFromStart`)
        (:`Update`
          (`SceneComponent.K2_SetWorldLocation` _staticmeshcomponent (`KismetMathLibrary.MakeVector` _returnvalue_x _returnvalue_y (`KismetMathLibrary.Lerp` _startz (- _startz 800.0) _newtrack_0)) false false))))))

(fn `UserConstructionScript`)
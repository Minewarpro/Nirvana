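; BP_Ring is a placeable ring of five SArceau pieces that widens when OnArenaCleaned fires.
; After a short delay, a slowed timeline plays from the start and lerps each piece's X and Y scale while Z stays fixed.
; Each piece has its own start and end size, so the smaller ones grow most and the nested set spreads outward into a tighter band.
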(event `/Game/NIRVANA/Core/Placeables/Management/BPI_ArenaManager.OnArenaCleaned`
  (params (ArenaManager :type "/Game/NIRVANA/Core/Placeables/Management/BP_ArenaManager Object Reference"))
  (`KismetSystemLibrary.Delay` 1.5)
  (`TimelineComponent.SetPlayRate` (`self.Timeline`) (/ 1.0 3.0))
  (bind (_direction _scale_alpha) (`Timeline|Timeline` :!via `PlayFromStart`)
    (:`Update`
      (bind _returnvalue (`KismetMathLibrary.Lerp` 1.907866 2.187011 _scale_alpha))
      (`SceneComponent.SetRelativeScale3D` (`self.S_Arceau_A1`) (`KismetMathLibrary.MakeVector` _returnvalue _returnvalue 1.0))
      (bind _returnvalue_2 (`KismetMathLibrary.Lerp` 1.434963 2.030404 _scale_alpha))
      (`SceneComponent.SetRelativeScale3D` (`self.S_Arceau_A2`) (`KismetMathLibrary.MakeVector` _returnvalue_2 _returnvalue_2 1.0))
      (bind _returnvalue_3 (`KismetMathLibrary.Lerp` 1.016897 1.917607 _scale_alpha))
      (`SceneComponent.SetRelativeScale3D` (`self.S_Arceau_A3`) (`KismetMathLibrary.MakeVector` _returnvalue_3 _returnvalue_3 1.0))
      (bind _returnvalue_4 (`KismetMathLibrary.Lerp` 0.601433 1.780459 _scale_alpha))
      (`SceneComponent.SetRelativeScale3D` (`self.S_Arceau_A4`) (`KismetMathLibrary.MakeVector` _returnvalue_4 _returnvalue_4 1.0))
      (bind _returnvalue_5 (`KismetMathLibrary.Lerp` 0.218682 1.67888 _scale_alpha))
      (`SceneComponent.SetRelativeScale3D` (`self.S_Arceau_A5`) (`KismetMathLibrary.MakeVector` _returnvalue_5 _returnvalue_5 1.0)))))

(fn `UserConstructionScript`)
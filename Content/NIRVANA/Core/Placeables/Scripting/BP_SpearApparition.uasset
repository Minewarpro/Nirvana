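; Placeable spear that rises into view while spinning, activates a linked bridge and can run a cinematic.
; Apparition drives timelines that lift it by Hauteur and yaw it, with spin rate set by LoopDuration.
; StartSequencer disables input, blends to a camera, plays the sequence and switches weapon; EndCine restores view and input, then destroys the spear.
; The trigger box overlap does nothing, and HideBack is never called here.
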(event `self.ReceiveBeginPlay`
  (cast `/Game/NIRVANA/Core/Characters/FirstPerson/BP_FirstPersonCharacter` (`GameplayStatics.GetPlayerCharacter` 0))
  (set `self.PlayerRef` null)
  (set `self.InitRotate` (`self.K2_GetActorRotation`)))

(event `Apparition`
  (bind (_returnvalue_x _returnvalue_y) (`KismetMathLibrary.BreakVector` (`self.K2_GetActorLocation`)))
  (bind (_temp_location_x _temp_location_y _temp_location_z) (`KismetMathLibrary.BreakVector` (`self.Temp Location`)))
  ;[1 1 1] Apparition de la lance
  (`/Game/NIRVANA/Core/Placeables/Gameplay/BP_MovablePlatform.Activate` (`self.Bridge Ref`))
  (set `self.Temp Location` (`self.K2_GetActorLocation`))
  (`|ExecutionSequence`
    (:`then_0`
      (bind (_direction _alpha) (`Timeline|Apparition TL` :!via `PlayFromStart`)
        (:`Update`
          (`self.K2_SetActorLocation` (`KismetMathLibrary.MakeVector` _returnvalue_x _returnvalue_y (`KismetMathLibrary.Lerp` _temp_location_z (+ _temp_location_z (`self.Hauteur`)) _alpha)))
          (`self.K2_SetActorRotation` (`KismetMathLibrary.MakeRotator` 0.0 0.0 (`KismetMathLibrary.Lerp` 0.0 270.0 _alpha))))))
    (:`then_1`
      (`self.Rotate`))))

(event `self.Box.OnComponentBeginOverlap`
  (params (OverlappedComponent :type "PrimitiveComponent Object Reference") (OtherActor :type "Actor Object Reference") (OtherComp :type "PrimitiveComponent Object Reference") (OtherBodyIndex :type Integer) (bFromSweep :type Boolean) (SweepResult :type "HitResult Structure (by ref)"))
  ;[1 1 1] Trigger pour cinématique
  (if (== OtherActor (`self.PlayerRef`))
    _))

(event `StartSequencer`
  (bind _returnvalue (`GameplayStatics.GetPlayerController` 0))
  (bind _playerref (`self.PlayerRef`))
  ;[1 1 1] Sequencer
  (`self.DisableInput` (`self.PlayerRef`) _returnvalue)
  (set `self.CamToReturn` (`GameplayStatics.GetPlayerCharacter` 0))
  (`PlayerController.SetViewTargetWithBlend` _returnvalue (`self.CamToBlend`) (`self.BlendTime`) "VTBlend_Linear" 0.0 false)
  (`MovieSceneSequencePlayer.Play` (`LevelSequenceActor.SequencePlayer` (`self.Sequencer`)))
  (`/Game/NIRVANA/Core/Characters/FirstPerson/BP_FirstPersonCharacter.Change Weapon` _playerref (`/Game/NIRVANA/Core/Characters/FirstPerson/BP_FirstPersonCharacter.Current Weapon` _playerref) 2))

(event `Rotate`
  (bind (_initrotate_roll _initrotate_pitch _initrotate_yaw) (`KismetMathLibrary.BreakRotator` (`self.InitRotate`)))
  ;[1 1 1] Rotate lance
  (`TimelineComponent.SetPlayRate` (`self.Timeline`) (/ 1.0 (`self.LoopDuration`)))
  (bind (_direction _newtrack_0) (`Timeline|Timeline`)
    (:`Update`
      (`self.K2_SetActorRotation` (`KismetMathLibrary.MakeRotator` _initrotate_roll _initrotate_pitch (`KismetMathLibrary.Lerp` _initrotate_yaw (+ 0.0 360.0) _newtrack_0))))))

(event `EndCine`
  (`PlayerController.SetViewTargetWithBlend` (`GameplayStatics.GetPlayerController` 0) (`self.CamToReturn`) (`self.BlendTime`) "VTBlend_Linear" 0.0 false)
  (`self.EnableInput` (`self.PlayerRef`) (`GameplayStatics.GetPlayerController` 0))
  (`self.K2_DestroyActor`))

(event `HideBack`
  (bind (_returnvalue_x _returnvalue_y _returnvalue_z) (`KismetMathLibrary.BreakVector` (`self.K2_GetActorLocation`)))
  ;[1 1 1] Hide Lance
  (`self.K2_SetActorLocation` (`KismetMathLibrary.MakeVector` _returnvalue_x _returnvalue_y (- _returnvalue_z (`self.Hauteur`)))))

(fn `UserConstructionScript`)
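; BP_LiftCircle is a one-shot descending lift, armed when OnArenaCleaned fires.
; Once armed, the player entering its Box disarms it and starts a slowed timeline that lerps the Cylinder from its start position to the Stop component.
; The same timeline moves the referenced BallToMove's Boule by that displacement, keeping its offset from the platform.
; The construction script shifts Stop by StopLoc to set the destination.
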(event `self.ReceiveBeginPlay`
  ;[1 1 1] Begin play + références
  (set `self.Origin` (`SceneComponent.K2_GetComponentLocation` (`self.Cylinder`)))
  (bind _asbp_first_person_character (cast `/Game/NIRVANA/Core/Characters/FirstPerson/BP_FirstPersonCharacter` (`GameplayStatics.GetPlayerCharacter` 0)))
  (set `self.PlayerRef` _asbp_first_person_character))

(event `self.  Box.OnComponentBeginOverlap`
  (params (OverlappedComponent :type "PrimitiveComponent Object Reference") (OtherActor :type "Actor Object Reference") (OtherComp :type "PrimitiveComponent Object Reference") (OtherBodyIndex :type Integer) (bFromSweep :type Boolean) (SweepResult :type "HitResult Structure (by ref)"))
  ;[1 1 1] Ascenseur Go down
  (if (`self.Activated`)
    (if (== OtherActor (`self.PlayerRef`))
      (set `self.BallOrigin` (`SceneComponent.K2_GetComponentLocation` (`/Game/NIRVANA/Effects/AutelBoule/BP_FloatingBall.Boule` (`self.BallToMove`))))
      (set `self.Activated` false)
      (`TimelineComponent.SetPlayRate` (`self.Lift Down TL`) (/ 1.0 15.0))
      (bind (_direction _newtrack_0) (`Timeline|Lift Down TL` :!via `PlayFromStart`)
        (:`Update`
          (`SceneComponent.K2_SetWorldLocation` (`self.Cylinder`) (`KismetMathLibrary.VLerp` (`self.Origin`) (`SceneComponent.K2_GetComponentLocation` (`self.Stop`)) _newtrack_0) false false)
          (`SceneComponent.K2_SetWorldLocation` (`/Game/NIRVANA/Effects/AutelBoule/BP_FloatingBall.Boule` (`self.BallToMove`)) (`KismetMathLibrary.VLerp` (`self.BallOrigin`) (+ (- (`self.BallOrigin`) (`self.Origin`)) (`SceneComponent.K2_GetComponentLocation` (`self.Stop`))) _newtrack_0) false false))))))

(event `/Game/NIRVANA/Core/Placeables/Management/BPI_ArenaManager.OnArenaCleaned`
  (params (ArenaManager :type "/Game/NIRVANA/Core/Placeables/Management/BP_ArenaManager Object Reference"))
  ;[1 1 1] Activation on arena cleaned
  (set `self.Activated` true))

(fn `UserConstructionScript`
  (bind _stop (`self.Stop`))
  (`SceneComponent.K2_SetRelativeLocation` _stop (+ (`SceneComponent.RelativeLocation` _stop) (`self.StopLoc`)) false false))
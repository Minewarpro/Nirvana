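; BP_TutoLaserStartSequence is a placeable one-shot trigger volume that switches a set of tutorial lasers on or off.
; It caches the first-person player character on BeginPlay and reacts only when that character enters its box while the trigger is activated.
; On overlap it deactivates itself, then calls CreateLaser or ShutDown on every laser in LaserRefs, depending on the StartLoop flag.
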(event `self.ReceiveBeginPlay`
  (bind _asbp_first_person_character (cast `/Game/NIRVANA/Core/Characters/FirstPerson/BP_FirstPersonCharacter` (`GameplayStatics.GetPlayerCharacter` 0)))
  (set `self.PlayerRef` _asbp_first_person_character))

(event `self.Box.OnComponentBeginOverlap`
  (params (OverlappedComponent :type "PrimitiveComponent Object Reference") (OtherActor :type "Actor Object Reference") (OtherComp :type "PrimitiveComponent Object Reference") (OtherBodyIndex :type Integer) (bFromSweep :type Boolean) (SweepResult :type "HitResult Structure (by ref)"))
  (if (and (== OtherActor (`self.PlayerRef`)) (`self.IsActivated`))
    (set `self.IsActivated` false)
    (if (`self.StartLoop`)
      (for _array_element (`self.LaserRefs`)
        (`/Game/NIRVANA/Core/Placeables/Gameplay/BP_Lasers.Create Laser` _array_element))
      (else
        (for _array_element_2 (`self.LaserRefs`)
          (`/Game/NIRVANA/Core/Placeables/Gameplay/BP_Lasers.ShutDown` _array_element_2))))))

(fn `UserConstructionScript`)
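; Tutorial trigger that introduces dash or slide through an enemy ambush in slow motion.
; When the player enters the box while it is active, it fires once, spawning ranged enemies at the Spawners' transforms.
; After delays, a timeline lowers global time dilation, enemies shoot a set pattern, and a hint widget appears.
; The matching dash or crouch input reverses the slow motion and removes the hint.
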(event `self.ReceiveBeginPlay`
  (bind _asbp_first_person_character (cast `/Game/NIRVANA/Core/Characters/FirstPerson/BP_FirstPersonCharacter` (`GameplayStatics.GetPlayerCharacter` 0)))
  (set `self.PlayerRef` _asbp_first_person_character))

(event `self.Box.OnComponentBeginOverlap`
  (params (OverlappedComponent :type "PrimitiveComponent Object Reference") (OtherActor :type "Actor Object Reference") (OtherComp :type "PrimitiveComponent Object Reference") (OtherBodyIndex :type Integer) (bFromSweep :type Boolean) (SweepResult :type "HitResult Structure (by ref)"))
  (if (== OtherActor (`self.PlayerRef`))
    (if (`self.Activated`)
      (set `self.Activated` false)
      (for _array_element (`self.Spawners`)
        (bind _returnvalue (`|SpawnActorFromClass` "/Game/NIRVANA/Core/Characters/Enemies/Range/BP_EnemyRange_V1.BP_EnemyRange_V1_C" (`self.GetTransform` _array_element) "Undefined" "MultiplyWithRoot" null null null))
        (`KismetArrayLibrary.Array_Add` (`self.Ennemies`) _returnvalue))
      (`KismetSystemLibrary.Delay` (`self.Delay`))
      (`self.SlowMoStart`)
      (`KismetSystemLibrary.Delay` (`self.Delay`))
      (`self.Fire`)
      (if (`self.TrueDashFalseSlide`)
        (set `self.NeedDash` true)
        (bind _returnvalue_2 (`|CreateWidget` "/Game/NIRVANA/UI/Player/WB_TutoInfos.WB_TutoInfos_C" null false false false true))
        (bind _output_get (set `self.TutoInfo` _returnvalue_2))
        (`UserWidget.AddToViewport` _output_get 0)
        (else
          (set `self.NeedSlide` true)
          (bind _returnvalue_3 (`|CreateWidget` "/Game/NIRVANA/UI/Player/WB_TutoInfos.WB_TutoInfos_C" null false false false false true))
          (bind _output_get_2 (set `self.TutoInfo` _returnvalue_3))
          (`UserWidget.AddToViewport` _output_get_2 0))))))

(event `Fire`
  (for _array_element (`self.Ennemies`)
    (set `/Game/NIRVANA/Core/Characters/Enemies/Range/BP_EnemyRange.PatternIndex` (`self.PatternToSet`) _array_element)
    (`/Game/NIRVANA/Core/Characters/Enemies/Range/BP_EnemyRange.Shoot` _array_element)))

(event `SlowMoStart`
  (bind (_direction _slowmo) (`Timeline|Timeline` :!via `PlayFromStart` :!label _label)
    (:`Update`
      (`GameplayStatics.SetGlobalTimeDilation` (`KismetMathLibrary.Lerp` 1.0 0.1 _slowmo)))))

(event `SlowMoEnd`
  (goto _label :!via `ReverseFromEnd`))

(event `EnhancedInput|/Game/NIRVANA/Core/Characters/FirstPerson/Input/Actions/IA_Dash`
  (params (ActionValue :type Boolean) (ElapsedSeconds :type "Float (double-precision)") (TriggeredSeconds :type "Float (double-precision)") (InputAction :type "InputAction Object Reference" :default "/Game/NIRVANA/Core/Characters/FirstPerson/Input/Actions/IA_Dash.IA_Dash"))
  (:`Started`
    (if (`self.NeedDash`)
      (`self.SlowMoEnd`)
      (set `self.NeedDash` false)
      (`Widget.RemoveFromParent` (`self.TutoInfo`)))))

(event `EnhancedInput|/Game/NIRVANA/Core/Characters/FirstPerson/Input/Actions/IA_Crouch`
  (params (ActionValue :type Boolean) (ElapsedSeconds :type "Float (double-precision)") (TriggeredSeconds :type "Float (double-precision)") (InputAction :type "InputAction Object Reference" :default "/Game/NIRVANA/Core/Characters/FirstPerson/Input/Actions/IA_Crouch.IA_Crouch"))
  (:`Started`
    (if (`self.NeedSlide`)
      (`self.SlowMoEnd`)
      (set `self.NeedSlide` false)
      (`Widget.RemoveFromParent` (`self.TutoInfo`)))))

(fn `UserConstructionScript`)
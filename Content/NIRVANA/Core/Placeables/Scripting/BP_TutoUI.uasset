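; BP_TutoUI is a placeable trigger box that shows tutorial prompts in a WB_TutoInfos widget.
; With GameStart set, it opens with mouse then movement hints, advanced by look and move inputs, and only then arms its box.
; When the player overlaps the armed box, it shows one of six movement hints chosen by index.
; That widget is removed after a delay, or after a jump or dash input for event boxes.
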(event `self.ReceiveBeginPlay`
  (bind _asbp_first_person_character (cast `/Game/NIRVANA/Core/Characters/FirstPerson/BP_FirstPersonCharacter` (`GameplayStatics.GetPlayerCharacter` 0)))
  (set `self.PlayerRef` _asbp_first_person_character)
  (set `self.BoxActivated` true)
  (if (`self.GameStart`)
    (`KismetSystemLibrary.Delay` 0.2)
    (`self.StartTutoUI`)))

(event `StartTutoUI`
  (bind _returnvalue (`|CreateWidget` "/Game/NIRVANA/UI/Player/WB_TutoInfos.WB_TutoInfos_C" null true))
  (bind _output_get (set `self.TutoInfos` _returnvalue))
  (`UserWidget.AddToViewport` _output_get 0)
  (`KismetSystemLibrary.Delay` 0.5)
  (set `self.Skip1` true)
  (set `self.BoxActivated` false))

(event `EnhancedInput|/Game/NIRVANA/Core/Characters/FirstPerson/Input/Actions/IA_Look`
  (params (ActionValue :type "Vector2D Structure") (ElapsedSeconds :type "Float (double-precision)") (TriggeredSeconds :type "Float (double-precision)") (InputAction :type "InputAction Object Reference" :default "/Game/NIRVANA/Core/Characters/FirstPerson/Input/Actions/IA_Look.IA_Look"))
  (bind _tutoinfos (`self.TutoInfos`))
  (:`Started`
    (if (`self.Skip1`)
      (`KismetSystemLibrary.Delay` 1.5)
      (`Widget.SetVisibility` (`/Game/NIRVANA/UI/Player/WB_TutoInfos.Mouse` _tutoinfos) "Hidden")
      (`Widget.SetVisibility` (`/Game/NIRVANA/UI/Player/WB_TutoInfos.ZQSD` _tutoinfos) "Visible")
      (set `self.Skip1` false)
      (set `self.Skip2` true))))

(event `EnhancedInput|/Game/NIRVANA/Core/Characters/FirstPerson/Input/Actions/IA_Move`
  (params (ActionValue :type "Vector2D Structure") (ElapsedSeconds :type "Float (double-precision)") (TriggeredSeconds :type "Float (double-precision)") (InputAction :type "InputAction Object Reference" :default "/Game/NIRVANA/Core/Characters/FirstPerson/Input/Actions/IA_Move.IA_Move"))
  (:`Triggered`
    (if (`self.Skip2`)
      (`KismetSystemLibrary.Delay` 1.5)
      (`Widget.SetVisibility` (`/Game/NIRVANA/UI/Player/WB_TutoInfos.ZQSD` (`self.TutoInfos`)) "Hidden")
      (set `self.Skip2` false)
      (set `self.BoxActivated` true))))

(event `self.Box.OnComponentBeginOverlap`
  (params (OverlappedComponent :type "PrimitiveComponent Object Reference") (OtherActor :type "Actor Object Reference") (OtherComp :type "PrimitiveComponent Object Reference") (OtherBodyIndex :type Integer) (bFromSweep :type Boolean) (SweepResult :type "HitResult Structure (by ref)"))
  (bind _tutoinfos (`self.TutoInfos`))
  (if (== OtherActor (`self.PlayerRef`))
    (if (`self.BoxActivated`)
      (`|ExecutionSequence`
        (:`then_0`
          (if (not (`self.GameStart`))
            (bind _returnvalue (`|CreateWidget` "/Game/NIRVANA/UI/Player/WB_TutoInfos.WB_TutoInfos_C"))
            (bind _output_get (set `self.TutoInfos` _returnvalue))
            (`UserWidget.AddToViewport` _output_get 0)))
        (:`then_1`
          (`Widget.SetVisibility` (select `int` (`self.TextToShow0To5`) :`0` (`/Game/NIRVANA/UI/Player/WB_TutoInfos.Space` _tutoinfos) :`1` (`/Game/NIRVANA/UI/Player/WB_TutoInfos.DoubleJump` _tutoinfos) :`2` (`/Game/NIRVANA/UI/Player/WB_TutoInfos.DashTuto` _tutoinfos) :`3` (`/Game/NIRVANA/UI/Player/WB_TutoInfos.Mantle` _tutoinfos) :`4` (`/Game/NIRVANA/UI/Player/WB_TutoInfos.DashCooldown` _tutoinfos) :`5` (`/Game/NIRVANA/UI/Player/WB_TutoInfos.DashSide` _tutoinfos) :!type "Widget Object Reference") "Visible")
          (set `self.BoxActivated` false)
          (if (`self.IsEvent`)
            (if (`self.IsJumpOrDash`)
              (set `self.Skip3` true)
              (else
                (set `self.SkipDash` true)))
            (else
              (`KismetSystemLibrary.Delay` 4.0)
              (`Widget.RemoveFromParent` (`self.TutoInfos`)))))))))

(event `EnhancedInput|/Game/NIRVANA/Core/Characters/FirstPerson/Input/Actions/IA_Jump`
  (params (ActionValue :type Boolean) (ElapsedSeconds :type "Float (double-precision)") (TriggeredSeconds :type "Float (double-precision)") (InputAction :type "InputAction Object Reference" :default "/Game/NIRVANA/Core/Characters/FirstPerson/Input/Actions/IA_Jump.IA_Jump"))
  (:`Started`
    (if (`self.Skip3`)
      (`KismetSystemLibrary.Delay` 2.0)
      (`Widget.RemoveFromParent` (`self.TutoInfos`)))))

(event `EnhancedInput|/Game/NIRVANA/Core/Characters/FirstPerson/Input/Actions/IA_Dash`
  (params (ActionValue :type Boolean) (ElapsedSeconds :type "Float (double-precision)") (TriggeredSeconds :type "Float (double-precision)") (InputAction :type "InputAction Object Reference" :default "/Game/NIRVANA/Core/Characters/FirstPerson/Input/Actions/IA_Dash.IA_Dash"))
  (:`Started`
    (if (`self.SkipDash`)
      (`KismetSystemLibrary.Delay` 2.0)
      (`Widget.RemoveFromParent` (`self.TutoInfos`)))))

(fn `UserConstructionScript`)
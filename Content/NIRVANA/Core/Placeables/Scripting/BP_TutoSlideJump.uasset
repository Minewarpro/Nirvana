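; BP_TutoSlideJump is a placeable tutorial trigger that slows time to a near freeze until the player presses jump.
; When the first-person character enters its Box while Activated, it disarms itself and allows the slow motion to be cancelled.
; A timeline eases global time dilation down, and the first IA_Jump press afterward reverses that timeline to restore normal speed.
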(event `self.ReceiveBeginPlay`
  (bind _asbp_first_person_character (cast `/Game/NIRVANA/Core/Characters/FirstPerson/BP_FirstPersonCharacter` (`GameplayStatics.GetPlayerCharacter` 0)))
  (set `self.PlayerRef` _asbp_first_person_character))

(event `self.Box.OnComponentBeginOverlap`
  (params (OverlappedComponent :type "PrimitiveComponent Object Reference") (OtherActor :type "Actor Object Reference") (OtherComp :type "PrimitiveComponent Object Reference") (OtherBodyIndex :type Integer) (bFromSweep :type Boolean) (SweepResult :type "HitResult Structure (by ref)"))
  (if (== OtherActor (`self.PlayerRef`))
    (if (`self.Activated`)
      (set `self.Activated` false)
      (set `self.CanStopSlowMo` true)
      (`self.SlowMoStart`))))

(event `SlowMoStart`
  (bind (_direction _slowmo) (`Timeline|Timeline` :!via `PlayFromStart` :!label _label)
    (:`Update`
      (`GameplayStatics.SetGlobalTimeDilation` (`KismetMathLibrary.Lerp` 1.0 0.01 _slowmo)))))

(event `SlowMoEnd`
  (goto _label :!via `Reverse`))

(event `EnhancedInput|/Game/NIRVANA/Core/Characters/FirstPerson/Input/Actions/IA_Jump`
  (params (ActionValue :type Boolean) (ElapsedSeconds :type "Float (double-precision)") (TriggeredSeconds :type "Float (double-precision)") (InputAction :type "InputAction Object Reference" :default "/Game/NIRVANA/Core/Characters/FirstPerson/Input/Actions/IA_Jump.IA_Jump"))
  (:`Started`
    (if (`self.CanStopSlowMo`)
      (`self.SlowMoEnd`)
      (set `self.CanStopSlowMo` false))))

(fn `UserConstructionScript`)
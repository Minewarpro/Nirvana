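; BP_TutoWallsForDash is a placeable set of three walls, named for the dash tutorial, that slides once when the player enters its trigger box.
; The overlap clears the Activated flag and plays the WallSlide timeline at a rate set by NewTime.
; Separate tracks, mapped in reverse order, lerp each wall along local X to EndLoc.
; The construction script applies the trigger's location and size and the wall scale multiplier.
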(event `self.Box.OnComponentBeginOverlap`
  (params (OverlappedComponent :type "PrimitiveComponent Object Reference") (OtherActor :type "Actor Object Reference") (OtherComp :type "PrimitiveComponent Object Reference") (OtherBodyIndex :type Integer) (bFromSweep :type Boolean) (SweepResult :type "HitResult Structure (by ref)"))
  (bind _asbp_first_person_character (cast `/Game/NIRVANA/Core/Characters/FirstPerson/BP_FirstPersonCharacter` (`GameplayStatics.GetPlayerCharacter` 0)))
  (if (and (== _asbp_first_person_character OtherActor) (`self.Activated`))
    (set `self.Activated` false)
    (`self.StartWallMove`)))

(event `StartWallMove`
  (`TimelineComponent.SetPlayRate` (`self.WallSlide`) (/ 1.0 (`self.NewTime`)))
  (bind (_direction _wall1 _wall2 _wall3) (`Timeline|WallSlide`)
    (:`Update`
      (`SceneComponent.K2_SetRelativeLocation` (`self.Wall1`) (`KismetMathLibrary.MakeVector` (`KismetMathLibrary.Lerp` 0.0 (`self.EndLoc`) _wall3)) false false)
      (`SceneComponent.K2_SetRelativeLocation` (`self.Wall2`) (`KismetMathLibrary.MakeVector` (`KismetMathLibrary.Lerp` 0.0 (`self.EndLoc`) _wall2) -190.0) false false)
      (`SceneComponent.K2_SetRelativeLocation` (`self.Wall3`) (`KismetMathLibrary.MakeVector` (`KismetMathLibrary.Lerp` 0.0 (`self.EndLoc`) _wall1) -380.0) false false))))

(fn `UserConstructionScript`
  (bind _box (`self.Box`))
  (bind _wall1 (`self.Wall1`))
  (`SceneComponent.K2_SetRelativeLocation` _box (`self.TriggerLoc`) false false)
  (`SceneComponent.SetRelativeScale3D` _box (`self.TriggerSize`))
  (`SceneComponent.SetWorldScale3D` _wall1 (* (`SceneComponent.K2_GetComponentScale` _wall1) (`self.WallSize`)))
  (`SceneComponent.SetWorldScale3D` (`self.Wall2`) (* (`SceneComponent.K2_GetComponentScale` _wall1) (`self.WallSize`)))
  (`SceneComponent.SetWorldScale3D` (`self.Wall3`) (* (`SceneComponent.K2_GetComponentScale` _wall1) (`self.WallSize`))))
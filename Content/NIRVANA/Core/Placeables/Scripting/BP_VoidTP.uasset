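; BP_VoidTP is a placeable void volume that catches the player and enemies falling or walking into its box.
; On player overlap it either kills the player when IsKilling is set, or fades to black, moves them to the Tp point, sets control rotation and fades back in.
; Overlapping BP_Enemy actors always die.
; The construction script applies per-instance box scale and teleport coordinates.
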(event `self.ReceiveBeginPlay`
  (bind _asbp_first_person_character (cast `/Game/NIRVANA/Core/Characters/FirstPerson/BP_FirstPersonCharacter` (`GameplayStatics.GetPlayerCharacter` 0)))
  (set `self.PlayerRef` _asbp_first_person_character))

(event `self.Box.OnComponentBeginOverlap`
  (params (OverlappedComponent :type "PrimitiveComponent Object Reference") (OtherActor :type "Actor Object Reference") (OtherComp :type "PrimitiveComponent Object Reference") (OtherBodyIndex :type Integer) (bFromSweep :type Boolean) (SweepResult :type "HitResult Structure (by ref)"))
  (if (== OtherActor (`self.PlayerRef`))
    (if (`self.IsKilling`)
      (`/Game/NIRVANA/Core/Characters/FirstPerson/BP_FirstPersonCharacter.Death` (`self.PlayerRef`))
      (else
        (`PlayerCameraManager.StartCameraFade` :`self` (`GameplayStatics.GetPlayerCameraManager` 0) :`ToAlpha` 1.0 :`Duration` 0.5)
        (`KismetSystemLibrary.Delay` 0.5)
        (`self.K2_SetActorLocation` (`self.PlayerRef`) (`SceneComponent.K2_GetComponentLocation` (`self.Tp`)) false false)
        (`Controller.SetControlRotation` (`GameplayStatics.GetPlayerController` 0) (`self.RotationTP`))
        (`PlayerCameraManager.StartCameraFade` :`self` (`GameplayStatics.GetPlayerCameraManager` 0) :`FromAlpha` 1.0 :`ToAlpha` 0.0 :`Duration` 0.5)))
    (else
      (bind _asbp_enemy (cast `/Game/NIRVANA/Core/Characters/Enemies/Common/BP_Enemy` OtherActor))
      (`/Game/NIRVANA/Core/Characters/Enemies/Common/BP_Enemy.Death` _asbp_enemy))))

(fn `UserConstructionScript`
  (`SceneComponent.SetRelativeScale3D` (`self.Box`) (`self.BoxScale`))
  (`SceneComponent.K2_SetRelativeLocation` (`self.Tp`) (`self.CoordsTP`) false false))
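; BP_TutoClicDroit is a placeable tutorial trigger teaching the right-click secondary shot, then a left-click follow-up.
; When activated, the player's overlap disables it, locks input, snaps control rotation and shows a WB_TutoInfos prompt under timeline-driven global slow motion.
; Right-click fires secondary, briefly restores time, then slows again for the second prompt.
; Left-click fires primary, removes the widget and restores input and time.
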(event `self.ReceiveBeginPlay`
  (bind _asbp_first_person_character (cast `/Game/NIRVANA/Core/Characters/FirstPerson/BP_FirstPersonCharacter` (`GameplayStatics.GetPlayerCharacter` 0)))
  (set `self.PlayerRef` _asbp_first_person_character))

(event `self.Box.OnComponentBeginOverlap`
  (params (OverlappedComponent :type "PrimitiveComponent Object Reference") (OtherActor :type "Actor Object Reference") (OtherComp :type "PrimitiveComponent Object Reference") (OtherBodyIndex :type Integer) (bFromSweep :type Boolean) (SweepResult :type "HitResult Structure (by ref)"))
  (bind _returnvalue (`GameplayStatics.GetPlayerController` 0))
  (if (and (== OtherActor (`self.PlayerRef`)) (`self.Activated`))
    (set `self.Activated` false)
    (`self.DisableInput` (`self.PlayerRef`) _returnvalue)
    (`Controller.SetControlRotation` _returnvalue (`self.RotationLock`))
    (`self.SlowMoStart`)
    (bind _returnvalue_2 (`|CreateWidget` "/Game/NIRVANA/UI/Player/WB_TutoInfos.WB_TutoInfos_C"))
    (bind _output_get (set `self.TutoInfos` _returnvalue_2))
    (`UserWidget.AddToViewport` _output_get 0)
    (`Widget.SetVisibility` (`/Game/NIRVANA/UI/Player/WB_TutoInfos.ClicDroit` (`self.TutoInfos`)) "Visible")
    (set `self.CanRightClick` true)))

(event `SlowMoStart`
  (`TimelineComponent.SetPlayRate` (`self.Timeline`) (/ 1.0 0.5))
  (bind (_direction _slowmo) (`Timeline|Timeline` :!via `PlayFromStart` :!label _label)
    (:`Update`
      (`GameplayStatics.SetGlobalTimeDilation` (`KismetMathLibrary.Lerp` 1.0 0.05 _slowmo)))))

(event `SlowMoEnd`
  (`TimelineComponent.SetPlayRate` (`self.Timeline`) (/ 1.0 0.2))
  (goto _label :!via `ReverseFromEnd`))

(event `EnhancedInput|/Game/NIRVANA/Core/Characters/FirstPerson/Input/Actions/IA_SecondaryShoot`
  (params (ActionValue :type Boolean) (ElapsedSeconds :type "Float (double-precision)") (TriggeredSeconds :type "Float (double-precision)") (InputAction :type "InputAction Object Reference" :default "/Game/NIRVANA/Core/Characters/FirstPerson/Input/Actions/IA_SecondaryShoot.IA_SecondaryShoot"))
  (:`Started`
    (if (`self.CanRightClick`)
      (`/Game/NIRVANA/Core/Weapons/Common/BP_Weapon.Secondary Fire Start` (`/Game/NIRVANA/Core/Characters/FirstPerson/BP_FirstPersonCharacter.Get Weapon` (`self.PlayerRef`)))
      (`Widget.SetVisibility` (`/Game/NIRVANA/UI/Player/WB_TutoInfos.ClicDroit` (`self.TutoInfos`)) "Hidden")
      (set `self.CanRightClick` false)
      (`self.SlowMoEnd`)
      (`KismetSystemLibrary.Delay` 0.5)
      (`Widget.SetVisibility` (`/Game/NIRVANA/UI/Player/WB_TutoInfos.ClicDroitP2` (`self.TutoInfos`)) "Visible")
      (`self.SlowMoStart`)
      (set `self.CanLeftClick` true))))

(event `EnhancedInput|/Game/NIRVANA/Core/Characters/FirstPerson/Input/Actions/IA_Shoot`
  (params (ActionValue :type Boolean) (ElapsedSeconds :type "Float (double-precision)") (TriggeredSeconds :type "Float (double-precision)") (InputAction :type "InputAction Object Reference" :default "/Game/NIRVANA/Core/Characters/FirstPerson/Input/Actions/IA_Shoot.IA_Shoot"))
  (:`Started`
    (if (`self.CanLeftClick`)
      (`/Game/NIRVANA/Core/Weapons/Common/BP_Weapon.Fire Start` (`/Game/NIRVANA/Core/Characters/FirstPerson/BP_FirstPersonCharacter.Get Weapon` (`self.PlayerRef`)))
      (`Widget.RemoveFromParent` (`self.TutoInfos`))
      (set `self.CanLeftClick` false)
      (`self.EnableInput` (`self.PlayerRef`) (`GameplayStatics.GetPlayerController` 0))
      (`self.SlowMoEnd`))))

(fn `UserConstructionScript`)
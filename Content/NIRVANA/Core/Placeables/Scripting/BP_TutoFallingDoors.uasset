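; Tutorial trigger that drops a referenced door as the player approaches, to teach sliding.
; On overlap, a one-shot timeline partly lowers the door; if slow-mo is enabled, it disables input, eases global time dilation down and shows a slide prompt.
; Crouch calls the player's slide and, during the prompt, restores time and input, then lowers the door fully after a delay.
; Camera-focus and mapping-context logic is left unwired.
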(event `self.ReceiveBeginPlay`
  (bind (_returnvalue_x _returnvalue_y _returnvalue_z) (`KismetMathLibrary.BreakVector` (`SceneComponent.K2_GetComponentLocation` (`StaticMeshActor.StaticMeshComponent` (`self.DoorToDown`)))))
  ;[1 1 1] BeginPlay
  (bind _asbp_first_person_character (cast `/Game/NIRVANA/Core/Characters/FirstPerson/BP_FirstPersonCharacter` (`GameplayStatics.GetPlayerCharacter` 0)))
  (set `self.PlayerRef` _asbp_first_person_character)
  (set `self.StartZ` _returnvalue_z)
  (set `self.MiddleZ` (- (`self.StartZ`) 650.0)))

(event `self.Box.OnComponentBeginOverlap`
  (params (OverlappedComponent :type "PrimitiveComponent Object Reference") (OtherActor :type "Actor Object Reference") (OtherComp :type "PrimitiveComponent Object Reference") (OtherBodyIndex :type Integer) (bFromSweep :type Boolean) (SweepResult :type "HitResult Structure (by ref)"))
  (bind _startz (`self.StartZ`))
  (bind _staticmeshcomponent (`StaticMeshActor.StaticMeshComponent` (`self.DoorToDown`)))
  (bind (_returnvalue_x _returnvalue_y) (`KismetMathLibrary.BreakVector` (`SceneComponent.K2_GetComponentLocation` _staticmeshcomponent)))
  ;[1 1 1] CloseDoor
  (if (== OtherActor (`self.PlayerRef`))
    (if (`self.IsActivated`)
      (set `self.IsActivated` false)
      (`|ExecutionSequence`
        (:`then_0`
          (bind (_direction _newtrack_0) (`Timeline|Timeline` :!via `PlayFromStart`)
            (:`Update`
              (`SceneComponent.K2_SetWorldLocation` _staticmeshcomponent (`KismetMathLibrary.MakeVector` _returnvalue_x _returnvalue_y (`KismetMathLibrary.Lerp` _startz (- _startz 650.0) _newtrack_0)) false false))))
        (:`then_1`
          (if (`self.SlowMoActivated`)
            (`self.DisableInput` (`self.PlayerRef`) (`GameplayStatics.GetPlayerController` 0))
            (`KismetSystemLibrary.Delay` 0.4)
            (`self.SlowMoStart`)
            (set `self.CanStopSlowMo` true)
            (bind _returnvalue (`|CreateWidget` "/Game/NIRVANA/UI/Player/WB_TutoInfos.WB_TutoInfos_C" null false false false false true))
            (bind _output_get (set `self.TutoInfo` _returnvalue))
            (`UserWidget.AddToViewport` _output_get 0)))))))

(event `SlowMoStart`
  ;[1 1 1] SlowMoManager
  (`TimelineComponent.SetPlayRate` (`self.SlowMotionStart`) (/ 1.0 0.5))
  (bind (_direction _slowmo) (`Timeline|SlowMotionStart` :!via `PlayFromStart` :!label _label)
    (:`Update`
      (`GameplayStatics.SetGlobalTimeDilation` (`KismetMathLibrary.Lerp` 1.0 0.1 _slowmo)))))

(event `SlowMoEnd`
  ;[1 1 1] SlowMoManager
  (`TimelineComponent.SetPlayRate` (`self.SlowMotionStart`) (/ 1.0 0.2))
  (goto _label :!via `ReverseFromEnd`))

(event `EnhancedInput|/Game/NIRVANA/Core/Characters/FirstPerson/Input/Actions/IA_Crouch`
  (params (ActionValue :type Boolean) (ElapsedSeconds :type "Float (double-precision)") (TriggeredSeconds :type "Float (double-precision)") (InputAction :type "InputAction Object Reference" :default "/Game/NIRVANA/Core/Characters/FirstPerson/Input/Actions/IA_Crouch.IA_Crouch"))
  (bind _middlez (`self.MiddleZ`))
  (bind _staticmeshcomponent (`StaticMeshActor.StaticMeshComponent` (`self.DoorToDown`)))
  (bind (_returnvalue_x _returnvalue_y) (`KismetMathLibrary.BreakVector` (`SceneComponent.K2_GetComponentLocation` _staticmeshcomponent)))
  ;[1 1 1] EndScript
  (:`Started`
    (`/Game/NIRVANA/Core/Characters/FirstPerson/BP_FirstPersonCharacter.BeginSlide` (`self.PlayerRef`))
    (if (`self.CanStopSlowMo`)
      (`|ExecutionSequence`
        (:`then_0`
          (`self.SlowMoEnd`)
          (set `self.CanStopSlowMo` false)
          (`self.EnableInput` (`self.PlayerRef`) (`GameplayStatics.GetPlayerController` 0))
          (`Widget.RemoveFromParent` (`self.TutoInfo`)))
        (:`then_1`
          (`KismetSystemLibrary.Delay` 1.0)
          (bind (_direction _newtrack_0) (`Timeline|CloseDoor` :!via `PlayFromStart`)
            (:`Update`
              (`SceneComponent.K2_SetWorldLocation` _staticmeshcomponent (`KismetMathLibrary.MakeVector` _returnvalue_x _returnvalue_y (`KismetMathLibrary.Lerp` _middlez (- _middlez 150.0) _newtrack_0)) false false))))))))

(fn `UserConstructionScript`)
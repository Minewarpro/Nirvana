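; BP_Health is a health loot pickup that restores health to the first-person player character.
; Overlapping its detection sphere while the player's health is below 100 starts a timeline that lerps the pickup from its start location toward the player's live position, like a magnet.
; Overlapping the other sphere adds HealthToAdd to the player and destroys the pickup, with no check on current health.
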(event `self.ReceiveBeginPlay`
  (bind _asbp_first_person_character (cast `/Game/NIRVANA/Core/Characters/FirstPerson/BP_FirstPersonCharacter` (`GameplayStatics.GetPlayerCharacter` 0)))
  (set `self.Player Ref` _asbp_first_person_character))

(event `self.Sphere Detectin.OnComponentBeginOverlap`
  (params (OverlappedComponent :type "PrimitiveComponent Object Reference") (OtherActor :type "Actor Object Reference") (OtherComp :type "PrimitiveComponent Object Reference") (OtherBodyIndex :type Integer) (bFromSweep :type Boolean) (SweepResult :type "HitResult Structure (by ref)"))
  (bind _player_ref (`self.Player Ref`))
  (if (== _player_ref OtherActor)
    (if (< (`/Game/NIRVANA/Core/Characters/FirstPerson/BP_FirstPersonCharacter.Current Health` _player_ref) 100.0)
      (`self.Start Travel`))))

(event `self.Sphere.OnComponentBeginOverlap`
  (params (OverlappedComponent :type "PrimitiveComponent Object Reference") (OtherActor :type "Actor Object Reference") (OtherComp :type "PrimitiveComponent Object Reference") (OtherBodyIndex :type Integer) (bFromSweep :type Boolean) (SweepResult :type "HitResult Structure (by ref)"))
  (bind _player_ref (`self.Player Ref`))
  (if (== _player_ref OtherActor)
    (`/Game/NIRVANA/Core/Characters/FirstPerson/BP_FirstPersonCharacter.Add Health` _player_ref (`self.Health To Add`))
    (`self.K2_DestroyActor`)))

(event `Start Travel`
  (set `self.Init Location` (`self.K2_GetActorLocation`))
  (bind (_direction _travel_alpha) (`Timeline|Travel TL`)
    (:`Update`
      (`self.K2_SetActorLocation` (`KismetMathLibrary.VLerp` (`self.Init Location`) (`self.K2_GetActorLocation` (`self.Player Ref`)) _travel_alpha)))))

(fn `UserConstructionScript`)
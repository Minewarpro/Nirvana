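; BP_EnemyProjectileApparition is the telegraph effect that plays where an enemy projectile is about to appear.
; The construction script sets the apparition Niagara effect's loop duration from the Duration variable.
; When that effect finishes, it passes its stored spawn location, motion, direction-change, damage, special-effect and scale settings to the bullet manager to activate a bullet, then destroys itself.
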(event `self.N_ApparitionBall.OnSystemFinished`
  (params (PSystem :type "NiagaraComponent Object Reference"))
  (bind _ref_bullet_manager (`self.Ref Bullet Manager`)
    (:`then`
      (`/Game/NIRVANA/Core/Characters/Enemies/Range/BP_BulletManager.Activate Bullet` _ref_bullet_manager (`self.Spawn Transform Location`) (`self.Direction`) (`self.Speed`) (`self.Damage`) (`self.Need Change Direction`) (`self.Delay Change DIrection`) (`self.New Direction`) (`self.New Speed`) (`self.Special Effect`) (`self.GetActorScale3D`) (`self.Enemie Ref`) false 0.0 0.0)
      (`self.K2_DestroyActor`))
    (:`else`)))

(fn `UserConstructionScript`
  (`NiagaraComponent.SetVariableFloat` (`self.N_ApparitionBall`) "Loop Duration" (`self.Duration`)))
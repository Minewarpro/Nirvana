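; BP_EnemyRange_V1 is a ranged enemy variant that inherits its shooting from a parent Blueprint.
; GetPatternIndex picks one of two StructPattern entries by Row: row 2 prefers the first, other rows the second, each falling back when its preference is disabled.
; Shoot only calls the parent; the weighted RandomPatternSelection, which strongly favors the second pattern, is left disconnected.
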(event `self.Shoot`
  (`parent.Shoot`))

(fn `GetPatternIndex`
  (params (Row :type Integer))
  (returns (Index :type Integer))
  (bind (_output_pattern _output_nbbulletloop _output_delayeachloop _output_projectilespeed _output_damage _output_dispertion _output_dispertionspeed _output_previsualisation _output_nbbulletrectangle _output_zoffsettransformlocation _output_directionbyoffset _output_disabled) (break `/Game/NIRVANA/Core/Characters/Enemies/Common/Struct_PatternValue` (`|GetArrayItem` (`self.StructPattern`))))
  (bind (_output_pattern_2 _output_nbbulletloop_2 _output_delayeachloop_2 _output_projectilespeed_2 _output_damage_2 _output_dispertion_2 _output_dispertionspeed_2 _output_previsualisation_2 _output_nbbulletrectangle_2 _output_zoffsettransformlocation_2 _output_directionbyoffset_2 _output_disabled_2) (break `/Game/NIRVANA/Core/Characters/Enemies/Common/Struct_PatternValue` (`|GetArrayItem` (`self.StructPattern`) 1)))
  (if (== Row 2)
    (if _output_disabled
      _
      (else
        (return 0)))
    (elif _output_disabled_2
      (return 0)
      (else
        _)))
  (return 1))

(fn `RandomPatternSelection`
  (locals (TempRandom :type Integer))
  (bind _output_get (set `local.TempRandom` (`KismetMathLibrary.RandomIntegerInRange` 0 99)))
  (if (< _output_get 90)
    (set `self.PatternIndex` 1)
    (else
      (set `self.PatternIndex` 0))))

(fn `UserConstructionScript`
  (`parent.UserConstructionScript`))
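; BP_EnemyRange_V2 is a ranged enemy Blueprint whose Shoot event only forwards to the parent implementation.
; RandomPatternSelection rolls a weighted random PatternIndex, heavily favoring pattern 0 over pattern 1, with pattern 2 disconnected.
; The graph that would call this roll and branch between the parent shot and StartSnipe is also disconnected, so neither runs from Shoot.
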(event `self.Shoot`
  (`parent.Shoot`))

(fn `RandomPatternSelection`
  (locals (TempRandom :type Integer))
  (bind _output_get (set `local.TempRandom` (`KismetMathLibrary.RandomIntegerInRange` 0 99)))
  (if (<= _output_get 85)
    (set `self.PatternIndex` 0)
    (else
      (set `self.PatternIndex` 1))))

(fn `UserConstructionScript`
  (`parent.UserConstructionScript`))
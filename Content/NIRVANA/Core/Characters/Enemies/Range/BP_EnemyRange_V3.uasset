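; BP_EnemyRange_V3 is a ranged enemy variant that extends its parent's shooting with a timed state change and row-based pattern selection.
; GetPatternIndex maps a row to a shot pattern, falling back through enabled StructPattern entries to index 3 when the candidates are disabled.
; Shoot records whether pattern 1 is active before the parent shot, then, if so, switches CurrentState for a few seconds before setting another state.
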(event `self.ReceiveBeginPlay`
  (`parent.ReceiveBeginPlay`))

(event `self.Shoot`
  (bind _output_get (set `self.PatternFreeze` (== (`self.PatternIndex`) 1)))
  (`parent.Shoot`)
  (if _output_get
    (set `self.CurrentState` "NewEnumerator7")
    (`KismetSystemLibrary.Delay` 4.0)
    (set `self.CurrentState` "NewEnumerator0")))

(fn `GetPatternIndex`
  (params (Row :type Integer))
  (returns (Index :type Integer))
  (bind (_output_pattern _output_nbbulletloop _output_delayeachloop _output_projectilespeed _output_damage _output_dispertion _output_dispertionspeed _output_previsualisation _output_nbbulletrectangle _output_zoffsettransformlocation _output_directionbyoffset _output_disabled) (break `/Game/NIRVANA/Core/Characters/Enemies/Common/Struct_PatternValue` (`|GetArrayItem` (`self.StructPattern`) 2)))
  (bind (_output_pattern_2 _output_nbbulletloop_2 _output_delayeachloop_2 _output_projectilespeed_2 _output_damage_2 _output_dispertion_2 _output_dispertionspeed_2 _output_previsualisation_2 _output_nbbulletrectangle_2 _output_zoffsettransformlocation_2 _output_directionbyoffset_2 _output_disabled_2) (break `/Game/NIRVANA/Core/Characters/Enemies/Common/Struct_PatternValue` (`|GetArrayItem` (`self.StructPattern`) 2)))
  (bind (_output_pattern_3 _output_nbbulletloop_3 _output_delayeachloop_3 _output_projectilespeed_3 _output_damage_3 _output_dispertion_3 _output_dispertionspeed_3 _output_previsualisation_3 _output_nbbulletrectangle_3 _output_zoffsettransformlocation_3 _output_directionbyoffset_3 _output_disabled_3) (break `/Game/NIRVANA/Core/Characters/Enemies/Common/Struct_PatternValue` (`|GetArrayItem` (`self.StructPattern`))))
  (bind (_output_pattern_4 _output_nbbulletloop_4 _output_delayeachloop_4 _output_projectilespeed_4 _output_damage_4 _output_dispertion_4 _output_dispertionspeed_4 _output_previsualisation_4 _output_nbbulletrectangle_4 _output_zoffsettransformlocation_4 _output_directionbyoffset_4 _output_disabled_4) (break `/Game/NIRVANA/Core/Characters/Enemies/Common/Struct_PatternValue` (`|GetArrayItem` (`self.StructPattern`) 1)))
  (bind (_output_pattern_5 _output_nbbulletloop_5 _output_delayeachloop_5 _output_projectilespeed_5 _output_damage_5 _output_dispertion_5 _output_dispertionspeed_5 _output_previsualisation_5 _output_nbbulletrectangle_5 _output_zoffsettransformlocation_5 _output_directionbyoffset_5 _output_disabled_5) (break `/Game/NIRVANA/Core/Characters/Enemies/Common/Struct_PatternValue` (`|GetArrayItem` (`self.StructPattern`) 1)))
  (if (== Row 2)
    ;[1 1 1] Row1
    (if _output_disabled
      (return 3)
      (else
        (return 2)))
    (elif (== Row 1)
      ;[1 1 1] Row2
      (if _output_disabled_4
        (if _output_disabled_2
          (return 3)
          (else
            (return 2)))
        (else
          (return 1)))
      (else
        ;[1 1 1] Row3
        (if _output_disabled_5
          (if _output_disabled_3
            (return 3)
            (else
              (return 0)))
          (else
            (return 1)))))))

(fn `UserConstructionScript`
  (`parent.UserConstructionScript`))
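; BP_EnemyRange_Showcase is a ranged enemy variant that shows off bullet patterns.
; On BeginPlay it caches the player and bullet manager, loads ShowedPattern as its pattern set and starts a looping timer that plays the attack montage.
; A separate Shoot event spawns the indexed pattern from the right wrist socket along the actor's forward vector, rather than aiming at the player.
; The Hit event is empty.
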(event `anim`
  (`|PlayMontage` (`self.Mesh`) "/Game/NIRVANA/Core/Characters/Enemies/Range/Anims/AM_AttackNormal.AM_AttackNormal"))

(event `/Game/NIRVANA/Core/Characters/FirstPerson/BPI_Hit.Hit`
  (params (Damages :type "Float (double-precision)") (Impulse :type "Vector Structure") (Location :type "Vector Structure") (Bone :type Name)))

(event `self.ReceiveBeginPlay`
  (bind _asbp_first_person_character (cast `/Game/NIRVANA/Core/Characters/FirstPerson/BP_FirstPersonCharacter` (`GameplayStatics.GetPlayerCharacter` 0)))
  (set `self.PlayerRef` _asbp_first_person_character)
  (bind _returnvalue (`GameplayStatics.GetActorOfClass` "/Game/NIRVANA/Core/Characters/Enemies/Range/BP_BulletManager.BP_BulletManager_C"))
  (set `self.Ref Bullet Manager` _returnvalue)
  (set `self.StructPattern` (`self.ShowedPattern`))
  (`KismetSystemLibrary.K2_SetTimerDelegate` (delegate `anim`) 8.0 true))

(event `self.Shoot`
  (bind (_output_pattern _output_nbbulletloop _output_delayeachloop _output_projectilespeed _output_damage _output_dispertion _output_dispertionspeed _output_previsualisation _output_nbbulletrectangle _output_zoffsettransformlocation _output_directionbyoffset) (break `/Game/NIRVANA/Core/Characters/Enemies/Common/Struct_PatternValue` (`|GetArrayItem` (`self.StructPattern`) (`self.PatternIndex`))))
  ;[1 1 1] Shoot
  (`self.Spawn Pattern` _output_pattern _output_nbbulletloop (`KismetMathLibrary.MakeVector` (.x (`SceneComponent.GetSocketLocation` (`self.Mesh`) "Bind_Wrist_RSocket")) (.y (`SceneComponent.GetSocketLocation` (`self.Mesh`) "Bind_Wrist_RSocket")) (+ (.z (`SceneComponent.GetSocketLocation` (`self.Mesh`) "Bind_Wrist_RSocket")) _output_zoffsettransformlocation)) (* (`self.GetActorForwardVector`) 200.0) _output_projectilespeed _output_damage _output_delayeachloop _output_previsualisation 1.0 _output_dispertion _output_dispertionspeed _output_nbbulletrectangle))

(fn `UserConstructionScript`
  (`parent.UserConstructionScript`))
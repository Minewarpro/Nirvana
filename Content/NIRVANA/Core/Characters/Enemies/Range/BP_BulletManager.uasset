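; BP_BulletManager is an object pool manager for enemy projectiles (BP_EnemieProjectile).
; On BeginPlay it pre-spawns about a thousand projectiles into the BulletPull array, ignoring spawn collision.
; ActivateBullet activates the first pooled projectile with movement, damage, delayed redirection, effect and scale parameters, then removes it from the pool, spawning another first if empty.
; Nothing in this Blueprint returns projectiles to the pool.
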(event `self.ReceiveBeginPlay`
  (for _ (range 1001)
    (`self.SpawnInitBullet`)))

(event `Activate Bullet`
  (params (`Spawn Location` :type "Vector Structure") (Direction :type "Vector Structure") (Speed :type "Float (single-precision)") (Damage :type "Float (double-precision)") (`Need Change Direction` :type Boolean) (`Delay Change DIrection` :type "Float (single-precision)") (`New Direction` :type "Vector Structure") (`New Speed` :type "Float (double-precision)") (`Special Effect` :type "/Game/NIRVANA/Core/Characters/Enemies/Common/Enum_SpecialEffectBullet Enum" :default "NewEnumerator1") (Scale :type "Vector Structure"))
  (bind _bulletpull (`self.BulletPull`))
  (bind _output (`|GetArrayItem` _bulletpull))
  (if (`KismetArrayLibrary.Array_IsEmpty` _bulletpull)
    (`self.SpawnInitBullet`))
  (`/Game/NIRVANA/Core/Characters/Enemies/Common/BP_EnemieProjectile.Activate` _output `Spawn Location` Direction Speed Damage `Need Change Direction` `Delay Change DIrection` `New Direction` `New Speed` `Special Effect` Scale)
  (`KismetArrayLibrary.Array_RemoveItem` _bulletpull _output))

(fn `SpawnInitBullet`
  (bind _returnvalue (`|SpawnActorFromClass` "/Game/NIRVANA/Core/Characters/Enemies/Common/BP_EnemieProjectile.BP_EnemieProjectile_C" (`KismetMathLibrary.MakeTransform` (0.0 0.0 0.0)) "AlwaysSpawn" "MultiplyWithRoot" null (0.0 0.0 0.0) 600.0 10.0 false 0.2 (0.0 0.0 0.0) 0.0 "NewEnumerator1" null))
  (`KismetArrayLibrary.Array_Add` (`self.BulletPull`) _returnvalue))

(fn `UserConstructionScript`)
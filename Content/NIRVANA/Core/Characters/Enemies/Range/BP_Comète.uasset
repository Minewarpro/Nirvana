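; BP_Comète is a telegraphed area attack, filed under ranged enemies, that explodes at its location after a delay.
; On BeginPlay, two decals get dynamic materials, with timelines fading in the base and growing a timer radius paced by TimeToExplode.
; When the timer finishes, it removes both decals, spawns a shockwave effect and sphere-traces, damaging the first hit if it is the first-person player character.
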(event `self.ReceiveBeginPlay`
  ;[1 1 1] Create Dynamic materials
  (bind _returnvalue (`KismetMaterialLibrary.CreateDynamicMaterialInstance` (`DecalComponent.GetDecalMaterial` (`self.Base`))))
  (bind _output_get (set `self.Mat_Inst` _returnvalue))
  (`DecalComponent.SetDecalMaterial` (`self.Base`) _output_get)
  (bind _returnvalue_2 (`KismetMaterialLibrary.CreateDynamicMaterialInstance` (`DecalComponent.GetDecalMaterial` (`self.Timer`))))
  (bind _output_get_2 (set `self.Mat_Inst_Timer` _returnvalue_2))
  (`DecalComponent.SetDecalMaterial` (`self.Timer`) _output_get_2)
  (`|ExecutionSequence`
    (:`then_0`
      ;[1 1 1] Base Apparition
      (`TimelineComponent.SetPlayRate` (`self.BaseAlpha TL`) (/ 1.0 0.5))
      (bind (_direction _alpha) (`Timeline|BaseAlpha TL`)
        (:`Update`
          (`MaterialInstanceDynamic.SetScalarParameterValue` (`self.Mat_Inst`) "Opacity" _alpha))))
    (:`then_1`
      ;[1 1 1] Timer Apparition
      (`TimelineComponent.SetPlayRate` (`self.Timer Alpha TL`) (/ 1.0 (/ (`self.TimeToExplode`) 0.6)))
      (bind (_direction_2 _alpha_2 _alphatarget) (`Timeline|Timer Alpha TL`)
        (:`Update`
          (`MaterialInstanceDynamic.SetScalarParameterValue` (`self.Mat_Inst_Timer`) "RadiusApparition" _alpha_2))
        (:`Finished`
          (`self.Explosion`))))))

(event `Explosion`
  (bind _returnvalue (`self.K2_GetActorLocation`))
  ;[1 1 1] Explosion
  (`ActorComponent.K2_DestroyComponent` (`self.Base`))
  (`ActorComponent.K2_DestroyComponent` (`self.Timer`))
  (`NiagaraFunctionLibrary.SpawnSystemAtLocation` "/Game/Collection_of_various_Niagara_VFX_Vol01/Pack/FXS/FXS_shockwave01.FXS_shockwave01" (`self.K2_GetActorLocation`) (struct) (0.7 0.7 0.7))
  (bind _outhit (`KismetSystemLibrary.SphereTraceSingleForObjects` _returnvalue (`KismetMathLibrary.MakeVector` (.x _returnvalue) (.y _returnvalue) (+ (.z _returnvalue) 100.0)) 120.0 (`self.Trace Objects Reponse`)))
  (bind _asbp_first_person_character (cast `/Game/NIRVANA/Core/Characters/FirstPerson/BP_FirstPersonCharacter` (`.HitActor` (`GameplayStatics.BreakHitResult` _outhit))))
  (`/Game/NIRVANA/Core/Characters/FirstPerson/BP_FirstPersonCharacter.Take Damage` _asbp_first_person_character (`self.Damages`) null))

(fn `UserConstructionScript`)
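; Ranged enemy character that fires data-driven bullet-hell patterns at the player and also has a telegraphed melee punch.
; Shoot dispatches the indexed StructPattern entry to pattern events using pooled bullets, preview spawners or comet rain, then disables it and spawns BP_PatternEnabler with its cooldown.
; EQS queries drive timeline-lerped strafing and fleeing, with a flee triggered below half health.
; Hits blend physical-animation stagger, and death updates ArenaManager and dissolves the mesh.
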(event Custom|Dissolve
  ;[1 1 1] Dissolve Effect
  (Components|Timeline|SetPlayRate (Variables|Default|GetDissolve%20TL) (/ 1.0 1.6))
  (bind _alpha_dissolve (Timeline|Dissolve%20TL Play)
    (:Update
      (Rendering|Material|SetScalarParameterValueonMaterials (Variables|Character|GetMesh) "Alpha" _alpha_dissolve)
      (Niagara|SetNiagaraVariable(Float) (Variables|Default|GetNS_Dissolve) "Alpha" _alpha_dissolve))
    (:Finished
      (Utilities|FlowControl|Delay 1.0)
      (Actor|DestroyActor))))

(event Custom|Flee
  (params (Task :type BT%20Task%20Flee%20Object%20Reference))
  ;[1 1 1] Tasks
  ;;[1 1 1] Flee
  (bind _returnvalue (AI|EQS|RunEQSQuery "/Game/NIRVANA/Core/Characters/Enemies/Range/EQS_Flee.EQS_Flee" self "AllMatching"))
  (bind _output_get (Variables|Tasks|SetEQS_Flee _returnvalue))
  (EventDispatchers|AssignOnQueryFinishedEvent _output_get (delegate Custom|OnQueryFinishedEvent_Event)))

(event Custom|Punch
  ;[1 0.02387 0] CloseAttack
  (Animation|Montage|PlayMontage (Variables|Character|GetMesh) "/Game/DevelopersContent/Core/Characters/Enemies/Common/Mixamo_Test/Anim/AM_MeleePunch.AM_MeleePunch" 3.0
    (:then
      (bind _returnvalue (Utilities|Time|SetTimerbyEvent (delegate Custom|RotateToPlayer) 0.01 true 0.0 -0.01))
      (Variables|Default|SetRotateLoop _returnvalue))))

(event Custom|Telegraphing
  ;[1 0.02387 0] CloseAttack
  (Utilities|Time|ClearandInvalidateTimerbyHandle (Variables|Default|GetRotateLoop))
  (Utilities|FlowControl|Delay (Variables|Default|GetTelegraphingDelay))
  (Animation|Montage|PlayMontage (Variables|Character|GetMesh) "/Game/DevelopersContent/Core/Characters/Enemies/Common/Mixamo_Test/Anim/AM_MeleePunch.AM_MeleePunch" 1.0 0.0 "EndCharge"
    (:OnCompleted
      _)
    (:OnInterrupted
      _))
  (Variables|Default|SetCurrentState "NewEnumerator0"))

(event Custom|RotateToPlayer
  (bind _playerref (Variables|Default|GetPlayerRef))
  (bind _returnvalue (Transformation|GetActorLocation _playerref))
  ;[1 0.02387 0] CloseAttack
  (Transformation|SetActorRotation (Math|Rotator|FindLookatRotation (Transformation|GetActorLocation) (Math|Vector|MakeVector (.x _returnvalue) (.y _returnvalue) (.z (Transformation|GetActorLocation))))))

(event Custom|OnQueryFinishedEvent_Event
  (params (QueryInstance :type Env%20Query%20Instance%20Blueprint%20Wrapper%20Object%20Reference) (QueryStatus :type EEnvQueryStatus%20Enum :default "Processing"))
  ;[1 1 1] Tasks
  ;;[1 1 1] Flee
  (bind (_position _valid) (CallFunction|GetBestItem QueryInstance))
  (if _valid
    (Variables|Tasks|SetTargetFleePosition (+ _position "0.000000,0.000000,200.000000"))
    (Variables|Tasks|SetInitPosition (Transformation|GetActorLocation))
    (Components|Timeline|SetPlayRate (Variables|Default|GetTL_Flee) (/ 1.0 0.75))
    (bind _returnvalue (Niagara|SpawnSystemAttached "/Game/NIRVANA/Core/Characters/Enemies/FX/NS_Flee.NS_Flee" (Variables|Character|GetMesh) "None" "0, 0, 0" "0, 0, 0" "KeepRelativeOffset" false))
    (Niagara|SetNiagaraVariable(LinearColor) _returnvalue "Main Color" (Variables|Default|GetFleeColor))
    (Variables|Default|SetNS_Flee%20Ref _returnvalue)
    (Variables|Default|SetFlee%20Direction (Math|Vector|GetUnitDirection(Vector) (Variables|Tasks|GetInitPosition) (Variables|Tasks|GetTargetFleePosition)))
    (bind _newtrack_0 (Timeline|TL_Flee PlayFromStart)
      (:Update
        (Transformation|SetActorLocation (Math|Vector|Lerp(Vector) (Variables|Tasks|GetInitPosition) (Variables|Tasks|GetTargetFleePosition) _newtrack_0) true false))
      (:Finished
        (Utilities|FlowControl|Sequence
          (:then_0
            (Utilities|IsValid (stale Custom|Flee Task)
              (:Is%20Valid
                (Default|FreeFlee (stale Custom|Flee Task)))))
          (:then_1
            (Variables|Default|SetCurrentState "NewEnumerator0")
            (Components|DestroyComponent (Variables|Default|GetNS_Flee%20Ref))))))
    (else
      (Variables|Default|SetCurrentState "NewEnumerator0")
      (Utilities|IsValid (stale Custom|Flee Task)
        (:Is%20Valid
          (Default|FreeFlee (stale Custom|Flee Task)))))))

(event Custom|Shoot
  (bind _patternindex (Variables|Default|GetPatternIndex))
  (bind _structpattern (Variables|Default|GetStructPattern))
  (bind _mesh (Variables|Character|GetMesh))
  (bind _structpattern_2 (Variables|Default|GetStructPattern))
  (bind _patternindex_2 (Variables|Default|GetPatternIndex))
  (bind _returnvalue (Transformation|GetSocketLocation _mesh "Bind_Wrist_RSocket"))
  (bind _output (Utilities|Array|Get(acopy) _structpattern_2 _patternindex_2))
  (bind _output_2 (Utilities|Array|Get(acopy) _structpattern _patternindex))
  (bind (_pattern _nbbulletloop _delayeachloop _projectilespeed _damage _dispertion _dispertionspeed _previsualisation _nbbulletrectangle _zoffsettransformlocation _directionbyoffset _disabled _delay) (Utilities|Struct|BreakStruct_PatternValue _output))
  (bind (_x _y _z) (Math|Vector|BreakVector _returnvalue))
  (bind _returnvalue_2 (+ _z (.zoffsettransformlocation _output_2)))
  (bind _returnvalue_3 (Math|Vector|MakeVector _x _y _returnvalue_2))
  ;[1 1 1] Shoot
  (Utilities|FlowControl|Sequence
    (:then_0
      (CallFunction|SpawnPattern (.pattern _output_2) (.nbbulletloop _output_2) _returnvalue_3 (Math|Vector|GetUnitDirection(Vector) (Math|Vector|SelectVector _returnvalue_3 _returnvalue (.directionbyoffset _output_2)) (Transformation|GetActorLocation (Variables|Default|GetPlayerRef))) (.projectilespeed _output_2) (.damage _output_2) (.delayeachloop _output_2) (.previsualisation _output_2) 1.0 (.dispertion _output_2) (.dispertionspeed _output_2) (.nbbulletrectangle _output_2))
      (Utilities|Array|SetArrayElem _structpattern_2 _patternindex (Utilities|Struct|MakeStruct_PatternValue _pattern _nbbulletloop _delayeachloop _projectilespeed _damage _dispertion _dispertionspeed _previsualisation _nbbulletrectangle _zoffsettransformlocation _directionbyoffset true _delay)))
    (:then_1
      (Variables|Default|SetToken false)
      (Game|SpawnActorfromClass "/Game/NIRVANA/Core/Characters/Enemies/Range/BP_PatternEnabler.BP_PatternEnabler_C" (Math|Transform|MakeTransform "0, 0, 0" "0, 0, 0" "1.000000,1.000000,1.000000") "Undefined" "MultiplyWithRoot" 0 _delay _patternindex_2 self 0))))

(event Custom|Strafe
  (params (QueryTemplate :type Env%20Query%20Object%20Reference))
  ;[1 1 1] Tasks
  ;;[1 1 1] Strafe
  (bind _returnvalue (AI|EQS|RunEQSQuery QueryTemplate self "SingleResult"))
  (bind _output_get (Variables|Tasks|SetEQS_Strafe _returnvalue))
  (EventDispatchers|BindEventtoOnQueryFinishedEvent _output_get (delegate Custom|OnQueryStrafeFinishedEvent)))

(event Custom|OnQueryStrafeFinishedEvent
  (params (QueryInstance :type Env%20Query%20Instance%20Blueprint%20Wrapper%20Object%20Reference) (QueryStatus :type EEnvQueryStatus%20Enum :default "Processing"))
  ;[1 1 1] Tasks
  ;;[1 1 1] Strafe
  (bind (_position _valid) (CallFunction|GetBestItem QueryInstance))
  (if _valid
    (Variables|Tasks|SetTargetFleePosition (+ _position "0.000000,0.000000,133.000000"))
    (Variables|Tasks|SetInitPosition (Transformation|GetActorLocation))
    (Components|Timeline|SetPlayRate (Variables|Default|GetTL_Strafe) (/ 1.0 1.0))
    (bind _newtrack_0 (Timeline|TL_Strafe PlayFromStart)
      (:Update
        (Transformation|SetActorLocation (Math|Vector|Lerp(Vector) (Variables|Tasks|GetInitPosition) (Variables|Tasks|GetTargetFleePosition) _newtrack_0) false false)))))

(event EventBeginPlay
  ;[1 0.6945 0.125 1 34] Begin Play
  (|CallParentFunction)
  (bind _returnvalue (Actor|GetActorOfClass "/Game/NIRVANA/Core/Characters/Enemies/Range/BP_BulletManager.BP_BulletManager_C"))
  (Variables|Default|SetRef%20Bullet%20Manager _returnvalue)
  (Class|PhysicalAnimationComponent|SetSkeletalMeshComponent (Variables|Default|GetPhysicalAnimation) (Variables|Character|GetMesh))
  (Class|PhysicalAnimationComponent|ApplyPhysicalAnimationSettingsBelow (Variables|Default|GetPhysicalAnimation) "Bind_Pelvis" (Utilities|Struct|MakePhysicalAnimationData true 3.5e+02 1e+02 5e+01 5e+01) false)
  (Class|SkeletalMeshComponent|SetAllBodiesBelowSimulatePhysics (Variables|Character|GetMesh) (Utilities|Name|MakeLiteralName "Bind_Pelvis") true false)
  (Class|SkeletalMeshComponent|SetAllBodiesBelowPhysicsBlendWeight (Variables|Character|GetMesh) (Utilities|Name|MakeLiteralName "Bind_Pelvis") 0.0 false false))

(event EventDeath
  (bind _mesh (Variables|Character|GetMesh))
  ;[0.0226 0.0399 0.08854] Death
  ;;[1 1 1] Tests Mathieu
  (Utilities|FlowControl|DoOnce false
    (:Completed
      (Components|DestroyComponent (Variables|Default|GetWidgetLifeBar))
      (Collision|SetCollisionResponsetoChannel (Variables|Default|GetCapsuleComponent) "ECC_GameTraceChannel3" "ECR_Ignore")
      (Collision|SetCollisionResponsetoChannel _mesh "ECC_GameTraceChannel3" "ECR_Ignore")
      (Collision|SetCollisionResponsetoChannel _mesh "ECC_GameTraceChannel5" "ECR_Ignore")
      (Collision|SetCollisionResponsetoChannel (Variables|Default|GetCapsuleComponent) "ECC_Pawn" "ECR_Ignore")
      (Class|Pawn|DetachfromControllerPendingDestroy self)
      (Animation|Montage|PlayMontage (Variables|Character|GetMesh) "/Game/NIRVANA/Core/Characters/Enemies/Range/Anims/Death_Montage.Death_Montage" 1.2
        (:then
          (CallFunction|Dissolve)
          (Audio|PlaySoundatLocation "/Game/NIRVANA/Core/Characters/Enemies/Range/Sounds/MS_MidDeath.MS_MidDeath" (Transformation|GetActorLocation) "0, 0, 0" 1.0 1.0 0.0 0 0 0 0)
          (Utilities|Array|RemoveItem (Variables|/Game/NIRVANA/Core/Placeables/Management/BP_ArenaManager.BP_ArenaManager_C|GetTotal%20EnemiesRange (Variables|Default|GetArenaManager)) self)
          (Default|AddNbKilledEnemy (Variables|Default|GetArenaManager))
          (|CallParentFunction))))))

(event EventHit
  (params (Damages :type Float%20%28double-precision%29) (Impulse :type Vector :default "0, 0, 0") (Location :type Vector :default "0, 0, 0") (Bone :type Name :default "None"))
  (bind _returnvalue (Utilities|Name|MakeLiteralName "Bind_Pelvis"))
  ;[1 0.3765 0.3765] Hit
  (Utilities|FlowControl|Sequence
    (:then_0
      (Class|SkeletalMeshComponent|SetAllBodiesBelowPhysicsBlendWeight (Variables|Character|GetMesh) _returnvalue 1.0 false false)
      (Components|Timeline|SetPlayRate (Variables|Default|GetTStagger) (/ 1.0 0.35))
      (if (Variables|Default|GetStagging)
        (bind _newtrack_0 (Timeline|TStagger Play)
          (:Update
            (Variables|Default|SetStagging true)
            (Class|SkeletalMeshComponent|SetAllBodiesBelowPhysicsBlendWeight (Variables|Character|GetMesh) _returnvalue _newtrack_0 false false))
          (:Finished
            (Class|SkeletalMeshComponent|ResetAllBodiesSimulatePhysics (Variables|Character|GetMesh))
            (Class|SkeletalMeshComponent|SetAllBodiesBelowPhysicsBlendWeight (Variables|Character|GetMesh) _returnvalue 0.0 false true)
            (Variables|Default|SetStagging false)))
        (else
          (Timeline|TStagger PlayFromStart))))
    (:then_1
      (Variables|Default|SetPreviousHealth (Variables|Default|GetCurrentHealth))
      (|CallParentFunction Damages Impulse Location Bone)
      (Default|SortingRange (Variables|Default|GetArenaManager))
      (if (and (>= (Variables|Default|GetPreviousHealth) (/ (Variables|Default|GetMaxHealth) 2.0)) (< (Variables|Default|GetCurrentHealth) (/ (Variables|Default|GetMaxHealth) 2.0)))
        (CallFunction|Flee)))))

(event Custom|Rectangle
  (params (NbBullet :type Integer) (Spawn%20Transform%20Location :type Vector) (Direction :type Vector) (Speed :type Float%20%28double-precision%29) (Damage :type Float%20%28double-precision%29) (Delay%20Each%20Loop :type Float%20%28double-precision%29) (Pre-Visualisation :type Boolean) (Projectile%20Scale :type Float%20%28double-precision%29) (Dispertion%20Speed :type Float%20%28double-precision%29) (NB%20Bullet%20Secondaire :type Integer) (Dispertion :type Boolean))
  (bind _returnvalue (Math|Conversions|RotationFromXVector Direction))
  (bind _returnvalue_2 (Math|Conversions|ToVector(Float) Projectile%20Scale))
  (bind _returnvalue_3 (* Projectile%20Scale 8e+01))
  (bind _returnvalue_4 (- NbBullet 1))
  (bind _returnvalue_5 (* Projectile%20Scale 8e+01))
  (bind _returnvalue_6 (- NB%20Bullet%20Secondaire 1))
  (bind _returnvalue_7 (Math|Vector|GetRightVector _returnvalue))
  ;[1 1 1] Rectangle
  (for _index (range 0 _returnvalue_4) ; Y
    (for _index_2 (range 0 _returnvalue_6) ; X
      (if Pre-Visualisation
        (Game|SpawnActorfromClass "/Game/NIRVANA/Core/Characters/Enemies/Common/BP_EnemyProjectileApparition.BP_EnemyProjectileApparition_C" (Math|Transform|MakeTransform (+ Spawn%20Transform%20Location (+ (* _returnvalue_7 (* (- _index (/ _returnvalue_4 2)) (select Dispertion _returnvalue_5 _returnvalue_3))) (* (Math|Vector|CrossProduct Direction _returnvalue_7) (* (- _index_2 (/ _returnvalue_6 2)) (select Dispertion _returnvalue_5 _returnvalue_3))))) "0, 0, 0" _returnvalue_2) "AlwaysSpawn" "MultiplyWithRoot" 0 0.5 (+ Spawn%20Transform%20Location (+ (* _returnvalue_7 (* (- _index (/ _returnvalue_4 2)) (select Dispertion _returnvalue_5 _returnvalue_3))) (* (Math|Vector|CrossProduct Direction _returnvalue_7) (* (- _index_2 (/ _returnvalue_6 2)) (select Dispertion _returnvalue_5 _returnvalue_3))))) (select Dispertion (Utilities|Dispertion Spawn%20Transform%20Location (+ Spawn%20Transform%20Location (+ (* _returnvalue_7 (* (- _index (/ _returnvalue_4 2)) (select Dispertion _returnvalue_5 _returnvalue_3))) (* (Math|Vector|CrossProduct Direction _returnvalue_7) (* (- _index_2 (/ _returnvalue_6 2)) (select Dispertion _returnvalue_5 _returnvalue_3))))) Direction Dispertion%20Speed false) Direction) Speed Damage false 0.2 "0.000000,0.000000,0.000000" 0.0 (Variables|Default|GetRef%20Bullet%20Manager) self "NewEnumerator1" 0)
        (else
          (Default|ActivateBullet (Variables|Default|GetRef%20Bullet%20Manager) (+ Spawn%20Transform%20Location (+ (* _returnvalue_7 (* (- _index (/ _returnvalue_4 2)) (select Dispertion _returnvalue_5 _returnvalue_3))) (* (Math|Vector|CrossProduct Direction _returnvalue_7) (* (- _index_2 (/ _returnvalue_6 2)) (select Dispertion _returnvalue_5 _returnvalue_3))))) (select Dispertion (Utilities|Dispertion Spawn%20Transform%20Location (+ Spawn%20Transform%20Location (+ (* _returnvalue_7 (* (- _index (/ _returnvalue_4 2)) (select Dispertion _returnvalue_5 _returnvalue_3))) (* (Math|Vector|CrossProduct Direction _returnvalue_7) (* (- _index_2 (/ _returnvalue_6 2)) (select Dispertion _returnvalue_5 _returnvalue_3))))) Direction Dispertion%20Speed false) Direction) Speed Damage false 0.0 "0, 0, 0" 0.0 "NewEnumerator1" _returnvalue_2 self false 0.0 0.0))))))

(event Custom|Horizontal%20Round
  (params (NbBullet :type Integer) (Spawn%20Transform%20Location :type Vector) (Direction :type Vector) (Speed :type Float%20%28double-precision%29) (Damage :type Float%20%28double-precision%29) (Delay%20Each%20Loop :type Float%20%28double-precision%29) (Pre-Visualisation :type Boolean) (Projectile%20Scale :type Float%20%28double-precision%29) (Dispertion%20Speed :type Float%20%28double-precision%29))
  (bind _returnvalue (Math|Conversions|ToVector(Float) Projectile%20Scale))
  (bind _returnvalue_2 (Math|Conversions|RotationFromXVector Direction))
  ;[1 1 1] Horizontal Round
  (bind _index (Utilities|ForLoopDelayed 0 (- NbBullet 1) Delay%20Each%20Loop)
    (:Loop%20Body
      (if Pre-Visualisation
        (Game|SpawnActorfromClass "/Game/NIRVANA/Core/Characters/Enemies/Common/BP_EnemyProjectileApparition.BP_EnemyProjectileApparition_C" (Math|Transform|MakeTransform (Math|Vector|MakeVector (.X (Math|Vector|BreakVector (+ (* (Math|Vector|RotateVectorAroundAxis (* (Math|Vector|GetRightVector _returnvalue_2) -1.0) (* _index (/ 1.8e+02 (Math|Conversions|ToFloat(Integer) NbBullet))) (Math|Vector|GetUpVector _returnvalue_2)) 2e+02) Spawn%20Transform%20Location))) (.Y (Math|Vector|BreakVector (+ (* (Math|Vector|RotateVectorAroundAxis (* (Math|Vector|GetRightVector _returnvalue_2) -1.0) (* _index (/ 1.8e+02 (Math|Conversions|ToFloat(Integer) NbBullet))) (Math|Vector|GetUpVector _returnvalue_2)) 2e+02) Spawn%20Transform%20Location))) (+ (.Z (Math|Vector|BreakVector (+ (* (Math|Vector|RotateVectorAroundAxis (* (Math|Vector|GetRightVector _returnvalue_2) -1.0) (* _index (/ 1.8e+02 (Math|Conversions|ToFloat(Integer) NbBullet))) (Math|Vector|GetUpVector _returnvalue_2)) 2e+02) Spawn%20Transform%20Location))) (* (stale _index) 5e+01))) "0, 0, 0" _returnvalue) "AlwaysSpawn" "MultiplyWithRoot" 0 0.5 (Math|Vector|MakeVector (.X (Math|Vector|BreakVector (+ (* (Math|Vector|RotateVectorAroundAxis (* (Math|Vector|GetRightVector _returnvalue_2) -1.0) (* _index (/ 1.8e+02 (Math|Conversions|ToFloat(Integer) NbBullet))) (Math|Vector|GetUpVector _returnvalue_2)) 2e+02) Spawn%20Transform%20Location))) (.Y (Math|Vector|BreakVector (+ (* (Math|Vector|RotateVectorAroundAxis (* (Math|Vector|GetRightVector _returnvalue_2) -1.0) (* _index (/ 1.8e+02 (Math|Conversions|ToFloat(Integer) NbBullet))) (Math|Vector|GetUpVector _returnvalue_2)) 2e+02) Spawn%20Transform%20Location))) (+ (.Z (Math|Vector|BreakVector (+ (* (Math|Vector|RotateVectorAroundAxis (* (Math|Vector|GetRightVector _returnvalue_2) -1.0) (* _index (/ 1.8e+02 (Math|Conversions|ToFloat(Integer) NbBullet))) (Math|Vector|GetUpVector _returnvalue_2)) 2e+02) Spawn%20Transform%20Location))) (* (stale _index) 5e+01))) (Utilities|Dispertion Spawn%20Transform%20Location (+ (* (Math|Vector|RotateVectorAroundAxis (* (Math|Vector|GetRightVector _returnvalue_2) -1.0) (* _index (/ 1.8e+02 (Math|Conversions|ToFloat(Integer) NbBullet))) (Math|Vector|GetUpVector _returnvalue_2)) 2e+02) Spawn%20Transform%20Location) Direction Dispertion%20Speed false) Speed Damage false 0.2 "0.000000,0.000000,0.000000" 0.0 (Variables|Default|GetRef%20Bullet%20Manager) self "NewEnumerator1" 0)
        (else
          (Default|ActivateBullet (Variables|Default|GetRef%20Bullet%20Manager) (Math|Vector|MakeVector (.X (Math|Vector|BreakVector (+ (* (Math|Vector|RotateVectorAroundAxis (* (Math|Vector|GetRightVector _returnvalue_2) -1.0) (* _index (/ 1.8e+02 (Math|Conversions|ToFloat(Integer) NbBullet))) (Math|Vector|GetUpVector _returnvalue_2)) 2e+02) Spawn%20Transform%20Location))) (.Y (Math|Vector|BreakVector (+ (* (Math|Vector|RotateVectorAroundAxis (* (Math|Vector|GetRightVector _returnvalue_2) -1.0) (* _index (/ 1.8e+02 (Math|Conversions|ToFloat(Integer) NbBullet))) (Math|Vector|GetUpVector _returnvalue_2)) 2e+02) Spawn%20Transform%20Location))) (+ (.Z (Math|Vector|BreakVector (+ (* (Math|Vector|RotateVectorAroundAxis (* (Math|Vector|GetRightVector _returnvalue_2) -1.0) (* _index (/ 1.8e+02 (Math|Conversions|ToFloat(Integer) NbBullet))) (Math|Vector|GetUpVector _returnvalue_2)) 2e+02) Spawn%20Transform%20Location))) (* (stale _index) 5e+01))) (Utilities|Dispertion Spawn%20Transform%20Location (+ (* (Math|Vector|RotateVectorAroundAxis (* (Math|Vector|GetRightVector _returnvalue_2) -1.0) (* _index (/ 1.8e+02 (Math|Conversions|ToFloat(Integer) NbBullet))) (Math|Vector|GetUpVector _returnvalue_2)) 2e+02) Spawn%20Transform%20Location) Direction Dispertion%20Speed false) Speed Damage false 0.0 "0, 0, 0" 0.0 "NewEnumerator1" _returnvalue self false 0.0 0.0))))))

(event Custom|Simple%20Pattern
  (params (NbBullet :type Integer) (Spawn%20Transform%20Location :type Vector) (Direction :type Vector) (Speed :type Float%20%28double-precision%29) (Damage :type Float%20%28double-precision%29) (Delay%20Each%20Loop :type Float%20%28double-precision%29) (Pre-Visualisation :type Boolean) (Projectile%20Scale :type Float%20%28double-precision%29))
  (bind _returnvalue (Math|Conversions|ToVector(Float) Projectile%20Scale))
  (bind _returnvalue_2 (Math|Random|RandomUnitVectorinConeinDegrees Direction 2.0))
  ;[1 1 1] Simple
  (bind _index (Utilities|ForLoopDelayed 0 (- NbBullet 1) Delay%20Each%20Loop)
    (:Loop%20Body
      (if Pre-Visualisation
        (Game|SpawnActorfromClass "/Game/NIRVANA/Core/Characters/Enemies/Common/BP_EnemyProjectileApparition.BP_EnemyProjectileApparition_C" (Math|Transform|MakeTransform Spawn%20Transform%20Location "0, 0, 0" _returnvalue) "AlwaysSpawn" "MultiplyWithRoot" 0 0.5 Spawn%20Transform%20Location _returnvalue_2 Speed Damage false 0.2 "0.000000,0.000000,0.000000" 0.0 (Variables|Default|GetRef%20Bullet%20Manager) self "NewEnumerator1" 0)
        (else
          (Default|ActivateBullet (Variables|Default|GetRef%20Bullet%20Manager) Spawn%20Transform%20Location _returnvalue_2 Speed Damage false 0.0 "0, 0, 0" 0.0 "NewEnumerator1" _returnvalue self true 1.0 (- 2e+04 (* _index (/ 20000 NbBullet)))))))))

(event Custom|PluieDeComete
  ;[1 1 1] Comete
  (bind _returnvalue (Utilities|Time|SetTimerbyEvent (delegate Custom|LaunchComete) (Variables|Comete|GetCometeInterval) true))
  (Variables|Comete|SetPluieDeCometeEvent _returnvalue)
  (Utilities|FlowControl|Delay (Variables|Comete|GetPluieDuration))
  (Utilities|Time|ClearandInvalidateTimerbyHandle (Variables|Comete|GetPluieDeCometeEvent)))

(event Custom|LaunchComete
  (bind _playerref (Variables|Default|GetPlayerRef))
  (bind _rangespawncomete (Variables|Comete|GetRangeSpawnComete))
  (bind _returnvalue (Transformation|GetActorLocation _playerref))
  (bind _returnvalue_2 (* _rangespawncomete -1.0))
  (bind (_x _y _z) (Math|Vector|BreakVector _returnvalue))
  ;[1 1 1] Comete
  (bind _output_get (Variables|Comete|SetCometeTempLocation (Math|Vector|MakeVector (+ _x (Math|Random|RandomFloatinRange _returnvalue_2 _rangespawncomete)) (+ _y (Math|Random|RandomFloatinRange _returnvalue_2 _rangespawncomete)) (+ _z 3e+02))))
  (bind _outhit (Collision|LineTraceByChannel _output_get (Math|Vector|MakeVector (.X (Math|Vector|BreakVector _output_get)) (.Y (Math|Vector|BreakVector _output_get)) (- (.Z (Math|Vector|BreakVector _output_get)) 1e+04)) "TraceTypeQuery1" false 0 "None" true "(R=1.000000,G=0.000000,B=0.000000,A=1.000000)" "(R=0.000000,G=1.000000,B=0.000000,A=1.000000)" 2.0))
  (if (.bBlockingHit (Collision|BreakHitResult _outhit))
    (Game|SpawnActorfromClass "/Game/NIRVANA/Core/Characters/Enemies/Range/BP_Comète.BP_Comète_C" (Math|Transform|MakeTransform (.ImpactPoint (Collision|BreakHitResult _outhit)) "0, 0, 0" "1.000000,1.000000,1.000000") "Undefined" "MultiplyWithRoot" 0 0)))

(event Custom|GrossBoule
  (params (NbBullet :type Integer) (Spawn%20Transform%20Location :type Vector) (Direction :type Vector) (Speed :type Float%20%28double-precision%29) (Damage :type Float%20%28double-precision%29) (Delay%20Each%20Loop :type Float%20%28double-precision%29) (Pre-Visualisation :type Boolean) (Projectile%20Scale :type Float%20%28double-precision%29))
  ;[1 1 1] GrossBoule
  (Utilities|ForLoopDelayed 0 (- NbBullet 1) Delay%20Each%20Loop
    (:Loop%20Body
      (if Pre-Visualisation
        (Game|SpawnActorfromClass "/Game/NIRVANA/Core/Characters/Enemies/Common/BP_EnemyProjectileApparition.BP_EnemyProjectileApparition_C" (Math|Transform|MakeTransform Spawn%20Transform%20Location "0, 0, 0" "10.000000,10.000000,10.000000") "AlwaysSpawn" "MultiplyWithRoot" 0 2.0 Spawn%20Transform%20Location Direction Speed Damage false 0.2 "0.000000,0.000000,0.000000" 0.0 (Variables|Default|GetRef%20Bullet%20Manager) self "NewEnumerator1" 0)
        (else
          (Default|ActivateBullet (Variables|Default|GetRef%20Bullet%20Manager) Spawn%20Transform%20Location Direction Speed Damage false 0.0 "0, 0, 0" 0.0 "NewEnumerator3" "10.000000,10.000000,10.000000" self false 0.0 0.0))))))

(event Custom|Horizontal%20Round%20Mitrallette
  (params (NbBullet :type Integer) (Spawn%20Transform%20Location :type Vector) (Direction :type Vector) (Speed :type Float%20%28double-precision%29) (Damage :type Float%20%28double-precision%29) (Delay%20Each%20Loop :type Float%20%28double-precision%29) (Pre-Visualisation :type Boolean) (Projectile%20Scale :type Float%20%28double-precision%29) (Dispertion%20Speed :type Float%20%28double-precision%29))
  (bind _returnvalue (Math|Conversions|ToVector(Float) Projectile%20Scale))
  (bind _returnvalue_2 (Math|Conversions|RotationFromXVector Direction))
  ;[1 1 1] Horizontal Round
  (bind _index (Utilities|ForLoopDelayed 0 (- NbBullet 1) Delay%20Each%20Loop)
    (:Loop%20Body
      (if Pre-Visualisation
        (Game|SpawnActorfromClass "/Game/NIRVANA/Core/Characters/Enemies/Common/BP_EnemyProjectileApparition.BP_EnemyProjectileApparition_C" (Math|Transform|MakeTransform (Math|Vector|MakeVector (.X (Math|Vector|BreakVector (+ (* (Math|Vector|RotateVectorAroundAxis (* (Math|Vector|GetRightVector _returnvalue_2) -1.0) (* _index (/ 1.8e+02 (Math|Conversions|ToFloat(Integer) NbBullet))) (Math|Vector|GetUpVector _returnvalue_2)) 2e+02) Spawn%20Transform%20Location))) (.Y (Math|Vector|BreakVector (+ (* (Math|Vector|RotateVectorAroundAxis (* (Math|Vector|GetRightVector _returnvalue_2) -1.0) (* _index (/ 1.8e+02 (Math|Conversions|ToFloat(Integer) NbBullet))) (Math|Vector|GetUpVector _returnvalue_2)) 2e+02) Spawn%20Transform%20Location))) (+ (.Z (Math|Vector|BreakVector (+ (* (Math|Vector|RotateVectorAroundAxis (* (Math|Vector|GetRightVector _returnvalue_2) -1.0) (* _index (/ 1.8e+02 (Math|Conversions|ToFloat(Integer) NbBullet))) (Math|Vector|GetUpVector _returnvalue_2)) 2e+02) Spawn%20Transform%20Location))) (* (stale _index) 5e+01))) "0, 0, 0" _returnvalue) "AlwaysSpawn" "MultiplyWithRoot" 0 (+ 0.5 (* _index 0.1)) (Math|Vector|MakeVector (.X (Math|Vector|BreakVector (+ (* (Math|Vector|RotateVectorAroundAxis (* (Math|Vector|GetRightVector _returnvalue_2) -1.0) (* _index (/ 1.8e+02 (Math|Conversions|ToFloat(Integer) NbBullet))) (Math|Vector|GetUpVector _returnvalue_2)) 2e+02) Spawn%20Transform%20Location))) (.Y (Math|Vector|BreakVector (+ (* (Math|Vector|RotateVectorAroundAxis (* (Math|Vector|GetRightVector _returnvalue_2) -1.0) (* _index (/ 1.8e+02 (Math|Conversions|ToFloat(Integer) NbBullet))) (Math|Vector|GetUpVector _returnvalue_2)) 2e+02) Spawn%20Transform%20Location))) (+ (.Z (Math|Vector|BreakVector (+ (* (Math|Vector|RotateVectorAroundAxis (* (Math|Vector|GetRightVector _returnvalue_2) -1.0) (* _index (/ 1.8e+02 (Math|Conversions|ToFloat(Integer) NbBullet))) (Math|Vector|GetUpVector _returnvalue_2)) 2e+02) Spawn%20Transform%20Location))) (* (stale _index) 5e+01))) (Utilities|Dispertion Spawn%20Transform%20Location (+ (* (Math|Vector|RotateVectorAroundAxis (* (Math|Vector|GetRightVector _returnvalue_2) -1.0) (* _index (/ 1.8e+02 (Math|Conversions|ToFloat(Integer) NbBullet))) (Math|Vector|GetUpVector _returnvalue_2)) 2e+02) Spawn%20Transform%20Location) Direction Dispertion%20Speed false) Speed Damage false 0.2 "0.000000,0.000000,0.000000" 0.0 (Variables|Default|GetRef%20Bullet%20Manager) 0 "NewEnumerator5" 0)
        (else
          (Default|ActivateBullet (Variables|Default|GetRef%20Bullet%20Manager) (Math|Vector|MakeVector (.X (Math|Vector|BreakVector (+ (* (Math|Vector|RotateVectorAroundAxis (* (Math|Vector|GetRightVector _returnvalue_2) -1.0) (* _index (/ 1.8e+02 (Math|Conversions|ToFloat(Integer) NbBullet))) (Math|Vector|GetUpVector _returnvalue_2)) 2e+02) Spawn%20Transform%20Location))) (.Y (Math|Vector|BreakVector (+ (* (Math|Vector|RotateVectorAroundAxis (* (Math|Vector|GetRightVector _returnvalue_2) -1.0) (* _index (/ 1.8e+02 (Math|Conversions|ToFloat(Integer) NbBullet))) (Math|Vector|GetUpVector _returnvalue_2)) 2e+02) Spawn%20Transform%20Location))) (+ (.Z (Math|Vector|BreakVector (+ (* (Math|Vector|RotateVectorAroundAxis (* (Math|Vector|GetRightVector _returnvalue_2) -1.0) (* _index (/ 1.8e+02 (Math|Conversions|ToFloat(Integer) NbBullet))) (Math|Vector|GetUpVector _returnvalue_2)) 2e+02) Spawn%20Transform%20Location))) (* (stale _index) 5e+01))) (Utilities|Dispertion Spawn%20Transform%20Location (+ (* (Math|Vector|RotateVectorAroundAxis (* (Math|Vector|GetRightVector _returnvalue_2) -1.0) (* _index (/ 1.8e+02 (Math|Conversions|ToFloat(Integer) NbBullet))) (Math|Vector|GetUpVector _returnvalue_2)) 2e+02) Spawn%20Transform%20Location) Direction Dispertion%20Speed false) Speed Damage false 0.0 "0, 0, 0" 0.0 "NewEnumerator5" _returnvalue self false 0.0 0.0))))))

(event Custom|Circle%20Explosion
  (params (NbBullet :type Integer) (Spawn%20Transform%20Location :type Vector) (Direction :type Vector) (Speed :type Float%20%28double-precision%29) (Damage :type Float%20%28double-precision%29) (Delay%20Each%20Loop :type Float%20%28double-precision%29) (Pre-Visualisation :type Boolean) (Projectile%20Scale :type Float%20%28double-precision%29) (Dispertion%20Speed :type Float%20%28double-precision%29))
  (bind _returnvalue (Math|Conversions|ToFloat(Integer) NbBullet))
  (bind _returnvalue_2 (/ 3.6e+02 _returnvalue))
  ;[1 1 1] Circle Explosion
  (for _index (range 0 1) ; Etages
    (bind _index_2 (Utilities|ForLoopDelayed 0 (- NbBullet 1) Delay%20Each%20Loop)
      (:Loop%20Body
        (if Pre-Visualisation
          (Game|SpawnActorfromClass "/Game/NIRVANA/Core/Characters/Enemies/Common/BP_EnemyProjectileApparition.BP_EnemyProjectileApparition_C" (Math|Transform|MakeTransform (Math|Vector|MakeVector (.X (Math|Vector|BreakVector (+ (* (Math|Vector|RotateVectorAroundAxis Direction (+ (* _index_2 _returnvalue_2) (+ _returnvalue_2 (* _returnvalue_2 (Math|Float|SelectFloat 0.0 0.5 (== (Math|Integer|%(Integer) _index 2) 0))))) "0.000000,0.000000,1.000000") 1e+02) Spawn%20Transform%20Location))) (.Y (Math|Vector|BreakVector (+ (* (Math|Vector|RotateVectorAroundAxis Direction (+ (* _index_2 _returnvalue_2) (+ _returnvalue_2 (* _returnvalue_2 (Math|Float|SelectFloat 0.0 0.5 (== (Math|Integer|%(Integer) _index 2) 0))))) "0.000000,0.000000,1.000000") 1e+02) Spawn%20Transform%20Location))) (+ (.Z (Math|Vector|BreakVector (+ (* (Math|Vector|RotateVectorAroundAxis Direction (+ (* _index_2 _returnvalue_2) (+ _returnvalue_2 (* _returnvalue_2 (Math|Float|SelectFloat 0.0 0.5 (== (Math|Integer|%(Integer) _index 2) 0))))) "0.000000,0.000000,1.000000") 1e+02) Spawn%20Transform%20Location))) (* _index 1e+02))) "0, 0, 0" (Math|Conversions|ToVector(Float) Projectile%20Scale)) "AlwaysSpawn" "MultiplyWithRoot" 0 0.5 (Math|Vector|MakeVector (.X (Math|Vector|BreakVector (+ (* (Math|Vector|RotateVectorAroundAxis Direction (+ (* _index_2 _returnvalue_2) (+ _returnvalue_2 (* _returnvalue_2 (Math|Float|SelectFloat 0.0 0.5 (== (Math|Integer|%(Integer) _index 2) 0))))) "0.000000,0.000000,1.000000") 1e+02) Spawn%20Transform%20Location))) (.Y (Math|Vector|BreakVector (+ (* (Math|Vector|RotateVectorAroundAxis Direction (+ (* _index_2 _returnvalue_2) (+ _returnvalue_2 (* _returnvalue_2 (Math|Float|SelectFloat 0.0 0.5 (== (Math|Integer|%(Integer) _index 2) 0))))) "0.000000,0.000000,1.000000") 1e+02) Spawn%20Transform%20Location))) (+ (.Z (Math|Vector|BreakVector (+ (* (Math|Vector|RotateVectorAroundAxis Direction (+ (* _index_2 _returnvalue_2) (+ _returnvalue_2 (* _returnvalue_2 (Math|Float|SelectFloat 0.0 0.5 (== (Math|Integer|%(Integer) _index 2) 0))))) "0.000000,0.000000,1.000000") 1e+02) Spawn%20Transform%20Location))) (* _index 1e+02))) (Math|Vector|MakeVector (.X (Math|Vector|BreakVector (Math|Vector|RotateVectorAroundAxis Direction (+ (* _index_2 _returnvalue_2) (+ _returnvalue_2 (* _returnvalue_2 (Math|Float|SelectFloat 0.0 0.5 (== (Math|Integer|%(Integer) _index 2) 0))))) "0.000000,0.000000,1.000000"))) (.Y (Math|Vector|BreakVector (Math|Vector|RotateVectorAroundAxis Direction (+ (* _index_2 _returnvalue_2) (+ _returnvalue_2 (* _returnvalue_2 (Math|Float|SelectFloat 0.0 0.5 (== (Math|Integer|%(Integer) _index 2) 0))))) "0.000000,0.000000,1.000000"))) 0.0) Speed Damage false 0.2 "0.000000,0.000000,0.000000" 0.0 (Variables|Default|GetRef%20Bullet%20Manager) self "NewEnumerator1" 0)
          (else
            (Default|ActivateBullet (Variables|Default|GetRef%20Bullet%20Manager) (Math|Vector|MakeVector (.X (Math|Vector|BreakVector (+ (* (Math|Vector|RotateVectorAroundAxis Direction (+ (* _index_2 _returnvalue_2) (+ _returnvalue_2 (* _returnvalue_2 (Math|Float|SelectFloat 0.0 0.5 (== (Math|Integer|%(Integer) _index 2) 0))))) "0.000000,0.000000,1.000000") 1e+02) Spawn%20Transform%20Location))) (.Y (Math|Vector|BreakVector (+ (* (Math|Vector|RotateVectorAroundAxis Direction (+ (* _index_2 _returnvalue_2) (+ _returnvalue_2 (* _returnvalue_2 (Math|Float|SelectFloat 0.0 0.5 (== (Math|Integer|%(Integer) _index 2) 0))))) "0.000000,0.000000,1.000000") 1e+02) Spawn%20Transform%20Location))) (+ (.Z (Math|Vector|BreakVector (+ (* (Math|Vector|RotateVectorAroundAxis Direction (+ (* _index_2 _returnvalue_2) (+ _returnvalue_2 (* _returnvalue_2 (Math|Float|SelectFloat 0.0 0.5 (== (Math|Integer|%(Integer) _index 2) 0))))) "0.000000,0.000000,1.000000") 1e+02) Spawn%20Transform%20Location))) (* _index 1e+02))) (Math|Vector|MakeVector (.X (Math|Vector|BreakVector (Math|Vector|RotateVectorAroundAxis Direction (+ (* _index_2 _returnvalue_2) (+ _returnvalue_2 (* _returnvalue_2 (Math|Float|SelectFloat 0.0 0.5 (== (Math|Integer|%(Integer) _index 2) 0))))) "0.000000,0.000000,1.000000"))) (.Y (Math|Vector|BreakVector (Math|Vector|RotateVectorAroundAxis Direction (+ (* _index_2 _returnvalue_2) (+ _returnvalue_2 (* _returnvalue_2 (Math|Float|SelectFloat 0.0 0.5 (== (Math|Integer|%(Integer) _index 2) 0))))) "0.000000,0.000000,1.000000"))) 0.0) Speed Damage false 0.0 "0, 0, 0" 0.0 "NewEnumerator1" "1.500000,1.500000,1.500000" self false 0.0 0.0)))))))

(event Custom|ShotgunExplosion
  (params (NbBullet :type Integer) (Spawn%20Transform%20Location :type Vector) (Direction :type Vector) (Speed :type Float%20%28double-precision%29) (Damage :type Float%20%28double-precision%29) (Delay%20Each%20Loop :type Float%20%28double-precision%29) (Pre-Visualisation :type Boolean) (Projectile%20Scale :type Float%20%28double-precision%29) (Dispertion%20Speed :type Float%20%28double-precision%29))
  (bind _returnvalue (Math|Conversions|ToVector(Float) Projectile%20Scale))
  (bind _returnvalue_2 (Math|Random|RandomUnitVectorinConeinDegrees Direction 3.6e+02))
  ;[1 1 1] Shotgun
  (Utilities|ForLoopDelayed 0 (- NbBullet 1) 0.0
    (:Loop%20Body
      (if Pre-Visualisation
        (Game|SpawnActorfromClass "/Game/NIRVANA/Core/Characters/Enemies/Common/BP_EnemyProjectileApparition.BP_EnemyProjectileApparition_C" (Math|Transform|MakeTransform Spawn%20Transform%20Location "0, 0, 0" _returnvalue) "AlwaysSpawn" "MultiplyWithRoot" 0 0.5 Spawn%20Transform%20Location _returnvalue_2 Speed Damage false 0.2 "0.000000,0.000000,0.000000" 0.0 (Variables|Default|GetRef%20Bullet%20Manager) self "NewEnumerator1" 0)
        (else
          (Default|ActivateBullet (Variables|Default|GetRef%20Bullet%20Manager) Spawn%20Transform%20Location _returnvalue_2 Speed Damage false 0.0 "0, 0, 0" 0.0 "NewEnumerator1" _returnvalue self false 0.0 0.0))))))

(event Custom|Shotgun
  (params (NbBullet :type Integer) (Spawn%20Transform%20Location :type Vector) (Direction :type Vector) (Speed :type Float%20%28double-precision%29) (Damage :type Float%20%28double-precision%29) (Delay%20Each%20Loop :type Float%20%28double-precision%29) (Pre-Visualisation :type Boolean) (Projectile%20Scale :type Float%20%28double-precision%29) (Dispertion%20Speed :type Float%20%28double-precision%29))
  (bind _returnvalue (Math|Conversions|ToVector(Float) Projectile%20Scale))
  (bind _returnvalue_2 (Math|Random|RandomUnitVectorinConeinDegrees Direction 2e+01))
  ;[1 1 1] Shotgun
  (Utilities|ForLoopDelayed 0 2 0.2
    (:Loop%20Body
      (Utilities|ForLoopDelayed 0 (- NbBullet 1) 0.0
        (:Loop%20Body
          (if Pre-Visualisation
            (Game|SpawnActorfromClass "/Game/NIRVANA/Core/Characters/Enemies/Common/BP_EnemyProjectileApparition.BP_EnemyProjectileApparition_C" (Math|Transform|MakeTransform Spawn%20Transform%20Location "0, 0, 0" _returnvalue) "AlwaysSpawn" "MultiplyWithRoot" 0 0.5 Spawn%20Transform%20Location _returnvalue_2 Speed Damage false 0.2 "0.000000,0.000000,0.000000" 0.0 (Variables|Default|GetRef%20Bullet%20Manager) self "NewEnumerator1" 0)
            (else
              (Default|ActivateBullet (Variables|Default|GetRef%20Bullet%20Manager) Spawn%20Transform%20Location _returnvalue_2 Speed Damage false 0.0 "0, 0, 0" 0.0 "NewEnumerator1" _returnvalue self false 0.0 0.0))))))))

(fn ConstructionScript
  (|CallParentFunction))

(fn SpawnPattern
  (params (Pattern :type Enum_Pattern%20Enum :default "NewEnumerator1") (NbBullet :type Integer) (Spawn%20Transform%20Location :type Vector) (Direction :type Vector) (Speed :type Float%20%28double-precision%29) (Damage :type Float%20%28double-precision%29) (Delay%20Each%20Loop :type Float%20%28double-precision%29) (Pre-Visualisation :type Boolean) (Projectile%20Scale :type Float%20%28double-precision%29) (Dispertion :type Boolean) (Dispertion%20Speed :type Float%20%28double-precision%29) (Nb%20Bullet%20Secondaire%20%28%20Rectangle%20%29 :type Integer))
  (switch Utilities|FlowControl|Switch|SwitchonEnum_Pattern Pattern
    (:NewEnumerator1
      (CallFunction|SimplePattern NbBullet Spawn%20Transform%20Location Direction Speed Damage Delay%20Each%20Loop Pre-Visualisation Projectile%20Scale))
    (:NewEnumerator9
      (CallFunction|CircleExplosion NbBullet Spawn%20Transform%20Location Direction Speed Damage Delay%20Each%20Loop Pre-Visualisation Projectile%20Scale Dispertion%20Speed))
    (:NewEnumerator13
      (CallFunction|Rectangle NbBullet Spawn%20Transform%20Location Direction Speed Damage Delay%20Each%20Loop Pre-Visualisation Projectile%20Scale Dispertion%20Speed Nb%20Bullet%20Secondaire%20%28%20Rectangle%20%29 Dispertion))
    (:NewEnumerator16
      (CallFunction|HorizontalRound NbBullet Spawn%20Transform%20Location Direction Speed Damage Delay%20Each%20Loop Pre-Visualisation Projectile%20Scale Dispertion%20Speed))
    (:NewEnumerator21
      (CallFunction|Shotgun NbBullet Spawn%20Transform%20Location Direction Speed Damage Delay%20Each%20Loop Pre-Visualisation Projectile%20Scale Dispertion%20Speed))
    (:NewEnumerator22
      (CallFunction|ShotgunExplosion NbBullet Spawn%20Transform%20Location Direction Speed Damage Delay%20Each%20Loop Pre-Visualisation Projectile%20Scale Dispertion%20Speed))
    (:NewEnumerator23
      (CallFunction|GrossBoule NbBullet Spawn%20Transform%20Location Direction Speed Damage Delay%20Each%20Loop Pre-Visualisation Projectile%20Scale))
    (:NewEnumerator24
      (CallFunction|PluieDeComete))
    (:NewEnumerator25
      (CallFunction|HorizontalRoundMitrallette NbBullet Spawn%20Transform%20Location Direction Speed Damage Delay%20Each%20Loop Pre-Visualisation Projectile%20Scale Dispertion%20Speed))))

(fn GetBestItem
  (params (EQS :type Env%20Query%20Instance%20Blueprint%20Wrapper%20Object%20Reference))
  (bind _output_get (LocalVariables|SetToSort EQS))
  (bind (_resultlocations _returnvalue) (AI|EQS|GetQueryResultsasLocations _output_get))
  (if _returnvalue
    (bind _output_get_2 (LocalVariables|SetPoints _resultlocations))
    (for (_ _array_index) _output_get_2
      (if (< (LocalVariables|GetBest) (Class|EnvQueryInstanceBlueprintWrapper|GetItemScore (LocalVariables|GetToSort) _array_index))
        (LocalVariables|SetBestIndex _array_index)
        (LocalVariables|SetBest (Class|EnvQueryInstanceBlueprintWrapper|GetItemScore (LocalVariables|GetToSort) _array_index))))
    (if (== (LocalVariables|GetBest) 0.0)
      (return "0, 0, 0" false)
      (else
        (return (Utilities|Array|Get(acopy) (LocalVariables|GetPoints) (LocalVariables|GetBestIndex)) true)))
    (else
      (return "0, 0, 0" false))))

(fn GetPatternIndex
  (params (Row :type Integer))
  (return 0))

(fn EnablePattern
  (params (PatternIndex :type Integer))
  (bind _structpattern (Variables|Default|GetStructPattern))
  (bind _output (Utilities|Array|Get(acopy) _structpattern PatternIndex))
  (bind (_pattern _nbbulletloop _delayeachloop _projectilespeed _damage _dispertion _dispertionspeed _previsualisation _nbbulletrectangle _zoffsettransformlocation _directionbyoffset _disabled _delay) (Utilities|Struct|BreakStruct_PatternValue _output))
  (if (>= PatternIndex (Utilities|Array|Length _structpattern))
    (return false)
    (else
      (Utilities|Array|SetArrayElem _structpattern PatternIndex (Utilities|Struct|MakeStruct_PatternValue _pattern _nbbulletloop _delayeachloop _projectilespeed _damage _dispertion _dispertionspeed _previsualisation _nbbulletrectangle _zoffsettransformlocation _directionbyoffset false _delay))
      (return true))))
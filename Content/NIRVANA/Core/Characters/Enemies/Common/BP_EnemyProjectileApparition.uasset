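; BP_EnemyProjectileApparition is the appearance effect that precedes an enemy projectile, delaying the shot until its Niagara ball effect finishes.
; The construction script sets the effect's loop duration from the game instance's projectile apparition time.
; When the system finishes, it spawns BP_EnemieProjectile at the actor's scale, passing on direction, speed, damage and optional delayed direction-change settings, then destroys itself.
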(event `self.N_ApparitionBall.OnSystemFinished`
  (params (PSystem :type "NiagaraComponent Object Reference"))
  (`|SpawnActorFromClass` "/Game/NIRVANA/Core/Characters/Enemies/Common/BP_EnemieProjectile.BP_EnemieProjectile_C" (`KismetMathLibrary.MakeTransform` (`self.Spawn Transform Location`) (struct) (`self.GetActorScale3D`)) "AlwaysSpawn" "MultiplyWithRoot" null (`self.Direction`) (`self.Speed`) (`self.Damage`) (`self.Need Change Direction`) (`self.Delay Change DIrection`) (`self.New Direction`) (`self.New Speed`) null)
  (`self.K2_DestroyActor`))

(fn `UserConstructionScript`
  (bind (_projectilevariables_size _projectilevariables_speed _projectilevariables_apparitiontime) (break `/Game/DevelopersContent/Core/Placeables/Struct_ProjectileTool` (`/Game/NIRVANA/Core/GameModes/Game_Instance.ProjectileVariables` (cast `/Game/NIRVANA/Core/GameModes/Game_Instance` (`GameplayStatics.GetGameInstance`) :!pure true))))
  (`NiagaraComponent.SetVariableFloat` (`self.N_ApparitionBall`) "Loop Duration" _projectilevariables_apparitiontime))
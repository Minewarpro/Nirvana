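; Pooled enemy projectile that damages the player on overlap and deactivates on any overlap, hit or lifetime timeout.
; Activate repositions and scales it, picks a speed-based material from BP_BulletManager, then launches it through physics velocity.
; An optional delayed redirect can run Mini Spiral or Ceiling Spiral timelines that modulate speed along the new direction.
; Deactivation hides it, disables physics and collision, and returns it to the manager's BulletPull.
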(event `Change Velocity`
  (`PrimitiveComponent.SetPhysicsLinearVelocity` (`self.Collision`) (* (`self.New Direction`) (`self.New Speed`)) false "None"))

(event `self.ReceiveBeginPlay`
  (bind _returnvalue (`GameplayStatics.GetActorOfClass` "/Game/NIRVANA/Core/Characters/Enemies/Range/BP_BulletManager.BP_BulletManager_C"))
  (set `self.Ref Bullet Manager` _returnvalue))

(event `Activate`
  (params (`Spawn Location` :type "Vector Structure") (Direction :type "Vector Structure") (Speed :type "Float (single-precision)") (Damage :type "Float (double-precision)") (`Need Change Direction` :type Boolean) (`Delay Change DIrection` :type "Float (single-precision)") (`New Direction` :type "Vector Structure") (`New Speed` :type "Float (double-precision)") (`Special Effect` :type "/Game/NIRVANA/Core/Characters/Enemies/Common/Enum_SpecialEffectBullet Enum" :default "NewEnumerator1") (Scale :type "Vector Structure") (EnemieRef :type "/Game/NIRVANA/Core/Characters/Enemies/Common/BP_Enemy Object Reference"))
  (bind _collision (`self.Collision`))
  (`self.Set Values` `Spawn Location` Direction Speed Damage `Need Change Direction` `Delay Change DIrection` `New Direction` `New Speed` `Special Effect` Scale EnemieRef)
  (`KismetSystemLibrary.K2_SetTimerDelegate` (delegate `Desactivate`) (`self.Life Time`))
  (`self.SetActorHiddenInGame` false)
  (`PrimitiveComponent.SetSimulatePhysics` _collision true)
  (`PrimitiveComponent.SetCollisionEnabled` _collision "QueryAndPhysics")
  (`PrimitiveComponent.SetPhysicsLinearVelocity` (`self.Collision`) (* (`self.Direction`) (`self.Speed`)) false "None")
  (`|ExecutionSequence`
    (:`then_0`
      (bind _asbp_first_person_character (cast `/Game/NIRVANA/Core/Characters/FirstPerson/BP_FirstPersonCharacter` (`GameplayStatics.GetPlayerCharacter` 0)))
      (set `self.Player Ref` _asbp_first_person_character))
    (:`then_1`
      (if (`self.Need Change Direction`)
        (`KismetSystemLibrary.Delay` (`self.Delay Change DIrection`))
        (`self.Change Velocity`)
        (switch `/Game/NIRVANA/Core/Characters/Enemies/Common/Enum_SpecialEffectBullet` (`self.Special Effect`)
          (:`NewEnumerator0`
            (`self.Mini Spiral Effect`))
          (:`NewEnumerator2`
            (`self.Ceiling Spiral`)))))))

(event `Desactivate`
  (bind _collision (`self.Collision`))
  (if (not (`self.bHidden`))
    (`self.SetActorHiddenInGame` true)
    (`PrimitiveComponent.SetPhysicsLinearVelocity` (`self.Collision`) (0.0 0.0 0.0) false "None")
    (`PrimitiveComponent.SetSimulatePhysics` _collision false)
    (`PrimitiveComponent.SetCollisionEnabled` _collision "NoCollision")
    (`KismetArrayLibrary.Array_Add` (`/Game/NIRVANA/Core/Characters/Enemies/Range/BP_BulletManager.BulletPull` (`self.Ref Bullet Manager`)) self)))

(event `self.Collision.OnComponentBeginOverlap`
  (params (OverlappedComponent :type "PrimitiveComponent Object Reference") (OtherActor :type "Actor Object Reference") (OtherComp :type "PrimitiveComponent Object Reference") (OtherBodyIndex :type Integer) (bFromSweep :type Boolean) (SweepResult :type "HitResult Structure (by ref)"))
  (if (== OtherActor (`self.Player Ref`))
    (`/Game/NIRVANA/Core/Characters/FirstPerson/BP_FirstPersonCharacter.Take Damage` (`self.Player Ref`) (`self.Damage`) self)
    (`self.Desactivate`)
    (else
      (cast `/Game/NIRVANA/Core/Characters/Enemies/Common/BP_Enemy` OtherActor
        (:`then`
          _)
        (:`CastFailed`
          _))
      (`self.Desactivate`))))

(event `self.Collision.OnComponentHit`
  (params (HitComponent :type "PrimitiveComponent Object Reference") (OtherActor :type "Actor Object Reference") (OtherComp :type "PrimitiveComponent Object Reference") (NormalImpulse :type "Vector Structure") (Hit :type "HitResult Structure (by ref)"))
  (`self.Desactivate`))

(event `Mini Spiral Effect`
  (`TimelineComponent.SetPlayRate` (`self.Mini Spiral Speed Effect`) (/ 1.0 0.4))
  (bind (_direction _speed) (`Timeline|Mini Spiral Speed Effect`)
    (:`Update`
      (`PrimitiveComponent.SetPhysicsLinearVelocity` (`self.Collision`) (* (`self.New Direction`) (* _speed (`self.New Speed`))) false "None"))))

(event `Ceiling Spiral`
  (`TimelineComponent.SetPlayRate` (`self.Ceiling Spiral TL`) (/ 1.0 7.0))
  (bind (_direction _speed) (`Timeline|Ceiling Spiral TL`)
    (:`Update`
      (`PrimitiveComponent.SetPhysicsLinearVelocity` (`self.Collision`) (* (`self.New Direction`) (* _speed (`self.New Speed`))) false "None"))))

(fn `Set Values`
  (params (SpawnLocation :type "Vector Structure") (Direction :type "Vector Structure") (Speed :type "Float (single-precision)") (Damage :type "Float (double-precision)") (`Need Change Direction` :type Boolean) (`Delay Change DIrection` :type "Float (single-precision)") (`New Direction` :type "Vector Structure") (`New Speed` :type "Float (double-precision)") (`Special Effect` :type "/Game/NIRVANA/Core/Characters/Enemies/Common/Enum_SpecialEffectBullet Enum" :default "NewEnumerator1") (Scale :type "Vector Structure") (EnemieRef :type "/Game/NIRVANA/Core/Characters/Enemies/Common/BP_Enemy Object Reference"))
  (bind _speed (`local.Speed`))
  (`self.K2_SetActorLocation` SpawnLocation false true)
  (`self.SetActorScale3D` Scale)
  (set `self.Direction` Direction)
  (set `self.Speed` Speed)
  (set `self.Damage` Damage)
  (set `self.Need Change Direction` `Need Change Direction`)
  (set `self.Delay Change DIrection` `Delay Change DIrection`)
  (set `self.New Direction` `New Direction`)
  (set `self.New Speed` `New Speed`)
  (set `self.Special Effect` `Special Effect`)
  (set `self.EnemieRef` EnemieRef)
  (if (< _speed 1000.0)
    (`PrimitiveComponent.SetMaterial` (`self.Sphere`) 0 (`/Game/NIRVANA/Core/Characters/Enemies/Range/BP_BulletManager.MaterialBullet=500` (`self.Ref Bullet Manager`)))
    (elif (< _speed 2000.0)
      (`PrimitiveComponent.SetMaterial` (`self.Sphere`) 0 (`/Game/NIRVANA/Core/Characters/Enemies/Range/BP_BulletManager.MaterialBullet=1000` (`self.Ref Bullet Manager`)))
      (else
        (`PrimitiveComponent.SetMaterial` (`self.Sphere`) 0 (`/Game/NIRVANA/Core/Characters/Enemies/Range/BP_BulletManager.MaterialBullet=2000` (`self.Ref Bullet Manager`)))))))

(fn `Start Special Effect`
  (switch `/Game/NIRVANA/Core/Characters/Enemies/Common/Enum_SpecialEffectBullet` (`self.Special Effect`)
    (:`NewEnumerator0`
      (`self.Mini Spiral Effect`))))

(fn `UserConstructionScript`)
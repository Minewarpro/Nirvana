(event `self.ReceiveBeginPlay`
  ;[1 0.6941 0.1255 1 34] Begin Play
  (bind _asbp_first_person_character (cast `/Game/NIRVANA/Core/Characters/FirstPerson/BP_FirstPersonCharacter` (`GameplayStatics.GetPlayerCharacter` 0)))
  (bind _output_get (set `self.PlayerRef` _asbp_first_person_character))
  (bind _output_get_2 (set `self.BlackBoard` (`AIBlueprintHelperLibrary.GetBlackboard` (`AIBlueprintHelperLibrary.GetAIController` self))))
  (`BlackboardComponent.SetValueAsObject` _output_get_2 "PlayerRef" _output_get)
  (set `self.CurrentHealth` (`self.MaxHealth`))
  (set `PrimitiveComponent.bGenerateOverlapEvents` false (`self.Weapon`))
  (`AIController.K2_SetFocus` (`AIBlueprintHelperLibrary.GetAIController` self) (`self.PlayerRef`))
  (set `self.Temp Max Walk Speed` (`CharacterMovementComponent.MaxWalkSpeed` (`self.CharacterMovement`)))
  (`PhysicalAnimationComponent.SetSkeletalMeshComponent` (`self.PhysicalAnimation`) (`self.Mesh`))
  (`PhysicalAnimationComponent.ApplyPhysicalAnimationSettingsBelow` (`self.PhysicalAnimation`) "Spine1" (make `PhysicalAnimationData` true 750.0 50.0 250.0 100.0) true)
  (`SkeletalMeshComponent.SetAllBodiesBelowSimulatePhysics` (`self.Mesh`) "Spine1" true true)
  (`SkeletalMeshComponent.SetAllBodiesBelowPhysicsBlendWeight` (`self.Mesh`) "Spine1" 0.0 false true))

(event `Cross hair hit alpha decrease`
  ;[0.6667 0.6667 0.6667] Cross Widget
  (set `/Game/NIRVANA/Core/Characters/FirstPerson/BP_FirstPersonCharacter.Crosshair Hit Alpha` 1.0 (`self.PlayerRef`))
  (bind (_direction _alpha) (`Timeline|Timeline_0` :!via `PlayFromStart`)
    (:`Update`
      (set `/Game/NIRVANA/Core/Characters/FirstPerson/BP_FirstPersonCharacter.Crosshair Hit Alpha` _alpha (`self.PlayerRef`)))))

(event `self.Weapon.OnComponentBeginOverlap`
  (params (OverlappedComponent :type "PrimitiveComponent Object Reference") (OtherActor :type "Actor Object Reference") (OtherComp :type "PrimitiveComponent Object Reference") (OtherBodyIndex :type Integer) (bFromSweep :type Boolean) (SweepResult :type "HitResult Structure (by ref)"))
  ;[1 1 1] Hit Player (cut)
  (bind _asbp_first_person_character (cast `/Game/NIRVANA/Core/Characters/FirstPerson/BP_FirstPersonCharacter` OtherActor))
  (`/Game/NIRVANA/Core/Characters/FirstPerson/BP_FirstPersonCharacter.Take Damage` _asbp_first_person_character 31.0 null))

(event `Death`
  (params (`Anim Index` :type Integer))
  ;[0.0226 0.0399 0.08854] Death
  (`NiagaraFunctionLibrary.SpawnSystemAtLocation` "/Game/DevelopersContent/Core/Characters/Enemies/Common/Effects/NS_KillBlood.NS_KillBlood" (`self.K2_GetActorLocation`))
  (`self.SpawnHealth`)
  (`GameplayStatics.PlaySoundAtLocation` (`self.Sound`) (`self.K2_GetActorLocation`) (struct) 1.0 1.0 0.0 null null null null)
  (`/Game/NIRVANA/Core/Placeables/Management/BP_ArenaManager.CheckNewWave` (`self.ArenaManager`) 0.1)
  (`self.K2_DestroyActor`))

(event `/Game/NIRVANA/Core/Characters/FirstPerson/BPI_Hit.Hit`
  (params (Damages :type "Float (double-precision)") (Impulse :type "Vector Structure") (Location :type "Vector Structure") (Bone :type Name))
  ;[1 0.3765 0.3765] Hit
  (`self.Cross hair hit alpha decrease `)
  (`GameplayStatics.PlaySound2D` "/Game/NIRVANA/Core/Characters/FirstPerson/Hit.Hit" 1.0 1.0 0.0 null null)
  (set `self.CurrentHealth` (- (`self.CurrentHealth`) Damages))
  (`SkeletalMeshComponent.SetAllBodiesBelowPhysicsBlendWeight` (`self.Mesh`) Bone 1.0 false true)
  (`|ExecutionSequence`
    (:`then_0`
      (`TimelineComponent.SetPlayRate` (`self.TStagger`) (/ 1.0 0.35))
      (bind (_direction _newtrack_0) (`Timeline|TStagger` :!via `PlayFromStart`)
        (:`Update`
          (`SkeletalMeshComponent.SetAllBodiesBelowPhysicsBlendWeight` (`self.Mesh`) Bone _newtrack_0 false true))))
    (:`then_1`
      (if (<= (`self.CurrentHealth`) 0.0)
        (`self.Death` 2)
        (else
          (`self.SetLifeBar`)
          (`MeshComponent.SetScalarParameterValueOnMaterials` (`self.Mesh`) "Hit" 0.1)
          (`KismetSystemLibrary.Delay` 0.2)
          (`MeshComponent.SetScalarParameterValueOnMaterials` (`self.Mesh`) "Hit" 0.0))))))

(event `/Game/NIRVANA/Core/Characters/Enemies/Common/BPI_EnemyAI.JumpToDestination`
  (params (Destination :type "Vector Structure"))
  ;[0.2282 0.8281 0.1553] NavLink Jump
  (if (`|EnumInequality` (`self.CurrentState`) "NewEnumerator4")
    (set `self.CurrentState` "NewEnumerator4")
    (bind _notifyname (`|PlayMontage` (`self.Mesh`) "/Game/DevelopersContent/Core/Characters/Enemies/Common/Mixamo_Test/Anim/AM_Jumping_Start.AM_Jumping_Start")
      (:`OnNotifyBegin`
        (if (== _notifyname "JumpStart")
          (bind _outlaunchvelocity (`GameplayStatics.SuggestProjectileVelocity_CustomArc` (`self.K2_GetActorLocation`) (+ Destination (0.0 0.0 160.0)) (`MovementComponent.GetGravityZ` (`self.CharacterMovement`)) 0.3))
          (`self.LaunchCharacter` _outlaunchvelocity true true))))))

(event `self.OnLanded`
  (params (Hit :type "HitResult Structure (by ref)"))
  ;[0.2282 0.8281 0.1553] NavLink Jump
  (bind _notifyname (`|PlayMontage` (`self.Mesh`) "/Game/DevelopersContent/Core/Characters/Enemies/Common/Mixamo_Test/Anim/AM_Falling_To_Landing.AM_Falling_To_Landing" 1.0 0.23)
    (:`OnNotifyBegin`
      (if (== _notifyname "CanWalk")
        (set `self.CurrentState` "NewEnumerator0")))))

(fn `IsOnScreen`
  (params (angle :type "Float (double-precision)" :default 45.0))
  (returns (Value :type Boolean))
  (bind _playerref (`self.PlayerRef`)
    (:`then`
      (bind (_returnvalue_x _returnvalue_y) (`KismetMathLibrary.BreakVector` (`self.GetActorForwardVector` _playerref)))
      (bind (_returnvalue_x_2 _returnvalue_y_2) (`KismetMathLibrary.BreakVector` (- (`self.K2_GetActorLocation`) (`self.K2_GetActorLocation` _playerref))))
      (if (> (`local.angle`) (`KismetMathLibrary.Lerp` 180.0 0.0 (`KismetMathLibrary.Dot_VectorVector` (`KismetMathLibrary.MakeVector` _returnvalue_x _returnvalue_y) (`KismetMathLibrary.Normal` (`KismetMathLibrary.MakeVector` _returnvalue_x_2 _returnvalue_y_2)))))
        (bind (_outhit _returnvalue) (`KismetSystemLibrary.LineTraceSingle` (`self.K2_GetActorLocation` (`self.PlayerRef`)) (`self.K2_GetActorLocation`) "TraceTypeQuery1"))
        (return (not _returnvalue))
        (else
          (return false))))
    (:`else`
      (return false))))

(fn `JumpVelocity`
  (params (startingPoint :type "Vector Structure") (ladingPoint :type "Vector Structure") (JumpDuration :type "Float (double-precision)"))
  (returns (Velocity :type "Vector Structure"))
  (locals (duration :type "Float (double-precision)"))
  (bind _duration (`local.duration`))
  (set `local.duration` JumpDuration)
  (return (`KismetMathLibrary.MakeVector` (/ (- (.x ladingPoint) (.x startingPoint)) _duration) (/ (- (.y ladingPoint) (.y startingPoint)) _duration) (/ (- (.z ladingPoint) (+ (.z startingPoint) (* (`KismetMathLibrary.Square` (`local.duration`)) -0.5 982.0 1.0))) _duration))))

(fn `SetLifeBar`
  (bind _aswb_enemy_life_bar (cast `/Game/DevelopersContent/Core/Characters/Enemies/Common/WB_EnemyLifeBar` (`WidgetComponent.GetWidget` (`self.WidgetLifeBar`))))
  (`/Game/DevelopersContent/Core/Characters/Enemies/Common/WB_EnemyLifeBar.SetProgressBar` _aswb_enemy_life_bar (`KismetMathLibrary.FClamp` (/ (`self.CurrentHealth`) (`self.MaxHealth`))))
  (return))

(fn `Spawn Munition`
  (locals (`Chance to spawn` :type Integer :default 80))
  (bind _playerref (`self.PlayerRef`))
  (for _array_element (`/Game/NIRVANA/Core/Characters/FirstPerson/BP_FirstPersonCharacter.MyWeapons` _playerref)
    (bind _returnvalue (`|EnumEquality` _array_element "NewEnumerator7"))
    (set `local.Chance to spawn` (select `bool` _returnvalue :`false` (select `bool` (`|EnumEquality` _array_element (`/Game/NIRVANA/Core/Characters/FirstPerson/BP_FirstPersonCharacter.Current Weapon` _playerref)) :`false` 80 :`true` 35) :`true` 12))
    (for _ (range (+ (select `bool` _returnvalue :`false` (`KismetMathLibrary.RandomIntegerInRange` 0 2)) 1))
      (if (< (`KismetMathLibrary.RandomIntegerInRange` 1 100) (`local.Chance to spawn`))
        (`|SpawnActorFromClass` "/Game/NIRVANA/Core/Weapons/Common/BP_Munition.BP_Munition_C" (`KismetMathLibrary.MakeTransform` (`self.K2_GetActorLocation`)) "AlwaysSpawn" "MultiplyWithRoot" null _array_element null)))))

(fn `SpawnHealth`
  (bind (_returnvalue_x _returnvalue_y _returnvalue_z) (`KismetMathLibrary.BreakVector` (`self.K2_GetActorLocation`)))
  (bind _playerref (`self.PlayerRef`))
  (if (not (== (`/Game/NIRVANA/Core/Characters/FirstPerson/BP_FirstPersonCharacter.Current Health` _playerref) (`/Game/NIRVANA/Core/Characters/FirstPerson/BP_FirstPersonCharacter.MaxHealth` _playerref)))
    (if (< (`KismetMathLibrary.RandomFloat`) 1.0)
      (`|SpawnActorFromClass` "/Game/NIRVANA/Core/Loots/Health/BP_Health.BP_Health_C" (`KismetMathLibrary.MakeTransform` (`KismetMathLibrary.MakeVector` _returnvalue_x _returnvalue_y (+ _returnvalue_z 40.0))) "Undefined" "MultiplyWithRoot" null null))
    (return)))

(fn `UserConstructionScript`
  (bind _weapon (`self.Weapon`))
  ;[1 1 1] cut
  (bind _returnvalue (`AddComponent|NODE_AddBoxComponent-0` :`bManualAttachment` true))
  (set `self.Weapon` _returnvalue)
  (bind _enumvalue (foreach `ECollisionChannel` false)
    (:`LoopBody`
      (`PrimitiveComponent.SetCollisionResponseToChannel` _weapon _enumvalue "ECR_Ignore"))
    (:`then`
      (`PrimitiveComponent.SetCollisionResponseToChannel` _weapon "ECC_Pawn" "ECR_Overlap")
      (`SceneComponent.K2_AttachToComponent` (`self.Weapon`) (`self.Mesh`) "LeftHandSocket" "SnapToTarget" "SnapToTarget" "KeepRelative" true))))
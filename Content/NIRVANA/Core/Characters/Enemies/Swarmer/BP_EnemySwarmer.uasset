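; Melee Swarmer enemy that periodically focuses on a nearby player and attacks with standing or dashing slashes, its weapon overlap dealing damage.
; The dash is timeline-driven, bending toward the player through traced, navmesh-projected points and stopping when none is valid.
; Hits drive a physical-animation stagger above the spine.
; Death removes it from the ArenaManager, calls the manager's swarmer spawn check and dissolves the body before destroying it.
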(event `SetFocus`
  (bind _returnvalue (`AIBlueprintHelperLibrary.GetAIController` self))
  (if (<= (`KismetMathLibrary.Vector_Distance` (`self.K2_GetActorLocation` (`self.PlayerRef`)) (`self.K2_GetActorLocation`)) (`self.DistanceToFocus`))
    (`AIController.K2_SetFocus` _returnvalue (`self.PlayerRef`))
    (else
      (`AIController.K2_ClearFocus` _returnvalue))))

(event `self.ReceiveBeginPlay`
  ;[1 0.6945 0.125 1 34] Begin Play
  (`parent.ReceiveBeginPlay`)
  (`PhysicalAnimationComponent.SetSkeletalMeshComponent` (`self.PhysicalAnimation`) (`self.Mesh`))
  (`PhysicalAnimationComponent.ApplyPhysicalAnimationSettingsBelow` (`self.PhysicalAnimation`) "Bind_Spine_01" (make `PhysicalAnimationData` true 60.0 15.0 50.0 50.0) false)
  (`SkeletalMeshComponent.SetAllBodiesBelowSimulatePhysics` (`self.Mesh`) "Bind_Spine_01" true false)
  (`SkeletalMeshComponent.SetAllBodiesBelowPhysicsBlendWeight` (`self.Mesh`) "Bind_Spine_01" 0.0 false false)
  (bind _returnvalue (`KismetSystemLibrary.K2_SetTimerDelegate` (delegate `SetFocus`) 0.5 true))
  (set `self.EventHandler_Focus` _returnvalue))

(event `Slash`
  (bind _slashtargetposition (`self.SlashTargetPosition`))
  (bind _slashinitposition (`self.SlashInitPosition`))
  (bind _returnvalue (`self.K2_GetActorLocation` (`self.PlayerRef`)))
  (bind _returnvalue_2 (+ _returnvalue (* (`KismetMathLibrary.GetDirectionUnitVector` _returnvalue (`self.K2_GetActorLocation`)) 150.0)))
  (bind _returnvalue_3 (`KismetMathLibrary.Vector_Distance` _slashtargetposition _returnvalue_2))
  ;[0.75 0.2422 0.3822 1 34] Slash
  (`GameplayStatics.PlaySoundAtLocation` "/Game/NIRVANA/Core/Characters/Enemies/Swarmer/Sounds/MS_SwarmerAttack.MS_SwarmerAttack" _slashinitposition (struct) 1.0 1.0 0.0 null null null null)
  (`TimelineComponent.SetPlayRate` (`self.TL_Slash`) (/ (`self.SlashSpeed`) (`KismetMathLibrary.Vector_Distance` _slashinitposition (`self.SlashTargetPosition`))))
  (`ActorComponent.Activate` (`self.FXS_Shooting02`) false)
  (bind (_direction _newtrack_0) (`Timeline|TL_Slash` :!via `PlayFromStart` :!label _label)
    (:`Update`
      (bind _returnvalue_4 (`KismetMathLibrary.VLerp` (`self.SlashInitPosition`) (`KismetMathLibrary.VLerp` _slashtargetposition (`KismetMathLibrary.MakeVector` (.x _returnvalue_2) (.y _returnvalue_2) (.z _slashtargetposition)) (`KismetMathLibrary.SelectFloat` 0.0 (/ 400.0 (`KismetMathLibrary.FClamp` _returnvalue_3 400.0 579.0)) (>= _returnvalue_3 1420.0))) _newtrack_0))
      (bind (_outhit _returnvalue_5) (`KismetSystemLibrary.LineTraceSingle` (- _returnvalue_4 (0.0 0.0 45.0)) (+ _returnvalue_4 (0.0 0.0 -175.0)) "TraceTypeQuery1" true))
      (bind _projectedlocation (`NavigationSystemV1.K2_ProjectPointToNavigation` (`.Location` (`GameplayStatics.BreakHitResult` _outhit)) null "/Game/NIRVANA/Core/Characters/Enemies/Swarmer/NQF_Swarmer.NQF_Swarmer_C" (10.0 10.0 50.0)))
      (if (and _returnvalue_5 (`KismetMathLibrary.NotEqualExactly_VectorVector` _projectedlocation))
        (`self.K2_SetActorLocation` (+ _projectedlocation (0.0 0.0 120.0)) true)
        (else
          (`|ExecutionSequence`
            (:`then_0`
              (goto _label :!via `Stop`))
            (:`then_1`
              (`|PlayMontage` (`self.Mesh`) "/Game/NIRVANA/Core/Characters/Enemies/Swarmer/Anims/attack/AM_DashPunch.AM_DashPunch" 1.0 0.0 "Slash" :!label _label_2
                (:`then`
                  (`self.Reverse Sword Emissive`))
                (:`OnCompleted`
                  (set `self.CurrentState` "NewEnumerator0" :!label _label_3))
                (:`OnInterrupted`
                  (`self.Reverse Sword Emissive`)
                  (set `PrimitiveComponent.bGenerateOverlapEvents` false (`self.Weapon`))
                  (goto _label_3))))))))
    (:`Finished`
      (goto _label_2))))

(event `/Game/NIRVANA/Core/Characters/FirstPerson/BPI_Hit.Hit`
  (params (Damages :type "Float (double-precision)"))
  ;[1 0.3765 0.3765] Hit
  (`|ExecutionSequence`
    (:`then_0`
      (`SkeletalMeshComponent.SetAllBodiesBelowPhysicsBlendWeight` (`self.Mesh`) "Bind_Spine_01" 1.0 false false)
      (`TimelineComponent.SetPlayRate` (`self.TStagger`) (/ 1.0 0.35))
      (if (`self.Stagging`)
        (bind (_direction _newtrack_0) (`Timeline|TStagger` :!label _label_4)
          (:`Update`
            (set `self.Stagging` true)
            (`SkeletalMeshComponent.SetAllBodiesBelowPhysicsBlendWeight` (`self.Mesh`) "Bind_Spine_01" _newtrack_0 false false))
          (:`Finished`
            (`SkeletalMeshComponent.ResetAllBodiesSimulatePhysics` (`self.Mesh`))
            (`SkeletalMeshComponent.SetAllBodiesBelowPhysicsBlendWeight` (`self.Mesh`) "Bind_Spine_01" 0.0 false true)
            (set `self.Stagging` false)))
        (else
          (goto _label_4 :!via `PlayFromStart`))))
    (:`then_1`
      (`parent.Hit` Damages))))

(event `SlashBegin`
  ;[1 0.02387 0] CloseAttack
  ;;[1 1 1] Dash
  (set `self.CurrentState` "NewEnumerator3")
  (`|PlayMontage` (`self.Mesh`) "/Game/NIRVANA/Core/Characters/Enemies/Swarmer/Anims/attack/AM_DashPunch.AM_DashPunch"
    (:`then`
      (`ActorComponent.Activate` (`self.NS_ChargeSwarmer`) true)
      (bind (_direction _alpha) (`Timeline|Sword Amissive Alpha` :!via `PlayFromStart` :!label _label_5)
        (:`Update`
          (`MeshComponent.SetScalarParameterValueOnMaterials` (`self.Mesh`) "Alpha Sword" _alpha))))))

(event `SlashInPlace`
  ;[1 0.02387 0] CloseAttack
  (set `self.CurrentState` "NewEnumerator3")
  (`|PlayMontage` (`self.Mesh`) "/Game/NIRVANA/Core/Characters/Enemies/Swarmer/Anims/attack/AM_StandingPunch1.AM_StandingPunch1"
    (:`OnCompleted`
      _)
    (:`OnInterrupted`
      _))
  (set `self.CurrentState` "NewEnumerator0"))

(event `Reverse Sword Emissive`
  ;[1 0.02387 0] CloseAttack
  ;;[1 1 1] Dash
  (goto _label_5 :!via `Reverse`))

(event `self.Weapon.OnComponentBeginOverlap`
  (params (OverlappedComponent :type "PrimitiveComponent Object Reference") (OtherActor :type "Actor Object Reference") (OtherComp :type "PrimitiveComponent Object Reference") (OtherBodyIndex :type Integer) (bFromSweep :type Boolean) (SweepResult :type "HitResult Structure (by ref)"))
  ;[1 1 1] Cut Overlap
  (bind _asbp_first_person_character (cast `/Game/NIRVANA/Core/Characters/FirstPerson/BP_FirstPersonCharacter` OtherActor))
  (`/Game/NIRVANA/Core/Characters/FirstPerson/BP_FirstPersonCharacter.Take Damage` _asbp_first_person_character 15.0 null))

(event `Dissolve`
  ;[1 1 1] Dissolve Effect
  (`TimelineComponent.SetPlayRate` (`self.Dissolve TL`) (/ 1.0 1.6))
  (`ActorComponent.Activate` (`self.NS_EnemiesDeath`) true)
  (bind (_direction _alpha_dissolve) (`Timeline|Dissolve TL`)
    (:`Update`
      (`MeshComponent.SetScalarParameterValueOnMaterials` (`self.Mesh`) "Alpha" _alpha_dissolve)
      (`NiagaraComponent.SetVariableFloat` (`self.NS_Dissolve`) "Alpha" _alpha_dissolve))
    (:`Finished`
      (`KismetSystemLibrary.Delay` 1.0)
      (`self.K2_DestroyActor`))))

(event `self.Death`
  (bind _mesh (`self.Mesh`))
  ;[0.0226 0.0399 0.08854] Death
  (`/Engine/EditorBlueprintResources/StandardMacros.DoOnce` false
    (:`Completed`
      (`KismetArrayLibrary.Array_RemoveItem` (`/Game/NIRVANA/Core/Placeables/Management/BP_ArenaManager.Total EnemiesSwarmer` (`self.ArenaManager`)) self)
      (`KismetSystemLibrary.K2_ClearAndInvalidateTimerHandle` (`self.EventHandler_Focus`))
      (`ActorComponent.K2_DestroyComponent` (`self.WidgetLifeBar`))
      (`PrimitiveComponent.SetCollisionResponseToChannel` _mesh "ECC_GameTraceChannel3" "ECR_Ignore")
      (`PrimitiveComponent.SetCollisionResponseToChannel` (`self.CapsuleComponent`) "ECC_GameTraceChannel3" "ECR_Ignore")
      (`PrimitiveComponent.SetCollisionResponseToChannel` _mesh "ECC_GameTraceChannel5" "ECR_Ignore")
      (`PrimitiveComponent.SetCollisionResponseToChannel` (`self.CapsuleComponent`) "ECC_Pawn" "ECR_Ignore")
      (`PrimitiveComponent.SetCollisionResponseToChannel` _mesh "ECC_Pawn" "ECR_Ignore")
      (`self.DetachFromControllerPendingDestroy` self)
      (`|PlayMontage` (`self.Mesh`) "/Game/NIRVANA/Core/Characters/Enemies/Swarmer/Anims/other/AM_Death.AM_Death" 0.3 0.5
        (:`then`
          (`self.Dissolve`)
          (`/Game/NIRVANA/Core/Placeables/Management/BP_ArenaManager.TestingSwarmerSpawn` (`self.ArenaManager`))
          (`parent.Death`))))))

(fn `UserConstructionScript`
  (bind _charactermovement (`self.CharacterMovement`))
  (`parent.UserConstructionScript`)
  (set `CharacterMovementComponent.MaxWalkSpeed` (`self.Max Walk Speed`) _charactermovement)
  (set `CharacterMovementComponent.MaxAcceleration` (`self.Max Acceleration`) _charactermovement))
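; Phase 2 boss enemy Blueprint that extends a parent's shooting and hit logic with randomized attack patterns and damage-triggered repositioning.
; Shoot picks a random pattern, or the first during the special state, retries on a timer if disabled, and restores its Token after the pattern's delay.
; Each time accumulated damage reaches a fifth of max health, it enters that state, snaps to its spawn location and plays the shoot montage before reverting.
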(event `self.ReceiveBeginPlay`
  ;[1 0.6941 0.1255 1 34] Begin
  (`parent.ReceiveBeginPlay`)
  (set `self.Token` true)
  (bind _output_get (set `self.DistantRange` 3000.0))
  (`BlackboardComponent.SetValueAsFloat` (`self.BlackBoard`) "Range" _output_get)
  (set `self.InitPos` (`self.K2_GetActorLocation`)))

(event `self.Shoot`
  ;[1 1 1] Shoot
  (bind _output_get (set `self.PatternIndex` (`KismetMathLibrary.SelectInt` 0 (`self.GetPatternIndex` 0) (`|EnumEquality` (`self.CurrentState`) "NewEnumerator7"))))
  (bind (_output_pattern _output_nbbulletloop _output_delayeachloop _output_projectilespeed _output_damage _output_dispertion _output_dispertionspeed _output_previsualisation _output_nbbulletrectangle _output_zoffsettransformlocation _output_directionbyoffset _output_disabled _output_delay) (break `/Game/NIRVANA/Core/Characters/Enemies/Common/Struct_PatternValue` (`|GetArrayItem` (`self.StructPattern`) _output_get)))
  (if _output_disabled
    (`KismetSystemLibrary.K2_SetTimerDelegate` (delegate `self.Shoot`) 0.6)
    (else
      (`parent.Shoot`)
      (`KismetSystemLibrary.Delay` _output_delay)
      (set `self.Token` true))))

(event `/Game/NIRVANA/Core/Characters/FirstPerson/BPI_Hit.Hit`
  (params (Damages :type "Float (double-precision)") (Impulse :type "Vector Structure") (Location :type "Vector Structure") (Bone :type Name))
  (`parent.Hit` Damages Impulse Location Bone)
  (bind _output_get (set `self.CurrentDealtDamages` (+ Damages (`self.CurrentDealtDamages`))))
  (if (>= _output_get (* (`self.MaxHealth`) 0.2))
    (set `self.CurrentDealtDamages` 0.0)
    (set `self.CurrentState` "NewEnumerator7")
    (`self.K2_SetActorLocation` (`self.InitPos`))
    (`|PlayMontage` (`self.Mesh`) "/Game/NIRVANA/Core/Characters/Enemies/Range/Anims/AM_Shoot.AM_Shoot"
      (:`OnCompleted`
        _)
      (:`OnInterrupted`
        _))
    (`KismetSystemLibrary.Delay` 1.2)
    (set `self.CurrentState` "NewEnumerator0")))

(fn `GetPatternIndex`
  (params (Row :type Integer))
  (returns (Index :type Integer))
  (return (`KismetMathLibrary.RandomInteger` (`KismetArrayLibrary.Array_Length` (`self.StructPattern`)))))

(fn `UserConstructionScript`
  (`parent.UserConstructionScript`))
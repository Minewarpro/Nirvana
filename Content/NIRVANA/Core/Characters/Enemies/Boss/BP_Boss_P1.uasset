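; Phase 1 boss that runs an endless bullet-pattern attack alongside a flower-and-root cycle.
; The attack loop fires a random StructPattern entry forward from the boss, waits that pattern's delay, then repeats.
; Killing all flowers makes BP_Root_P1 stretch, perform a random swipe, then shrink, which respawns the flowers in numbers that rise as boss health drops.
; Damage lowers health and updates crosshair, sound and life bar feedback.
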(event `/Game/NIRVANA/Core/Characters/FirstPerson/BPI_Hit.Hit`
  (params (Damages :type "Float (double-precision)") (Impulse :type "Vector Structure") (Location :type "Vector Structure") (Bone :type Name))
  ;[0.526 0.01096 0.01096] Overrided
)

(event `self.Death`
  ;[0.526 0.01096 0.01096] Overrided
  (`self.K2_DestroyActor`))

(event `self.ReceiveBeginPlay`
  ;[1 0.6941 0.1255 1 34] BeginPlay
  (bind _asbp_first_person_character (cast `/Game/NIRVANA/Core/Characters/FirstPerson/BP_FirstPersonCharacter` (`GameplayStatics.GetPlayerCharacter` 0)))
  (set `self.PlayerRef` _asbp_first_person_character)
  (set `self.CurrentHealth` (`self.MaxHealth`))
  (set `PrimitiveComponent.bGenerateOverlapEvents` false (`self.Weapon`))
  (bind _returnvalue (`GameplayStatics.GetActorOfClass` "/Game/NIRVANA/Core/Characters/Enemies/Range/BP_BulletManager.BP_BulletManager_C"))
  (set `self.Ref Bullet Manager` _returnvalue)
  (bind _returnvalue_2 (`GameplayStatics.GetActorOfClass` "/Game/NIRVANA/Core/Characters/Enemies/Boss/Root/BP_Root_P1.BP_Root_P1_C"))
  (set `self.Root` _returnvalue_2)
  (`self.OnActivated`)
  (bind _outactors (`GameplayStatics.GetAllActorsOfClass` "/Game/NIRVANA/Core/Characters/Enemies/Boss/BP_Flower_P1.BP_Flower_P1_C"))
  (bind _output_get (set `self.Flowers` _outactors))
  (for _array_element _output_get
    (`KismetArrayLibrary.Array_Add` (`self.FlowersPositions`) (`self.K2_GetActorLocation` _array_element)))
  (set `self.nbFlowers` (`KismetArrayLibrary.Array_Length` _output_get)))

(event `OnFlowerKilled`
  (params (flower :type "/Game/NIRVANA/Core/Characters/Enemies/Boss/BP_Flower_P1 Object Reference"))
  (bind _flowers (`self.Flowers`))
  (bind _returnvalue (/ (`self.CurrentHealth`) (`self.MaxHealth`)))
  ;[1 1 1] Events
  ;;[0.2777 0.7448 0.2941] Flowers
  (`KismetArrayLibrary.Array_RemoveItem` _flowers flower)
  (if (`KismetArrayLibrary.Array_IsEmpty` _flowers)
    (`KismetArrayLibrary.Array_Clear` (`self.Flowers`))
    (set `self.nbFlowers` (`KismetMathLibrary.SelectInt` (`KismetMathLibrary.SelectInt` 4 3 (<= _returnvalue 0.2)) 2 (<= _returnvalue 0.6)))
    (`/Game/NIRVANA/Core/Characters/Enemies/Boss/Root/BP_Root_P1.Stretch` (`self.Root`))))

(event `OnFlowerAppeared`
  (params (Flower :type "/Game/NIRVANA/Core/Characters/Enemies/Boss/BP_Flower_P1 Object Reference"))
  ;[1 1 1] Events
  ;;[0.2777 0.7448 0.2941] Flowers
  (`KismetArrayLibrary.Array_Add` (`self.Flowers`) Flower))

(event `Event Damage`
  (params (Damages :type "Float (double-precision)"))
  ;[1 0.3765 0.3765] Hit
  (`self.Cross hair hit alpha decrease `)
  (`GameplayStatics.PlaySound2D` null 1.0 1.0 0.0 null null)
  (set `self.CurrentHealth` (- (`self.CurrentHealth`) Damages))
  (if (not (<= (`self.CurrentHealth`) 0.0))
    (`self.SetLifeBar`)))

(event `OnRootFinishSwipe`
  (params (Root :type "/Game/NIRVANA/Core/Characters/Enemies/Boss/Root/BP_Root_P1 Object Reference"))
  ;[1 1 1] Events
  ;;[0.4062 0.2731 0.164] Root
  (`/Game/NIRVANA/Core/Characters/Enemies/Boss/Root/BP_Root_P1.Shrink` (`self.Root`)))

(event `OnActivated`
  ;[0.3586 0.2914 1] Activated
  (`self.Attack`))

(event `OnRootStretched`
  (bind _root (`self.Root`))
  ;[1 1 1] Events
  ;;[0.4062 0.2731 0.164] Root
  (switch `int` (`KismetMathLibrary.RandomInteger` 4)
    (:`Default`
      (`/Game/NIRVANA/Core/Characters/Enemies/Boss/Root/BP_Root_P1.HorizontalSwipe` _root (+ (`KismetMathLibrary.RandomInteger` 2) 2) 40.0 :!label _label))
    (:`0`
      (goto _label))
    (:`1`
      (`/Game/NIRVANA/Core/Characters/Enemies/Boss/Root/BP_Root_P1.VerticalSwipe` _root 65.0))
    (:`2`
      (`/Game/NIRVANA/Core/Characters/Enemies/Boss/Root/BP_Root_P1.VerticalSideSwipe` _root true 65.0 25.0))
    (:`3`
      (`/Game/NIRVANA/Core/Characters/Enemies/Boss/Root/BP_Root_P1.VerticalSideSwipe` _root false 65.0 25.0))))

(event `Attack`
  ;[1 1 1] Attack Loop
  (set `self.PatternIndex` (`self.GetPatternIndex` 0))
  (`self.Shoot`))

(event `self.Shoot`
  (bind _pos (`self.GetShootOrigin`))
  (bind _y (.y _pos))
  (bind (_output_pattern _output_nbbulletloop _output_delayeachloop _output_projectilespeed _output_damage _output_dispertion _output_dispertionspeed _output_previsualisation _output_nbbulletrectangle _output_zoffsettransformlocation _output_directionbyoffset _output_disabled _output_delay) (break `/Game/NIRVANA/Core/Characters/Enemies/Common/Struct_PatternValue` (`|GetArrayItem` (`self.StructPattern`) (`self.PatternIndex`))))
  (bind _returnvalue (`KismetMathLibrary.MakeVector` (.x _pos) (`KismetMathLibrary.SelectFloat` (+ _y 1300.0) _y (`|EnumEquality` _output_pattern "NewEnumerator17")) (+ (.z _pos) _output_zoffsettransformlocation)))
  ;[1 1 1] Shoot
  (`self.Spawn Pattern` _output_pattern _output_nbbulletloop _returnvalue (`KismetMathLibrary.GetDirectionUnitVector` (`KismetMathLibrary.SelectVector` _returnvalue _pos) (`self.GetTarget`)) _output_projectilespeed _output_damage _output_delayeachloop _output_previsualisation 1.0 _output_dispertion _output_dispertionspeed _output_nbbulletrectangle)
  (`KismetSystemLibrary.Delay` _output_delay)
  (`self.Attack`))

(event `OnRootShrinked`
  (bind _returnvalue (`self.K2_GetActorLocation`))
  ;[1 1 1] Events
  ;;[0.4062 0.2731 0.164] Root
  (for _index (range (`self.nbFlowers`))
    (bind _returnvalue_2 (== _index 2))
    (bind _returnvalue_3 (`|SpawnActorFromClass` "/Game/NIRVANA/Core/Characters/Enemies/Boss/BP_Flower_P1.BP_Flower_P1_C" (`KismetMathLibrary.MakeTransform` (`KismetMathLibrary.SelectVector` (`|GetArrayItem` (`self.FlowersPositions`) _index) (`KismetMathLibrary.SelectVector` (+ _returnvalue (0.0 0.0 600.0)) (`KismetMathLibrary.SelectVector` (+ _returnvalue (400.0 0.0 600.0)) (+ _returnvalue (-400.0 0.0 600.0)) _returnvalue_2) (and _returnvalue_2 (== (`self.nbFlowers`) 3))) (< _index 2))) "AlwaysSpawn" "MultiplyWithRoot" null null null))
    (`KismetArrayLibrary.Array_Add` (`self.Flowers`) _returnvalue_3)))

(fn `GetPatternIndex`
  (params (Row :type Integer))
  (returns (Index :type Integer))
  (return (`KismetMathLibrary.RandomInteger` (`KismetArrayLibrary.Array_Length` (`self.StructPattern`)))))

(fn `GetShootOrigin`
  (returns (Pos :type "Vector Structure"))
  (return (+ (`self.K2_GetActorLocation`) (* (`self.GetActorForwardVector`) 80.0))))

(fn `GetTarget`
  (returns (Pos :type "Vector Structure"))
  (return (+ (`self.K2_GetActorLocation`) (* (`self.GetActorForwardVector`) 500.0))))

(fn `UserConstructionScript`
  (`parent.UserConstructionScript`))
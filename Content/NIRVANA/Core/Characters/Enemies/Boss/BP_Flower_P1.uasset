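; Flower enemy for the phase 1 boss fight that rises from below ground, then attacks the player as a damageable boss weak point.
; A timeline drives the rise and rotation, then notifies BP_Boss_P1 and activates the flower as vulnerable.
; Hits damage both boss and flower, and death notifies the boss before destroying the actor.
; Shot origin and target come from a mesh socket and the player's location.
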(event `self.ReceiveBeginPlay`
  ;[1 0.6941 0.1255 1 34] BeginPlay
  (bind _asbp_first_person_character (cast `/Game/NIRVANA/Core/Characters/FirstPerson/BP_FirstPersonCharacter` (`GameplayStatics.GetPlayerCharacter` 0)))
  (set `self.PlayerRef` _asbp_first_person_character)
  (bind _output_get (set `self.Pos` (`self.K2_GetActorLocation`)))
  (`self.K2_SetActorLocationAndRotation` (- _output_get (0.0 0.0 1500.0)) (struct :`Roll` 90.0))
  (bind _returnvalue (`GameplayStatics.GetActorOfClass` "/Game/NIRVANA/Core/Characters/Enemies/Boss/BP_Boss_P1.BP_Boss_P1_C"))
  (bind _output_get_2 (set `self.Boss` _returnvalue))
  (if (== (`GameplayStatics.GetObjectClass` _output_get_2) "/Game/NIRVANA/Core/Characters/Enemies/Boss/BP_Boss_P1.BP_Boss_P1_C")
    (`KismetSystemLibrary.PrintString` "Got Boss" true true (struct :`G` 1.0 :`A` 1.0))
    (else
      (`KismetSystemLibrary.PrintString` "Error Boss" true true (struct :`R` 1.0 :`A` 1.0))))
  (`parent.ReceiveBeginPlay`)
  (`self.Appearing`))

(event `self.OnActivated`
  ;[0.3586 0.2914 1] Activated
  (set `self.vulnerable` true)
  (`self.Attack`))

(event `Appearing`
  (bind _pos (`self.Pos`))
  ;[0.5117 0.6979 0.2326] Appearing
  (`TimelineComponent.SetPlayRate` (`self.TL_Appearing`) (/ 1.0 (`self.AppearingDuration`)))
  (bind (_direction _translate _rotation) (`Timeline|TL_Appearing` :!via `PlayFromStart`)
    (:`Update`
      (`self.K2_SetActorLocationAndRotation` (`KismetMathLibrary.VLerp` (- _pos (0.0 0.0 1500.0)) _pos _translate) (`KismetMathLibrary.MakeRotator` _rotation)))
    (:`Finished`
      (`self.OnFlowerAppeared` (`self.Boss`) self)
      (`self.OnActivated`))))

(event `self.Death`
  ;[0.0226 0.0399 0.08854] Death
  (`self.SetActorHiddenInGame` true)
  (`self.K2_SetActorLocation` (0.0 0.0 999999.0) false true)
  (`self.OnFlowerKilled` (`self.Boss`) self)
  (`self.K2_DestroyActor`))

(event `/Game/NIRVANA/Core/Characters/FirstPerson/BPI_Hit.Hit`
  (params (Damages :type "Float (double-precision)") (Impulse :type "Vector Structure") (Location :type "Vector Structure") (Bone :type Name))
  ;[1 0.3765 0.3765] Hit
  (if (`self.vulnerable`)
    (`|ExecutionSequence`
      (:`then_0`
        ;;[1 1 1] Boss
        (`self.Event Damage` (`self.Boss`) Damages))
      (:`then_1`
        ;;[1 1 1] Flower
        (`self.Cross hair hit alpha decrease `)
        (`GameplayStatics.PlaySound2D` null 1.0 1.0 0.0 null null)
        (set `self.CurrentHealth` (- (`self.CurrentHealth`) Damages))
        (if (<= (`self.CurrentHealth`) 0.0)
          (`self.Death`)
          (else
            (`self.SetLifeBar`)))))))

(fn `GetShootOrigin`
  (returns (Pos :type "Vector Structure"))
  (return (`SceneComponent.GetSocketLocation` (`self.Mesh`) "polySurface6Socket")))

(fn `GetTarget`
  (returns (Pos :type "Vector Structure"))
  (return (`self.K2_GetActorLocation` (`self.PlayerRef`))))

(fn `UserConstructionScript`
  (`parent.UserConstructionScript`))
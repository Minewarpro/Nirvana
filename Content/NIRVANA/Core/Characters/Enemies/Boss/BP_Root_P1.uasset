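; Root appendage actor for the phase 1 boss that attacks by swiping and damages the player on contact.
; The construction script attaches overlap capsules along the Root's sockets, skipping the last.
; On BeginPlay, a delayed timeline rolls it down and back, then notifies BP_Boss_P1.
; A repeating horizontal yaw sweep is uncalled here, and the vertical swipe sets play rate only on the horizontal timeline.
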(event `self.ReceiveBeginPlay`
  (bind _asbp_first_person_character (cast `/Game/NIRVANA/Core/Characters/FirstPerson/BP_FirstPersonCharacter` (`GameplayStatics.GetPlayerCharacter` 0))
    (:`then`
      (set `self.PlayerRef` _asbp_first_person_character))
    (:`CastFailed`
      _))
  (bind _returnvalue (`GameplayStatics.GetActorOfClass` "/Game/NIRVANA/Core/Characters/Enemies/Boss/BP_Boss_P1.BP_Boss_P1_C"))
  (set `self.Boss` _returnvalue)
  (`self.VerticalSwipe`))

(event `CapsuleBeginOverlap`
  (params (OverlappedComponent :type "PrimitiveComponent Object Reference") (OtherActor :type "Actor Object Reference") (OtherComp :type "PrimitiveComponent Object Reference") (OtherBodyIndex :type Integer) (bFromSweep :type Boolean) (SweepResult :type "HitResult Structure (by ref)"))
  (bind _playerref (`self.PlayerRef`))
  (if (== OtherActor _playerref)
    (`/Game/NIRVANA/Core/Characters/FirstPerson/BP_FirstPersonCharacter.Take Damage` _playerref 5.0 null)))

(event `HorizontalSwipe`
  (params (Count :type Integer))
  ;[1 1 1] Swipes
  ;;[1 1 1] Horizontal
  (if (> Count 0)
    (`TimelineComponent.SetPlayRate` (`self.TL_Horizontal`) (/ 1.0 (`self.SwipeDuration`)))
    (`/Engine/EditorBlueprintResources/StandardMacros.FlipFlop`
      (:`A`
        (bind (_direction _progress) (`Timeline|TL_Horizontal` :!via `PlayFromStart` :!label _label)
          (:`Update`
            (`self.K2_SetActorRelativeRotation` (`KismetMathLibrary.MakeRotator` 0.0 0.0 (`KismetMathLibrary.Lerp` -65.0 65.0 _progress))))
          (:`Finished`
            (`self.HorizontalSwipe` (- Count 1)))))
      (:`B`
        (goto _label :!via `ReverseFromEnd`)))
    (else
      (`/Game/NIRVANA/Core/Characters/Enemies/Boss/BP_Boss_P1.OnRootFinishSwipe` (`self.Boss`) self))))

(event `VerticalSwipe`
  (bind (_initrot_roll _initrot_pitch _initrot_yaw) (`KismetMathLibrary.BreakRotator` (`self.InitRot`)))
  ;[1 1 1] Swipes
  ;;[1 1 1] Vertical
  (set `self.InitRot` (`self.K2_GetActorRotation`))
  (`KismetSystemLibrary.Delay` 2.0)
  (`TimelineComponent.SetPlayRate` (`self.TL_Horizontal`) (/ 1.0 (`self.SwipeDuration`)))
  (bind (_direction _x _y _z) (`Timeline|TL_Vertical` :!via `PlayFromStart` :!label _label_2)
    (:`Update`
      (`self.K2_SetActorRelativeRotation` (`KismetMathLibrary.MakeRotator` (`KismetMathLibrary.Lerp` _initrot_roll -65.0 _x))))
    (:`Finished`
      (`/Engine/EditorBlueprintResources/StandardMacros.FlipFlop`
        (:`A`
          (`TimelineComponent.SetPlayRate` (`self.TL_Horizontal`) (/ 1.0 (/ (`self.SwipeDuration`) 4.0)))
          (goto _label_2 :!via `Reverse`))
        (:`B`
          (`/Game/NIRVANA/Core/Characters/Enemies/Boss/BP_Boss_P1.OnRootFinishSwipe` (`self.Boss`) self))))))

(fn `UserConstructionScript`
  (bind _root (`self.root`))
  (bind _returnvalue (`SceneComponent.GetAllSocketNames` (`self.root`)))
  (for _array_element _returnvalue
    (if (!= (`|GetArrayItem` _returnvalue (`KismetArrayLibrary.Array_LastIndex` _returnvalue)) _array_element)
      (if (== (`|GetArrayItem` _returnvalue) _array_element)
        (bind _returnvalue_2 (`AddComponent|NODE_AddCapsuleComponent-1` :`bManualAttachment` true))
        (add `PrimitiveComponent.OnComponentBeginOverlap` _returnvalue_2 (`|CreateDelegate` :!event `CapsuleBeginOverlap`))
        (`SceneComponent.K2_AttachToComponent` _returnvalue_2 _root _array_element "KeepRelative" "KeepRelative" "KeepRelative" true)
        (else
          (bind _returnvalue_3 (`AddComponent|NODE_AddCapsuleComponent-0` :`bManualAttachment` true))
          (add `PrimitiveComponent.OnComponentBeginOverlap` _returnvalue_3 (`|CreateDelegate` :!event `CapsuleBeginOverlap`))
          (`SceneComponent.K2_AttachToComponent` _returnvalue_3 _root _array_element "KeepRelative" "KeepRelative" "KeepRelative" true))))))
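; BP_MusicStartLevel is a level music starter that sets the music state from its MusicEvent value.
; On BeginPlay it runs StarterMusic automatically only when MainMenu is true, after a one-tick delay.
; StarterMusic calls SetState with MusicEvent, then passes the same value to Game_Instance through ChangeMusicState.
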(event `self.ReceiveBeginPlay`
  (if (`self.MainMenu`)
    (`KismetSystemLibrary.DelayUntilNextTick`)
    (`self.StarterMusic`)))

(event `StarterMusic`
  (`AkGameplayStatics.SetState` (`self.MusicEvent`))
  (bind _asgame_instance (cast `/Game/NIRVANA/Core/GameModes/Game_Instance` (`GameplayStatics.GetGameInstance`)))
  (`/Game/NIRVANA/Core/GameModes/Game_Instance.ChangeMusicState` _asgame_instance (`self.MusicEvent`)))

(fn `UserConstructionScript`)
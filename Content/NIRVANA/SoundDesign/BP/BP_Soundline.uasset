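; BP_Soundline is a Wwise sound emitter that follows the player along a spline, making one sound behave like a line source.
; On BeginPlay it posts its AkEvent on the AkCompSpline component, then moves that component to the spline point closest to the player character, raised slightly in Z.
; A short Delay and the MoveAudio event repeat the move in a timed loop instead of using Tick.
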(event `self.ReceiveBeginPlay`
  (bind (_returnvalue_x _returnvalue_y _returnvalue_z) (`KismetMathLibrary.BreakVector` (`SplineComponent.FindLocationClosestToWorldLocation` (`self.Spline`) (`self.K2_GetActorLocation` (`GameplayStatics.GetPlayerCharacter` 0)) "World")))
  ;[0.7899 1 0.5518] [SD]
  (`AkGameObject.PostAkEvent` :`self` (`self.AkComp_Spline`) :`AkEvent` (`self.Ak Event`))
  (`SceneComponent.K2_SetWorldLocation` (`self.AkComp_Spline`) (`KismetMathLibrary.MakeVector` _returnvalue_x _returnvalue_y (+ _returnvalue_z 50.0)) false false :!label _label)
  (`KismetSystemLibrary.Delay` 0.05)
  (`self.MoveAudio`))

(event `MoveAudio`
  ;[0.7899 1 0.5518] [SD]
  (goto _label))

(fn `UserConstructionScript`)
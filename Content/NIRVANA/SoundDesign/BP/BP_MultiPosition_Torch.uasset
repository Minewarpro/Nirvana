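; Sound design actor that plays Wwise torch audio at the locations of all torches in the level through a single multi-position Ak component.
; On BeginPlay it gathers transforms of actors tagged TorchBlue, applies them as MultiSources positions and posts an Ak event.
; It then repeats this for TorchRed, appending to the same uncleared array, so the second pass covers both colors on the same component.
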(event `self.ReceiveBeginPlay`
  ;[0.7899 1 0.5518] [SD] Multi positions for torches
  (`|ExecutionSequence`
    (:`then_0`
      (bind _outactors (`GameplayStatics.GetAllActorsWithTag` "TorchBlue"))
      (for _array_element _outactors
        (`KismetArrayLibrary.Array_Add` (`self.Transform`) (`self.GetTransform` _array_element)))
      (`AkGameplayStatics.SetMultiplePositions` (`self.AkComp_MultiPosition`) (`self.Transform`) "MultiSources")
      (`AkGameObject.PostAkEvent` :`self` (`self.AkComp_MultiPosition`) :`AkEvent` (`self.AkEvent`)))
    (:`then_1`
      (`GameplayStatics.GetAllActorsWithTag` "TorchRed")
      (for _array_element_2 _
        (`KismetArrayLibrary.Array_Add` (`self.Transform`) (`self.GetTransform` _array_element_2)))
      (`AkGameplayStatics.SetMultiplePositions` (`self.AkComp_MultiPosition`) (`self.Transform`) "MultiSources")
      (`AkGameObject.PostAkEvent` :`self` (`self.AkComp_MultiPosition`) :`AkEvent` (`self.AkEvent`)))))

(fn `UserConstructionScript`)
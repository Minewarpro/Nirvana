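; BP_BoxMusic is a trigger volume that changes the game's music state when the player walks into it.
; On BeginPlay it caches the first-person character, and its box overlap responds only to that actor.
; The overlap sets its MusicState, passes it to the Game Instance, saves, then destroys the box, so each trigger fires once.
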(event `self.ReceiveBeginPlay`
  ;[0.7899 1 0.5518] [SD] Trigger music state
  (bind _asbp_first_person_character (cast `/Game/NIRVANA/Core/Characters/FirstPerson/BP_FirstPersonCharacter` (`GameplayStatics.GetPlayerCharacter` 0)))
  (set `self.PlayerRef` _asbp_first_person_character))

(event `self.TriggerBox.OnComponentBeginOverlap`
  (params (OverlappedComponent :type "PrimitiveComponent Object Reference") (OtherActor :type "Actor Object Reference") (OtherComp :type "PrimitiveComponent Object Reference") (OtherBodyIndex :type Integer) (bFromSweep :type Boolean) (SweepResult :type "HitResult Structure (by ref)"))
  ;[0.7899 1 0.5518] [SD] Trigger music state
  (if (== OtherActor (`self.PlayerRef`))
    (`AkGameplayStatics.SetState` (`self.MusicState`))
    (bind _asgame_instance (cast `/Game/NIRVANA/Core/GameModes/Game_Instance` (`GameplayStatics.GetGameInstance`)))
    (`/Game/NIRVANA/Core/GameModes/Game_Instance.ChangeMusicState` _asgame_instance (`self.MusicState`))
    (`/Game/NIRVANA/Core/GameModes/Game_Instance.Save` _asgame_instance)
    (`self.K2_DestroyActor`)))

(fn `UserConstructionScript`)
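; BP_Obelisque_A is an obelisk prop, filed under architectural lights, set up to move its static mesh vertically.
; BeginPlay randomizes the MoveTL timeline's play rate and a peak height, so instances can differ in pace and range.
; The timeline's update lerps the mesh's relative Z from zero to that height.
; The graph never starts the timeline, so any motion would depend on autoplay.
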(event `self.ReceiveBeginPlay`
  (`TimelineComponent.SetPlayRate` (`self.Move TL`) (/ 1.0 (`KismetMathLibrary.RandomFloatInRange` 6.0 7.0)))
  (set `self.High` (`KismetMathLibrary.RandomFloatInRange` 50.0 150.0)))

(fn `UserConstructionScript`)
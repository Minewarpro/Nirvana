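; BP_FloatingProp is a prop Blueprint that animates its static mesh with a vertical offset and yaw rotation to make it float.
; At BeginPlay, an optional Random flag picks amplitude and rotation within set bounds, along with a random duration.
; A Timeline, with play rate scaled to that duration, drives both relative height and yaw from a single Progress track.
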(event `self.ReceiveBeginPlay`
  (`|ExecutionSequence`
    (:`then_0`
      (if (`self.Random`)
        (set `self.Amplitude` (`KismetMathLibrary.RandomFloatInRange` (`self.AmplitudeMin`) (`self.AmplitudeMax`)))
        (set `self.Rotation` (`KismetMathLibrary.RandomFloatInRange` (`self.RotationMin`) (`self.RotationMax`)))
        (set `self.Seconds` (`KismetMathLibrary.RandomFloatInRange` 5.0 10.0))))
    (:`then_1`
      (`TimelineComponent.SetPlayRate` (`self.Timeline`) (/ 1.0 (`self.Seconds`)))
      (bind (_direction _progress) (`Timeline|Timeline`)
        (:`Update`
          (`SceneComponent.K2_SetRelativeLocationAndRotation` (`self.StaticMesh`) (`KismetMathLibrary.MakeVector` 0.0 0.0 (* _progress (`self.Amplitude`))) (`KismetMathLibrary.MakeRotator` 0.0 0.0 (* _progress (`self.Rotation`))) false false))))))

(fn `UserConstructionScript`)
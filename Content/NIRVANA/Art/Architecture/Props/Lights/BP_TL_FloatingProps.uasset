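; Manager Blueprint that animates every BP_FloatingProp in the level with a floating and spinning motion.
; On BeginPlay it gathers the props and randomizes amplitude and rotation within each prop's own ranges for those flagged Random.
; One shared timeline, TL_Float, drives all their meshes: yaw is set to Rotation times progress, while height accumulates progress times Amplitude on each update.
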(event `self.ReceiveBeginPlay`
  (bind _outactors (`GameplayStatics.GetAllActorsOfClass` "/Game/NIRVANA/Art/Architecture/Props/Lights/BP_FloatingProp.BP_FloatingProp_C"))
  (bind _output_get (set `self.FloatingProps` _outactors))
  (for _array_element _output_get
    (if (`/Game/NIRVANA/Art/Architecture/Props/Lights/BP_FloatingProp.Random` _array_element)
      (set `/Game/NIRVANA/Art/Architecture/Props/Lights/BP_FloatingProp.Amplitude` (`KismetMathLibrary.RandomFloatInRange` (`/Game/NIRVANA/Art/Architecture/Props/Lights/BP_FloatingProp.AmplitudeMin` _array_element) (`/Game/NIRVANA/Art/Architecture/Props/Lights/BP_FloatingProp.AmplitudeMax` _array_element)) _array_element)
      (set `/Game/NIRVANA/Art/Architecture/Props/Lights/BP_FloatingProp.Rotation` (`KismetMathLibrary.RandomFloatInRange` (`/Game/NIRVANA/Art/Architecture/Props/Lights/BP_FloatingProp.RotationMin` _array_element) (`/Game/NIRVANA/Art/Architecture/Props/Lights/BP_FloatingProp.RotationMax` _array_element)) _array_element)))
  (bind (_direction _progress) (`Timeline|TL_Float` :`NewTime` (`self.TimeAnim`))
    (:`Update`
      (for _array_element_2 (`self.FloatingProps`)
        (`|ExecutionSequence`
          (:`then_0`
            (bind _staticmesh (`/Game/NIRVANA/Art/Architecture/Props/Lights/BP_FloatingProp.StaticMesh` _array_element_2))
            (bind (_relativerotation_roll _relativerotation_pitch) (`KismetMathLibrary.BreakRotator` (`SceneComponent.RelativeRotation` _staticmesh)))
            (`SceneComponent.K2_SetRelativeRotation` _staticmesh (`KismetMathLibrary.MakeRotator` _relativerotation_roll _relativerotation_pitch (* (`/Game/NIRVANA/Art/Architecture/Props/Lights/BP_FloatingProp.Rotation` _array_element_2) _progress)) false false))
          (:`then_1`
            (bind (_relativelocation_x _relativelocation_y _relativelocation_z) (`KismetMathLibrary.BreakVector` (`SceneComponent.RelativeLocation` _staticmesh)))
            (`SceneComponent.K2_SetRelativeLocation` _staticmesh (`KismetMathLibrary.MakeVector` _relativelocation_x _relativelocation_y (+ _relativelocation_z (* _progress (`/Game/NIRVANA/Art/Architecture/Props/Lights/BP_FloatingProp.Amplitude` _array_element_2)))) false false)))))))

(fn `UserConstructionScript`)
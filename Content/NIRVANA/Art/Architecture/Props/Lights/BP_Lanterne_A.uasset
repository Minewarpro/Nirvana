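; Lantern prop Blueprint that animates its static mesh with a vertical and rotational motion.
; On BeginPlay it can randomize amplitude and rotation within set ranges to vary instances, then plays the MoveLantern timeline.
; Each update sets yaw from the curve scaled by rotation and adds the curve scaled by amplitude to the current Z, so vertical movement accumulates per frame.
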(event `self.ReceiveBeginPlay`
  (bind _staticmesh (`self.StaticMesh`))
  (bind _staticmesh_2 (`self.StaticMesh`))
  (bind (_relativelocation_x _relativelocation_y _relativelocation_z) (`KismetMathLibrary.BreakVector` (`SceneComponent.RelativeLocation` _staticmesh)))
  (bind (_relativerotation_roll _relativerotation_pitch) (`KismetMathLibrary.BreakRotator` (`SceneComponent.RelativeRotation` _staticmesh_2)))
  (if (`self.Random`)
    (set `self.Amplitude` (`KismetMathLibrary.RandomFloatInRange` (`self.AmpliyudeMin`) (`self.AmpliyudeMax`)))
    (set `self.Rotation` (`KismetMathLibrary.RandomFloatInRange` (`self.RotationMin`) (`self.RotationMax`)))
    (bind (_direction _move) (`Timeline|MoveLantern` :`NewTime` (`self.TimeAnim`) :!label _label)
      (:`Update`
        (`SceneComponent.K2_SetRelativeRotation` _staticmesh_2 (`KismetMathLibrary.MakeRotator` _relativerotation_roll _relativerotation_pitch (* _move (`self.Rotation`))) false false)
        (`SceneComponent.K2_SetRelativeLocation` _staticmesh (`KismetMathLibrary.MakeVector` _relativelocation_x _relativelocation_y (+ _relativelocation_z (* _move (`self.Amplitude`)))) false false)))
    (else
      (goto _label))))

(fn `UserConstructionScript`)
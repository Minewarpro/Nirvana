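; Decorative architecture prop, a sphere for chains, that spins three glowing mesh parts from BeginPlay.
; The construction script gives each mesh a dynamic material instance and sets its emissive strength.
; The Circles event plays the Rotato timeline at a slowed rate, driving each mesh's relative rotation through rotator lerps on pitch and yaw or roll, with different ranges and alpha multipliers so they turn out of step.
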(event `self.ReceiveBeginPlay`
  (`self.Circles`))

(event `Circles`
  (`TimelineComponent.SetPlayRate` (`self.Rotato`) (/ 1.0 5.0))
  (bind (_direction _newtrack_0) (`Timeline|Rotato` :!via `PlayFromStart`)
    (:`Update`
      (`SceneComponent.K2_SetRelativeRotation` (`self.StaticMesh`) (`KismetMathLibrary.RLerp` (struct) (struct :`Pitch` 360.0 :`Roll` 360.0) (* _newtrack_0 2.0)) false false)
      (`SceneComponent.K2_SetRelativeRotation` (`self.StaticMesh1`) (`KismetMathLibrary.RLerp` (struct :`Pitch` -180.0 :`Roll` -180.0) (struct :`Pitch` 180.0 :`Roll` 180.0) (* _newtrack_0 1.5)) false false)
      (`SceneComponent.K2_SetRelativeRotation` (`self.StaticMesh2`) (`KismetMathLibrary.RLerp` (struct :`Pitch` 180.0 :`Roll` 180.0) (struct :`Pitch` -180.0 :`Roll` -180.0) (* _newtrack_0 1.0)) false false))))

(fn `UserConstructionScript`
  (bind _returnvalue (`PrimitiveComponent.CreateDynamicMaterialInstance` (`self.StaticMesh`) 0 null "None"))
  (`MaterialInstanceDynamic.SetScalarParameterValue` _returnvalue "Strenght Emissive" 1.0)
  (bind _returnvalue_2 (`PrimitiveComponent.CreateDynamicMaterialInstance` (`self.StaticMesh1`) 0 null "None"))
  (`MaterialInstanceDynamic.SetScalarParameterValue` _returnvalue_2 "Strenght Emissive" 1.0)
  (bind _returnvalue_3 (`PrimitiveComponent.CreateDynamicMaterialInstance` (`self.StaticMesh2`) 0 null "None"))
  (`MaterialInstanceDynamic.SetScalarParameterValue` _returnvalue_3 "Strenght Emissive" 1.0))
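; BP_Caisson is an incubation pod prop with an animated energy effect and an optional human occupant.
; The construction script sets the occupant's rotation and male, female or empty mesh, and removes both point lights when HasLight is off.
; After a configurable delay on BeginPlay, two timelines animate "Panner" parameters on dynamic materials in an endless loop, first across the pod, then along VerticalOut.
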(event `self.ReceiveBeginPlay`
  (bind _returnvalue (`PrimitiveComponent.CreateDynamicMaterialInstance` (`self.VerticalOut`) 0 "/Game/NIRVANA/MaterialLibrary/Environement/MasterMat/Material_Instance/MM_VerticaleLumineux_1_Inst.MM_VerticaleLumineux_1_Inst" "None"))
  (set `self.MatEnergy` _returnvalue)
  (bind _returnvalue_2 (`PrimitiveComponent.CreateDynamicMaterialInstance` (`self.Caisson`) 2 "/Game/NIRVANA/MaterialLibrary/Environement/MasterMat/Material_Instance/MI_Caisson_A.MI_Caisson_A" "None"))
  (set `self.Material` _returnvalue_2)
  (`KismetSystemLibrary.Delay` (`self.PannerDelay`))
  (`self.Panner`))

(event `Panner`
  (`TimelineComponent.SetPlayRate` (`self.PannerMove`) (/ 1.0 6.0))
  (bind (_direction _newtrack_0) (`Timeline|PannerMove` :!via `PlayFromStart`)
    (:`Update`
      (`MaterialInstanceDynamic.SetScalarParameterValue` (`self.Material`) "Panner" (`KismetMathLibrary.Lerp` 0.0 1.0 _newtrack_0)))
    (:`Finished`
      (`self.EnergyOut`))))

(event `EnergyOut`
  (`TimelineComponent.SetPlayRate` (`self.SendOut`) (/ 1.0 2.0))
  (bind (_direction _newtrack_0) (`Timeline|SendOut` :!via `PlayFromStart`)
    (:`Update`
      (`MaterialInstanceDynamic.SetScalarParameterValue` (`self.MatEnergy`) "Panner" (`KismetMathLibrary.Lerp` -0.35 1.35 _newtrack_0)))
    (:`Finished`
      (`KismetSystemLibrary.Delay` 0.5)
      (`self.Panner`))))

(fn `UserConstructionScript`
  (`|ExecutionSequence`
    (:`then_0`
      (`SceneComponent.K2_SetRelativeRotation` (`self.Type`) (select `bool` (`self.IsRotate`) :`false` (struct :`Pitch` 16.593628 :`Yaw` -78.585561) :`true` (struct :`Pitch` -16.571984 :`Yaw` 98.40392 :`Roll` -7.390005) :!type "Rotator Structure") false false)
      (if (`self.Has Human`)
        (`StaticMeshComponent.SetStaticMesh` (`self.Type`) (select `bool` (`self.IsFemale`) :`false` "/Game/NIRVANA/Art/Architecture/Props/Caisson/S_Homme_Incubation_A.S_Homme_Incubation_A" :`true` "/Game/NIRVANA/Art/Architecture/Props/Caisson/S_Femme_Incubation_A.S_Femme_Incubation_A" :!type "StaticMesh Object Reference"))
        (else
          (`StaticMeshComponent.SetStaticMesh` (`self.Type`) null))))
    (:`then_1`
      (if (not (`self.HasLight`))
        (`ActorComponent.K2_DestroyComponent` (`self.PointLight`))
        (`ActorComponent.K2_DestroyComponent` (`self.PointLight1`))))))
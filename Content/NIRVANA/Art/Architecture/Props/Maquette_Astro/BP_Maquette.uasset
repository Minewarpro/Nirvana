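; BP_Maquette is an animated astronomical model prop whose center, two hoops (Arceau) and exterior float and spin.
; On BeginPlay, two slowed timelines start: Levitation lerps the relative height of all four parts, while Rotation turns the hoops.
; The hoops rotate on different axis pairs, with the second driven at double alpha.
; The construction script applies the Size variable as relative scale to all four parts.
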(event `self.ReceiveBeginPlay`
  (`self.Levitate`)
  (`self.Rotate`))

(event `Levitate`
  (`TimelineComponent.SetPlayRate` (`self.Levitation`) (/ 1.0 10.0))
  (bind (_direction _newtrack_0) (`Timeline|Levitation` :!via `PlayFromStart`)
    (:`Update`
      (`SceneComponent.K2_SetRelativeLocation` (`self.Center`) (`KismetMathLibrary.MakeVector` 0.0 0.0 (`KismetMathLibrary.Lerp` 0.0 100.0 _newtrack_0)) false false)
      (`SceneComponent.K2_SetRelativeLocation` (`self.Arceau1`) (`KismetMathLibrary.MakeVector` 0.0 0.0 (`KismetMathLibrary.Lerp` 0.0 100.0 _newtrack_0)) false false)
      (`SceneComponent.K2_SetRelativeLocation` (`self.Arceau2`) (`KismetMathLibrary.MakeVector` 0.0 0.0 (`KismetMathLibrary.Lerp` 0.0 100.0 _newtrack_0)) false false)
      (`SceneComponent.K2_SetRelativeLocation` (`self.Exterior`) (`KismetMathLibrary.MakeVector` 0.0 0.0 (`KismetMathLibrary.Lerp` 0.0 100.0 _newtrack_0)) false false))))

(event `Rotate`
  (`TimelineComponent.SetPlayRate` (`self.Rotation`) (/ 1.0 5.0))
  (bind (_direction _newtrack_0) (`Timeline|Rotation` :!via `PlayFromStart`)
    (:`Update`
      (`SceneComponent.K2_SetRelativeRotation` (`self.Arceau1`) (`KismetMathLibrary.RLerp` (struct) (struct :`Pitch` 360.0 :`Yaw` 360.0) _newtrack_0) false false)
      (`SceneComponent.K2_SetRelativeRotation` (`self.Arceau2`) (`KismetMathLibrary.RLerp` (struct) (struct :`Pitch` 360.0 :`Roll` 360.0) (* _newtrack_0 2.0)) false false))))

(fn `UserConstructionScript`
  (`SceneComponent.SetRelativeScale3D` (`self.Center`) (`self.Size`))
  (`SceneComponent.SetRelativeScale3D` (`self.Arceau1`) (`self.Size`))
  (`SceneComponent.SetRelativeScale3D` (`self.Arceau2`) (`self.Size`))
  (`SceneComponent.SetRelativeScale3D` (`self.Exterior`) (`self.Size`)))
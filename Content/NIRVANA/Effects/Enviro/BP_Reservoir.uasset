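; BP_Reservoir is an environment effect actor that animates a reservoir mesh with vertical movement and spin.
; On BeginPlay, the HautBas timeline lerps the mesh's relative height from zero toward OffsetHaut, while the Rotation timeline drives yaw through a full turn.
; Each timeline's play rate is the inverse of its own duration variable.
; The construction script applies ScaleReservoir as the mesh's world scale.
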(event `self.ReceiveBeginPlay`
  (`self.CycleMove`)
  (`self.Rotate`))

(event `CycleMove`
  (`TimelineComponent.SetPlayRate` (`self.HautBas`) (/ 1.0 (`self.NewTime`)))
  (bind (_direction _hautbas) (`Timeline|HautBas`)
    (:`Update`
      (`SceneComponent.K2_SetRelativeLocation` (`self.StaticMesh`) (`KismetMathLibrary.MakeVector` 0.0 0.0 (`KismetMathLibrary.Lerp` 0.0 (`self.OffsetHaut`) _hautbas)) false false))))

(event `Rotate`
  (`TimelineComponent.SetPlayRate` (`self.Rotation`) (/ 1.0 (`self.NewTimeRotate`)))
  (bind (_direction _newtrack_0) (`Timeline|Rotation`)
    (:`Update`
      (`SceneComponent.K2_SetRelativeRotation` (`self.StaticMesh`) (`KismetMathLibrary.MakeRotator` 0.0 0.0 (`KismetMathLibrary.Lerp` 0.0 360.0 _newtrack_0)) false false))))

(fn `UserConstructionScript`
  (`SceneComponent.SetWorldScale3D` (`self.StaticMesh`) (`self.ScaleReservoir`)))
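; BP_MeshesAfterCine puts statue and beam meshes into their post-cinematic state, as its name suggests.
; The SetLocations event raises six referenced statue actors by fixed world Z offsets, with one height for four and a lower one for two, then destroys four beam actors.
; The moves are instant, unswept and relative, so repeated calls would stack; nothing in this Blueprint calls the event.
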(event `self.ReceiveBeginPlay`)

(event `SetLocations`
  (`self.K2_AddActorWorldOffset` (`self.Statue1`) (0.0 0.0 4231.0) false false)
  (`self.K2_AddActorWorldOffset` (`self.Statue2`) (0.0 0.0 4231.0) false false)
  (`self.K2_AddActorWorldOffset` (`self.Statue3`) (0.0 0.0 4231.0) false false)
  (`self.K2_AddActorWorldOffset` (`self.Statue4`) (0.0 0.0 4231.0) false false)
  (`self.K2_AddActorWorldOffset` (`self.Statue5`) (0.0 0.0 3734.0) false false)
  (`self.K2_AddActorWorldOffset` (`self.Statue6`) (0.0 0.0 3734.0) false false)
  (`self.K2_DestroyActor` (`self.Beam1`))
  (`self.K2_DestroyActor` (`self.Beam2`))
  (`self.K2_DestroyActor` (`self.Beam3`))
  (`self.K2_DestroyActor` (`self.Beam4`)))

(fn `UserConstructionScript`)
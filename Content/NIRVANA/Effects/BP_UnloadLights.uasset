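; Trigger actor that transitions the level's directional light and height fog to target settings, then removes them.
; BeginPlay caches original values; the player's first Box overlap applies toggles immediately and blends the rest through the Switching timeline, paced by TimelineRate.
; That arms DestroyBox, whose next player overlap destroys the referenced light, skylight, fog and sky atmosphere.
; The construction script sizes both boxes and positions DestroyBox.
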(event `self.ReceiveBeginPlay`
  (bind _component (`ExponentialHeightFog.Component` (`self.Fog`)))
  (bind _lightcomponent (`Light.LightComponent` (`self.Directionnal`)))
  (bind (_secondfogdata_fogdensity _secondfogdata_fogheightfalloff _secondfogdata_fogheightoffset) (break `ExponentialHeightFogData` (`ExponentialHeightFogComponent.SecondFogData` _component)))
  (set `self.DLOriginTemperatur` (`LightComponent.Temperature` _lightcomponent))
  (set `self.DLOriginIntensity` (`LightComponentBase.Intensity` _lightcomponent))
  (set `self.DLOriginVolScatInt` (`LightComponentBase.VolumetricScatteringIntensity` _lightcomponent))
  (set `self.DLOriginBloomScale` (`LightComponent.BloomScale` _lightcomponent))
  (set `self.DLOriginBloomMaxBright` (`LightComponent.BloomMaxBrightness` _lightcomponent))
  (set `self.DLOriginLightFunctionScale` (`LightComponent.LightFunctionScale` _lightcomponent))
  (set `self.DLOriginFadeDist` (`LightComponent.LightFunctionFadeDistance` _lightcomponent))
  (set `self.DLOriginDisabledBrightness` (`LightComponent.DisabledBrightness` _lightcomponent))
  (set `self.FOGOriginDensity` (`ExponentialHeightFogComponent.FogDensity` _component))
  (set `self.FOGOriginHeighFalloff` (`ExponentialHeightFogComponent.FogHeightFalloff` _component))
  (set `self.FOGOriginInscateringCol` (`ExponentialHeightFogComponent.FogInscatteringLuminance` _component))
  (set `self.FOGOriginSecondDensity` _secondfogdata_fogdensity)
  (set `self.FOGOriginSecondFalloff` _secondfogdata_fogheightfalloff)
  (set `self.FOGOriginSecondOffset` _secondfogdata_fogheightoffset)
  (set `self.FOGOriginVolumetricDist` (`ExponentialHeightFogComponent.VolumetricFogStartDistance` _component))
  (set `self.FOGOriginStartDistance` (`ExponentialHeightFogComponent.StartDistance` _component))
  (set `self.FOGOriginScattDistrib` (`ExponentialHeightFogComponent.VolumetricFogScatteringDistribution` _component)))

(event `SwitchLights`
  (bind _lightcomponent (`Light.LightComponent` (`self.Directionnal`)))
  (bind _lightcomponent_2 (`Light.LightComponent` (`self.Directionnal`)))
  (bind _component (`ExponentialHeightFog.Component` (`self.Fog`)))
  (`TimelineComponent.SetPlayRate` (`self.Switching`) (/ 1.0 (`self.TimelineRate`)))
  (`LightComponent.SetUseTemperature` _lightcomponent_2 (`self.NewUseTemprature`))
  (`LightComponent.SetEnableLightShaftBloom` _lightcomponent_2 (`self.New Shaft Bloom`))
  (`ExponentialHeightFogComponent.SetVolumetricFog` (`ExponentialHeightFog.Component` (`self.Fog`)) (`self.New Volumetric Fog`))
  (bind (_direction _newtrack_0) (`Timeline|Switching` :!via `PlayFromStart`)
    (:`Update`
      (`LightComponent.SetTemperature` _lightcomponent (`KismetMathLibrary.Lerp` (`self.DLOriginTemperatur`) (`self.DLTargetTemp`) _newtrack_0))
      (`LightComponent.SetIntensity` _lightcomponent (`KismetMathLibrary.Lerp` (`self.DLOriginIntensity`) (`self.DLTargerIntensity`) _newtrack_0))
      (`LightComponent.SetVolumetricScatteringIntensity` _lightcomponent (`KismetMathLibrary.Lerp` (`self.DLOriginVolScatInt`) (`self.DLTargetVolScatInt`) _newtrack_0))
      (`LightComponent.SetBloomScale` _lightcomponent (`KismetMathLibrary.Lerp` (`self.DLOriginBloomScale`) (`self.DLTargetBloomScale`) _newtrack_0))
      (`LightComponent.SetBloomMaxBrightness` _lightcomponent (`KismetMathLibrary.Lerp` (`self.DLOriginBloomMaxBright`) (`self.DLTargetBloomMaxBright`) _newtrack_0))
      (`LightComponent.SetLightFunctionScale` _lightcomponent (`KismetMathLibrary.VLerp` (`self.DLOriginLightFunctionScale`) (`self.DLTargetLightFuncScale`) _newtrack_0))
      (`LightComponent.SetLightFunctionFadeDistance` _lightcomponent (`KismetMathLibrary.Lerp` (`self.DLOriginFadeDist`) (`self.DLTargetFadeDist`) _newtrack_0))
      (`LightComponent.SetLightFunctionDisabledBrightness` _lightcomponent (`KismetMathLibrary.Lerp` (`self.DLOriginDisabledBrightness`) (`self.DLTargetDisabledBirght`) _newtrack_0))
      (`ExponentialHeightFogComponent.SetFogDensity` _component (`KismetMathLibrary.Lerp` (`self.FOGOriginDensity`) (`self.FogTargetDensity`) _newtrack_0))
      (`ExponentialHeightFogComponent.SetFogHeightFalloff` _component (`KismetMathLibrary.Lerp` (`self.FOGOriginHeighFalloff`) (`self.FogTargetHeightFalloff`) _newtrack_0))
      (`ExponentialHeightFogComponent.SetFogInscatteringColor` _component (`KismetMathLibrary.LinearColorLerp` (`self.FOGOriginInscateringCol`) (`self.FogTargetInscatteringColor`) _newtrack_0))
      (`ExponentialHeightFogComponent.SetSecondFogDensity` _component (`KismetMathLibrary.Lerp` (`self.FOGOriginSecondDensity`) (`self.FogTargetSecondDensity`) _newtrack_0))
      (`ExponentialHeightFogComponent.SetVolumetricFogScatteringDistribution` _component (`KismetMathLibrary.Lerp` (`self.FOGOriginScattDistrib`) (`self.FogTargetScattDistrib`) _newtrack_0))
      (`ExponentialHeightFogComponent.SetSecondFogHeightFalloff` _component (`KismetMathLibrary.Lerp` (`self.FOGOriginSecondFalloff`) (`self.FogTargetSecondFalloff`) _newtrack_0))
      (`ExponentialHeightFogComponent.SetSecondFogHeightOffset` _component (`KismetMathLibrary.Lerp` (`self.FOGOriginSecondOffset`) (`self.FogTargetSecondOffset`) _newtrack_0))
      (`ExponentialHeightFogComponent.SetVolumetricFogDistance` _component (`KismetMathLibrary.Lerp` (`self.FOGOriginVolumetricDist`) (`self.FogTargetVolumetricDist`) _newtrack_0))
      (`ExponentialHeightFogComponent.SetStartDistance` _component (`KismetMathLibrary.Lerp` (`self.FOGOriginStartDistance`) (`self.FogTargetStartDist`) _newtrack_0)))))

(event `self.Box.OnComponentBeginOverlap`
  (params (OverlappedComponent :type "PrimitiveComponent Object Reference") (OtherActor :type "Actor Object Reference") (OtherComp :type "PrimitiveComponent Object Reference") (OtherBodyIndex :type Integer) (bFromSweep :type Boolean) (SweepResult :type "HitResult Structure (by ref)"))
  (cast `/Game/NIRVANA/Core/Characters/FirstPerson/BP_FirstPersonCharacter` OtherActor)
  (if (`self.Activated`)
    (set `self.Activated` false)
    (set `self.Destructible` true)
    (`self.SwitchLights`)))

(event `DestroyAll`
  (`self.K2_DestroyActor` (`self.Directionnal`))
  (`self.K2_DestroyActor` (`self.SkyLight`))
  (`self.K2_DestroyActor` (`self.Fog`))
  (`self.K2_DestroyActor` (`self.SkyAtmo`)))

(event `self.DestroyBox.OnComponentBeginOverlap`
  (params (OverlappedComponent :type "PrimitiveComponent Object Reference") (OtherActor :type "Actor Object Reference") (OtherComp :type "PrimitiveComponent Object Reference") (OtherBodyIndex :type Integer) (bFromSweep :type Boolean) (SweepResult :type "HitResult Structure (by ref)"))
  (cast `/Game/NIRVANA/Core/Characters/FirstPerson/BP_FirstPersonCharacter` OtherActor)
  (if (`self.Destructible`)
    (set `self.Destructible` false)
    (`self.DestroyAll`)))

(fn `UserConstructionScript`
  (bind _destroybox (`self.DestroyBox`))
  (`SceneComponent.K2_SetRelativeLocation` _destroybox (`self.BoxDestroLoc`) false false)
  (`SceneComponent.SetRelativeScale3D` _destroybox (`self.BoxDestroyScale`))
  (`SceneComponent.SetRelativeScale3D` (`self.Box`) (`self.TriggerScale`)))
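; BP_FresqueUne is a tutorial mural that hands the player the Vajra weapon and opens when shot with it.
; Overlapping the grab trigger equips the Vajra, arms the mural and shows the WB_TutoInfos widget and text.
; Each Vajra projectile hit recolours the mural through a material parameter.
; The third hit lowers it on a timeline, resets the weapon's overheat and briefly shows the overheat tip.
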(event `self.ReceiveBeginPlay`
  (bind _asbp_first_person_character (cast `/Game/NIRVANA/Core/Characters/FirstPerson/BP_FirstPersonCharacter` (`GameplayStatics.GetPlayerCharacter` 0)))
  (set `self.PlayerRef` _asbp_first_person_character)
  (`PrimitiveComponent.CreateDynamicMaterialInstance` (`self.FresqueMesh`) 0 null "None"))

(event `self.GrabVajra.OnComponentBeginOverlap`
  (params (OverlappedComponent :type "PrimitiveComponent Object Reference") (OtherActor :type "Actor Object Reference") (OtherComp :type "PrimitiveComponent Object Reference") (OtherBodyIndex :type Integer) (bFromSweep :type Boolean) (SweepResult :type "HitResult Structure (by ref)"))
  ;[1 1 1] Grab Vajra
  (if (and (== OtherActor (`self.PlayerRef`)) (`self.CanGrab`))
    (`self.EquipVajra`)
    (set `self.CanGrab` false)))

(event `DestroyVajra`
  (`ActorComponent.K2_DestroyComponent` (`self.Vajra`)))

(event `EquipVajra`
  (bind _playerref (`self.PlayerRef`))
  ;[1 1 1] Grab Vajra
  (set `self.Activated` true)
  (`/Game/NIRVANA/Core/Characters/FirstPerson/BP_FirstPersonCharacter.EquipWeapons` _playerref (`self.EquipWeapons`))
  (`/Game/NIRVANA/Core/Characters/FirstPerson/BP_FirstPersonCharacter.Change Weapon` _playerref "NewEnumerator11" 1)
  (bind _asbp_vajra (cast `/Game/NIRVANA/Core/Weapons/Vajra/BP_Vajra` (`/Game/NIRVANA/Core/Characters/FirstPerson/BP_FirstPersonCharacter.Get Weapon` _playerref)))
  (set `self.VajraRef` _asbp_vajra)
  (set `/Game/NIRVANA/Core/Characters/FirstPerson/BP_FirstPersonCharacter.Can Change weapon` true _playerref)
  (bind _returnvalue (`|CreateWidget` "/Game/NIRVANA/UI/Player/WB_TutoInfos.WB_TutoInfos_C" null false false false false false true))
  (bind _output_get (set `self.TutoInfos` _returnvalue))
  (`UserWidget.AddToViewport` _output_get 0)
  (`SceneComponent.SetHiddenInGame` (`self.TextRender`) false false))

(event `self.Box.OnComponentBeginOverlap`
  (params (OverlappedComponent :type "PrimitiveComponent Object Reference") (OtherActor :type "Actor Object Reference") (OtherComp :type "PrimitiveComponent Object Reference") (OtherBodyIndex :type Integer) (bFromSweep :type Boolean) (SweepResult :type "HitResult Structure (by ref)"))
  ;[1 1 1] Open Fresque
  (bind _asbp_projectile_vajra (cast `/Game/NIRVANA/Core/Weapons/Vajra/BP_ProjectileVajra` OtherActor))
  (if (and (== (`/Game/NIRVANA/Core/Weapons/Vajra/BP_ProjectileVajra.MiddleCollision` _asbp_projectile_vajra) OtherComp) (`self.Activated`))
    (set `self.ShootIndex` (+ (`self.ShootIndex`) 1))
    (`|ExecutionSequence`
      (:`then_0`
        (if (not (`self.CanOpen`))
          (`self.ChangeMaterial`)
          (if (== (`self.ShootIndex`) 3)
            (set `self.CanOpen` true))))
      (:`then_1`
        (if (`self.CanOpen`)
          (`self.ChangeMaterial`)
          (`self.OpenMural`)
          (set `self.CanOpen` false)
          (set `self.Activated` false)))
      (:`then_2`
        (if (`self.TutoEnd`)
          (`Widget.SetVisibility` (`/Game/NIRVANA/UI/Player/WB_TutoInfos.Shoot` (`self.TutoInfos`)) "Hidden")
          (set `self.TutoEnd` false))))))

(event `OpenMural`
  (bind _vajraref (`self.VajraRef`))
  ;[1 1 1] Open Fresque
  (`|ExecutionSequence`
    (:`then_0`
      (bind (_direction _newtrack_0) (`Timeline|Opening` :!via `PlayFromStart`)
        (:`Update`
          (`SceneComponent.K2_SetRelativeLocation` (`self.FresqueMesh`) (`KismetMathLibrary.MakeVector` 0.0 0.0 (`KismetMathLibrary.Lerp` 400.0 -400.0 _newtrack_0)) false false))))
    (:`then_1`
      (`/Game/NIRVANA/Core/Weapons/Vajra/BP_Vajra.Add Surchauffe` _vajraref (* (`/Game/NIRVANA/Core/Weapons/Vajra/BP_Vajra.Surchauffe Value` _vajraref) -1.0))
      (`Widget.SetVisibility` (`/Game/NIRVANA/UI/Player/WB_TutoInfos.OverHeat` (`self.TutoInfos`)) "Visible")
      (`KismetSystemLibrary.Delay` 5.0)
      (`Widget.RemoveFromParent` (`self.TutoInfos`)))))

(event `ChangeMaterial`
  ;[1 1 1] Open Fresque
  (`MeshComponent.SetVectorParameterValueOnMaterials` (`self.FresqueMesh`) "SurfaceColor" (select `int` (`self.ShootIndex`) :`0` (1.0 0.0 0.0) :`1` (0.0 1.0 0.0) :`2` (0.0 0.0 1.0) :`3` (0.0 0.0 0.0) :!type "Vector Structure")))

(fn `UserConstructionScript`
  (`SceneComponent.SetHiddenInGame` (`self.TextRender`) true false))
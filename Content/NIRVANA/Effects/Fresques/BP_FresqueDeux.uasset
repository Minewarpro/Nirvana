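; Fresco actor that plays a two-part cinematic once the arena is cleared, if still active.
; It hides the HUD, plays two level sequences with a fade and camera switch between them, then teleports the player, calls UpAutel on the altar and restores view and input.
; A CenterFall timeline tips the scene with shake and smoke, but its chakram-hit trigger is disconnected, leaving the bound hit event empty.
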(event `self.ReceiveBeginPlay`
  (bind _asbp_first_person_character (cast `/Game/NIRVANA/Core/Characters/FirstPerson/BP_FirstPersonCharacter` (`GameplayStatics.GetPlayerCharacter` 0)))
  (set `self.PlayerRef` _asbp_first_person_character))

(event `/Game/NIRVANA/Core/Placeables/Management/BPI_ArenaManager.OnArenaCleaned`
  (params (ArenaManager :type "/Game/NIRVANA/Core/Placeables/Management/BP_ArenaManager Object Reference"))
  (`KismetSystemLibrary.Delay` 1.0)
  (if (`self.IsActive`)
    (set `self.IsActive` false)
    (`self.PlayFresque`)))

(event `PlayFresque`
  (bind _returnvalue (`GameplayStatics.GetPlayerController` 0))
  (bind _returnvalue_2 (`GameplayStatics.GetPlayerController` 0))
  (bind _sequenceplayer (`LevelSequenceActor.SequencePlayer` (`self.SecondSequencerToPlay`)))
  (bind _sequenceplayer_2 (`LevelSequenceActor.SequencePlayer` (`self.SequencerToPlay`)))
  (`Widget.SetVisibility` (`/Game/NIRVANA/Core/Characters/FirstPerson/BP_FirstPersonCharacter.WB_Base_Ref` (`self.PlayerRef`)) "Hidden")
  (set `/Game/NIRVANA/Core/Characters/FirstPerson/BP_FirstPersonCharacter.inCinematic` true (`self.PlayerRef`))
  (`MovieSceneSequencePlayer.Play` _sequenceplayer_2)
  (`KismetSystemLibrary.Delay` (`TimeManagementBlueprintLibrary.Conv_QualifiedFrameTimeToSeconds` (`MovieSceneSequencePlayer.GetDuration` _sequenceplayer_2)))
  (`PlayerCameraManager.StartCameraFade` :`self` (`GameplayStatics.GetPlayerCameraManager` 0) :`ToAlpha` 1.0 :`Duration` 0.5)
  (`KismetSystemLibrary.Delay` 0.5)
  (`self.DisableInput` (`self.PlayerRef`) _returnvalue)
  (set `self.CamToReturn` (`Controller.GetViewTarget` _returnvalue))
  (`PlayerController.SetViewTargetWithBlend` _returnvalue (`self.CamToBlend`) 0.0 "VTBlend_Linear" 0.0 false)
  (`MovieSceneSequencePlayer.Play` _sequenceplayer)
  (`KismetSystemLibrary.Delay` (`TimeManagementBlueprintLibrary.Conv_QualifiedFrameTimeToSeconds` (`MovieSceneSequencePlayer.GetDuration` _sequenceplayer)))
  (set `/Game/NIRVANA/Core/Characters/FirstPerson/BP_FirstPersonCharacter.inCinematic` false (`self.PlayerRef`))
  (`self.K2_SetActorLocation` (`self.PlayerRef`) (82432.999906 -17789.864547 9430.617932) false false)
  (`Controller.SetControlRotation` (`GameplayStatics.GetPlayerController` 0) (`self.RotationTP`))
  (`/Game/DevelopersContent/DevelopersTools/BP_Autel_Chakram.UpAutel` (`self.AutelToMove`))
  (`PlayerController.SetViewTargetWithBlend` _returnvalue_2 (`self.CamToReturn`) 0.0 "VTBlend_Linear" 0.0 false)
  (`PlayerCameraManager.StartCameraFade` :`self` (`GameplayStatics.GetPlayerCameraManager` 0) :`FromAlpha` 1.0 :`Duration` 0.5)
  (`self.EnableInput` (`self.PlayerRef`) _returnvalue_2))

(event `HitFresque`
  (params (HitComponent :type "PrimitiveComponent Object Reference") (OtherActor :type "Actor Object Reference") (OtherComp :type "PrimitiveComponent Object Reference") (NormalImpulse :type "Vector Structure") (Hit :type "HitResult Structure (by ref)")))

(event `CenterFall`
  (`TimelineComponent.SetPlayRate` (`self.Fall`) (/ 1.0 3.0))
  (bind (_direction _newtrack_0) (`Timeline|Fall` :!via `PlayFromStart`)
    (:`Update`
      (`SceneComponent.K2_SetRelativeRotation` (`self.Scene`) (`KismetMathLibrary.MakeRotator` 0.0 (`KismetMathLibrary.Lerp` 0.0 -90.0 _newtrack_0)) false false))
    (:`Finished`
      (`PlayerCameraManager.StartCameraShake` :`self` (`GameplayStatics.GetPlayerCameraManager` 0) :`ShakeClass` "/Game/NIRVANA/Effects/Cinematics/CamShake_BridgeFall.CamShake_BridgeFall_C")
      (`ActorComponent.Activate` (`self.FXS_Smoke03`) false))))

(fn `UserConstructionScript`
  (for _array_element (`SceneComponent.GetChildrenComponents` (`self.Middle`) false)
    (bind _asstatic_mesh_component (cast `StaticMeshComponent` _array_element))
    (add `PrimitiveComponent.OnComponentHit` _asstatic_mesh_component (`|CreateDelegate` :!event `HitFresque`))))
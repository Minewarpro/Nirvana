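; BP_LightSetup switches off a level's lighting setup at runtime by hiding its referenced environment actors when play begins.
; On BeginPlay it loops through four actor arrays (directional lights, sky lights, sky atmospheres and fogs) and sets each actor hidden in game.
; The construction script is empty, and nothing in the Blueprint fills the arrays or unhides the actors.
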(event `self.ReceiveBeginPlay`
  (for _array_element (`self.Directionals`)
    (`self.SetActorHiddenInGame` _array_element true))
  (for _array_element_2 (`self.SkyLights`)
    (`self.SetActorHiddenInGame` _array_element_2 true))
  (for _array_element_3 (`self.SkyAtmos`)
    (`self.SetActorHiddenInGame` _array_element_3 true))
  (for _array_element_4 (`self.Fogs`)
    (`self.SetActorHiddenInGame` _array_element_4 true)))

(fn `UserConstructionScript`)
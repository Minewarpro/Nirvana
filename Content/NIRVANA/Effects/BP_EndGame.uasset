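; End-game trigger actor that plays the ending credits and returns to the main menu.
; When the first-person character overlaps the box while Activated, it fires once, destroys BPVoid, fades to black, disables input and shows WB_Ending.
; Timelines fade in ESMA and Mastoc, then CreditsText re-calls itself, stepping backwards through parallel arrays of roles, names and portraits.
; A closing Carton fade precedes loading MainMenu_V1.
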(event `self.Box.OnComponentBeginOverlap`
  (params (OverlappedComponent :type "PrimitiveComponent Object Reference") (OtherActor :type "Actor Object Reference") (OtherComp :type "PrimitiveComponent Object Reference") (OtherBodyIndex :type Integer) (bFromSweep :type Boolean) (SweepResult :type "HitResult Structure (by ref)"))
  (bind _fadeduration (`self.FadeDuration`))
  (bind _playerref (`self.PlayerRef`))
  (bind _asbp_first_person_character (cast `/Game/NIRVANA/Core/Characters/FirstPerson/BP_FirstPersonCharacter` OtherActor))
  (set `self.PlayerRef` _asbp_first_person_character)
  (if (`self.Activated`)
    (set `self.Activated` false)
    (`self.K2_DestroyActor` (`self.BP_Void`))
    (`PlayerCameraManager.StartCameraFade` :`self` (`GameplayStatics.GetPlayerCameraManager` 0) :`ToAlpha` 1.0 :`Duration` _fadeduration :`bHoldWhenFinished` true)
    (`KismetSystemLibrary.Delay` _fadeduration)
    (`self.DisableInput` _playerref (`GameplayStatics.GetPlayerController` 0))
    (`Widget.SetVisibility` (`/Game/NIRVANA/Core/Characters/FirstPerson/BP_FirstPersonCharacter.WB_Base_Ref` _playerref) "Hidden")
    (bind _returnvalue (`|CreateWidget` "/Game/NIRVANA/UI/WB_Ending.WB_Ending_C"))
    (`UserWidget.AddToViewport` _returnvalue 0)
    (`TimelineComponent.SetPlayRate` (`self.ESMA`) (/ 1.0 2.0))
    (bind (_direction _newtrack_0) (`Timeline|ESMA` :!via `PlayFromStart`)
      (:`Update`
        (`Image.SetOpacity` (`/Game/NIRVANA/UI/WB_Ending.ESMA` _returnvalue) (`KismetMathLibrary.Lerp` 0.0 1.0 _newtrack_0)))
      (:`Finished`
        (`TimelineComponent.SetPlayRate` (`self.Mastoc`) (/ 1.0 2.0))
        (bind (_direction_2 _newtrack_0_2) (`Timeline|Mastoc` :!via `PlayFromStart`)
          (:`Update`
            (`Image.SetOpacity` (`/Game/NIRVANA/UI/WB_Ending.Mastoc` _returnvalue) (`KismetMathLibrary.Lerp` 0.0 1.0 _newtrack_0_2)))
          (:`Finished`
            (`self.CreditsText`)))))))

(event `CreditsText`
  (bind _returnvalue (- (`self.CreditsId`) 1))
  (`TimelineComponent.SetPlayRate` (`self.NamesDesign`) (/ 1.0 6.0))
  (bind _fonction (`/Game/NIRVANA/UI/WB_Ending.Fonction` (stale `self.Box.OnComponentBeginOverlap` _returnvalue)))
  (set `TextBlock.Text` (`|GetArrayItem` (`self.Fonctions`) _returnvalue) _fonction)
  (bind _name1 (`/Game/NIRVANA/UI/WB_Ending.Name1` (stale `self.Box.OnComponentBeginOverlap` _returnvalue)))
  (set `TextBlock.Text` (`|GetArrayItem` (`self.Names1`) _returnvalue) _name1)
  (bind _name2 (`/Game/NIRVANA/UI/WB_Ending.Name2` (stale `self.Box.OnComponentBeginOverlap` _returnvalue)))
  (set `TextBlock.Text` (`|GetArrayItem` (`self.Names2`) _returnvalue) _name2)
  (bind _name3 (`/Game/NIRVANA/UI/WB_Ending.Name3` (stale `self.Box.OnComponentBeginOverlap` _returnvalue)))
  (set `TextBlock.Text` (`|GetArrayItem` (`self.Names3`) _returnvalue) _name3)
  (bind _portrait1 (`/Game/NIRVANA/UI/WB_Ending.Portrait1` (stale `self.Box.OnComponentBeginOverlap` _returnvalue)))
  (`Image.SetBrushFromTexture` _portrait1 (`|GetArrayItem` (`self.Portraits1`) _returnvalue) true)
  (bind _portrait2 (`/Game/NIRVANA/UI/WB_Ending.Portrait2` (stale `self.Box.OnComponentBeginOverlap` _returnvalue)))
  (`Image.SetBrushFromTexture` _portrait2 (`|GetArrayItem` (`self.Portraits2`) _returnvalue) true)
  (bind _portrait3 (`/Game/NIRVANA/UI/WB_Ending.Portrait3` (stale `self.Box.OnComponentBeginOverlap` _returnvalue)))
  (`Image.SetBrushFromTexture` _portrait3 (`|GetArrayItem` (`self.Portraits3`) _returnvalue) true)
  (bind (_direction _design _name1_2 _name2_2 _name3_2) (`Timeline|NamesDesign` :!via `PlayFromStart`)
    (:`Update`
      (`TextBlock.SetOpacity` _fonction (`KismetMathLibrary.Lerp` 0.0 1.0 _design))
      (`TextBlock.SetOpacity` _name1 (`KismetMathLibrary.Lerp` 0.0 1.0 _name1_2))
      (`TextBlock.SetOpacity` _name2 (`KismetMathLibrary.Lerp` 0.0 1.0 _name2_2))
      (`TextBlock.SetOpacity` _name3 (`KismetMathLibrary.Lerp` 0.0 1.0 _name3_2))
      (`Image.SetOpacity` _portrait1 (`KismetMathLibrary.Lerp` 0.0 1.0 _name1_2))
      (`Image.SetOpacity` _portrait2 (`KismetMathLibrary.Lerp` 0.0 1.0 _name2_2))
      (`Image.SetOpacity` _portrait3 (`KismetMathLibrary.Lerp` 0.0 1.0 _name3_2)))
    (:`Finished`
      (set `self.CreditsId` (- (`self.CreditsId`) 1))
      (if (> (`self.CreditsId`) 0)
        (`self.CreditsText`)
        (else
          (`TimelineComponent.SetPlayRate` (`self.opacity`) (/ 1.0 5.0))
          (bind (_direction_2 _newtrack_0) (`Timeline|opacity` :!via `PlayFromStart`)
            (:`Update`
              (`Image.SetOpacity` (`/Game/NIRVANA/UI/WB_Ending.Carton` (stale `self.Box.OnComponentBeginOverlap` _returnvalue)) (`KismetMathLibrary.Lerp` 0.0 1.0 _newtrack_0)))
            (:`Finished`
              (`GameplayStatics.OpenLevelBySoftObjectPtr` "/Game/DevelopersContent/Maps/Playtests/MainMenu_V1.MainMenu_V1"))))))))

(fn `UserConstructionScript`)
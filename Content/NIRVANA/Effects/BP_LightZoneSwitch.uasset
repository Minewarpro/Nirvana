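; Atmosphere controller that shifts directional light, height fog and sky atmosphere as the player moves between level zones.
; BeginPlay applies the initial Scientifique look, with bright volumetric fog.
; Two trigger boxes, placed by construction-script variables, each fire a one-shot, slowed Timeline that lerps to the Military or Hall look.
; Start values are hard-coded, so Hall assumes Military already ran, and nothing transitions back.
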(event `self.ReceiveBeginPlay`
  (bind _asbp_first_person_character (cast `/Game/NIRVANA/Core/Characters/FirstPerson/BP_FirstPersonCharacter` (`GameplayStatics.GetPlayerCharacter` 0)))
  (set `self.PlayerRef` _asbp_first_person_character)
  (`self.ScientifiqueSetup`))

(event `ScientifiqueSetup`
  (bind _directionallight (`self.DirectionalLight`))
  (bind _exponentialheightfog (`self.ExponentialHeightFog`))
  (`LightComponent.SetIntensity` _directionallight 5.0)
  (`DirectionalLightComponent.SetEnableLightShaftOcclusion` _directionallight true)
  (`ExponentialHeightFogComponent.SetFogDensity` _exponentialheightfog 0.2)
  (`ExponentialHeightFogComponent.SetFogHeightFalloff` _exponentialheightfog 0.32084)
  (`ExponentialHeightFogComponent.SetStartDistance` _exponentialheightfog 600.0)
  (`ExponentialHeightFogComponent.SetVolumetricFog` _exponentialheightfog true)
  (`ExponentialHeightFogComponent.SetFogInscatteringColor` _exponentialheightfog (struct :`R` 1.0 :`G` 1.0 :`B` 1.0 :`A` 1.0)))

(event `self.BoxMilitary.OnComponentBeginOverlap`
  (params (OverlappedComponent :type "PrimitiveComponent Object Reference") (OtherActor :type "Actor Object Reference") (OtherComp :type "PrimitiveComponent Object Reference") (OtherBodyIndex :type Integer) (bFromSweep :type Boolean) (SweepResult :type "HitResult Structure (by ref)"))
  (if (and (== OtherActor (`self.PlayerRef`)) (`self.ActivatedMilitary`))
    (set `self.ActivatedMilitary` false)
    (`self.TransitionToMilitary`)))

(event `self.BoxReligieuse1.OnComponentBeginOverlap`
  (params (OverlappedComponent :type "PrimitiveComponent Object Reference") (OtherActor :type "Actor Object Reference") (OtherComp :type "PrimitiveComponent Object Reference") (OtherBodyIndex :type Integer) (bFromSweep :type Boolean) (SweepResult :type "HitResult Structure (by ref)"))
  (if (and (== OtherActor (`self.PlayerRef`)) (`self.ActivatedHall`))
    (set `self.ActivatedHall` false)
    (`self.TransitionToHall`)))

(event `TransitionToMilitary`
  (bind _directionallight (`self.DirectionalLight`))
  (bind _exponentialheightfog (`self.ExponentialHeightFog`))
  ;[1 1 1] Transition vers military
  (`TimelineComponent.SetPlayRate` (`self.Military`) (/ 1.0 5.0))
  (`LightComponent.SetUseTemperature` (`self.DirectionalLight`) true)
  (bind (_direction _newtrack_0) (`Timeline|Military` :!via `PlayFromStart`)
    (:`Update`
      (`LightComponent.SetIntensity` _directionallight (`KismetMathLibrary.Lerp` 5.0 10.0 _newtrack_0))
      (`LightComponent.SetTemperature` _directionallight (`KismetMathLibrary.Lerp` 6500.0 4000.0 _newtrack_0))
      (`DirectionalLightComponent.SetLightSourceAngle` _directionallight (`KismetMathLibrary.Lerp` 0.5357 0.6957 _newtrack_0))
      (`DirectionalLightComponent.SetDynamicShadowDistanceMovableLight` _directionallight (`KismetMathLibrary.Lerp` 40000.0 30000.0 _newtrack_0))
      (`LightComponent.SetLightFunctionScale` _directionallight (`KismetMathLibrary.VLerp` (1024.0 1024.0 1024.0) (4235.0 4235.0 4235.0) _newtrack_0))
      (`LightComponent.SetLightFunctionFadeDistance` _directionallight (`KismetMathLibrary.Lerp` 100000.0 77466.1875 _newtrack_0))
      (`LightComponent.SetLightFunctionDisabledBrightness` _directionallight (`KismetMathLibrary.Lerp` 0.5 0.696 _newtrack_0))
      (`ExponentialHeightFogComponent.SetFogDensity` _exponentialheightfog (`KismetMathLibrary.Lerp` 0.2 0.0332 _newtrack_0))
      (`ExponentialHeightFogComponent.SetFogHeightFalloff` _exponentialheightfog (`KismetMathLibrary.Lerp` 0.32084 0.2 _newtrack_0))
      (`ExponentialHeightFogComponent.SetFogInscatteringColor` _exponentialheightfog (`KismetMathLibrary.LinearColorLerp` (struct :`R` 1.0 :`G` 1.0 :`B` 1.0 :`A` 1.0) (struct :`R` 1.0 :`G` 0.407843 :`B` 0.317647 :`A` 1.0) _newtrack_0))
      (`ExponentialHeightFogComponent.SetVolumetricFogScatteringDistribution` _exponentialheightfog (`KismetMathLibrary.Lerp` 0.2 0.0 _newtrack_0)))))

(event `TransitionToHall`
  (bind _directionallight (`self.DirectionalLight`))
  (bind _exponentialheightfog (`self.ExponentialHeightFog`))
  ;[1 1 1] Trasition vers hall
  (`TimelineComponent.SetPlayRate` (`self.Hall`) (/ 1.0 5.0))
  (`LightComponent.SetEnableLightShaftBloom` (`self.DirectionalLight`) true)
  (`ExponentialHeightFogComponent.SetVolumetricFog` (`self.ExponentialHeightFog`) false)
  (bind (_direction _newtrack_0) (`Timeline|Hall`)
    (:`Update`
      (`LightComponent.SetTemperature` _directionallight (`KismetMathLibrary.Lerp` 4000.0 7241.0 _newtrack_0))
      (`LightComponent.SetIntensity` _directionallight (`KismetMathLibrary.Lerp` 10.0 1.0 _newtrack_0))
      (`LightComponent.SetVolumetricScatteringIntensity` _directionallight (`KismetMathLibrary.Lerp` 1.0 50.0 _newtrack_0))
      (`LightComponent.SetBloomScale` _directionallight (`KismetMathLibrary.Lerp` 0.2 0.02 _newtrack_0))
      (`LightComponent.SetBloomMaxBrightness` _directionallight (`KismetMathLibrary.Lerp` 100.0 5.421 _newtrack_0))
      (`DirectionalLightComponent.SetDynamicShadowDistanceMovableLight` _directionallight (`KismetMathLibrary.Lerp` 30000.0 40000.0 _newtrack_0))
      (`LightComponent.SetLightFunctionScale` _directionallight (`KismetMathLibrary.VLerp` (4235.0 4235.0 4235.0) (1024.0 1024.0 1024.0) _newtrack_0))
      (`LightComponent.SetLightFunctionFadeDistance` _directionallight (`KismetMathLibrary.Lerp` 77466.1875 100000.0 _newtrack_0))
      (`LightComponent.SetLightFunctionDisabledBrightness` _directionallight (`KismetMathLibrary.Lerp` 0.696 0.5 _newtrack_0))
      (`SkyAtmosphereComponent.SetBottomRadius` (`self.SkyAtmosphere`) (`KismetMathLibrary.Lerp` 6360.0 7000.0 _newtrack_0))
      (`ExponentialHeightFogComponent.SetFogDensity` _exponentialheightfog (`KismetMathLibrary.Lerp` 0.0332 0.05 _newtrack_0))
      (`ExponentialHeightFogComponent.SetFogHeightFalloff` _exponentialheightfog (`KismetMathLibrary.Lerp` 0.2 0.001 _newtrack_0))
      (`ExponentialHeightFogComponent.SetFogInscatteringColor` _exponentialheightfog (`KismetMathLibrary.LinearColorLerp` (struct :`R` 1.0 :`G` 0.407843 :`B` 0.317647 :`A` 1.0) (struct) _newtrack_0)))))

(fn `UserConstructionScript`
  (bind _boxmilitary (`self.BoxMilitary`))
  (bind _boxreligieuse1 (`self.BoxReligieuse1`))
  (`SceneComponent.K2_SetRelativeLocation` _boxmilitary (`self.MilitaryBoxLocation`) false false)
  (`SceneComponent.SetRelativeScale3D` _boxmilitary (`self.MilitaryBoxScale`))
  (`SceneComponent.K2_SetRelativeLocation` _boxreligieuse1 (`self.HallBoxLocation`) false false)
  (`SceneComponent.SetRelativeScale3D` _boxreligieuse1 (`self.HallBoxScale`)))
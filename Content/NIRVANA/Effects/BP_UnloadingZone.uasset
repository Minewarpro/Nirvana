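; BP_UnloadingZone is a trigger volume that unloads a streamed level when the player enters it.
; On BeginPlay it caches the first-person character, and its box overlap fires only for that character while the zone is active.
; The first valid overlap deactivates the zone, starts a non-blocking unload of the configured level, and writes the zone's level value to ActualLevel on the Game Instance.
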(event `self.ReceiveBeginPlay`
  (bind _asbp_first_person_character (cast `/Game/NIRVANA/Core/Characters/FirstPerson/BP_FirstPersonCharacter` (`GameplayStatics.GetPlayerCharacter` 0)))
  (set `self.PlayerRef` _asbp_first_person_character))

(event `self.Box.OnComponentBeginOverlap`
  (params (OverlappedComponent :type "PrimitiveComponent Object Reference") (OtherActor :type "Actor Object Reference") (OtherComp :type "PrimitiveComponent Object Reference") (OtherBodyIndex :type Integer) (bFromSweep :type Boolean) (SweepResult :type "HitResult Structure (by ref)"))
  (if (and (== OtherActor (`self.PlayerRef`)) (`self.IsActive`))
    (set `self.IsActive` false)
    (`GameplayStatics.UnloadStreamLevelBySoftObjectPtr` (`self.Level`))
    (set `/Game/NIRVANA/Core/GameModes/Game_Instance.ActualLevel` (`self.Actual Level For Instance`) (cast `/Game/NIRVANA/Core/GameModes/Game_Instance` (`GameplayStatics.GetGameInstance`) :!pure true))))

(fn `UserConstructionScript`)
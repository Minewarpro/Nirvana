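; BP_LoadingZone is a trigger volume that streams in a level when the player walks into it.
; On BeginPlay it caches the first-person player character as PlayerRef.
; When that character overlaps the Box while IsActive is set, it clears the flag and asynchronously loads the assigned Level, making it visible once loaded, so it fires only once.
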(event `self.ReceiveBeginPlay`
  (bind _asbp_first_person_character (cast `/Game/NIRVANA/Core/Characters/FirstPerson/BP_FirstPersonCharacter` (`GameplayStatics.GetPlayerCharacter` 0)))
  (set `self.PlayerRef` _asbp_first_person_character))

(event `self.Box.OnComponentBeginOverlap`
  (params (OverlappedComponent :type "PrimitiveComponent Object Reference") (OtherActor :type "Actor Object Reference") (OtherComp :type "PrimitiveComponent Object Reference") (OtherBodyIndex :type Integer) (bFromSweep :type Boolean) (SweepResult :type "HitResult Structure (by ref)"))
  (if (and (== OtherActor (`self.PlayerRef`)) (`self.IsActive`))
    (set `self.IsActive` false)
    (`GameplayStatics.LoadStreamLevelBySoftObjectPtr` (`self.Level`) true)))

(fn `UserConstructionScript`)
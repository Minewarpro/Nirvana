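; Lava spline actor that lays deformed mesh segments along a spline, with no active gameplay logic.
; The construction script adds one spline mesh per full section length, setting its material, forward axis and collision, with optional section sizing from actor X scale.
; Helper functions sample segment endpoints by distance and clamp tangents to section length.
; PositionBlending shortens each start distance in proportion to its index, so overlap grows along the spline.
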(fn `Get End Pos/Tan`
  (params (Index :type Integer))
  (returns (Position :type "Vector Structure") (Tangent :type "Vector Structure"))
  (bind _sectionlength (`self.SectionLength`))
  (bind _spline (`self.Spline`))
  (bind _returnvalue (* (+ Index 1) _sectionlength))
  (return (`SplineComponent.GetLocationAtDistanceAlongSpline` _spline _returnvalue "Local") (`KismetMathLibrary.ClampVectorSize` (`SplineComponent.GetTangentAtDistanceAlongSpline` _spline _returnvalue "Local") 0.0 _sectionlength)))

(fn `Get Start Pos/Tan`
  (params (Index :type Integer))
  (returns (Position :type "Vector Structure") (Tangent :type "Vector Structure"))
  (bind _sectionlength (`self.SectionLength`))
  (bind _spline (`self.Spline`))
  (bind _returnvalue (* Index (- _sectionlength (`self.PositionBlending`))))
  (return (`SplineComponent.GetLocationAtDistanceAlongSpline` _spline _returnvalue "Local") (`KismetMathLibrary.ClampVectorSize` (`SplineComponent.GetTangentAtDistanceAlongSpline` _spline _returnvalue "Local") 0.0 _sectionlength)))

(fn `UserConstructionScript`
  (locals (LoopIndex :type Integer))
  (bind _returnvalue_x (`KismetMathLibrary.BreakVector` (`self.GetActorScale3D`)))
  (if (`self.AllowScaling`)
    ;[1 1 1] Adding spline scaling option
    (set `self.SectionLength` (* _returnvalue_x 100.0)))
  (if true
    ;[1 1 1] Must be full length meshes.
    (for _index (range (`KismetMathLibrary.FTrunc` (/ (`SplineComponent.GetSplineLength` (`self.Spline`)) (`self.SectionLength`))))
      (set `local.LoopIndex` _index)
      (bind _returnvalue (`AddComponent|NODE_AddSplineMeshComponent-0` :!label _label))
      (`StaticMeshComponent.SetStaticMesh` _returnvalue (`self.SplineMesh`))
      (`SplineMeshComponent.SetForwardAxis` _returnvalue (`self.Set Forward Axis`) true)
      (bind (_position _tangent) (`self.Get Start Pos/Tan` (`local.LoopIndex`)))
      (bind (_position_2 _tangent_2) (`self.Get End Pos/Tan` (`local.LoopIndex`)))
      (`SplineMeshComponent.SetStartAndEnd` _returnvalue _position _tangent _position_2 _tangent_2 true)
      (`PrimitiveComponent.SetMaterial` _returnvalue 0 (`self.LavaMaterial`))
      (`PrimitiveComponent.SetCollisionEnabled` _returnvalue (`self.CollisionType`)))
    (else
      ;[1 1 1] Spline length / by section length to get number of spline meshes
      (for _index_2 (range (+ (`KismetMathLibrary.FTrunc` (/ (`SplineComponent.GetSplineLength` (`self.Spline`)) (`self.SectionLength`))) 1))
        (set `local.LoopIndex` _index_2)
        (goto _label)))))
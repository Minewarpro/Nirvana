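; Trigger actor that plays placeholder voice lines at the player's location, once, when the player enters its box while it is active.
; It plays either one sound or a recursive delay-timed sequence, read from the array's end backwards.
; A finished sequence can make a fresque grabbable or arm another trigger.
; With GameStart set, it instead plays a hardcoded intro chain at BeginPlay and deactivates itself.
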(event `self.ReceiveBeginPlay`
  (bind _asbp_first_person_character (cast `/Game/NIRVANA/Core/Characters/FirstPerson/BP_FirstPersonCharacter` (`GameplayStatics.GetPlayerCharacter` 0)))
  (set `self.PlayerRef` _asbp_first_person_character)
  (if (`self.GameStart`)
    (`self.StartGameSound`)
    (set `self.Activated` false)))

(event `self.Box.OnComponentBeginOverlap`
  (params (OverlappedComponent :type "PrimitiveComponent Object Reference") (OtherActor :type "Actor Object Reference") (OtherComp :type "PrimitiveComponent Object Reference") (OtherBodyIndex :type Integer) (bFromSweep :type Boolean) (SweepResult :type "HitResult Structure (by ref)"))
  (bind _playerref (`self.PlayerRef`))
  (if (`self.Activated`)
    (if (== OtherActor _playerref)
      (if (`self.IsSequence`)
        (set `self.Activated` false)
        (`self.SequenceVoices`)
        (else
          (`GameplayStatics.PlaySoundAtLocation` (`self.VoiceToTrigger`) (`self.K2_GetActorLocation` _playerref) (struct) (`self.Volume Multiplier`) 1.0 0.0 null null null null)
          (set `self.Activated` false))))))

(event `StartGameSound`
  (`GameplayStatics.PlaySoundAtLocation` (`self.VoiceStart`) (`self.K2_GetActorLocation` (`self.PlayerRef`)) (struct) 2.0 1.0 0.0 null null null null)
  (`KismetSystemLibrary.Delay` (+ (`SoundBase.Duration` (`self.VoiceStart`)) 0.3))
  (set `self.VoiceStart` "/Game/NIRVANA/Sound/Voices/PLAYER-ARI/J_005_V05.J_005_V05")
  (`GameplayStatics.PlaySoundAtLocation` (`self.VoiceStart`) (`self.K2_GetActorLocation` (`self.PlayerRef`)) (struct) 2.0 1.0 0.0 null null null null)
  (`KismetSystemLibrary.Delay` (+ (`SoundBase.Duration` (`self.VoiceStart`)) 0.3))
  (set `self.VoiceStart` "/Game/NIRVANA/Sound/Voices/V04-DIANA/D_008_01.D_008_01")
  (`GameplayStatics.PlaySoundAtLocation` (`self.VoiceStart`) (`self.K2_GetActorLocation` (`self.PlayerRef`)) (struct) 2.0 1.0 0.0 null null null null)
  (`KismetSystemLibrary.Delay` (+ (`SoundBase.Duration` (`self.VoiceStart`)) 0.3))
  (set `self.VoiceStart` "/Game/NIRVANA/Sound/Voices/PLAYER-ARI/J_006_V01.J_006_V01")
  (`GameplayStatics.PlaySoundAtLocation` (`self.VoiceStart`) (`self.K2_GetActorLocation` (`self.PlayerRef`)) (struct) 2.0 1.0 0.0 null null null null)
  (`KismetSystemLibrary.Delay` (+ (`SoundBase.Duration` (`self.VoiceStart`)) 0.3))
  (set `self.VoiceStart` "/Game/NIRVANA/Sound/Voices/V03-SIMON/C_009_01.C_009_01")
  (`GameplayStatics.PlaySoundAtLocation` (`self.VoiceStart`) (`self.K2_GetActorLocation` (`self.PlayerRef`)) (struct) 2.0 1.0 0.0 null null null null))

(event `SequenceVoices`
  (bind _sizeofsequence (`self.SizeOfSequence`))
  (bind _output (`|GetArrayItem` (`self.VoicesInSequence`) (- (`self.SizeOfSequence`) 1)))
  (if (> (`self.SizeOfSequence`) 0)
    (set `self.DelayForSequence` (+ (`SoundBase.Duration` _output) 0.5))
    (`GameplayStatics.PlaySoundAtLocation` _output (`self.K2_GetActorLocation` (`self.PlayerRef`)) (struct) (`self.Volume Multiplier`) 1.0 0.0 null null null null)
    (set `self.SizeOfSequence` (- _sizeofsequence 1))
    (`KismetSystemLibrary.Delay` (`self.DelayForSequence`))
    (if (> _sizeofsequence 0)
      (`self.SequenceVoices`)
      (else
        (`|ExecutionSequence`
          (:`then_0`
            (if (`self.ActivateFrasque`)
              (`self.ActivateFresque`)))
          (:`then_1`
            (if (`self.ActivateTrigger`)
              (set `/Game/DevelopersContent/Core/VoicePlaceholders/BP_VoiceTrigger.Activated` true (`self.TriggerToActivate`)))))))))

(event `ActivateFresque`
  (set `/Game/NIRVANA/Effects/Fresques/BP_FresqueUne.CanGrab` true (`self.FresqueToActivate`)))

(fn `UserConstructionScript`)
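; Enemy spawn area: a box volume, sized in the construction script, that spawns range or swarmer enemies at random points inside it.
; SpawnNPC hands the ArenaManager to range enemies and increments a non-negative NPC count; the swarmer branch does neither.
; Spawn points come from random box offsets rotated by actor yaw and projected onto the navmesh, retrying recursively when the result is near world origin.
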(fn `Add NPC`
  (params (Nb :type Integer))
  (bind _returnvalue (+ (`self.Nb NPCs`) Nb))
  (set `self.Nb NPCs` (`KismetMathLibrary.SelectInt` _returnvalue 0 (> _returnvalue 0)))
  (return))

(fn `Get Random Point in Area`
  (returns (`Random Point` :type "Vector Structure"))
  (locals (ImpactPoint :type "Vector Structure"))
  (bind (_returnvalue_roll _returnvalue_pitch _returnvalue_yaw) (`KismetMathLibrary.BreakRotator` (`self.K2_GetActorRotation`)))
  (bind _box (`self.Box`))
  (bind _returnvalue (`SceneComponent.K2_GetComponentLocation` _box))
  (bind _returnvalue_2 (`KismetMathLibrary.RandomPointInBoundingBox` _returnvalue (* (`BoxComponent.BoxExtent` _box) (`self.GetActorScale3D`))))
  (bind _output_get (set `local.ImpactPoint` (`NavigationSystemV1.K2_ProjectPointToNavigation` (+ (* (`KismetMathLibrary.RotateAngleAxis` (`KismetMathLibrary.GetDirectionUnitVector` _returnvalue _returnvalue_2) _returnvalue_yaw (0.0 0.0 1.0)) (`KismetMathLibrary.Vector_Distance` _returnvalue_2 _returnvalue)) _returnvalue) null null (1.0 1.0 300.0))))
  (if (== _output_get (0.0 0.0 0.0) :`ErrorTolerance` 100.0)
    (`self.Get Random Point in Area`)
    (else
      (return (`local.ImpactPoint`)))))

(fn `SpawnNPC`
  (params (ArenaManager :type "/Game/NIRVANA/Core/Placeables/Management/BP_ArenaManager Object Reference"))
  (returns (`Spawned npc` :type "/Game/NIRVANA/Core/Characters/Enemies/Range/BP_EnemyRange Object Reference"))
  (bind _random_point (`self.Get Random Point in Area`))
  (bind _asbp_enemy_range (castclass `/Game/NIRVANA/Core/Characters/Enemies/Range/BP_EnemyRange` null)
    (:`then`
      (bind _returnvalue (`|SpawnActorFromClass` _asbp_enemy_range (`KismetMathLibrary.MakeTransform` _random_point) "Undefined" "MultiplyWithRoot" null ArenaManager null))
      (`self.Add NPC` 1)
      (return _returnvalue))
    (:`CastFailed`
      (`|SpawnActorFromClass` (castclass `/Game/NIRVANA/Core/Characters/Enemies/Swarmer/BP_EnemySwarmer` null :!pure true) (`KismetMathLibrary.MakeTransform` _random_point) "Undefined" "MultiplyWithRoot" null null null)
      (return null))))

(fn `UserConstructionScript`
  (`BoxComponent.SetBoxExtent` (`self.Box`) (`self.In Box Extent`) true))
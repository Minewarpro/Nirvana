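; Boss root appendage for BP_Boss_P1 that stretches into the arena, swipes and damages the player on touch.
; Stretch and Shrink lerp the actor along Y while setting AnimBP state flags, then notify the boss.
; Timeline-driven rotations perform recursive horizontal sweeps, raise-and-slam vertical swipes and angled side swipes, ending in Withdraw, which resets rotation and reports back.
; The construction script attaches overlap capsules to all but the last mesh socket.
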(event `SetABP_Ref`
  (params (ABP :type "/Game/DevelopersContent/Core/Characters/Enemies/Boss/Root/ABP_root Object Reference"))
  (set `self.ABP_Skeleton` ABP))

(event `self.ReceiveBeginPlay`
  ;[1 0.6941 0.1255 1 24] Begin
  (bind _asbp_first_person_character (cast `/Game/NIRVANA/Core/Characters/FirstPerson/BP_FirstPersonCharacter` (`GameplayStatics.GetPlayerCharacter` 0))
    (:`then`
      (set `self.PlayerRef` _asbp_first_person_character))
    (:`CastFailed`
      _))
  (bind _returnvalue (`GameplayStatics.GetActorOfClass` "/Game/DevelopersContent/Core/Characters/Enemies/Boss/BP_Boss_P1.BP_Boss_P1_C"))
  (set `self.Boss` _returnvalue)
  (bind _output_get (set `self.InitPos` (`self.K2_GetActorLocation`)))
  (`self.K2_SetActorLocation` (- _output_get (0.0 1500.0 0.0))))

(event `CapsuleBeginOverlap`
  (params (OverlappedComponent :type "PrimitiveComponent Object Reference") (OtherActor :type "Actor Object Reference") (OtherComp :type "PrimitiveComponent Object Reference") (OtherBodyIndex :type Integer) (bFromSweep :type Boolean) (SweepResult :type "HitResult Structure (by ref)"))
  (bind _playerref (`self.PlayerRef`))
  ;[0.6213 0.4386 1] Player Hit
  (if (== OtherActor _playerref)
    (`/Game/NIRVANA/Core/Characters/FirstPerson/BP_FirstPersonCharacter.Take Damage` _playerref 5.0 null)))

(event `Stretch`
  (bind _initpos (`self.InitPos`))
  (bind _abp_skeleton (`self.ABP_Skeleton`))
  ;[1 1 1] States Change
  (`TimelineComponent.SetPlayRate` (`self.TL_Stretch`) (/ 1.0 6.0))
  (set `/Game/DevelopersContent/Core/Characters/Enemies/Boss/Root/ABP_root.Withdraw` false _abp_skeleton)
  (set `/Game/DevelopersContent/Core/Characters/Enemies/Boss/Root/ABP_root.ChangeState` true _abp_skeleton)
  (set `/Game/DevelopersContent/Core/Characters/Enemies/Boss/Root/ABP_root.InstantShrink` false _abp_skeleton)
  (bind (_direction _progress) (`Timeline|TL_Stretch` :!via `PlayFromStart`)
    (:`Update`
      (`self.K2_SetActorLocation` (`KismetMathLibrary.VLerp` (- _initpos (0.0 1500.0 0.0)) _initpos _progress)))
    (:`Finished`
      (set `/Game/DevelopersContent/Core/Characters/Enemies/Boss/Root/ABP_root.ChangeState` false (`self.ABP_Skeleton`))
      (`/Game/DevelopersContent/Core/Characters/Enemies/Boss/BP_Boss_P1.OnRootStretched` (`self.Boss`)))))

(event `Shrink`
  (bind _initpos (`self.InitPos`))
  (bind _abp_skeleton (`self.ABP_Skeleton`))
  ;[1 1 1] States Change
  (`TimelineComponent.SetPlayRate` (`self.TL_Shrink`) (/ 1.0 6.0))
  (set `/Game/DevelopersContent/Core/Characters/Enemies/Boss/Root/ABP_root.Withdraw` true _abp_skeleton)
  (set `/Game/DevelopersContent/Core/Characters/Enemies/Boss/Root/ABP_root.ChangeState` true _abp_skeleton)
  (set `/Game/DevelopersContent/Core/Characters/Enemies/Boss/Root/ABP_root.InstantShrink` false _abp_skeleton)
  (bind (_direction _progress) (`Timeline|TL_Shrink` :!via `PlayFromStart`)
    (:`Update`
      (`self.K2_SetActorLocation` (`KismetMathLibrary.VLerp` _initpos (- _initpos (0.0 1500.0 0.0)) _progress)))
    (:`Finished`
      (`/Game/DevelopersContent/Core/Characters/Enemies/Boss/BP_Boss_P1.OnRootShrinked` (`self.Boss`)))))

(event `Withdraw`
  (bind (_initrot_roll _initrot_pitch _initrot_yaw) (`KismetMathLibrary.BreakRotator` (`self.InitRot`)))
  ;[1 0.6941 0.1255] Withdraw
  (set `self.InitRot` (`self.K2_GetActorRotation`))
  (`TimelineComponent.SetPlayRate` (`self.TL_Vertical`) (/ 1.0 (`self.SwipeDuration`)))
  (bind (_direction _x _y _z) (`Timeline|TL_Withdraw` :!via `PlayFromStart`)
    (:`Update`
      (`self.K2_SetActorRelativeRotation` (`KismetMathLibrary.MakeRotator` (`KismetMathLibrary.Lerp` _initrot_roll 0.0 _x) (`KismetMathLibrary.Lerp` _initrot_pitch 0.0 _y) (`KismetMathLibrary.Lerp` _initrot_yaw 0.0 _z))))
    (:`Finished`
      (`/Game/DevelopersContent/Core/Characters/Enemies/Boss/BP_Boss_P1.OnRootFinishSwipe` (`self.Boss`) self))))

(event `HorizontalSwipe`
  (params (Count :type Integer :default 1) (Angle :type "Float (double-precision)" :default 40.0))
  (bind _returnvalue (/ Angle 2.0))
  (bind (_initrot_roll _initrot_pitch _initrot_yaw) (`KismetMathLibrary.BreakRotator` (`self.InitRot`)))
  (bind _returnvalue_2 (`KismetMathLibrary.SelectFloat` _returnvalue (* _returnvalue -1.0) (`self.Left`)))
  ;[1 1 1] Horizontal
  (set `self.InitRot` (`self.K2_GetActorRotation`))
  (if (> Count 0)
    (`TimelineComponent.SetPlayRate` (`self.TL_Horizontal`) (/ 1.0 (`self.SwipeDuration`)))
    (bind (_direction _progress) (`Timeline|TL_Horizontal` :!via `PlayFromStart`)
      (:`Update`
        (`self.K2_SetActorRelativeRotation` (`KismetMathLibrary.MakeRotator` _initrot_roll _initrot_pitch (`KismetMathLibrary.Lerp` _initrot_yaw (+ _initrot_yaw (`KismetMathLibrary.SelectFloat` _returnvalue_2 (* _returnvalue_2 2.0) (`self.First`))) _progress))))
      (:`Finished`
        (set `self.Left` (not (`self.Left`)))
        (set `self.First` false)
        (`self.HorizontalSwipe` (- Count 1) Angle)))
    (else
      (set `self.First` true)
      (`self.Withdraw`))))

(event `VerticalSwipe`
  (params (Height :type "Float (double-precision)" :default 65.0))
  (bind (_initrot_roll _initrot_pitch _initrot_yaw) (`KismetMathLibrary.BreakRotator` (`self.InitRot`)))
  (bind _tl_vertical (`self.TL_Vertical`))
  ;[1 1 1] Vertical
  (set `self.InitRot` (`self.K2_GetActorRotation`))
  (`TimelineComponent.SetPlayRate` _tl_vertical (/ 1.0 (`self.SwipeDuration`)))
  (bind (_direction _x) (`Timeline|TL_Vertical` :!via `PlayFromStart` :!label _label)
    (:`Update`
      (`self.K2_SetActorRelativeRotation` (`KismetMathLibrary.MakeRotator` (`KismetMathLibrary.Lerp` _initrot_roll (* Height -1.0) _x) _initrot_pitch _initrot_yaw)))
    (:`Finished`
      (`/Engine/EditorBlueprintResources/StandardMacros.FlipFlop`
        (:`A`
          (`KismetSystemLibrary.Delay` 0.8)
          (`TimelineComponent.SetPlayRate` _tl_vertical (/ 1.0 (/ (`self.SwipeDuration`) 10.0)))
          (goto _label :!via `ReverseFromEnd`))
        (:`B`
          (`self.Withdraw`))))))

(event `VerticalSideSwipe`
  (params (Left :type Boolean :default true) (Height :type "Float (double-precision)" :default 65.0) (Angle :type "Float (double-precision)" :default 25.0))
  (bind _returnvalue (* Height -1.0))
  (bind (_initrot_roll _initrot_pitch) (`KismetMathLibrary.BreakRotator` (`self.InitRot`)))
  (bind (_initrot_roll_2 _initrot_pitch_2 _initrot_yaw) (`KismetMathLibrary.BreakRotator` (`self.InitRot`)))
  (bind _returnvalue_2 (* (`KismetMathLibrary.SelectFloat` -1.0 1.0 Left) Angle))
  ;[1 1 1] Vertical Side
  (set `self.InitRot` (`self.K2_GetActorRotation`))
  (`TimelineComponent.SetPlayRate` (`self.TL_VerticalSide`) (/ 1.0 (`self.SwipeDuration`)))
  (set `self.CurrentMovement` "NewEnumerator0")
  (bind (_direction _progress) (`Timeline|TL_VerticalSide` :!via `PlayFromStart` :!label _label_2)
    (:`Update`
      (switch `/Game/DevelopersContent/Core/Characters/Enemies/Boss/Root/Enum_Root` (`self.CurrentMovement`)
        (:`NewEnumerator0`
          (`self.K2_SetActorRelativeRotation` (`KismetMathLibrary.MakeRotator` (`KismetMathLibrary.Lerp` _initrot_roll_2 _returnvalue _progress) _initrot_pitch_2 (`KismetMathLibrary.Lerp` _initrot_yaw _returnvalue_2 _progress))))
        (:`NewEnumerator1`
          (`self.K2_SetActorRelativeRotation` (`KismetMathLibrary.MakeRotator` (`KismetMathLibrary.Lerp` _returnvalue _initrot_roll _progress) _initrot_pitch _returnvalue_2)))))
    (:`Finished`
      (switch `/Game/DevelopersContent/Core/Characters/Enemies/Boss/Root/Enum_Root` (`self.CurrentMovement`)
        (:`NewEnumerator0`
          (set `self.CurrentMovement` "NewEnumerator1")
          (`TimelineComponent.SetPlayRate` (`self.TL_VerticalSide`) (/ 1.0 (`self.SwipeDuration`)))
          (goto _label_2 :!via `PlayFromStart`))
        (:`NewEnumerator1`
          (`self.Withdraw`))))))

(fn `UserConstructionScript`
  (bind _root (`self.root`))
  (bind _returnvalue (`SceneComponent.GetAllSocketNames` (`self.root`)))
  (for _array_element _returnvalue
    (if (!= (`|GetArrayItem` _returnvalue (`KismetArrayLibrary.Array_LastIndex` _returnvalue)) _array_element)
      (if (== (`|GetArrayItem` _returnvalue) _array_element)
        (bind _returnvalue_2 (`AddComponent|NODE_AddCapsuleComponent-1` :`bManualAttachment` true))
        (add `PrimitiveComponent.OnComponentBeginOverlap` _returnvalue_2 (`|CreateDelegate` :!event `CapsuleBeginOverlap`))
        (`SceneComponent.K2_AttachToComponent` _returnvalue_2 _root _array_element "KeepRelative" "KeepRelative" "KeepRelative" true)
        (else
          (bind _returnvalue_3 (`AddComponent|NODE_AddCapsuleComponent-0` :`bManualAttachment` true))
          (add `PrimitiveComponent.OnComponentBeginOverlap` _returnvalue_3 (`|CreateDelegate` :!event `CapsuleBeginOverlap`))
          (`SceneComponent.K2_AttachToComponent` _returnvalue_3 _root _array_element "KeepRelative" "KeepRelative" "KeepRelative" true))))))
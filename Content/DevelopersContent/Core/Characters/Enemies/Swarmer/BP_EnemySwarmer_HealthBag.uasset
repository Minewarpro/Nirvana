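; Swarmer enemy variant that acts as a respawning health source, calling SpawnHealth when killed.
; Hits reduce health, update the life bar and crosshair, flash the material and drive a timeline-blended physical-animation stagger on bones below the spine.
; Death plays a montage alongside a material and Niagara dissolve.
; After dissolving, the actor hides off-map, then returns to its starting position with full health.
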(event `self.ReceiveBeginPlay`
  (bind _asbp_first_person_character (cast `/Game/NIRVANA/Core/Characters/FirstPerson/BP_FirstPersonCharacter` (`GameplayStatics.GetPlayerCharacter` 0)))
  (set `self.PlayerRef` _asbp_first_person_character)
  (set `self.CurrentHealth` (`self.MaxHealth`))
  (set `self.InitPos` (`self.K2_GetActorLocation`))
  (`PhysicalAnimationComponent.SetSkeletalMeshComponent` (`self.PhysicalAnimation`) (`self.Mesh`))
  (`PhysicalAnimationComponent.ApplyPhysicalAnimationSettingsBelow` (`self.PhysicalAnimation`) "Bind_Spine_01" (make `PhysicalAnimationData` true 60.0 15.0 50.0 50.0) false)
  (`SkeletalMeshComponent.SetAllBodiesBelowSimulatePhysics` (`self.Mesh`) "Bind_Spine_01" true false)
  (`SkeletalMeshComponent.SetAllBodiesBelowPhysicsBlendWeight` (`self.Mesh`) "Bind_Spine_01" 0.0 false false))

(event `self.Dissolve`
  (`TimelineComponent.SetPlayRate` (`self.Dissolve TL`) (/ 1.0 1.6))
  (bind (_direction _alpha_dissolve) (`Timeline|Timeline_2`)
    (:`Update`
      (`MeshComponent.SetScalarParameterValueOnMaterials` (`self.Mesh`) "Alpha" _alpha_dissolve)
      (`NiagaraComponent.SetVariableFloat` (`self.NS_Dissolve`) "Alpha" _alpha_dissolve))
    (:`Finished`
      (`KismetSystemLibrary.Delay` 1.0)
      (`self.SetActorHiddenInGame` true)
      (`self.K2_SetActorLocation` (9999999.0 999999.0 0.0))
      (`KismetSystemLibrary.Delay` 2.0)
      (`self.K2_SetActorLocation` (`self.InitPos`))
      (`self.SetActorHiddenInGame` false)
      (`MeshComponent.SetScalarParameterValueOnMaterials` (`self.Mesh`) "Alpha" 0.0)
      (`NiagaraComponent.SetVariableFloat` (`self.NS_Dissolve`) "Alpha" 0.0)
      (set `self.dying` false)
      (set `self.CurrentHealth` (`self.MaxHealth`)))))

(event `self.Hit`
  (params (Damages :type "Float (double-precision)"))
  (`|ExecutionSequence`
    (:`then_0`
      (`self.Cross hair hit alpha decrease `)
      (set `self.CurrentHealth` (- (`self.CurrentHealth`) Damages))
      (if (<= (`self.CurrentHealth`) 0.0)
        (`self.Death`)
        (else
          (`self.SetLifeBar`)
          (`MeshComponent.SetScalarParameterValueOnMaterials` (`self.Mesh`) "Hit" 0.1)
          (`KismetSystemLibrary.Delay` 0.2)
          (`MeshComponent.SetScalarParameterValueOnMaterials` (`self.Mesh`) "Hit" 0.0))))
    (:`then_1`
      (`SkeletalMeshComponent.SetAllBodiesBelowPhysicsBlendWeight` (`self.Mesh`) "Bind_Spine_01" 1.0 false false)
      (`TimelineComponent.SetPlayRate` (`self.TStagger`) (/ 1.0 0.35))
      (if (`self.Stagging`)
        (bind (_direction _newtrack_0) (`Timeline|Timeline_1` :!label _label)
          (:`Update`
            (set `self.Stagging` true)
            (`SkeletalMeshComponent.SetAllBodiesBelowPhysicsBlendWeight` (`self.Mesh`) "Bind_Spine_01" _newtrack_0 false false))
          (:`Finished`
            (`SkeletalMeshComponent.ResetAllBodiesSimulatePhysics` (`self.Mesh`))
            (`SkeletalMeshComponent.SetAllBodiesBelowPhysicsBlendWeight` (`self.Mesh`) "Bind_Spine_01" 0.0 false true)
            (set `self.Stagging` false)))
        (else
          (goto _label :!via `PlayFromStart`))))))

(event `self.Death`
  (if (not (`self.dying`))
    (set `self.dying` true)
    (`|PlayMontage` (`self.Mesh`) "/Game/NIRVANA/Core/Characters/Enemies/Range/Anims/Death_Montage.Death_Montage" 1.2
      (:`then`
        (`self.Dissolve`)
        (`self.SpawnHealth`)))))

(fn `UserConstructionScript`
  (`parent.UserConstructionScript`))
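; Walking variant of the Swarmer enemy that paces back and forth along a straight line from its spawn point.
; On BeginPlay it caches the player character and its start location, stopping if the player cast fails.
; Two AIMoveTo events then alternate between a Distance offset on world Y and the origin, each triggering the other on success or failure.
; The stored player reference is unused in this graph.
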(event `/Game/NIRVANA/Core/Characters/FirstPerson/BPI_Hit.Hit`
  (params (Damages :type "Float (double-precision)") (Impulse :type "Vector Structure") (Location :type "Vector Structure") (Bone :type Name)))

(event `self.ReceiveBeginPlay`
  (bind _asbp_first_person_character (cast `/Game/NIRVANA/Core/Characters/FirstPerson/BP_FirstPersonCharacter` (`GameplayStatics.GetPlayerCharacter` 0)))
  (set `self.PlayerRef` _asbp_first_person_character)
  (set `self.InitPos` (`self.K2_GetActorLocation`))
  (`self.MoveTarget`))

(event `MoveTarget`
  (bind _movementresult (`|AIMoveTo` self (+ (`self.InitPos`) (`KismetMathLibrary.MakeVector` 0.0 (`self.Distance`))) null)
    (:`then`
      (`KismetSystemLibrary.PrintString` (`|GetEnumeratorNameAsString` _movementresult)))
    (:`OnSuccess`
      (`self.MoveOrigin` :!label _label))
    (:`OnFail`
      (goto _label))))

(event `MoveOrigin`
  (`|AIMoveTo` self (`self.InitPos`) null
    (:`OnSuccess`
      _)
    (:`OnFail`
      _))
  (`self.MoveTarget`))

(fn `UserConstructionScript`
  (`parent.UserConstructionScript`))
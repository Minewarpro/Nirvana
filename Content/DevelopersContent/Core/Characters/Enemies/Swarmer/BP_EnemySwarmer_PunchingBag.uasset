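; Punching-bag variant of the Swarmer enemy that reacts to hits with a material flash and a physics-driven stagger.
; BeginPlay stores the player character and sets up Physical Animation with simulated bodies below Bind_Spine_01, starting with zero physics blend.
; Hit briefly raises the "Hit" material parameter and sets full physics blend below the spine.
; A timeline then drives that blend weight and restores the animated pose on finish.
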(event `self.ReceiveBeginPlay`
  (bind _asbp_first_person_character (cast `/Game/NIRVANA/Core/Characters/FirstPerson/BP_FirstPersonCharacter` (`GameplayStatics.GetPlayerCharacter` 0)))
  (set `self.PlayerRef` _asbp_first_person_character)
  (`PhysicalAnimationComponent.SetSkeletalMeshComponent` (`self.PhysicalAnimation`) (`self.Mesh`))
  (`PhysicalAnimationComponent.ApplyPhysicalAnimationSettingsBelow` (`self.PhysicalAnimation`) "Bind_Spine_01" (make `PhysicalAnimationData` true 60.0 15.0 50.0 50.0) false)
  (`SkeletalMeshComponent.SetAllBodiesBelowSimulatePhysics` (`self.Mesh`) "Bind_Spine_01" true false)
  (`SkeletalMeshComponent.SetAllBodiesBelowPhysicsBlendWeight` (`self.Mesh`) "Bind_Spine_01" 0.0 false false))

(event `/Game/NIRVANA/Core/Characters/FirstPerson/BPI_Hit.Hit`
  (params (Damages :type "Float (double-precision)"))
  (`|ExecutionSequence`
    (:`then_0`
      (`MeshComponent.SetScalarParameterValueOnMaterials` (`self.Mesh`) "Hit" 0.1)
      (`KismetSystemLibrary.Delay` 0.2)
      (`MeshComponent.SetScalarParameterValueOnMaterials` (`self.Mesh`) "Hit" 0.0))
    (:`then_1`
      (`SkeletalMeshComponent.SetAllBodiesBelowPhysicsBlendWeight` (`self.Mesh`) "Bind_Spine_01" 1.0 false false)
      (`TimelineComponent.SetPlayRate` (`self.TStagger`) (/ 1.0 0.35))
      (if (`self.Stagging`)
        (bind (_direction _newtrack_0) (`Timeline|Timeline_1` :!label _label)
          (:`Update`
            (set `self.Stagging` true)
            (`SkeletalMeshComponent.SetAllBodiesBelowPhysicsBlendWeight` (`self.Mesh`) "Bind_Spine_01" _newtrack_0 false false))
          (:`Finished`
            (`SkeletalMeshComponent.ResetAllBodiesSimulatePhysics` (`self.Mesh`))
            (`SkeletalMeshComponent.SetAllBodiesBelowPhysicsBlendWeight` (`self.Mesh`) "Bind_Spine_01" 0.0 false true)
            (set `self.Stagging` false)))
        (else
          (goto _label :!via `PlayFromStart`))))))

(fn `UserConstructionScript`
  (`parent.UserConstructionScript`))
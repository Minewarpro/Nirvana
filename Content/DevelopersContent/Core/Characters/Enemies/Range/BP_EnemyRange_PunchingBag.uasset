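; Punching-bag variant of the ranged enemy that flashes and physically staggers when hit.
; BeginPlay caches the first-person player and configures physical animation below the pelvis bone.
; Hit briefly raises a material parameter, then a timeline drives the physics blend weight of those bodies, continuing if already staggering.
; When the timeline finishes, it resets body simulation and clears the stagger flag.
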(event `self.ReceiveBeginPlay`
  (bind _asbp_first_person_character (cast `/Game/NIRVANA/Core/Characters/FirstPerson/BP_FirstPersonCharacter` (`GameplayStatics.GetPlayerCharacter` 0)))
  (set `self.PlayerRef` _asbp_first_person_character)
  (`PhysicalAnimationComponent.SetSkeletalMeshComponent` (`self.PhysicalAnimation`) (`self.Mesh`))
  (`PhysicalAnimationComponent.ApplyPhysicalAnimationSettingsBelow` (`self.PhysicalAnimation`) "Bind_Pelvis" (make `PhysicalAnimationData` true 350.0 100.0 50.0 50.0) false)
  (`SkeletalMeshComponent.SetAllBodiesBelowSimulatePhysics` (`self.Mesh`) "Bind_Pelvis" true false)
  (`SkeletalMeshComponent.SetAllBodiesBelowPhysicsBlendWeight` (`self.Mesh`) "Bind_Pelvis" 0.0 false false))

(event `/Game/NIRVANA/Core/Characters/FirstPerson/BPI_Hit.Hit`
  (params (Damages :type "Float (double-precision)") (Impulse :type "Vector Structure") (Location :type "Vector Structure") (Bone :type Name))
  (`|ExecutionSequence`
    (:`then_0`
      (`MeshComponent.SetScalarParameterValueOnMaterials` (`self.Mesh`) "Hit" 0.1)
      (`KismetSystemLibrary.Delay` 0.2)
      (`MeshComponent.SetScalarParameterValueOnMaterials` (`self.Mesh`) "Hit" 0.0))
    (:`then_1`
      (`SkeletalMeshComponent.SetAllBodiesBelowPhysicsBlendWeight` (`self.Mesh`) "Bind_Pelvis" 1.0 false false)
      (`TimelineComponent.SetPlayRate` (`self.TStagger`) (/ 1.0 0.35))
      (if (`self.Stagging`)
        (bind (_direction _newtrack_0) (`Timeline|Timeline_1` :!label _label)
          (:`Update`
            (set `self.Stagging` true)
            (`SkeletalMeshComponent.SetAllBodiesBelowPhysicsBlendWeight` (`self.Mesh`) "Bind_Pelvis" _newtrack_0 false false))
          (:`Finished`
            (`SkeletalMeshComponent.ResetAllBodiesSimulatePhysics` (`self.Mesh`))
            (`SkeletalMeshComponent.SetAllBodiesBelowPhysicsBlendWeight` (`self.Mesh`) "Bind_Pelvis" 0.0 false true)
            (set `self.Stagging` false)))
        (else
          (goto _label :!via `PlayFromStart`))))))

(fn `UserConstructionScript`
  (`parent.UserConstructionScript`))
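; BP_AR is an assault rifle weapon that fires hitscan shots from the player's camera, rate-limited by a delay.
; FireHold plays the first-person fire montage and sphere-traces within a random spread cone.
; A wide trace gives aim forgiveness, retried with a narrow one when it hits WorldStatic geometry.
; Blocking hits send damage through HitMessage and play a shotgun sound; ammo check and decrement are disconnected.
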(event `self.ReceiveBeginPlay`
  (`parent.ReceiveBeginPlay`))

(event `self.Fire Hold`
  (bind _firstpersoncamera (`/Game/NIRVANA/Core/Characters/FirstPerson/BP_FirstPersonCharacter.FirstPersonCamera` (`self.Player Ref`)))
  (bind _returnvalue (`SceneComponent.K2_GetComponentLocation` _firstpersoncamera))
  (bind _returnvalue_2 (`KismetMathLibrary.GetForwardVector` (`SceneComponent.K2_GetComponentRotation` _firstpersoncamera)))
  (bind _returnvalue_3 (+ _returnvalue (* (`KismetMathLibrary.RandomUnitVectorInConeInDegrees` _returnvalue_2 (`self.Cone Half Angle in Degrees`)) 99999999.0)))
  ;[0.1771 0.04611 0.05078] Fire
  (if (`self.CanShoot`)
    (`|ExecutionSequence`
      (:`then_0`
        (`KismetSystemLibrary.Delay` (`self.Delay Shoot`))
        (set `self.CanShoot` true))
      (:`then_1`
        (set `self.CanShoot` false)
        (`self.ShootAnimation`)
        (bind _outhit (`KismetSystemLibrary.SphereTraceSingle` :`Start` (+ _returnvalue (* _returnvalue_2 50.0)) :`End` _returnvalue_3 :`Radius` 65.0 :`TraceChannel` "TraceTypeQuery4" :`bTraceComplex` true :`DrawTime` 2.0))
        (bind (_bblockinghit _binitialoverlap _time _distance _location _impactpoint _normal _impactnormal _physmat _hitactor _hitcomponent) (`GameplayStatics.BreakHitResult` _outhit))
        (`KismetSystemLibrary.PrintString` (`KismetSystemLibrary.GetDisplayName` _hitactor))
        (if (`|EnumEquality` (`PrimitiveComponent.GetCollisionObjectType` _hitcomponent) "ECC_WorldStatic")
          (bind _outhit_2 (`KismetSystemLibrary.SphereTraceSingle` :`Start` _returnvalue :`End` _returnvalue_3 :`Radius` 5.0 :`TraceChannel` "TraceTypeQuery4" :`bTraceComplex` true :`DrawTime` 2.0))
          (bind (_bblockinghit_2 _binitialoverlap_2 _time_2 _distance_2 _location_2 _impactpoint_2 _normal_2 _impactnormal_2 _physmat_2 _hitactor_2) (`GameplayStatics.BreakHitResult` _outhit_2))
          (if _bblockinghit_2
            (message `/Game/NIRVANA/Core/Characters/FirstPerson/BPI_Hit.Hit` _hitactor_2 (`self.Damages`) (0.0 0.0 0.0) (0.0 0.0 0.0) "None")
            (`GameplayStatics.PlaySound2D` "/Game/DevelopersContent/Core/Weapons/ShotGun/Sound/ShotGun_Fire.ShotGun_Fire" 1.0 1.0 0.0 null null))
          (elif _bblockinghit
            (message `/Game/NIRVANA/Core/Characters/FirstPerson/BPI_Hit.Hit` _hitactor (`self.Damages`) (0.0 0.0 0.0) (0.0 0.0 0.0) "None")
            (`GameplayStatics.PlaySound2D` "/Game/DevelopersContent/Core/Weapons/ShotGun/Sound/ShotGun_Fire.ShotGun_Fire" 1.0 1.0 0.0 null null)))))))

(event `ShootAnimation`
  ;[0.4583 1 0.8771] Animaton
  (`|PlayMontage` (`/Game/NIRVANA/Core/Characters/FirstPerson/BP_FirstPersonCharacter.Mesh_1P` (`self.Player Ref`)) "/Game/DevelopersContent/Core/Characters/FirstPerson/Animations/ARs/A_FP_PCH_AR_Fire_Montage.A_FP_PCH_AR_Fire_Montage"))

(fn `UserConstructionScript`
  (`parent.UserConstructionScript`))
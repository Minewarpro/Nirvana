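; Big Uzi projectile Blueprint that launches along its direction and explodes on contact with anything other than the player, or after a timeout.
; BeginPlay sets the collision component's physics velocity, and overlap or hit events trigger Destroy.
; Destroy plays Niagara and audio effects, sends HitMessage damage to filtered actor classes in a sphere overlap, then removes the projectile and collision components before delayed actor destruction.
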(event `Destroy`
  (bind _ns_aoe_explosion_2 (`self.NS_AOE_Explosion_2`))
  (`SceneComponent.SetVisibility` _ns_aoe_explosion_2 true false)
  (`ActorComponent.Activate` _ns_aoe_explosion_2 false)
  (`AddComponent|NODE_AddAudioComponent-1`)
  (for _array_element (`self.Actor Class Filter`)
    (bind _outactors (`KismetSystemLibrary.SphereOverlapActors` (`SceneComponent.K2_GetComponentLocation` (`self.Collision`)) 850.0 (`self.Object Types`) _array_element))
    (`|ExecutionSequence`
      (:`then_1`
        (for _array_element_2 _outactors
          (message `/Game/NIRVANA/Core/Characters/FirstPerson/BPI_Hit.Hit` _array_element_2 (`self.Damage`) (0.0 0.0 0.0) (0.0 0.0 0.0) "None")))))
  (`ActorComponent.K2_DestroyComponent` (`self.Projectile`))
  (`ActorComponent.K2_DestroyComponent` (`self.Collision`))
  (`KismetSystemLibrary.Delay` 5.0)
  (`self.K2_DestroyActor`))

(event `self.Collision.OnComponentBeginOverlap`
  (params (OverlappedComponent :type "PrimitiveComponent Object Reference") (OtherActor :type "Actor Object Reference") (OtherComp :type "PrimitiveComponent Object Reference") (OtherBodyIndex :type Integer) (bFromSweep :type Boolean) (SweepResult :type "HitResult Structure (by ref)"))
  (if (!= OtherActor (`self.Player Ref`))
    (`self.Destroy` :!label _label)))

(event `self.Collision.OnComponentHit`
  (params (HitComponent :type "PrimitiveComponent Object Reference") (OtherActor :type "Actor Object Reference") (OtherComp :type "PrimitiveComponent Object Reference") (NormalImpulse :type "Vector Structure") (Hit :type "HitResult Structure (by ref)"))
  (if (!= OtherActor (`self.Player Ref`))
    (goto _label)))

(event `self.ReceiveBeginPlay`
  (`PrimitiveComponent.SetPhysicsLinearVelocity` (`self.Collision`) (* (`self.Direction`) (`self.Speed`)) false "None")
  (`KismetSystemLibrary.Delay` 10.0)
  (`self.Destroy`))

(fn `UserConstructionScript`)
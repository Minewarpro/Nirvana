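; BP_DoorClose is a placeable trigger that moves two referenced door actors when the player enters its box, closing them going by the asset name.
; It caches the first-person character on BeginPlay and responds only to that actor's overlap.
; If Activated is set, it instantly shifts DoorLeft and DoorRight in opposite directions along world Y by a fixed offset, then clears the flag so it does not repeat.
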(event `self.ReceiveBeginPlay`
  (bind _asbp_first_person_character (cast `/Game/NIRVANA/Core/Characters/FirstPerson/BP_FirstPersonCharacter` (`GameplayStatics.GetPlayerCharacter` 0)))
  (set `self.PlayerRef` _asbp_first_person_character))

(event `self.Box.OnComponentBeginOverlap`
  (params (OverlappedComponent :type "PrimitiveComponent Object Reference") (OtherActor :type "Actor Object Reference") (OtherComp :type "PrimitiveComponent Object Reference") (OtherBodyIndex :type Integer) (bFromSweep :type Boolean) (SweepResult :type "HitResult Structure (by ref)"))
  (bind _doorleft (`self.DoorLeft`))
  (bind _doorright (`self.DoorRight`))
  (bind (_returnvalue_x _returnvalue_y _returnvalue_z) (`KismetMathLibrary.BreakVector` (`self.K2_GetActorLocation` _doorleft)))
  (bind (_returnvalue_x_2 _returnvalue_y_2 _returnvalue_z_2) (`KismetMathLibrary.BreakVector` (`self.K2_GetActorLocation` _doorright)))
  (if (== OtherActor (`self.PlayerRef`))
    (if (`self.Activated`)
      (`self.K2_SetActorLocation` _doorleft (`KismetMathLibrary.MakeVector` _returnvalue_x (+ _returnvalue_y 700.0) _returnvalue_z) false false)
      (`self.K2_SetActorLocation` _doorright (`KismetMathLibrary.MakeVector` _returnvalue_x_2 (- _returnvalue_y_2 700.0) _returnvalue_z_2) false false)
      (set `self.Activated` false))))

(fn `UserConstructionScript`)
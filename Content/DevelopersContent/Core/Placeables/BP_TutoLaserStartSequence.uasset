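; Tutorial trigger box that switches a set of lasers on or off when the player enters it, optionally slowing time for a tutorial moment.
; Overlap fires once, then creates or shuts down every referenced laser depending on StartLoop.
; With SlowMotion enabled, a timeline ramps global time dilation down to near standstill, and pressing the dash input reverses it back to normal speed.
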(event `self.ReceiveBeginPlay`
  (bind _asbp_first_person_character (cast `/Game/NIRVANA/Core/Characters/FirstPerson/BP_FirstPersonCharacter` (`GameplayStatics.GetPlayerCharacter` 0)))
  (set `self.PlayerRef` _asbp_first_person_character))

(event `self.Box.OnComponentBeginOverlap`
  (params (OverlappedComponent :type "PrimitiveComponent Object Reference") (OtherActor :type "Actor Object Reference") (OtherComp :type "PrimitiveComponent Object Reference") (OtherBodyIndex :type Integer) (bFromSweep :type Boolean) (SweepResult :type "HitResult Structure (by ref)"))
  (if (and (== OtherActor (`self.PlayerRef`)) (`self.IsActivated`))
    (set `self.IsActivated` false)
    (`|ExecutionSequence`
      (:`then_0`
        (if (`self.StartLoop`)
          (for _array_element (`self.LaserRefs`)
            (`/Game/DevelopersContent/Core/Placeables/Gameplay/BP_Lasers.Create Laser` _array_element))
          (else
            (for _array_element_2 (`self.LaserRefs`)
              (`/Game/DevelopersContent/Core/Placeables/Gameplay/BP_Lasers.ShutDown` _array_element_2)))))
      (:`then_1`
        (if (`self.SlowMotion`)
          (`self.SlowMoStart`)
          (set `self.CanStopSlowMotion` true))))))

(event `SlowMoStart`
  (`TimelineComponent.SetPlayRate` (`self.Timeline`) (/ 1.0 0.5))
  (bind (_direction _slowmo) (`Timeline|Timeline` :!via `PlayFromStart` :!label _label)
    (:`Update`
      (`GameplayStatics.SetGlobalTimeDilation` (`KismetMathLibrary.Lerp` 1.0 0.05 _slowmo)))))

(event `SlowMoEnd`
  (`TimelineComponent.SetPlayRate` (`self.Timeline`) (/ 1.0 0.2))
  (goto _label :!via `ReverseFromEnd`))

(event `EnhancedInput|/Game/NIRVANA/Core/Characters/FirstPerson/Input/Actions/IA_Dash`
  (params (ActionValue :type Boolean) (ElapsedSeconds :type "Float (double-precision)") (TriggeredSeconds :type "Float (double-precision)") (InputAction :type "InputAction Object Reference" :default "/Game/NIRVANA/Core/Characters/FirstPerson/Input/Actions/IA_Dash.IA_Dash"))
  (:`Started`
    (if (`self.CanStopSlowMotion`)
      (set `self.CanStopSlowMotion` false)
      (`self.SlowMoEnd`))))

(fn `UserConstructionScript`)
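; BP_SpawnManager is a placeable trigger that spawns a preset group of enemies when the player enters its box.
; On overlap by the cached first-person player character, it runs only while Activated is set, then clears the flag so it fires once.
; SpawnLoop walks the MapSpawn map of spawners to enemy types and asks the ArenaManager to spawn each pair.
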(event `self.ReceiveBeginPlay`
  (bind _asbp_first_person_character (cast `/Game/NIRVANA/Core/Characters/FirstPerson/BP_FirstPersonCharacter` (`GameplayStatics.GetPlayerCharacter` 0)))
  (set `self.PlayerRef` _asbp_first_person_character))

(event `self.Box.OnComponentBeginOverlap`
  (params (OverlappedComponent :type "PrimitiveComponent Object Reference") (OtherActor :type "Actor Object Reference") (OtherComp :type "PrimitiveComponent Object Reference") (OtherBodyIndex :type Integer) (bFromSweep :type Boolean) (SweepResult :type "HitResult Structure (by ref)"))
  (if (`self.Activated`)
    (if (== OtherActor (`self.PlayerRef`))
      (`self.SpawnLoop`)
      (set `self.Activated` false))))

(event `SpawnLoop`
  (bind _mapspawn (`self.MapSpawn`))
  (bind _keys (`BlueprintMapLibrary.Map_Keys` _mapspawn))
  (bind _values (`BlueprintMapLibrary.Map_Values` _mapspawn))
  (for (_array_element _array_index) _keys
    (`/Game/NIRVANA/Core/Placeables/Management/BP_ArenaManager.SpawnEnemy` (`self.ArenaManager`) (`|GetArrayItem` _values _array_index) _array_element)))

(fn `UserConstructionScript`)
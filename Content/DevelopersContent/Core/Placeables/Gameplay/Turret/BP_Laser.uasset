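; Turret laser hazard that cycles on and off, damaging any BP_FirstPersonCharacter that overlaps its beam.
; BeginPlay sets both Niagara beam ends and sizes the capsule along local X from Distance, then loops anticipation, active and inactive phases through delays, skipping anticipation when InactiveTime is not longer than AnticipationDelay.
; Each hit briefly switches capsule overlap events off and on; SetCapsule, an EndLocation-based alignment, is not called here.
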(event `self.ReceiveBeginPlay`
  (bind _capsule (`self.Capsule`))
  (bind _returnvalue (/ (`self.Distance`) 2.0))
  (`|ExecutionSequence`
    (:`then_0`
      (`NiagaraComponent.SetVariableVec3` (`self.NS_LaserEnemie`) "Beam End" (`self.End Location`))
      (`NiagaraComponent.SetVariableVec3` (`self.NS_LaserAnticipation`) "Beam End" (`self.End Location`))
      (`SceneComponent.K2_SetRelativeLocation` _capsule (`KismetMathLibrary.MakeVector` _returnvalue) false true)
      (`CapsuleComponent.SetCapsuleHalfHeight` _capsule _returnvalue true)
      (`SceneComponent.K2_SetRelativeRotation` _capsule (struct :`Pitch` 90.0) false false))
    (:`then_1`
      (`self.Anticipation`))))

(event `Anticipation`
  (`SceneComponent.SetHiddenInGame` (`self.NS_LaserAnticipation`) false false)
  (`KismetSystemLibrary.Delay` (`self.AnticipationDelay`))
  (`SceneComponent.SetHiddenInGame` (`self.NS_LaserAnticipation`) true false)
  (`self.Activate`))

(event `Activate`
  (`SceneComponent.SetHiddenInGame` (`self.NS_LaserEnemie`) false false)
  (set `PrimitiveComponent.bGenerateOverlapEvents` true (`self.Capsule`))
  (`KismetSystemLibrary.Delay` (`self.Laser Life Time `))
  (`self.Desactivate`))

(event `Desactivate`
  (`SceneComponent.SetHiddenInGame` (`self.NS_LaserEnemie`) true false)
  (set `PrimitiveComponent.bGenerateOverlapEvents` false (`self.Capsule`))
  (if (> (`self.Inactive Time`) (`self.AnticipationDelay`))
    (`KismetSystemLibrary.Delay` (- (`self.Inactive Time`) (`self.AnticipationDelay`)))
    (`self.Anticipation`)
    (else
      (`KismetSystemLibrary.Delay` (`self.Inactive Time`))
      (`self.Activate`))))

(event `self.Capsule.OnComponentBeginOverlap`
  (params (OverlappedComponent :type "PrimitiveComponent Object Reference") (OtherActor :type "Actor Object Reference") (OtherComp :type "PrimitiveComponent Object Reference") (OtherBodyIndex :type Integer) (bFromSweep :type Boolean) (SweepResult :type "HitResult Structure (by ref)"))
  (bind _capsule (`self.Capsule`))
  (bind _asbp_first_person_character (cast `/Game/NIRVANA/Core/Characters/FirstPerson/BP_FirstPersonCharacter` OtherActor))
  (`/Game/NIRVANA/Core/Characters/FirstPerson/BP_FirstPersonCharacter.Take Damage` _asbp_first_person_character (`self.Damage`) null)
  (set `PrimitiveComponent.bGenerateOverlapEvents` false _capsule)
  (`KismetSystemLibrary.Delay` 0.05)
  (set `PrimitiveComponent.bGenerateOverlapEvents` true _capsule))

(fn `Set Capsule`
  (bind _capsule (`self.Capsule`))
  (bind (_returnvalue_roll _returnvalue_pitch _returnvalue_yaw) (`KismetMathLibrary.BreakRotator` (`KismetMathLibrary.FindLookAtRotation` (`SceneComponent.K2_GetComponentLocation` (`self.NS_LaserEnemie`)) (`self.End Location`))))
  (`SceneComponent.K2_SetRelativeLocation` _capsule (/ (- (`self.End Location`) (`SceneComponent.K2_GetComponentLocation` (`self.NS_LaserEnemie`))) 2.0) false false)
  (`SceneComponent.K2_SetRelativeRotation` _capsule (`KismetMathLibrary.MakeRotator` _returnvalue_roll (+ _returnvalue_pitch 90.0) _returnvalue_yaw) false false)
  (`CapsuleComponent.SetCapsuleHalfHeight` (`self.Capsule`) (/ (`KismetMathLibrary.Vector_Distance` (`SceneComponent.K2_GetComponentLocation` (`self.NS_LaserEnemie`)) (`self.End Location`)) 2.0) true)
  (`CapsuleComponent.SetCapsuleRadius` (`self.Capsule`) 22.0 true))

(fn `UserConstructionScript`)
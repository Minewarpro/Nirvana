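; BP_Lasers is a placeable row of laser emitters that fire damaging BP_Laser beams, optionally on begin play.
; The construction script builds evenly spaced emitter meshes.
; CreateLaser uses a delayed-loop macro to stagger firing, line-tracing each emitter's forward vector to size and attach its spawned beam.
; With a long enough inactive time, Anticipation cycles emitter colors red and yellow on the beam timing until ShutDown destroys the beams.
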(event `self.ReceiveBeginPlay`
  ;[0.2396 0.2396 0.2396] Begin play
  (if (`self.Start Active`)
    (`self.Create Laser`)))

(event `Create Laser`
  ;[0.3385 0.2327 0.2327 1 50] Create Laser
  (`KismetSystemLibrary.Delay` (`self.DelayStart`))
  (bind _array_element (`self.Each Loop Delayed` (`self.All Lasers`) (`self.DelayLinear`))
    (:`Loop Body`
      (bind _returnvalue (`SceneComponent.K2_GetComponentLocation` _array_element))
      (bind _outhit (`KismetSystemLibrary.LineTraceSingle` _returnvalue (+ _returnvalue (* (`SceneComponent.GetForwardVector` _array_element) 999999999.0)) "TraceTypeQuery1"))
      (bind (_bblockinghit _binitialoverlap _time _distance _location) (`GameplayStatics.BreakHitResult` _outhit))
      (bind _returnvalue_2 (`|SpawnActorFromClass` "/Game/DevelopersContent/Core/Placeables/Gameplay/Turret/BP_Laser.BP_Laser_C" (`KismetMathLibrary.MakeTransform` (0.0 0.0 0.0)) "Undefined" "MultiplyWithRoot" null _location (`self.Damage`) (`self.Active Time`) _distance (`self.Inactive Time`) null))
      (`self.K2_AttachToComponent` _returnvalue_2 _array_element "None" "KeepRelative" "KeepRelative" "KeepRelative" true)
      (`KismetArrayLibrary.Array_Add` (`self.ProjectilesRefs`) _returnvalue_2)
      (if (>= (`self.Inactive Time`) 1.0)
        (`self.Anticipation`)
        (set `self.Running` true)))))

(event `ShutDown`
  (for _array_element (`self.ProjectilesRefs`)
    (`self.K2_DestroyActor` _array_element)
    (set `self.Running` false)))

(event `Anticipation`
  (for _array_element (`self.All Lasers`)
    (`MeshComponent.SetVectorParameterValueOnMaterials` _array_element "BaseColor" (1.0 0.0 0.0)))
  (`KismetSystemLibrary.Delay` (+ (`self.Active Time`) 1.0))
  (for _array_element_2 (`self.All Lasers`)
    (`MeshComponent.SetVectorParameterValueOnMaterials` _array_element_2 "BaseColor" (1.0 0.91 0.0)))
  (if (`self.Running`)
    (`KismetSystemLibrary.Delay` (- (`self.Inactive Time`) 1.0))
    (`self.Anticipation`)))

(fn `UserConstructionScript`
  ;[0.2396 0.2396 0.2396] Spawn Lasers
  (for _index (range (`self.Nb Lasers`))
    (bind _returnvalue (`AddComponent|NODE_AddStaticMeshComponent-0` :`RelativeTransform` (`KismetMathLibrary.MakeTransform` (`KismetMathLibrary.MakeVector` 0.0 (`KismetMathLibrary.Conv_IntToDouble` (* _index (`self.Distance Beetwen Lasers`)))))))
    (`KismetArrayLibrary.Array_Add` (`self.All Lasers`) _returnvalue)))
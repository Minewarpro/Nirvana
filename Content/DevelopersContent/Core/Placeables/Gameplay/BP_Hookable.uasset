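; BP_Hookable is a placeable hook point that tells the first-person player character when it is in range.
; Overlapping its sphere starts the player's hook tick; leaving ends it and hides the crosshair widget, which has functions to show or hide it.
; Desactivate makes the mesh ignore a custom trace channel and swaps its material, then Activate restores both after a configurable delay.
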(event `self.ReceiveBeginPlay`
  (bind _asbp_first_person_character (cast `/Game/NIRVANA/Core/Characters/FirstPerson/BP_FirstPersonCharacter` (`GameplayStatics.GetPlayerCharacter` 0)))
  (set `self.Player Ref` _asbp_first_person_character)
  (bind _aswb_hook_cross_hair (cast `/Game/DevelopersContent/Core/Weapons/MainGun/projectiles/WB_HookCrossHair` (`WidgetComponent.GetWidget` (`self.Widget`))))
  (set `self.WB_CrossHair` _aswb_hook_cross_hair))

(event `self.SphereCollision.OnComponentBeginOverlap`
  (params (OverlappedComponent :type "PrimitiveComponent Object Reference") (OtherActor :type "Actor Object Reference") (OtherComp :type "PrimitiveComponent Object Reference") (OtherBodyIndex :type Integer) (bFromSweep :type Boolean) (SweepResult :type "HitResult Structure (by ref)"))
  (bind _player_ref (`self.Player Ref`))
  (if (== OtherActor _player_ref)
    (`/Game/NIRVANA/Core/Characters/FirstPerson/BP_FirstPersonCharacter.Start Tick Hook` _player_ref)
    (set `self.IsInRange` true)
    (`KismetSystemLibrary.PrintString` "Enter Sphere")))

(event `self.SphereCollision.OnComponentEndOverlap`
  (params (OverlappedComponent :type "PrimitiveComponent Object Reference") (OtherActor :type "Actor Object Reference") (OtherComp :type "PrimitiveComponent Object Reference") (OtherBodyIndex :type Integer))
  (bind _player_ref (`self.Player Ref`))
  (if (== OtherActor _player_ref)
    (`/Game/NIRVANA/Core/Characters/FirstPerson/BP_FirstPersonCharacter.End Tick Hook` _player_ref)
    (`self.Desactive Cross Hair`)
    (set `self.IsInRange` false)))

(event `Desactivate`
  (bind _mesh (`self.Mesh`))
  (set `self.IsActive` false)
  (`PrimitiveComponent.SetCollisionResponseToChannel` _mesh "ECC_GameTraceChannel6" "ECR_Ignore")
  (`PrimitiveComponent.SetMaterial` _mesh 0 "/Game/DevelopersContent/Core/Characters/Enemies/Common/Mixamo_Skin/Alpha_Body_MAT_Inst1.Alpha_Body_MAT_Inst1")
  (`KismetSystemLibrary.Delay` (`self.DelayReactivate`))
  (`self.Activate`))

(event `Activate`
  (bind _mesh (`self.Mesh`))
  (set `self.IsActive` true)
  (`PrimitiveComponent.SetCollisionResponseToChannel` _mesh "ECC_GameTraceChannel6" "ECR_Block")
  (`PrimitiveComponent.SetMaterial` _mesh 0 "/Engine/MapTemplates/Materials/BasicAsset03.BasicAsset03"))

(event `Activate Trap`)

(fn `Active Cross Hair`
  (`SceneComponent.SetHiddenInGame` (`self.Widget`) false false))

(fn `Desactive Cross Hair`
  (`SceneComponent.SetHiddenInGame` (`self.Widget`) true false))

(fn `UserConstructionScript`)
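; BP_MovablePlatform is a placeable grid of platform meshes that shift vertically in response to player proximity.
; Its construction script generates static mesh components from grid counts and mesh bounds, storing Start and End locations separated by Height.
; While the player overlaps the detection box, Tick lerps each platform by clamped player distance, reaching End when near and Start when far.
; The timer-based move loop is never called.
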(event `self.ReceiveBeginPlay`
  (bind _asbp_first_person_character (cast `/Game/NIRVANA/Core/Characters/FirstPerson/BP_FirstPersonCharacter` (`GameplayStatics.GetPlayerCharacter` 0)))
  (set `self.Player Ref` _asbp_first_person_character))

(event `self.Box Detection.OnComponentBeginOverlap`
  (params (OverlappedComponent :type "PrimitiveComponent Object Reference") (OtherActor :type "Actor Object Reference") (OtherComp :type "PrimitiveComponent Object Reference") (OtherBodyIndex :type Integer) (bFromSweep :type Boolean) (SweepResult :type "HitResult Structure (by ref)"))
  (if (== OtherActor (`self.Player Ref`))
    (set `self.can move` true)))

(event `self.Box Detection.OnComponentEndOverlap`
  (params (OverlappedComponent :type "PrimitiveComponent Object Reference") (OtherActor :type "Actor Object Reference") (OtherComp :type "PrimitiveComponent Object Reference") (OtherBodyIndex :type Integer))
  (if (== OtherActor (`self.Player Ref`))
    (set `self.can move` false)))

(event `Start Move Loop`
  (bind _returnvalue (`KismetSystemLibrary.K2_SetTimerDelegate` (delegate `MovingPlatform`) 0.001 true))
  (set `self.Move Loop Event` _returnvalue))

(event `Stop Move Loop`
  (`KismetSystemLibrary.K2_ClearAndInvalidateTimerHandle` (`self.Move Loop Event`))
  (for _array_element (`self.Platforms`)
    (`SceneComponent.K2_SetRelativeLocation` _array_element (0.0 0.0 0.0) false false)))

(event `MovingPlatform`)

(event `self.ReceiveTick`
  (params (DeltaSeconds :type "Float (single-precision)"))
  (if (`self.can move`)
    (for (_array_element _array_index) (`self.Platforms`)
      (bind (_output_start _output_end) (break `/Game/DevelopersContent/Core/Placeables/SPlatform` (`|GetArrayItem` (`self.Locations`) _array_index)))
      (`SceneComponent.K2_SetRelativeLocation` _array_element (`KismetMathLibrary.VLerp` _output_end _output_start (`KismetMathLibrary.NormalizeToRange` (`KismetMathLibrary.FClamp` (`KismetMathLibrary.Vector_Distance` (`self.K2_GetActorLocation` (`self.Player Ref`)) (`SceneComponent.K2_GetComponentLocation` _array_element)) 500.0 1500.0) 500.0 1500.0)) false false))))

(fn `Clear all`
  (bind _platforms (`self.Platforms`))
  (for _array_element _platforms
    (`ActorComponent.K2_DestroyComponent` _array_element))
  (`KismetArrayLibrary.Array_Clear` _platforms)
  (`KismetArrayLibrary.Array_Clear` (`self.Locations`)))

(fn `Create Static Mesh`
  (for _array_element (`self.Locations`)
    (bind _returnvalue (`AddComponent|NODE_AddStaticMeshComponent-2` :`RelativeTransform` (`KismetMathLibrary.MakeTransform` (break `/Game/DevelopersContent/Core/Placeables/SPlatform` _array_element))))
    (`StaticMeshComponent.SetStaticMesh` _returnvalue (`self.Mesh`))
    (`KismetArrayLibrary.Array_Add` (`self.Platforms`) _returnvalue)))

(fn `Generate Bridge`
  (for _index (range (`self.Nb Platforms X`))
    (bind _returnvalue (* _index (* (.x (`.BoxExtent` (`KismetMathLibrary.BreakBoxSphereBounds` (`StaticMesh.GetBounds` (`self.Mesh`))))) 2.0)))
    (`KismetArrayLibrary.Array_Add` (`self.Locations`) (make `/Game/DevelopersContent/Core/Placeables/SPlatform` (`KismetMathLibrary.MakeVector` _returnvalue) (`KismetMathLibrary.MakeVector` _returnvalue 0.0 (`self.Height`))))
    (for _index_2 (range (`self.Nb Platforms Y`))
      (bind _returnvalue_2 (* _index_2 (* (.y (`.BoxExtent` (`KismetMathLibrary.BreakBoxSphereBounds` (`StaticMesh.GetBounds` (`self.Mesh`))))) 2.0)))
      (`KismetArrayLibrary.Array_Add` (`self.Locations`) (make `/Game/DevelopersContent/Core/Placeables/SPlatform` (`KismetMathLibrary.MakeVector` _returnvalue _returnvalue_2) (`KismetMathLibrary.MakeVector` _returnvalue _returnvalue_2 (`self.Height`))))))
  (`self.Create Static Mesh`))

(fn `UserConstructionScript`
  (bind _box_detection (`self.Box Detection`))
  (`self.Clear all`)
  (`self.Generate Bridge`)
  (`SceneComponent.K2_SetRelativeLocation` _box_detection (`self.Box Relative Location`) false false)
  (`BoxComponent.SetBoxExtent` _box_detection (`self.Box Extent`) true))
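; BP_Ring_Rotation is a placeable ring actor that spins a full turn around its yaw axis.
; BeginPlay stores the starting rotation and calls Rotate, which plays a timeline at a rate set by the inverse of LoopDuration.
; Each timeline update lerps yaw from the starting value through 360 degrees, keeping the original pitch and roll.
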(event `Rotate`
  (bind (_initrotate_roll _initrotate_pitch _initrotate_yaw) (`KismetMathLibrary.BreakRotator` (`self.InitRotate`)))
  (`TimelineComponent.SetPlayRate` (`self.Timeline`) (/ 1.0 (`self.LoopDuration`)))
  (bind (_direction _newtrack_1) (`Timeline|Timeline` :!via `PlayFromStart`)
    (:`Update`
      (`self.K2_SetActorRotation` (`KismetMathLibrary.MakeRotator` _initrotate_roll _initrotate_pitch (`KismetMathLibrary.Lerp` _initrotate_yaw (+ _initrotate_yaw 360.0) _newtrack_1))))))

(event `self.ReceiveBeginPlay`
  (set `self.InitRotate` (`self.K2_GetActorRotation`))
  (`self.Rotate`))

(fn `UserConstructionScript`)
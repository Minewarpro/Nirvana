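; BP_ChangeLevel is a placeable trigger volume that moves the first-person player to another level.
; On BeginPlay it caches the player character.
; When that character overlaps the trigger while Activated is set, it opens LevelToOpen, then clears the player's checkpoints.
; The construction script scales the trigger to BoxSize, sets the level name text and positions both text components from TextHeight.
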(event `self.ReceiveBeginPlay`
  (bind _asbp_first_person_character (cast `/Game/NIRVANA/Core/Characters/FirstPerson/BP_FirstPersonCharacter` (`GameplayStatics.GetPlayerCharacter` 0)))
  (set `self.PlayerRef` _asbp_first_person_character))

(event `self.Trigger.OnComponentBeginOverlap`
  (params (OverlappedComponent :type "PrimitiveComponent Object Reference") (OtherActor :type "Actor Object Reference") (OtherComp :type "PrimitiveComponent Object Reference") (OtherBodyIndex :type Integer) (bFromSweep :type Boolean) (SweepResult :type "HitResult Structure (by ref)"))
  (if (and (== OtherActor (`self.PlayerRef`)) (`self.Activated`))
    (`GameplayStatics.OpenLevelBySoftObjectPtr` (`self.LevelToOpen`))
    (`/Game/NIRVANA/Core/Characters/FirstPerson/BP_FirstPersonCharacter.Clear Checkpoints` (`self.PlayerRef`))))

(fn `UserConstructionScript`
  (bind _levelname (`self.LevelName`))
  (`SceneComponent.SetRelativeScale3D` (`self.Trigger`) (`self.BoxSize`))
  (`TextRenderComponent.K2_SetText` _levelname (`self.Value`))
  (`SceneComponent.K2_SetRelativeLocation` _levelname (`KismetMathLibrary.MakeVector` 0.0 0.0 (- (`self.TextHeight`) 50.0)) false false)
  (`SceneComponent.K2_SetRelativeLocation` (`self.TextRender`) (`KismetMathLibrary.MakeVector` 0.0 0.0 (`self.TextHeight`)) false false))
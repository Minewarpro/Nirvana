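; Boss actor, named for cinematic use, with helper functions for health and teleport-zone bookkeeping.
; BeginPlay caches the first-person player character.
; SubstractLife lowers health, updates the boss widget's life bar, then clamps negative health to zero.
; SetNewZone moves the occupied flag to a zone from GetValidZone, which re-rolls randomly until one is free, without moving the actor itself.
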(event `self.ReceiveBeginPlay`
  ;[1 1 1] Begin play
  (bind _asbp_first_person_character (cast `/Game/NIRVANA/Core/Characters/FirstPerson/BP_FirstPersonCharacter` (`GameplayStatics.GetPlayerCharacter` 0)))
  (set `self.Player Ref` _asbp_first_person_character))

(fn `Get Valid Zone`
  (returns (`New Zone` :type "/Game/DevelopersContent/Art/Boss/BP_BossZone Object Reference"))
  (locals (NewLocalVar :type "/Game/DevelopersContent/Art/Boss/BP_BossZone Object Reference"))
  (bind _output_get (set `local.NewLocalVar` (`KismetArrayLibrary.Array_Random` (`self.Zones to TP`)) :!label _label))
  (if (not (`/Game/DevelopersContent/Art/Boss/BP_BossZone.Is Occupated` _output_get))
    (return _output_get)
    (else
      (goto _label))))

(fn `Set New Zone`
  (bind _new_zone (`self.Get Valid Zone`))
  (set `/Game/DevelopersContent/Art/Boss/BP_BossZone.Is Occupated` false (`self.Current Zone`))
  (bind _output_get (set `self.Current Zone` _new_zone))
  (set `/Game/DevelopersContent/Art/Boss/BP_BossZone.Is Occupated` true _output_get)
  (return))

(fn `Substract Life`
  (params (`Life to Sub` :type "Float (double-precision)"))
  (bind _output_get (set `self.Current Health` (- (`self.Current Health`) `Life to Sub`)))
  (`ProgressBar.SetPercent` (`/Game/DevelopersContent/Art/Boss/WB_Boss.LifeBar` (`self.Widget Boss Ref`)) (/ _output_get (`self.Max Health`)))
  (if (< _output_get 0.0)
    (set `self.Current Health` 0.0)
    (return)
    (else
      (return))))

(fn `UserConstructionScript`)
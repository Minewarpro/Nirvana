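; Bullet-hell boss actor that alternates between Attack and Vulnerable states, with a health bar widget and Niagara hit and death effects.
; In Attack it teleports between free zones on a looping timer with a timeline glide and fires CurrentPattern through SpawnPattern.
; Patterns activate BP_BulletManager bullets, spawn previsualisation actors or rain comets.
; It takes damage only while Vulnerable, returning to Attack after a delay or enough damage.
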(event Custom|Hit%20Reaction
  ;[0.7693 1 0.6791] Hit Reaction
  (bind _newtrack_0 (Timeline|TL%20Hit PlayFromStart)
    (:Update
      (Niagara|SetNiagaraVariable(Float) (Variables|Default|GetNS_Boss) "Attraction force" (Math|Float|Lerp 0.0 -7e+03 _newtrack_0))
      (Niagara|SetNiagaraVariable(Float) (Variables|Default|GetNS_Boss) "Emissive Power" (Math|Float|Lerp 0.0 0.1 _newtrack_0)))))

(event Custom|Start%20TP%20Loop
  ;[1 0.07837 0 1 91] Attack State
  ;;[0.627 0.7768 1] Tp System
  (bind _returnvalue (Utilities|Time|SetTimerbyEvent (delegate Custom|TP) (Variables|TPSystem|GetTP%20Cooldown) true))
  (Variables|TPSystem|SetTP%20Loop%20Event _returnvalue))

(event Custom|TP
  ;[1 0.07837 0 1 91] Attack State
  ;;[0.627 0.7768 1] Tp System
  (Variables|TPSystem|SetisTP true)
  (Zone|SetNewZone)
  (Variables|TPSystem|SetTemp%20Location%20Boss (Transformation|GetActorLocation))
  (bind _location_alpha (Timeline|TL%20Move%20To%20New%20Zone PlayFromStart)
    (:Update
      (Transformation|SetActorLocation (Math|Vector|Lerp(Vector) (Variables|TPSystem|GetTemp%20Location%20Boss) (Transformation|GetActorLocation (Variables|TPSystem|GetCurrent%20Zone)) _location_alpha) false false))
    (:Finished
      (CallFunction|OnFinishTP))))

(event Custom|CheckShoot
  ;[1 0.07837 0 1 91] Attack State
  ;;[1 1 1] Shoot
  ;;;[0.4114 0.5677 0.3117 0.66] Check to Shoot
  (if (and (not (Variables|TPSystem|GetisTP)) (Variables|Shoot|GetcanShoot))
    (Utilities|Time|PauseTimerbyHandle (Variables|TPSystem|GetTP%20Loop%20Event))
    (CallFunction|Shoot)))

(event Custom|StartBehavior
  ;[1 0.6941 0.1255] Start
  (Rendering|SetActorHiddenInGame false)
  (UserInterface|Viewport|AddtoViewport (Variables|Ref|GetWidget%20Boss%20Ref) 0)
  (CallFunction|SwitchState "NewEnumerator1"))

(event Custom|SwitchState
  (params (targetState :type Enum_BossState%20Enum :default "NewEnumerator0"))
  (bind _spheremat (Variables|Default|GetSphereMat))
  ;[0.5885 0.2574 0.0705] States
  (bind _output_get (Variables|Default|Setstate targetState))
  (switch Utilities|FlowControl|Switch|SwitchonEnum_BossState _output_get
    (:NewEnumerator0
      (Rendering|Material|SetVectorParameterValue _spheremat "Color" "(R=1.000000,G=0.419608,B=0.000000,A=1.000000)" :!class /Script/Engine.MaterialInstanceDynamic)
      (Variables|Shoot|SetcanShoot false)
      (Utilities|Time|ClearandInvalidateTimerbyHandle (Variables|TPSystem|GetTP%20Loop%20Event))
      (Utilities|FlowControl|Delay 1e+01)
      (CallFunction|SwitchState "NewEnumerator1"))
    (:NewEnumerator1
      (Rendering|Material|SetVectorParameterValue _spheremat "Color" "(R=0.309804,G=0.258824,B=1.000000,A=1.000000)" :!class /Script/Engine.MaterialInstanceDynamic)
      (Variables|Shoot|SetcanShoot true)
      (CallFunction|StartTPLoop)
      (Utilities|FlowControl|Sequence
        (:then_0
          (Utilities|FlowControl|Delay 1.0)
          (CallFunction|CheckShoot))
        (:then_1
          (Utilities|FlowControl|Delay 45.0)
          (CallFunction|SwitchState "NewEnumerator0"))))))

(event Custom|Shoot
  (bind _returnvalue (Transformation|GetActorLocation))
  (bind (_x _y _z) (Math|Vector|BreakVector _returnvalue))
  ;[1 0.07837 0 1 91] Attack State
  ;;[1 1 1] Shoot
  (Variables|Shoot|SetcurrentPattern (CallFunction|GetPattern))
  (Variables|Shoot|SetcanShoot false)
  (CallFunction|SpawnPattern (.pattern (Variables|Shoot|GetcurrentPattern)) (.nbbulletloop (Variables|Shoot|GetcurrentPattern)) (Math|Vector|MakeVector _x _y (+ _z (.zoffsettransformlocation (Variables|Shoot|GetcurrentPattern)))) (Math|Vector|GetUnitDirection(Vector) (Math|Vector|SelectVector (Math|Vector|MakeVector _x _y (+ _z (.zoffsettransformlocation (Variables|Shoot|GetcurrentPattern)))) _returnvalue (.directionbyoffset (Variables|Shoot|GetcurrentPattern))) (Transformation|GetActorLocation (Variables|Ref|GetPlayer%20Ref))) (.projectilespeed (Variables|Shoot|GetcurrentPattern)) (.damage (Variables|Shoot|GetcurrentPattern)) (.delayeachloop (Variables|Shoot|GetcurrentPattern)) (.previsualisation (Variables|Shoot|GetcurrentPattern)) 1.0 (.dispertion (Variables|Shoot|GetcurrentPattern)) (.dispertionspeed (Variables|Shoot|GetcurrentPattern)) (.nbbulletrectangle (Variables|Shoot|GetcurrentPattern)))
  (Utilities|FlowControl|Delay (.duration (Variables|Shoot|GetcurrentPattern)))
  (CallFunction|OnFinishShoot))

(event Custom|Death
  ;[0.02353 0.03922 0.0902] Death
  (Development|PrintString "Boss Dead")
  (Components|Timeline|SetPlayRate (Variables|Default|GetParticlesExplosion) (/ 1.0 2.0))
  (bind _newtrack_0 (Timeline|ParticlesExplosion PlayFromStart)
    (:Update
      (Niagara|SetNiagaraVariable(Float) (Variables|Default|GetNS_Boss) "Falloff Exponent" (Math|Float|Lerp 0.5 3.0 _newtrack_0)))
    (:Finished
      (Components|DestroyComponent (Variables|Default|GetNS_Boss))
      (Widget|RemovefromParent (Variables|Ref|GetWidget%20Boss%20Ref))
      (Actor|DestroyActor)
      (Default|SequenceVoices (Variables|Ref|GetVoicesToLaunch)))))

(event Custom|OnFinishTP
  ;[1 1 1] CallBacks
  (Variables|TPSystem|SetisTP false)
  (CallFunction|CheckShoot))

(event Custom|OnFinishShoot
  ;[1 1 1] CallBacks
  (Utilities|Time|UnpauseTimerbyHandle (Variables|TPSystem|GetTP%20Loop%20Event))
  (Utilities|FlowControl|Delay (.delay (Variables|Shoot|GetcurrentPattern)))
  (CallFunction|CheckShoot)
  (Variables|Shoot|SetcanShoot true))

(event Custom|Hit_1
  (params (Damages :type Float%20%28double-precision%29))
  ;[0.7693 1 0.6791] Hit Reaction
  (if (Utilities|Enum|Equal(Enum) (Variables|Default|Getstate) "NewEnumerator0")
    (CallFunction|HitReaction)
    (bind _dead (CallFunction|SubstractLife Damages))
    (if _dead
      (CallFunction|Death)
      (elif (CallFunction|IsWeakened Damages)
        (Variables|HealthSystem|SetDealtDamage 0.0)
        (CallFunction|SwitchState "NewEnumerator1")))))

(event EventBeginPlay
  ;[1 1 1] Init
  (bind _asbp_first_person_character (Utilities|Casting|CastToBP_FirstPersonCharacter (Game|GetPlayerCharacter 0)))
  (Variables|Ref|SetPlayer%20Ref _asbp_first_person_character)
  (bind _returnvalue (Actor|GetActorOfClass "/Game/NIRVANA/Core/Characters/Enemies/Range/BP_BulletManager.BP_BulletManager_C"))
  (Variables|Ref|SetRef%20Bullet%20Manager _returnvalue)
  (bind _returnvalue_2 (UserInterface|CreateWidget "/Game/DevelopersContent/Art/Boss/WB_Boss.WB_Boss_C" (Game|GetPlayerController 0)))
  (Variables|Ref|SetWidget%20Boss%20Ref _returnvalue_2)
  (Components|Timeline|SetPlayRate (Variables|Default|GetTL%20Hit) (/ 1.0 0.1))
  (Variables|HealthSystem|SetCurrent%20Health (Variables|HealthSystem|GetMax%20Health))
  (Components|Timeline|SetPlayRate (Variables|Default|GetTL%20Move%20To%20New%20Zone) (/ 1.0 3.0))
  (Transformation|SetActorLocation (Transformation|GetActorLocation (Variables|TPSystem|GetCurrent%20Zone)) false false)
  (bind _returnvalue_3 (Rendering|Material|CreateDynamicMaterialInstance (Variables|Default|GetSphere) 0 "/Game/DevelopersContent/Art/Boss/M_BossOrb_Inst.M_BossOrb_Inst" "None" :!class /Script/Engine.PrimitiveComponent))
  (Variables|Default|SetSphereMat _returnvalue_3))

(event Custom|Rectangle
  (params (NbBullet :type Integer) (Spawn%20Transform%20Location :type Vector) (Direction :type Vector) (Speed :type Float%20%28double-precision%29) (Damage :type Float%20%28double-precision%29) (Delay%20Each%20Loop :type Float%20%28double-precision%29) (Pre-Visualisation :type Boolean) (Projectile%20Scale :type Float%20%28double-precision%29) (Dispertion%20Speed :type Float%20%28double-precision%29) (NB%20Bullet%20Secondaire :type Integer) (Dispertion :type Boolean))
  (bind _returnvalue (Math|Conversions|ToVector(Float) Projectile%20Scale))
  (bind _returnvalue_2 (+ Spawn%20Transform%20Location ""))
  (bind _returnvalue_3 (- NbBullet 1))
  (bind _returnvalue_4 (+ Spawn%20Transform%20Location ""))
  (bind _ref_bullet_manager (Variables|Ref|GetRef%20Bullet%20Manager))
  ;[1 1 1] Lines
  (for _index (range 0 _returnvalue_3) ; Horizontal
    (Game|SpawnActorfromClass "/Game/NIRVANA/Core/Characters/Enemies/Projectiles/BP_EnemyProjectileApparition.BP_EnemyProjectileApparition_C" (Math|Transform|MakeTransform (+ Spawn%20Transform%20Location (Math|Vector|MakeVector 0.0 0.0 (- (* _index 8e+01) (* (/ (Math|Conversions|ToFloat(Integer) _returnvalue_3) 2.0) 8e+01)))) "0, 0, 0" _returnvalue) "AlwaysSpawn" "MultiplyWithRoot" 0 0.5 (+ Spawn%20Transform%20Location (Math|Vector|MakeVector 0.0 0.0 (- (* _index 8e+01) (* (/ (Math|Conversions|ToFloat(Integer) _returnvalue_3) 2.0) 8e+01)))) Direction Speed Damage false 0.2 "0.000000,0.000000,0.000000" 0.0 _ref_bullet_manager 0 "NewEnumerator1" 0))
  (for _index_2 (range 0 (- NbBullet 1)) ; Vertical
    (Game|SpawnActorfromClass "/Game/NIRVANA/Core/Characters/Enemies/Projectiles/BP_EnemyProjectileApparition.BP_EnemyProjectileApparition_C" (Math|Transform|MakeTransform _returnvalue_4 "0, 0, 0" _returnvalue) "AlwaysSpawn" "MultiplyWithRoot" 0 0.5 _returnvalue_4 Direction Speed Damage false 0.2 "0.000000,0.000000,0.000000" 0.0 _ref_bullet_manager 0 "NewEnumerator1" 0))
  (for _index_3 (range 0 (- NbBullet 1)) ; Diagonal
    (Game|SpawnActorfromClass "/Game/NIRVANA/Core/Characters/Enemies/Projectiles/BP_EnemyProjectileApparition.BP_EnemyProjectileApparition_C" (Math|Transform|MakeTransform _returnvalue_2 "0, 0, 0" _returnvalue) "AlwaysSpawn" "MultiplyWithRoot" 0 0.5 _returnvalue_2 Direction Speed Damage false 0.2 "0.000000,0.000000,0.000000" 0.0 _ref_bullet_manager 0 "NewEnumerator1" 0)))

(event Custom|Horizontal%20Round
  (params (NbBullet :type Integer) (Spawn%20Transform%20Location :type Vector) (Direction :type Vector) (Speed :type Float%20%28double-precision%29) (Damage :type Float%20%28double-precision%29) (Delay%20Each%20Loop :type Float%20%28double-precision%29) (Pre-Visualisation :type Boolean) (Projectile%20Scale :type Float%20%28double-precision%29) (Dispertion%20Speed :type Float%20%28double-precision%29))
  (bind _returnvalue (Math|Conversions|ToVector(Float) Projectile%20Scale))
  (bind _returnvalue_2 (Math|Conversions|RotationFromXVector Direction))
  ;[1 1 1] Horizontal Round
  (bind _index (Utilities|ForLoopDelayed 0 (- NbBullet 1) Delay%20Each%20Loop)
    (:Loop%20Body
      (if Pre-Visualisation
        (Game|SpawnActorfromClass "/Game/NIRVANA/Core/Characters/Enemies/Projectiles/BP_EnemyProjectileApparition.BP_EnemyProjectileApparition_C" (Math|Transform|MakeTransform (Math|Vector|MakeVector (.X (Math|Vector|BreakVector (+ (* (Math|Vector|RotateVectorAroundAxis (* (Math|Vector|GetRightVector _returnvalue_2) -1.0) (* _index (/ 1.8e+02 (Math|Conversions|ToFloat(Integer) NbBullet))) (Math|Vector|GetUpVector _returnvalue_2)) 2e+02) Spawn%20Transform%20Location))) (.Y (Math|Vector|BreakVector (+ (* (Math|Vector|RotateVectorAroundAxis (* (Math|Vector|GetRightVector _returnvalue_2) -1.0) (* _index (/ 1.8e+02 (Math|Conversions|ToFloat(Integer) NbBullet))) (Math|Vector|GetUpVector _returnvalue_2)) 2e+02) Spawn%20Transform%20Location))) (+ (.Z (Math|Vector|BreakVector (+ (* (Math|Vector|RotateVectorAroundAxis (* (Math|Vector|GetRightVector _returnvalue_2) -1.0) (* _index (/ 1.8e+02 (Math|Conversions|ToFloat(Integer) NbBullet))) (Math|Vector|GetUpVector _returnvalue_2)) 2e+02) Spawn%20Transform%20Location))) (* (stale _index) 5e+01))) "0, 0, 0" _returnvalue) "AlwaysSpawn" "MultiplyWithRoot" 0 0.5 (Math|Vector|MakeVector (.X (Math|Vector|BreakVector (+ (* (Math|Vector|RotateVectorAroundAxis (* (Math|Vector|GetRightVector _returnvalue_2) -1.0) (* _index (/ 1.8e+02 (Math|Conversions|ToFloat(Integer) NbBullet))) (Math|Vector|GetUpVector _returnvalue_2)) 2e+02) Spawn%20Transform%20Location))) (.Y (Math|Vector|BreakVector (+ (* (Math|Vector|RotateVectorAroundAxis (* (Math|Vector|GetRightVector _returnvalue_2) -1.0) (* _index (/ 1.8e+02 (Math|Conversions|ToFloat(Integer) NbBullet))) (Math|Vector|GetUpVector _returnvalue_2)) 2e+02) Spawn%20Transform%20Location))) (+ (.Z (Math|Vector|BreakVector (+ (* (Math|Vector|RotateVectorAroundAxis (* (Math|Vector|GetRightVector _returnvalue_2) -1.0) (* _index (/ 1.8e+02 (Math|Conversions|ToFloat(Integer) NbBullet))) (Math|Vector|GetUpVector _returnvalue_2)) 2e+02) Spawn%20Transform%20Location))) (* (stale _index) 5e+01))) (Utilities|Dispertion Spawn%20Transform%20Location (+ (* (Math|Vector|RotateVectorAroundAxis (* (Math|Vector|GetRightVector _returnvalue_2) -1.0) (* _index (/ 1.8e+02 (Math|Conversions|ToFloat(Integer) NbBullet))) (Math|Vector|GetUpVector _returnvalue_2)) 2e+02) Spawn%20Transform%20Location) Direction Dispertion%20Speed false) Speed Damage false 0.2 "0.000000,0.000000,0.000000" 0.0 (Variables|Ref|GetRef%20Bullet%20Manager) 0 "NewEnumerator1" 0)
        (else
          (Default|ActivateBullet (Variables|Ref|GetRef%20Bullet%20Manager) (Math|Vector|MakeVector (.X (Math|Vector|BreakVector (+ (* (Math|Vector|RotateVectorAroundAxis (* (Math|Vector|GetRightVector _returnvalue_2) -1.0) (* _index (/ 1.8e+02 (Math|Conversions|ToFloat(Integer) NbBullet))) (Math|Vector|GetUpVector _returnvalue_2)) 2e+02) Spawn%20Transform%20Location))) (.Y (Math|Vector|BreakVector (+ (* (Math|Vector|RotateVectorAroundAxis (* (Math|Vector|GetRightVector _returnvalue_2) -1.0) (* _index (/ 1.8e+02 (Math|Conversions|ToFloat(Integer) NbBullet))) (Math|Vector|GetUpVector _returnvalue_2)) 2e+02) Spawn%20Transform%20Location))) (+ (.Z (Math|Vector|BreakVector (+ (* (Math|Vector|RotateVectorAroundAxis (* (Math|Vector|GetRightVector _returnvalue_2) -1.0) (* _index (/ 1.8e+02 (Math|Conversions|ToFloat(Integer) NbBullet))) (Math|Vector|GetUpVector _returnvalue_2)) 2e+02) Spawn%20Transform%20Location))) (* (stale _index) 5e+01))) (Utilities|Dispertion Spawn%20Transform%20Location (+ (* (Math|Vector|RotateVectorAroundAxis (* (Math|Vector|GetRightVector _returnvalue_2) -1.0) (* _index (/ 1.8e+02 (Math|Conversions|ToFloat(Integer) NbBullet))) (Math|Vector|GetUpVector _returnvalue_2)) 2e+02) Spawn%20Transform%20Location) Direction Dispertion%20Speed false) Speed Damage false 0.0 "0, 0, 0" 0.0 "NewEnumerator1" _returnvalue 0 false 0.0 0.0))))))

(event Custom|Simple%20Pattern
  (params (NbBullet :type Integer) (Spawn%20Transform%20Location :type Vector) (Direction :type Vector) (Speed :type Float%20%28double-precision%29) (Damage :type Float%20%28double-precision%29) (Delay%20Each%20Loop :type Float%20%28double-precision%29) (Pre-Visualisation :type Boolean) (Projectile%20Scale :type Float%20%28double-precision%29))
  (bind _returnvalue (Math|Conversions|ToVector(Float) Projectile%20Scale))
  (bind _returnvalue_2 (Math|Random|RandomUnitVectorinConeinDegrees Direction 2.0))
  ;[1 1 1] Simple
  (bind _index (Utilities|ForLoopDelayed 0 (- NbBullet 1) Delay%20Each%20Loop)
    (:Loop%20Body
      (if Pre-Visualisation
        (Game|SpawnActorfromClass "/Game/NIRVANA/Core/Characters/Enemies/Projectiles/BP_EnemyProjectileApparition.BP_EnemyProjectileApparition_C" (Math|Transform|MakeTransform Spawn%20Transform%20Location "0, 0, 0" _returnvalue) "AlwaysSpawn" "MultiplyWithRoot" 0 0.5 Spawn%20Transform%20Location _returnvalue_2 Speed Damage false 0.2 "0.000000,0.000000,0.000000" 0.0 (Variables|Ref|GetRef%20Bullet%20Manager) 0 "NewEnumerator1" 0)
        (else
          (Default|ActivateBullet (Variables|Ref|GetRef%20Bullet%20Manager) Spawn%20Transform%20Location _returnvalue_2 Speed Damage false 0.0 "0, 0, 0" 0.0 "NewEnumerator1" _returnvalue 0 true 1.0 (- 2e+04 (* _index (/ 20000 NbBullet)))))))))

(event Custom|PluieDeComete
  ;[1 1 1] Comete
  (bind _returnvalue (Utilities|Time|SetTimerbyEvent (delegate Custom|LaunchComete) (Variables|Shoot|GetCometeInterval) true))
  (Variables|Shoot|SetPluieDeCometeEvent _returnvalue)
  (Utilities|FlowControl|Delay (Variables|Shoot|GetPluieDuration))
  (Utilities|Time|ClearandInvalidateTimerbyHandle (Variables|Shoot|GetPluieDeCometeEvent)))

(event Custom|LaunchComete
  (bind _player_ref (Variables|Ref|GetPlayer%20Ref))
  (bind _rangespawncomete (Variables|Shoot|GetRangeSpawnComete))
  (bind _returnvalue (Transformation|GetActorLocation _player_ref))
  (bind _returnvalue_2 (* _rangespawncomete -1.0))
  (bind (_x _y _z) (Math|Vector|BreakVector _returnvalue))
  ;[1 1 1] Comete
  (bind _output_get (Variables|Shoot|SetCometeTempLocation (Math|Vector|MakeVector (+ _x (Math|Random|RandomFloatinRange _returnvalue_2 _rangespawncomete)) (+ _y (Math|Random|RandomFloatinRange _returnvalue_2 _rangespawncomete)) (+ _z 3e+02))))
  (bind _outhit (Collision|LineTraceByChannel _output_get (Math|Vector|MakeVector (.X (Math|Vector|BreakVector _output_get)) (.Y (Math|Vector|BreakVector _output_get)) (- (.Z (Math|Vector|BreakVector _output_get)) 1e+04)) "TraceTypeQuery1" false 0 "None" true "(R=1.000000,G=0.000000,B=0.000000,A=1.000000)" "(R=0.000000,G=1.000000,B=0.000000,A=1.000000)" 2.0))
  (if (.bBlockingHit (Collision|BreakHitResult _outhit))
    (Game|SpawnActorfromClass "/Game/NIRVANA/Core/Characters/Enemies/Range/BP_Comète.BP_Comète_C" (Math|Transform|MakeTransform (.ImpactPoint (Collision|BreakHitResult _outhit)) "0, 0, 0" "1.000000,1.000000,1.000000") "Undefined" "MultiplyWithRoot" 0 0)))

(event Custom|GrossBoule
  (params (NbBullet :type Integer) (Spawn%20Transform%20Location :type Vector) (Direction :type Vector) (Speed :type Float%20%28double-precision%29) (Damage :type Float%20%28double-precision%29) (Delay%20Each%20Loop :type Float%20%28double-precision%29) (Pre-Visualisation :type Boolean) (Projectile%20Scale :type Float%20%28double-precision%29))
  ;[1 1 1] GrossBoule
  (Utilities|ForLoopDelayed 0 (- NbBullet 1) Delay%20Each%20Loop
    (:Loop%20Body
      (if Pre-Visualisation
        (Game|SpawnActorfromClass "/Game/NIRVANA/Core/Characters/Enemies/Projectiles/BP_EnemyProjectileApparition.BP_EnemyProjectileApparition_C" (Math|Transform|MakeTransform Spawn%20Transform%20Location "0, 0, 0" "10.000000,10.000000,10.000000") "AlwaysSpawn" "MultiplyWithRoot" 0 2.0 Spawn%20Transform%20Location Direction Speed Damage false 0.2 "0.000000,0.000000,0.000000" 0.0 (Variables|Ref|GetRef%20Bullet%20Manager) 0 "NewEnumerator1" 0)
        (else
          (Default|ActivateBullet (Variables|Ref|GetRef%20Bullet%20Manager) Spawn%20Transform%20Location Direction Speed Damage false 0.0 "0, 0, 0" 0.0 "NewEnumerator3" "10.000000,10.000000,10.000000" 0 false 0.0 0.0))))))

(event Custom|Spirale%20Infernal
  (params (Spawn%20Transform%20Location :type Vector) (Direction :type Vector) (Speed :type Float%20%28double-precision%29) (Damage :type Float%20%28double-precision%29) (Nb%20Bullet :type Integer) (Pre-Visualisation :type Boolean) (Projectil%20Scale :type Float%20%28double-precision%29))
  (bind _returnvalue (Math|Conversions|ToVector(Float) Projectil%20Scale))
  (bind _returnvalue_2 (/ Speed 1.5))
  ;[1 1 1] Spirale Infernale
  (bind _index (Utilities|ForLoopDelayed 0 (- Nb%20Bullet 1) 0.05)
    (:Loop%20Body
      (for _index_2 (range 0 11)
        (if Pre-Visualisation
          (Game|SpawnActorfromClass "/Game/NIRVANA/Core/Characters/Enemies/Projectiles/BP_EnemyProjectileApparition.BP_EnemyProjectileApparition_C" (Math|Transform|MakeTransform (+ (* (Math|Vector|RotateVectorAroundAxis (Math|Vector|GetRightVector (Math|Conversions|RotationFromXVector Direction)) (+ (* _index_2 (/ 3.6e+02 12.0)) (* _index 5.0)) Direction) 15) Spawn%20Transform%20Location) "0, 0, 0" _returnvalue) "AlwaysSpawn" "MultiplyWithRoot" 0 0.5 (+ (* (Math|Vector|RotateVectorAroundAxis (Math|Vector|GetRightVector (Math|Conversions|RotationFromXVector Direction)) (+ (* _index_2 (/ 3.6e+02 12.0)) (* _index 5.0)) Direction) 15) Spawn%20Transform%20Location) (Math|Vector|RotateVectorAroundAxis (Math|Vector|GetRightVector (Math|Conversions|RotationFromXVector Direction)) (+ (* _index_2 (/ 3.6e+02 12.0)) (* _index 5.0)) Direction) _returnvalue_2 Damage true (* _index 0.09) Direction Speed (Variables|Ref|GetRef%20Bullet%20Manager) 0 "NewEnumerator1" 0)
          (else
            (Default|ActivateBullet (Variables|Ref|GetRef%20Bullet%20Manager) (Math|Vector|MakeVector (.X (Math|Vector|BreakVector (+ (* (Math|Vector|RotateVectorAroundAxis (Math|Vector|GetRightVector (Math|Conversions|RotationFromXVector Direction)) (+ (* _index_2 (/ 3.6e+02 12.0)) (* _index 5.0)) Direction) 15) Spawn%20Transform%20Location))) (.Y (Math|Vector|BreakVector (+ (* (Math|Vector|RotateVectorAroundAxis (Math|Vector|GetRightVector (Math|Conversions|RotationFromXVector Direction)) (+ (* _index_2 (/ 3.6e+02 12.0)) (* _index 5.0)) Direction) 15) Spawn%20Transform%20Location))) (.Z (Math|Vector|BreakVector (+ (* (Math|Vector|RotateVectorAroundAxis (Math|Vector|GetRightVector (Math|Conversions|RotationFromXVector Direction)) (+ (* _index_2 (/ 3.6e+02 12.0)) (* _index 5.0)) Direction) 15) Spawn%20Transform%20Location)))) (Math|Vector|RotateVectorAroundAxis (Math|Vector|GetRightVector (Math|Conversions|RotationFromXVector Direction)) (+ (* _index_2 (/ 3.6e+02 12.0)) (* _index 5.0)) Direction) _returnvalue_2 Damage true (* _index 0.09) Direction Speed "NewEnumerator1" _returnvalue 0 false 0.0 0.0)))))))

(event Custom|Horizontal%20Round%20Mitrallette
  (params (NbBullet :type Integer) (Spawn%20Transform%20Location :type Vector) (Direction :type Vector) (Speed :type Float%20%28double-precision%29) (Damage :type Float%20%28double-precision%29) (Delay%20Each%20Loop :type Float%20%28double-precision%29) (Pre-Visualisation :type Boolean) (Projectile%20Scale :type Float%20%28double-precision%29) (Dispertion%20Speed :type Float%20%28double-precision%29))
  (bind _returnvalue (Math|Conversions|ToVector(Float) Projectile%20Scale))
  (bind _returnvalue_2 (Math|Conversions|RotationFromXVector Direction))
  ;[1 1 1] Horizontal Round
  (bind _index (Utilities|ForLoopDelayed 0 (- NbBullet 1) Delay%20Each%20Loop)
    (:Loop%20Body
      (if Pre-Visualisation
        (Game|SpawnActorfromClass "/Game/NIRVANA/Core/Characters/Enemies/Projectiles/BP_EnemyProjectileApparition.BP_EnemyProjectileApparition_C" (Math|Transform|MakeTransform (Math|Vector|MakeVector (.X (Math|Vector|BreakVector (+ (* (Math|Vector|RotateVectorAroundAxis (* (Math|Vector|GetRightVector _returnvalue_2) -1.0) (* _index (/ 1.8e+02 (Math|Conversions|ToFloat(Integer) NbBullet))) (Math|Vector|GetUpVector _returnvalue_2)) 2e+02) Spawn%20Transform%20Location))) (.Y (Math|Vector|BreakVector (+ (* (Math|Vector|RotateVectorAroundAxis (* (Math|Vector|GetRightVector _returnvalue_2) -1.0) (* _index (/ 1.8e+02 (Math|Conversions|ToFloat(Integer) NbBullet))) (Math|Vector|GetUpVector _returnvalue_2)) 2e+02) Spawn%20Transform%20Location))) (+ (.Z (Math|Vector|BreakVector (+ (* (Math|Vector|RotateVectorAroundAxis (* (Math|Vector|GetRightVector _returnvalue_2) -1.0) (* _index (/ 1.8e+02 (Math|Conversions|ToFloat(Integer) NbBullet))) (Math|Vector|GetUpVector _returnvalue_2)) 2e+02) Spawn%20Transform%20Location))) (* (stale _index) 5e+01))) "0, 0, 0" _returnvalue) "AlwaysSpawn" "MultiplyWithRoot" 0 (+ 0.5 (* _index 0.1)) (Math|Vector|MakeVector (.X (Math|Vector|BreakVector (+ (* (Math|Vector|RotateVectorAroundAxis (* (Math|Vector|GetRightVector _returnvalue_2) -1.0) (* _index (/ 1.8e+02 (Math|Conversions|ToFloat(Integer) NbBullet))) (Math|Vector|GetUpVector _returnvalue_2)) 2e+02) Spawn%20Transform%20Location))) (.Y (Math|Vector|BreakVector (+ (* (Math|Vector|RotateVectorAroundAxis (* (Math|Vector|GetRightVector _returnvalue_2) -1.0) (* _index (/ 1.8e+02 (Math|Conversions|ToFloat(Integer) NbBullet))) (Math|Vector|GetUpVector _returnvalue_2)) 2e+02) Spawn%20Transform%20Location))) (+ (.Z (Math|Vector|BreakVector (+ (* (Math|Vector|RotateVectorAroundAxis (* (Math|Vector|GetRightVector _returnvalue_2) -1.0) (* _index (/ 1.8e+02 (Math|Conversions|ToFloat(Integer) NbBullet))) (Math|Vector|GetUpVector _returnvalue_2)) 2e+02) Spawn%20Transform%20Location))) (* (stale _index) 5e+01))) (Utilities|Dispertion Spawn%20Transform%20Location (+ (* (Math|Vector|RotateVectorAroundAxis (* (Math|Vector|GetRightVector _returnvalue_2) -1.0) (* _index (/ 1.8e+02 (Math|Conversions|ToFloat(Integer) NbBullet))) (Math|Vector|GetUpVector _returnvalue_2)) 2e+02) Spawn%20Transform%20Location) Direction Dispertion%20Speed false) Speed Damage false 0.2 "0.000000,0.000000,0.000000" 0.0 (Variables|Ref|GetRef%20Bullet%20Manager) 0 "NewEnumerator5" 0)
        (else
          (Default|ActivateBullet (Variables|Ref|GetRef%20Bullet%20Manager) (Math|Vector|MakeVector (.X (Math|Vector|BreakVector (+ (* (Math|Vector|RotateVectorAroundAxis (* (Math|Vector|GetRightVector _returnvalue_2) -1.0) (* _index (/ 1.8e+02 (Math|Conversions|ToFloat(Integer) NbBullet))) (Math|Vector|GetUpVector _returnvalue_2)) 2e+02) Spawn%20Transform%20Location))) (.Y (Math|Vector|BreakVector (+ (* (Math|Vector|RotateVectorAroundAxis (* (Math|Vector|GetRightVector _returnvalue_2) -1.0) (* _index (/ 1.8e+02 (Math|Conversions|ToFloat(Integer) NbBullet))) (Math|Vector|GetUpVector _returnvalue_2)) 2e+02) Spawn%20Transform%20Location))) (+ (.Z (Math|Vector|BreakVector (+ (* (Math|Vector|RotateVectorAroundAxis (* (Math|Vector|GetRightVector _returnvalue_2) -1.0) (* _index (/ 1.8e+02 (Math|Conversions|ToFloat(Integer) NbBullet))) (Math|Vector|GetUpVector _returnvalue_2)) 2e+02) Spawn%20Transform%20Location))) (* (stale _index) 5e+01))) (Utilities|Dispertion Spawn%20Transform%20Location (+ (* (Math|Vector|RotateVectorAroundAxis (* (Math|Vector|GetRightVector _returnvalue_2) -1.0) (* _index (/ 1.8e+02 (Math|Conversions|ToFloat(Integer) NbBullet))) (Math|Vector|GetUpVector _returnvalue_2)) 2e+02) Spawn%20Transform%20Location) Direction Dispertion%20Speed false) Speed Damage false 0.0 "0, 0, 0" 0.0 "NewEnumerator5" _returnvalue 0 false 0.0 0.0))))))

(event Custom|Ceiling%20Spiral
  (params (Spawn%20Transform%20Location :type Vector) (Direction :type Vector) (Speed :type Float%20%28double-precision%29) (Damage :type Float%20%28double-precision%29) (Nb%20Bullet :type Integer) (Pre-Visualisation :type Boolean) (Projectil%20Scale :type Float%20%28double-precision%29))
  (bind _returnvalue (Math|Conversions|ToVector(Float) Projectil%20Scale))
  ;[0.4157 1 0.302] Ceiling Spiral
  (bind _index (Utilities|ForLoopDelayed 0 (- Nb%20Bullet 1) 0.05)
    (:Loop%20Body
      (if (> _index 1)
        (for _index_2 (range 0 11)
          (if Pre-Visualisation
            (Game|SpawnActorfromClass "/Game/NIRVANA/Core/Characters/Enemies/Projectiles/BP_EnemyProjectileApparition.BP_EnemyProjectileApparition_C" (Math|Transform|MakeTransform (+ (* (Math|Vector|RotateVectorAroundAxis "1.000000,0.000000,0.000000" (+ (* _index_2 (/ 3.6e+02 12.0)) (* _index 5.0)) "0.000000,0.000000,1.000000") 100) Spawn%20Transform%20Location) "0, 0, 0" _returnvalue) "AlwaysSpawn" "MultiplyWithRoot" 0 0.5 (+ (* (Math|Vector|RotateVectorAroundAxis "1.000000,0.000000,0.000000" (+ (* _index_2 (/ 3.6e+02 12.0)) (* _index 5.0)) "0.000000,0.000000,1.000000") 100) Spawn%20Transform%20Location) (Math|Vector|RotateVectorAroundAxis "1.000000,0.000000,0.000000" (+ (* _index_2 (/ 3.6e+02 12.0)) (* _index 5.0)) "0.000000,0.000000,1.000000") 6e+02 Damage true (* _index 0.085) "0.000000,0.000000,-1.000000" Speed (Variables|Ref|GetRef%20Bullet%20Manager) 0 "NewEnumerator1" 0)
            (else
              (Default|ActivateBullet (Variables|Ref|GetRef%20Bullet%20Manager) (Math|Vector|MakeVector (.X (Math|Vector|BreakVector (+ (* (Math|Vector|RotateVectorAroundAxis "1.000000,0.000000,0.000000" (+ (* _index_2 (/ 3.6e+02 12.0)) (* _index 5.0)) "0.000000,0.000000,1.000000") 100) Spawn%20Transform%20Location))) (.Y (Math|Vector|BreakVector (+ (* (Math|Vector|RotateVectorAroundAxis "1.000000,0.000000,0.000000" (+ (* _index_2 (/ 3.6e+02 12.0)) (* _index 5.0)) "0.000000,0.000000,1.000000") 100) Spawn%20Transform%20Location))) (.Z (Math|Vector|BreakVector (+ (* (Math|Vector|RotateVectorAroundAxis "1.000000,0.000000,0.000000" (+ (* _index_2 (/ 3.6e+02 12.0)) (* _index 5.0)) "0.000000,0.000000,1.000000") 100) Spawn%20Transform%20Location)))) (Math|Vector|RotateVectorAroundAxis "1.000000,0.000000,0.000000" (+ (* _index_2 (/ 3.6e+02 12.0)) (* _index 5.0)) "0.000000,0.000000,1.000000") Speed Damage true (* _index 0.085) "0.000000,0.000000,-1.000000" Speed "NewEnumerator1" _returnvalue 0 false 0.0 0.0))))))))

(event Custom|Circle%20Explosion
  (params (NbBullet :type Integer) (Spawn%20Transform%20Location :type Vector) (Direction :type Vector) (Speed :type Float%20%28double-precision%29) (Damage :type Float%20%28double-precision%29) (Delay%20Each%20Loop :type Float%20%28double-precision%29) (Pre-Visualisation :type Boolean) (Projectile%20Scale :type Float%20%28double-precision%29) (Dispertion%20Speed :type Float%20%28double-precision%29))
  (bind _returnvalue (Math|Conversions|ToFloat(Integer) NbBullet))
  (bind _returnvalue_2 (- NbBullet 1))
  (bind _returnvalue_3 (/ 3.6e+02 _returnvalue))
  ;[0.4157 1 0.302] Circle Explosion
  (for _index (range 0 1) ; Etages
    (bind _index_2 (Utilities|ForLoopDelayed 0 _returnvalue_2 Delay%20Each%20Loop)
      (:Loop%20Body
        (if (not (Math|Boolean|ORBoolean (and (< (/ (Math|Conversions|ToFloat(Integer) _index_2) (Math|Conversions|ToFloat(Integer) _returnvalue_2)) 0.39) (> (/ (Math|Conversions|ToFloat(Integer) _index_2) (Math|Conversions|ToFloat(Integer) _returnvalue_2)) 0.27)) (and (< (/ (Math|Conversions|ToFloat(Integer) _index_2) (Math|Conversions|ToFloat(Integer) _returnvalue_2)) 0.72) (> (/ (Math|Conversions|ToFloat(Integer) _index_2) (Math|Conversions|ToFloat(Integer) _returnvalue_2)) 0.6)) (> (/ (Math|Conversions|ToFloat(Integer) _index_2) (Math|Conversions|ToFloat(Integer) _returnvalue_2)) 0.88)))
          (if Pre-Visualisation
            (Game|SpawnActorfromClass "/Game/NIRVANA/Core/Characters/Enemies/Projectiles/BP_EnemyProjectileApparition.BP_EnemyProjectileApparition_C" (Math|Transform|MakeTransform (Math|Vector|MakeVector (.X (Math|Vector|BreakVector (+ (* (Math|Vector|RotateVectorAroundAxis Direction (+ (* _index_2 _returnvalue_3) (+ _returnvalue_3 (* _returnvalue_3 (Math|Float|SelectFloat 0.0 0.5 (== (Math|Integer|%(Integer) _index 2) 0))))) "0.000000,0.000000,1.000000") 1e+02) Spawn%20Transform%20Location))) (.Y (Math|Vector|BreakVector (+ (* (Math|Vector|RotateVectorAroundAxis Direction (+ (* _index_2 _returnvalue_3) (+ _returnvalue_3 (* _returnvalue_3 (Math|Float|SelectFloat 0.0 0.5 (== (Math|Integer|%(Integer) _index 2) 0))))) "0.000000,0.000000,1.000000") 1e+02) Spawn%20Transform%20Location))) (+ (.Z (Math|Vector|BreakVector (+ (* (Math|Vector|RotateVectorAroundAxis Direction (+ (* _index_2 _returnvalue_3) (+ _returnvalue_3 (* _returnvalue_3 (Math|Float|SelectFloat 0.0 0.5 (== (Math|Integer|%(Integer) _index 2) 0))))) "0.000000,0.000000,1.000000") 1e+02) Spawn%20Transform%20Location))) (* _index 1e+02))) "0, 0, 0" (Math|Conversions|ToVector(Float) Projectile%20Scale)) "AlwaysSpawn" "MultiplyWithRoot" 0 0.5 (Math|Vector|MakeVector (.X (Math|Vector|BreakVector (+ (* (Math|Vector|RotateVectorAroundAxis Direction (+ (* _index_2 _returnvalue_3) (+ _returnvalue_3 (* _returnvalue_3 (Math|Float|SelectFloat 0.0 0.5 (== (Math|Integer|%(Integer) _index 2) 0))))) "0.000000,0.000000,1.000000") 1e+02) Spawn%20Transform%20Location))) (.Y (Math|Vector|BreakVector (+ (* (Math|Vector|RotateVectorAroundAxis Direction (+ (* _index_2 _returnvalue_3) (+ _returnvalue_3 (* _returnvalue_3 (Math|Float|SelectFloat 0.0 0.5 (== (Math|Integer|%(Integer) _index 2) 0))))) "0.000000,0.000000,1.000000") 1e+02) Spawn%20Transform%20Location))) (+ (.Z (Math|Vector|BreakVector (+ (* (Math|Vector|RotateVectorAroundAxis Direction (+ (* _index_2 _returnvalue_3) (+ _returnvalue_3 (* _returnvalue_3 (Math|Float|SelectFloat 0.0 0.5 (== (Math|Integer|%(Integer) _index 2) 0))))) "0.000000,0.000000,1.000000") 1e+02) Spawn%20Transform%20Location))) (* _index 1e+02))) (Math|Vector|MakeVector (.X (Math|Vector|BreakVector (Math|Vector|RotateVectorAroundAxis Direction (+ (* _index_2 _returnvalue_3) (+ _returnvalue_3 (* _returnvalue_3 (Math|Float|SelectFloat 0.0 0.5 (== (Math|Integer|%(Integer) _index 2) 0))))) "0.000000,0.000000,1.000000"))) (.Y (Math|Vector|BreakVector (Math|Vector|RotateVectorAroundAxis Direction (+ (* _index_2 _returnvalue_3) (+ _returnvalue_3 (* _returnvalue_3 (Math|Float|SelectFloat 0.0 0.5 (== (Math|Integer|%(Integer) _index 2) 0))))) "0.000000,0.000000,1.000000"))) 0.0) Speed Damage false 0.2 "0.000000,0.000000,0.000000" 0.0 (Variables|Ref|GetRef%20Bullet%20Manager) 0 "NewEnumerator1" 0)
            (else
              (Default|ActivateBullet (Variables|Ref|GetRef%20Bullet%20Manager) (Math|Vector|MakeVector (.X (Math|Vector|BreakVector (+ (* (Math|Vector|RotateVectorAroundAxis Direction (+ (* _index_2 _returnvalue_3) (+ _returnvalue_3 (* _returnvalue_3 (Math|Float|SelectFloat 0.0 0.5 (== (Math|Integer|%(Integer) _index 2) 0))))) "0.000000,0.000000,1.000000") 1e+02) Spawn%20Transform%20Location))) (.Y (Math|Vector|BreakVector (+ (* (Math|Vector|RotateVectorAroundAxis Direction (+ (* _index_2 _returnvalue_3) (+ _returnvalue_3 (* _returnvalue_3 (Math|Float|SelectFloat 0.0 0.5 (== (Math|Integer|%(Integer) _index 2) 0))))) "0.000000,0.000000,1.000000") 1e+02) Spawn%20Transform%20Location))) (+ (.Z (Math|Vector|BreakVector (+ (* (Math|Vector|RotateVectorAroundAxis Direction (+ (* _index_2 _returnvalue_3) (+ _returnvalue_3 (* _returnvalue_3 (Math|Float|SelectFloat 0.0 0.5 (== (Math|Integer|%(Integer) _index 2) 0))))) "0.000000,0.000000,1.000000") 1e+02) Spawn%20Transform%20Location))) (* _index 1e+02))) (Math|Vector|MakeVector (.X (Math|Vector|BreakVector (Math|Vector|RotateVectorAroundAxis Direction (+ (* _index_2 _returnvalue_3) (+ _returnvalue_3 (* _returnvalue_3 (Math|Float|SelectFloat 0.0 0.5 (== (Math|Integer|%(Integer) _index 2) 0))))) "0.000000,0.000000,1.000000"))) (.Y (Math|Vector|BreakVector (Math|Vector|RotateVectorAroundAxis Direction (+ (* _index_2 _returnvalue_3) (+ _returnvalue_3 (* _returnvalue_3 (Math|Float|SelectFloat 0.0 0.5 (== (Math|Integer|%(Integer) _index 2) 0))))) "0.000000,0.000000,1.000000"))) 0.0) Speed Damage false 0.0 "0, 0, 0" 0.0 "NewEnumerator1" "1.500000,1.500000,1.500000" 0 false 0.0 0.0))))))))

(event Custom|ShotgunExplosion
  (params (NbBullet :type Integer) (Spawn%20Transform%20Location :type Vector) (Direction :type Vector) (Speed :type Float%20%28double-precision%29) (Damage :type Float%20%28double-precision%29) (Delay%20Each%20Loop :type Float%20%28double-precision%29) (Pre-Visualisation :type Boolean) (Projectile%20Scale :type Float%20%28double-precision%29) (Dispertion%20Speed :type Float%20%28double-precision%29))
  (bind _returnvalue (Math|Conversions|ToVector(Float) Projectile%20Scale))
  (bind _returnvalue_2 (Math|Random|RandomUnitVectorinConeinDegrees Direction 3.6e+02))
  ;[1 1 1] Shotgun
  (Utilities|ForLoopDelayed 0 (- NbBullet 1) 0.0
    (:Loop%20Body
      (if Pre-Visualisation
        (Game|SpawnActorfromClass "/Game/NIRVANA/Core/Characters/Enemies/Projectiles/BP_EnemyProjectileApparition.BP_EnemyProjectileApparition_C" (Math|Transform|MakeTransform Spawn%20Transform%20Location "0, 0, 0" _returnvalue) "AlwaysSpawn" "MultiplyWithRoot" 0 0.5 Spawn%20Transform%20Location _returnvalue_2 Speed Damage false 0.2 "0.000000,0.000000,0.000000" 0.0 (Variables|Ref|GetRef%20Bullet%20Manager) 0 "NewEnumerator1" 0)
        (else
          (Default|ActivateBullet (Variables|Ref|GetRef%20Bullet%20Manager) Spawn%20Transform%20Location _returnvalue_2 Speed Damage false 0.0 "0, 0, 0" 0.0 "NewEnumerator1" _returnvalue 0 false 0.0 0.0))))))

(event Custom|Shotgun
  (params (NbBullet :type Integer) (Spawn%20Transform%20Location :type Vector) (Direction :type Vector) (Speed :type Float%20%28double-precision%29) (Damage :type Float%20%28double-precision%29) (Delay%20Each%20Loop :type Float%20%28double-precision%29) (Pre-Visualisation :type Boolean) (Projectile%20Scale :type Float%20%28double-precision%29) (Dispertion%20Speed :type Float%20%28double-precision%29))
  (bind _returnvalue (Math|Conversions|ToVector(Float) Projectile%20Scale))
  (bind _returnvalue_2 (Math|Random|RandomUnitVectorinConeinDegrees Direction 2e+01))
  ;[1 1 1] Shotgun
  (Utilities|ForLoopDelayed 0 2 0.2
    (:Loop%20Body
      (Utilities|ForLoopDelayed 0 (- NbBullet 1) 0.0
        (:Loop%20Body
          (if Pre-Visualisation
            (Game|SpawnActorfromClass "/Game/NIRVANA/Core/Characters/Enemies/Projectiles/BP_EnemyProjectileApparition.BP_EnemyProjectileApparition_C" (Math|Transform|MakeTransform Spawn%20Transform%20Location "0, 0, 0" _returnvalue) "AlwaysSpawn" "MultiplyWithRoot" 0 0.5 Spawn%20Transform%20Location _returnvalue_2 Speed Damage false 0.2 "0.000000,0.000000,0.000000" 0.0 (Variables|Ref|GetRef%20Bullet%20Manager) 0 "NewEnumerator1" 0)
            (else
              (Default|ActivateBullet (Variables|Ref|GetRef%20Bullet%20Manager) Spawn%20Transform%20Location _returnvalue_2 Speed Damage false 0.0 "0, 0, 0" 0.0 "NewEnumerator1" _returnvalue 0 false 0.0 0.0))))))))

(fn ConstructionScript)

(fn SubstractLife
  (params (Life%20to%20Sub :type Float%20%28double-precision%29))
  (bind _output_get (Variables|HealthSystem|SetCurrent%20Health (- (Variables|HealthSystem|GetCurrent%20Health) Life%20to%20Sub)))
  (if (<= _output_get 0.0)
    (Variables|HealthSystem|SetCurrent%20Health 0.0)
    (Progress|SetPercent (Variables|/Game/DevelopersContent/Art/Boss/WB_Boss.WB_Boss_C|GetLifeBar (Variables|Ref|GetWidget%20Boss%20Ref)) (/ (Variables|HealthSystem|GetCurrent%20Health) (Variables|HealthSystem|GetMax%20Health)))
    (return true)
    (else
      (Progress|SetPercent (Variables|/Game/DevelopersContent/Art/Boss/WB_Boss.WB_Boss_C|GetLifeBar (Variables|Ref|GetWidget%20Boss%20Ref)) (/ (Variables|HealthSystem|GetCurrent%20Health) (Variables|HealthSystem|GetMax%20Health)))
      (return false))))

(fn GetValidZone
  (bind _output_get (LocalVariables|SetNewLocalVar (.OutItem (Utilities|Array|Random (Variables|TPSystem|GetZones%20to%20TP))) :!label _label))
  (if (not (Variables|/Game/DevelopersContent/Art/Boss/BP_BossZone.BP_BossZone_C|GetIs%20Occupated _output_get))
    (return _output_get)
    (else
      (goto _label))))

(fn SetNewZone
  (bind _new_zone (Zone|GetValidZone))
  (Variables|/Game/DevelopersContent/Art/Boss/BP_BossZone.BP_BossZone_C|SetIs%20Occupated (Variables|TPSystem|GetCurrent%20Zone) false)
  (bind _output_get (Variables|TPSystem|SetCurrent%20Zone _new_zone))
  (Variables|/Game/DevelopersContent/Art/Boss/BP_BossZone.BP_BossZone_C|SetIs%20Occupated _output_get true)
  (return))

(fn SpawnPattern
  (params (Pattern :type Enum_Pattern%20Enum :default "NewEnumerator1") (NbBullet :type Integer) (Spawn%20Transform%20Location :type Vector) (Direction :type Vector) (Speed :type Float%20%28double-precision%29) (Damage :type Float%20%28double-precision%29) (Delay%20Each%20Loop :type Float%20%28double-precision%29) (Pre-Visualisation :type Boolean) (Projectile%20Scale :type Float%20%28double-precision%29) (Dispertion :type Boolean) (Dispertion%20Speed :type Float%20%28double-precision%29) (Nb%20Bullet%20Secondaire%20%28%20Rectangle%20%29 :type Integer))
  (switch Utilities|FlowControl|Switch|SwitchonEnum_Pattern Pattern
    (:NewEnumerator1
      (CallFunction|SimplePattern NbBullet Spawn%20Transform%20Location Direction Speed Damage Delay%20Each%20Loop Pre-Visualisation Projectile%20Scale))
    (:NewEnumerator9
      (CallFunction|CircleExplosion NbBullet Spawn%20Transform%20Location Direction Speed Damage Delay%20Each%20Loop Pre-Visualisation Projectile%20Scale Dispertion%20Speed))
    (:NewEnumerator8
      (CallFunction|SpiraleInfernal Spawn%20Transform%20Location Direction Speed Damage NbBullet Pre-Visualisation Projectile%20Scale))
    (:NewEnumerator13
      (CallFunction|Rectangle NbBullet Spawn%20Transform%20Location Direction Speed Damage Delay%20Each%20Loop Pre-Visualisation Projectile%20Scale Dispertion%20Speed Nb%20Bullet%20Secondaire%20%28%20Rectangle%20%29 Dispertion))
    (:NewEnumerator16
      (CallFunction|HorizontalRound NbBullet Spawn%20Transform%20Location Direction Speed Damage Delay%20Each%20Loop Pre-Visualisation Projectile%20Scale Dispertion%20Speed))
    (:NewEnumerator17
      (CallFunction|CeilingSpiral Spawn%20Transform%20Location Direction Speed Damage NbBullet Pre-Visualisation Projectile%20Scale))
    (:NewEnumerator21
      (CallFunction|Shotgun NbBullet Spawn%20Transform%20Location Direction Speed Damage Delay%20Each%20Loop Pre-Visualisation Projectile%20Scale Dispertion%20Speed))
    (:NewEnumerator22
      (CallFunction|ShotgunExplosion NbBullet Spawn%20Transform%20Location Direction Speed Damage Delay%20Each%20Loop Pre-Visualisation Projectile%20Scale Dispertion%20Speed))
    (:NewEnumerator23
      (CallFunction|GrossBoule NbBullet Spawn%20Transform%20Location Direction Speed Damage Delay%20Each%20Loop Pre-Visualisation Projectile%20Scale))
    (:NewEnumerator24
      (CallFunction|PluieDeComete))
    (:NewEnumerator25
      (CallFunction|HorizontalRoundMitrallette NbBullet Spawn%20Transform%20Location Direction Speed Damage Delay%20Each%20Loop Pre-Visualisation Projectile%20Scale Dispertion%20Speed))))

(fn GetPattern
  (return (Variables|Shoot|GetcurrentPattern)))

(fn IsWeakened
  (params (Damage :type Float%20%28double-precision%29))
  (bind _output_get (Variables|HealthSystem|SetDealtDamage (+ (Variables|HealthSystem|GetDealtDamage) (/ Damage (Variables|HealthSystem|GetMax%20Health)))))
  (return (>= _output_get 0.34)))
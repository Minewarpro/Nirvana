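; Trigger actor that plays a one-shot fresco (Fresque) sequence when the first-person player enters its box.
; It spawns ClassFresque at Spawn, starts a media video, and lerps the fresco to Offset via timeline.
; After delays chained from timeline updates, it lerps back, destroys the fresco and shifts WallToMove vertically.
; The construction script offsets both anchor points by configurable amounts.
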(event `self.ReceiveBeginPlay`
  ;[1 1 1] PlayerRef
  (bind _asbp_first_person_character (cast `/Game/NIRVANA/Core/Characters/FirstPerson/BP_FirstPersonCharacter` (`GameplayStatics.GetPlayerCharacter` 0)))
  (set `self.PlayrRef` _asbp_first_person_character))

(event `self.Box.OnComponentBeginOverlap`
  (params (OverlappedComponent :type "PrimitiveComponent Object Reference") (OtherActor :type "Actor Object Reference") (OtherComp :type "PrimitiveComponent Object Reference") (OtherBodyIndex :type Integer) (bFromSweep :type Boolean) (SweepResult :type "HitResult Structure (by ref)"))
  (bind _returnvalue (`SceneComponent.K2_GetComponentLocation` (`self.Spawn`)))
  ;[1 1 1] Conditions activation
  (if (== OtherActor (`self.PlayrRef`))
    (if (`self.Activated`)
      (set `self.Activated` false)
      ;[1 1 1] Spawn Fresque sur location + reference
      (bind _returnvalue_2 (`|SpawnActorFromClass` (`self.ClassFresque`) (`KismetMathLibrary.MakeTransform` _returnvalue) "Undefined" "MultiplyWithRoot" null null))
      (set `self.Fresque` _returnvalue_2)
      ;[1 1 1] Start video
      (`MediaPlayer.OpenSource` (`self.MediaPlayer`) "/Game/DevelopersContent/Effects/Fresque/Src_FresqueTest.Src_FresqueTest")
      ;[1 1 1] Move la fresque to offset
      (bind (_direction _newtrack_0) (`Timeline|ToOffset`)
        (:`Update`
          (`SceneComponent.K2_SetWorldLocation` (`Actor.RootComponent` (`self.Fresque`)) (`KismetMathLibrary.VLerp` _returnvalue (`SceneComponent.K2_GetComponentLocation` (`self.Offset`)) _newtrack_0) false false)
          ;[1 1 1] Retour au spawn
          (`KismetSystemLibrary.Delay` (`self.Timing`))
          (bind (_direction_2 _newtrack_0_2) (`Timeline|BackToSpawn`)
            (:`Update`
              (`SceneComponent.K2_SetWorldLocation` (`Actor.RootComponent` (`self.Fresque`)) (`KismetMathLibrary.VLerp` (`SceneComponent.K2_GetComponentLocation` (`self.Offset`)) (`SceneComponent.K2_GetComponentLocation` (`self.Spawn`)) _newtrack_0_2) false false)
              ;[1 1 1] destroy la fresque
              (`KismetSystemLibrary.Delay` 2.0)
              (`self.K2_DestroyActor` (`self.Fresque`))
              (bind (_direction_3 _newtrack_0_3) (`Timeline|Timeline`)
                (:`Update`
                  (`SceneComponent.K2_AddWorldOffset` (`Actor.RootComponent` (`self.WallToMove`)) (`KismetMathLibrary.MakeVector` 0.0 0.0 (* _newtrack_0_3 1.0)) false false))))))))))

(fn `UserConstructionScript`
  (bind _spawn (`self.Spawn`))
  (bind _offset (`self.Offset`))
  (bind (_relativelocation_x _relativelocation_y _relativelocation_z) (`KismetMathLibrary.BreakVector` (`SceneComponent.RelativeLocation` _spawn)))
  (bind (_relativelocation_x_2 _relativelocation_y_2 _relativelocation_z_2) (`KismetMathLibrary.BreakVector` (`SceneComponent.RelativeLocation` _offset)))
  (`SceneComponent.K2_SetRelativeLocation` _spawn (`KismetMathLibrary.MakeVector` (+ _relativelocation_x (`self.SpawnFresqueX`)) (+ _relativelocation_y (`self.SpawnFresqueY`)) (+ _relativelocation_z (`self.SpawnFresqueZ`))) false false)
  (`SceneComponent.K2_SetRelativeLocation` _offset (`KismetMathLibrary.MakeVector` (+ _relativelocation_x_2 (`self.OffsetFresX`)) (+ _relativelocation_y_2 (`self.OffsetFresY`)) (+ _relativelocation_z_2 (`self.OffsetFresZ`))) false false))
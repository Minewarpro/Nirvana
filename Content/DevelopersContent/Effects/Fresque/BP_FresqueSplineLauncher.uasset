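; Trigger actor that plays a fresco cinematic when the first-person player overlaps its box, then moves a wall.
; While activated, it fires once, disabling input, blending to a cinematic camera and playing the assigned level sequence.
; After a delay equal to the sequence duration, it restores the previous view target and input.
; A timeline then adds a vertical offset to the wall every update, so total travel depends on frame rate.
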(event `self.ReceiveBeginPlay`
  (bind _asbp_first_person_character (cast `/Game/NIRVANA/Core/Characters/FirstPerson/BP_FirstPersonCharacter` (`GameplayStatics.GetPlayerCharacter` 0)))
  (set `self.PlayerRef` _asbp_first_person_character))

(event `self.Box.OnComponentBeginOverlap`
  (params (OverlappedComponent :type "PrimitiveComponent Object Reference") (OtherActor :type "Actor Object Reference") (OtherComp :type "PrimitiveComponent Object Reference") (OtherBodyIndex :type Integer) (bFromSweep :type Boolean) (SweepResult :type "HitResult Structure (by ref)"))
  (if (== OtherActor (`self.PlayerRef`))
    (if (`self.Activated`)
      (`self.PlayCine`)
      (set `self.Activated` false))))

(event `PlayCine`
  (bind _returnvalue (`GameplayStatics.GetPlayerController` 0))
  (bind _sequenceplayer (`LevelSequenceActor.SequencePlayer` (`self.SequencerToPlay`)))
  (`self.DisableInput` (`self.PlayerRef`) _returnvalue)
  (set `self.CamToReturn` (`Controller.GetViewTarget` _returnvalue))
  (`PlayerController.SetViewTargetWithBlend` _returnvalue (`self.CamToBlend`) 0.2 "VTBlend_Linear" 0.0 false)
  (`MovieSceneSequencePlayer.Play` _sequenceplayer)
  (`|ExecutionSequence`
    (:`then_0`
      (`KismetSystemLibrary.Delay` (`TimeManagementBlueprintLibrary.Conv_QualifiedFrameTimeToSeconds` (`MovieSceneSequencePlayer.GetDuration` _sequenceplayer)))
      (`PlayerController.SetViewTargetWithBlend` (`GameplayStatics.GetPlayerController` 0) (`self.CamToReturn`) 0.2 "VTBlend_Linear" 0.0 false)
      (`self.EnableInput` (`self.PlayerRef`) (`GameplayStatics.GetPlayerController` 0))
      (bind (_direction _newtrack_0) (`Timeline|Timeline`)
        (:`Update`
          (`SceneComponent.K2_AddWorldOffset` (`Actor.RootComponent` (`self.wallToMove`)) (`KismetMathLibrary.MakeVector` 0.0 0.0 (* _newtrack_0 3.0)) false false))))))

(fn `UserConstructionScript`)
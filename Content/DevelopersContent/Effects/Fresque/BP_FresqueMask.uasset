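; A one-shot trigger for a fresco mask that starts a cinematic when the player enters its box.
; Overlap clears the Activated flag and plays the referenced level sequence, waits out its duration, then plays three delayed sounds at the player's location.
; The construction script positions and scales the trigger from variables and zeroes the Cube material's Speed parameter.
; ReadFresque, which animates that parameter and moves the Cube vertically by timeline, is never called here.
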(event `self.ReceiveBeginPlay`
  (bind _asbp_first_person_character (cast `/Game/NIRVANA/Core/Characters/FirstPerson/BP_FirstPersonCharacter` (`GameplayStatics.GetPlayerCharacter` 0)))
  (set `self.PlayerRef` _asbp_first_person_character))

(event `Play Sequencer`
  (bind _returnvalue (`self.K2_GetActorLocation` (`self.PlayerRef`)))
  (bind _sequenceplayer (`LevelSequenceActor.SequencePlayer` (`self.Sequencer`)))
  (`MovieSceneSequencePlayer.Play` _sequenceplayer)
  (`KismetSystemLibrary.Delay` (`TimeManagementBlueprintLibrary.Conv_QualifiedFrameTimeToSeconds` (`MovieSceneSequencePlayer.GetDuration` _sequenceplayer)))
  (`GameplayStatics.PlaySoundAtLocation` "/Game/NIRVANA/Sound/Voices/V03-SIMON/C_022_01.C_022_01" _returnvalue (struct) 1.0 1.0 0.0 null null null null)
  (`KismetSystemLibrary.Delay` 2.0)
  (`GameplayStatics.PlaySoundAtLocation` "/Game/NIRVANA/Sound/Voices/V02-BLAISE/B_021_02.B_021_02" _returnvalue (struct) 1.0 1.0 0.0 null null null null)
  (`KismetSystemLibrary.Delay` 3.0)
  (`GameplayStatics.PlaySoundAtLocation` "/Game/NIRVANA/Sound/Voices/PLAYER-ARI/J_023_V05.J_023_V05" _returnvalue (struct) 1.0 1.0 0.0 null null null null))

(event `self.Box.OnComponentBeginOverlap`
  (params (OverlappedComponent :type "PrimitiveComponent Object Reference") (OtherActor :type "Actor Object Reference") (OtherComp :type "PrimitiveComponent Object Reference") (OtherBodyIndex :type Integer) (bFromSweep :type Boolean) (SweepResult :type "HitResult Structure (by ref)"))
  (if (== OtherActor (`self.PlayerRef`))
    (if (`self.Activated`)
      (set `self.Activated` false)
      (`self.Play Sequencer`))))

(event `ReadFresque`
  (`KismetSystemLibrary.PrintString` "Start")
  (`MeshComponent.SetScalarParameterValueOnMaterials` (`self.Cube`) "Speed" (`self.Speed`))
  (`KismetSystemLibrary.Delay` (`self.Delay`))
  (`KismetSystemLibrary.PrintString` "Stop")
  (`MeshComponent.SetScalarParameterValueOnMaterials` (`self.Cube`) "Speed" 0.0)
  (bind (_direction _newtrack_0) (`Timeline|Timeline`)
    (:`Update`
      (`SceneComponent.K2_AddWorldOffset` (`self.Cube`) (`KismetMathLibrary.MakeVector` 0.0 0.0 (* _newtrack_0 3.0)) false false))))

(fn `UserConstructionScript`
  (bind _box (`self.Box`))
  (`SceneComponent.K2_SetRelativeLocation` _box (`KismetMathLibrary.MakeVector` (`self.TriggerLocX`) (`self.TriggerLocY`) (`self.TriggerLocZ`)) false false)
  (`SceneComponent.SetWorldScale3D` _box (`KismetMathLibrary.MakeVector` (`self.TriggerSizeX`) (`self.TriggerSizeY`) (`self.TriggerSizeZ`)))
  (`MeshComponent.SetScalarParameterValueOnMaterials` (`self.Cube`) "Speed" 0.0))
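; BP_MusicPlayer is a music player Blueprint that starts one selected track when play begins.
; On BeginPlay, it switches on the SwitchSound selection and plays the matching sound from the start, with one sound per named track.
; An unconnected array-based Stop call, noted as a way to stop all music, never runs, so the graph has no working stop logic.
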(event `self.ReceiveBeginPlay`
  (switch `/Game/DevelopersContent/Effects/Music/Enum_Music` (`self.Switch Sound`)
    (:`NewEnumerator0`
      (`AudioComponent.Play` (`self.Doom`) 0.0))
    (:`NewEnumerator1`
      (`AudioComponent.Play` (`self.Fumée`) 0.0))
    (:`NewEnumerator2`
      (`AudioComponent.Play` (`self.Pendulum`) 0.0))
    (:`NewEnumerator3`
      (`AudioComponent.Play` (`self.Ultrakill`) 0.0))
    (:`NewEnumerator4`
      (`AudioComponent.Play` (`self.HilightTribe`) 0.0))
    (:`NewEnumerator5`
      (`AudioComponent.Play` (`self.OxiDaksi`) 0.0))
    (:`NewEnumerator6`
      (`AudioComponent.Play` (`self.Justice`) 0.0))))

(fn `UserConstructionScript`)
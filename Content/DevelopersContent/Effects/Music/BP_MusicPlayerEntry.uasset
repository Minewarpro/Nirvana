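; BP_MusicPlayerEntry is a trigger volume that controls combat music as the first-person character enters and leaves its box.
; On overlap begin it fades the Combat audio in slowly.
; On overlap end it fades Combat out quickly, then after a short delay plays a CombatEnd audio component.
; Both events print debug strings.
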(event `self.Box.OnComponentBeginOverlap`
  (params (OverlappedComponent :type "PrimitiveComponent Object Reference") (OtherActor :type "Actor Object Reference") (OtherComp :type "PrimitiveComponent Object Reference") (OtherBodyIndex :type Integer) (bFromSweep :type Boolean) (SweepResult :type "HitResult Structure (by ref)"))
  (cast `/Game/NIRVANA/Core/Characters/FirstPerson/BP_FirstPersonCharacter` OtherActor)
  (`KismetSystemLibrary.PrintString` "CombatIn")
  (`AudioComponent.FadeIn` (`self.Combat`) 5.0 1.0 0.0 "Linear"))

(event `self.Box.OnComponentEndOverlap`
  (params (OverlappedComponent :type "PrimitiveComponent Object Reference") (OtherActor :type "Actor Object Reference") (OtherComp :type "PrimitiveComponent Object Reference") (OtherBodyIndex :type Integer))
  (cast `/Game/NIRVANA/Core/Characters/FirstPerson/BP_FirstPersonCharacter` OtherActor)
  (`KismetSystemLibrary.PrintString` "Combat out")
  (`AudioComponent.FadeOut` (`self.Combat`) 0.5 0.0 "Linear")
  (`KismetSystemLibrary.Delay` 0.2)
  (`AudioComponent.Play` (`self.CombatEnd`) 0.0))

(fn `UserConstructionScript`)
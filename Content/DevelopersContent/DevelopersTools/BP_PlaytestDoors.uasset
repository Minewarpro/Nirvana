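; Playtest developer tool that swings a pair of referenced door actors open when the player enters its box trigger.
; On BeginPlay it caches the first-person player character and both doors' starting rotations.
; A player overlap, gated and then cleared by the Activated flag, plays a timeline that lerps the doors 90 degrees in opposite yaw directions.
; Nothing in the graph closes the doors or resets the flag.
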(event `self.ReceiveBeginPlay`
  (bind _asbp_first_person_character (cast `/Game/NIRVANA/Core/Characters/FirstPerson/BP_FirstPersonCharacter` (`GameplayStatics.GetPlayerCharacter` 0)))
  (set `self.PlayerRef` _asbp_first_person_character)
  (set `self.DoorLOrigin` (`self.K2_GetActorRotation` (`self.DoorLeft`)))
  (set `self.DoorROrigin` (`self.K2_GetActorRotation` (`self.DoorRight`))))

(event `self.Box.OnComponentBeginOverlap`
  (params (OverlappedComponent :type "PrimitiveComponent Object Reference") (OtherActor :type "Actor Object Reference") (OtherComp :type "PrimitiveComponent Object Reference") (OtherBodyIndex :type Integer) (bFromSweep :type Boolean) (SweepResult :type "HitResult Structure (by ref)"))
  (bind (_doorlorigin_roll _doorlorigin_pitch _doorlorigin_yaw) (`KismetMathLibrary.BreakRotator` (`self.DoorLOrigin`)))
  (bind (_doorrorigin_roll _doorrorigin_pitch _doorrorigin_yaw) (`KismetMathLibrary.BreakRotator` (`self.DoorROrigin`)))
  (if (== OtherActor (`self.PlayerRef`))
    (if (`self.Activated`)
      (set `self.Activated` false)
      (bind (_direction _newtrack_0) (`Timeline|Timeline` :!via `PlayFromStart`)
        (:`Update`
          (`self.K2_SetActorRotation` (`self.DoorLeft`) (`KismetMathLibrary.RLerp` (`self.DoorLOrigin`) (`KismetMathLibrary.MakeRotator` _doorlorigin_roll _doorlorigin_pitch (- _doorlorigin_yaw 90.0)) _newtrack_0) false)
          (`self.K2_SetActorRotation` (`self.DoorRight`) (`KismetMathLibrary.RLerp` (`self.DoorROrigin`) (`KismetMathLibrary.MakeRotator` _doorrorigin_roll _doorrorigin_pitch (+ _doorrorigin_yaw 90.0)) _newtrack_0) false))))))

(fn `UserConstructionScript`)
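; Circular lift platform that activates when the arena is cleaned, then carries the player to a stop point and opens a pair of doors.
; OnArenaCleaned arms it and animates a linked light's intensity; player overlap with the box stops that animation and starts the move.
; A timeline lerps the cylinder, linked ball and light by one offset, then a second timeline swings the doors apart.
; The construction script offsets the stop point by StopLoc.
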(event `self.ReceiveBeginPlay`
  (set `self.Origin` (`SceneComponent.K2_GetComponentLocation` (`self.Cylinder`)))
  (set `self.LightOrigin` (`SceneComponent.K2_GetComponentLocation` (`Light.LightComponent` (`self.LightToMove`))))
  (set `self.BallOrigin` (`SceneComponent.K2_GetComponentLocation` (`/Game/NIRVANA/Effects/AutelBoule/BP_FloatingBall.DefaultSceneRoot` (`self.BallToMove`))))
  (bind _asbp_first_person_character (cast `/Game/NIRVANA/Core/Characters/FirstPerson/BP_FirstPersonCharacter` (`GameplayStatics.GetPlayerCharacter` 0)))
  (set `self.PlayerRef` _asbp_first_person_character)
  (set `self.OriginLeftDoor` (`self.K2_GetActorRotation` (`self.DoorLeft`)))
  (set `self.OriginRightDoor` (`self.K2_GetActorRotation` (`self.DoorRight`))))

(event `self.  Box.OnComponentBeginOverlap`
  (params (OverlappedComponent :type "PrimitiveComponent Object Reference") (OtherActor :type "Actor Object Reference") (OtherComp :type "PrimitiveComponent Object Reference") (OtherBodyIndex :type Integer) (bFromSweep :type Boolean) (SweepResult :type "HitResult Structure (by ref)"))
  (if (`self.Activated`)
    (if (== OtherActor (`self.PlayerRef`))
      (`self.StopLight`)
      (bind (_direction _newtrack_0) (`Timeline|Timeline` :!via `PlayFromStart`)
        (:`Update`
          (`SceneComponent.K2_SetWorldLocation` (`self.Cylinder`) (`KismetMathLibrary.VLerp` (`self.Origin`) (`SceneComponent.K2_GetComponentLocation` (`self.Stop`)) _newtrack_0) false false)
          (`SceneComponent.K2_SetWorldLocation` (`/Game/NIRVANA/Effects/AutelBoule/BP_FloatingBall.DefaultSceneRoot` (`self.BallToMove`)) (`KismetMathLibrary.VLerp` (`self.BallOrigin`) (+ (- (`self.BallOrigin`) (`self.Origin`)) (`SceneComponent.K2_GetComponentLocation` (`self.Stop`))) _newtrack_0) false false)
          (`SceneComponent.K2_SetWorldLocation` (`SpotLight.SpotLightComponent` (`self.LightToMove`)) (`KismetMathLibrary.VLerp` (`self.LightOrigin`) (+ (- (`self.LightOrigin`) (`self.Origin`)) (`SceneComponent.K2_GetComponentLocation` (`self.Stop`))) _newtrack_0) false false))
        (:`Finished`
          (`self.OpenDoor`))))))

(event `/Game/NIRVANA/Core/Placeables/Management/BPI_ArenaManager.OnArenaCleaned`
  (params (ArenaManager :type "/Game/NIRVANA/Core/Placeables/Management/BP_ArenaManager Object Reference"))
  (set `self.Activated` true)
  (`self.StartLight`))

(event `StartLight`
  (bind (_direction _newtrack_0) (`Timeline|Timeline_1` :!via `PlayFromStart` :!label _label)
    (:`Update`
      (`LightComponent.SetIntensity` (`Light.LightComponent` (`self.LightToMove`)) (`KismetMathLibrary.Lerp` 0.0 160.0 _newtrack_0)))))

(event `StopLight`
  (goto _label :!via `Stop`))

(event `OpenDoor`
  (bind (_originrightdoor_roll _originrightdoor_pitch _originrightdoor_yaw) (`KismetMathLibrary.BreakRotator` (`self.OriginRightDoor`)))
  (bind (_originleftdoor_roll _originleftdoor_pitch _originleftdoor_yaw) (`KismetMathLibrary.BreakRotator` (`self.OriginLeftDoor`)))
  (bind (_direction _newtrack_0) (`Timeline|Timeline_0`)
    (:`Update`
      (`self.K2_SetActorRotation` (`self.DoorLeft`) (`KismetMathLibrary.RLerp` (`KismetMathLibrary.MakeRotator` _originleftdoor_roll _originleftdoor_pitch _originleftdoor_yaw) (`KismetMathLibrary.MakeRotator` _originleftdoor_roll _originleftdoor_pitch (- _originleftdoor_yaw 90.0)) _newtrack_0) false)
      (`self.K2_SetActorRotation` (`self.DoorRight`) (`KismetMathLibrary.RLerp` (`KismetMathLibrary.MakeRotator` _originrightdoor_roll _originrightdoor_pitch _originrightdoor_yaw) (`KismetMathLibrary.MakeRotator` _originrightdoor_roll _originrightdoor_pitch (+ _originrightdoor_yaw 90.0)) _newtrack_0) false))))

(fn `UserConstructionScript`
  (bind _stop (`self.Stop`))
  (`SceneComponent.K2_SetRelativeLocation` _stop (+ (`SceneComponent.RelativeLocation` _stop) (`self.StopLoc`)) false false))
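; BP_SpawnTrigger is a developer-tools trigger volume that starts an enemy or object wave on a referenced arena when the player enters it.
; It caches the first-person player character on BeginPlay and compares it against actors overlapping its Box.
; While Activated is true, a player overlap calls SpawnWave on ArenaRef, then clears Activated so the trigger does not fire again.
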(event `self.ReceiveBeginPlay`
  (bind _asbp_first_person_character (cast `/Game/NIRVANA/Core/Characters/FirstPerson/BP_FirstPersonCharacter` (`GameplayStatics.GetPlayerCharacter` 0)))
  (set `self.PlayerRef` _asbp_first_person_character))

(event `self.Box.OnComponentBeginOverlap`
  (params (OverlappedComponent :type "PrimitiveComponent Object Reference") (OtherActor :type "Actor Object Reference") (OtherComp :type "PrimitiveComponent Object Reference") (OtherBodyIndex :type Integer) (bFromSweep :type Boolean) (SweepResult :type "HitResult Structure (by ref)"))
  (if (`self.Activated`)
    (if (== OtherActor (`self.PlayerRef`))
      (`/Game/NIRVANA/Core/Placeables/Management/BP_ArenaManager.SpawnWave` (`self.ArenaRef`))
      (set `self.Activated` false))))

(fn `UserConstructionScript`)
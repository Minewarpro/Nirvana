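; Developer test-arena control actor that lets the player configure and launch enemy spawns by walking into trigger volumes.
; Plus and minus triggers adjust a capped, displayed enemy count, while Type and Size triggers cycle options and shift indicator points.
; Size also slides a wall to change the arena, resetting to its cached origin.
; Start spawns the chosen enemy class at successive spawner locations, one per counted enemy.
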(event `self.ReceiveBeginPlay`
  ;[1 1 1] Begin play : Player ref + point origin
  (bind _asbp_first_person_character (cast `/Game/NIRVANA/Core/Characters/FirstPerson/BP_FirstPersonCharacter` (`GameplayStatics.GetPlayerCharacter` 0)))
  (set `self.PlayerRef` _asbp_first_person_character)
  (set `self.PointLoc` (`SceneComponent.RelativeLocation` (`self.Point`)))
  (set `self.Point2Loc` (`SceneComponent.RelativeLocation` (`self.Point1`)))
  (set `self.WallOrigin` (`SceneComponent.K2_GetComponentLocation` (`StaticMeshActor.StaticMeshComponent` (`self.WallToMove`)))))

(event `self.EnemyPlus.OnComponentBeginOverlap`
  (params (OverlappedComponent :type "PrimitiveComponent Object Reference") (OtherActor :type "Actor Object Reference") (OtherComp :type "PrimitiveComponent Object Reference") (OtherBodyIndex :type Integer) (bFromSweep :type Boolean) (SweepResult :type "HitResult Structure (by ref)"))
  (bind _nbennemy (`self.NbEnnemy`))
  ;[1 1 1] Gestion du nombre d'ennemis entre 0 et 6
  (if (== OtherActor (`self.PlayerRef`))
    (if (< (`self.NbEnnemy`) 6)
      (set `self.NbEnnemy` (+ _nbennemy 1))
      (`TextRenderComponent.K2_SetText` (`self.NBennemies`) (`KismetTextLibrary.Conv_IntToText` _nbennemy)))))

(event `self.Type.OnComponentBeginOverlap`
  (params (OverlappedComponent :type "PrimitiveComponent Object Reference") (OtherActor :type "Actor Object Reference") (OtherComp :type "PrimitiveComponent Object Reference") (OtherBodyIndex :type Integer) (bFromSweep :type Boolean) (SweepResult :type "HitResult Structure (by ref)"))
  (bind _point (`self.Point`))
  (bind (_relativelocation_x _relativelocation_y _relativelocation_z) (`KismetMathLibrary.BreakVector` (`SceneComponent.RelativeLocation` _point)))
  ;[1 1 1] Choix du type de mid à spawn
  (if (== OtherActor (`self.PlayerRef`))
    (if (< (`self.EnemyChoice`) 2)
      (set `self.EnemyChoice` (+ (`self.EnemyChoice`) 1))
      (`SceneComponent.K2_SetRelativeLocation` _point (`KismetMathLibrary.MakeVector` _relativelocation_x (- _relativelocation_y 165.0) _relativelocation_z) false false)
      (else
        (set `self.EnemyChoice` 0)
        (`SceneComponent.K2_SetRelativeLocation` (`self.Point`) (`self.PointLoc`) false false)))))

(event `self.EnemyMinus.OnComponentBeginOverlap`
  (params (OverlappedComponent :type "PrimitiveComponent Object Reference") (OtherActor :type "Actor Object Reference") (OtherComp :type "PrimitiveComponent Object Reference") (OtherBodyIndex :type Integer) (bFromSweep :type Boolean) (SweepResult :type "HitResult Structure (by ref)"))
  (bind _nbennemy (`self.NbEnnemy`))
  ;[1 1 1] Gestion du nombre d'ennemis entre 0 et 6
  (if (== OtherActor (`self.PlayerRef`))
    (if (> (`self.NbEnnemy`) 0)
      (set `self.NbEnnemy` (- _nbennemy 1))
      (`TextRenderComponent.K2_SetText` (`self.NBennemies`) (`KismetTextLibrary.Conv_IntToText` _nbennemy)))))

(event `self.Size.OnComponentBeginOverlap`
  (params (OverlappedComponent :type "PrimitiveComponent Object Reference") (OtherActor :type "Actor Object Reference") (OtherComp :type "PrimitiveComponent Object Reference") (OtherBodyIndex :type Integer) (bFromSweep :type Boolean) (SweepResult :type "HitResult Structure (by ref)"))
  (bind _point1 (`self.Point1`))
  (bind (_relativelocation_x _relativelocation_y _relativelocation_z) (`KismetMathLibrary.BreakVector` (`SceneComponent.RelativeLocation` _point1)))
  (bind _staticmeshcomponent (`StaticMeshActor.StaticMeshComponent` (`self.WallToMove`)))
  (bind (_returnvalue_x _returnvalue_y _returnvalue_z) (`KismetMathLibrary.BreakVector` (`SceneComponent.K2_GetComponentLocation` _staticmeshcomponent)))
  (if (== OtherActor (`self.PlayerRef`))
    (if (< (`self.SizeIndex`) 2)
      (set `self.SizeIndex` (+ (`self.SizeIndex`) 1))
      (`SceneComponent.K2_SetRelativeLocation` _point1 (`KismetMathLibrary.MakeVector` _relativelocation_x (+ _relativelocation_y 140.0) _relativelocation_z) false false)
      (`SceneComponent.K2_SetWorldLocation` _staticmeshcomponent (`KismetMathLibrary.MakeVector` _returnvalue_x (+ _returnvalue_y 1250.0) _returnvalue_z) false false)
      (else
        (set `self.SizeIndex` 0)
        (`SceneComponent.K2_SetRelativeLocation` (`self.Point1`) (`self.Point2Loc`) false false)
        (`SceneComponent.K2_SetWorldLocation` (`StaticMeshActor.StaticMeshComponent` (`self.WallToMove`)) (`self.WallOrigin`) false false)))))

(event `self.Start.OnComponentBeginOverlap`
  (params (OverlappedComponent :type "PrimitiveComponent Object Reference") (OtherActor :type "Actor Object Reference") (OtherComp :type "PrimitiveComponent Object Reference") (OtherBodyIndex :type Integer) (bFromSweep :type Boolean) (SweepResult :type "HitResult Structure (by ref)"))
  ;[1 1 1] Activation du spawn avec les paramètres de l'arene
  (if (== OtherActor (`self.PlayerRef`))
    (for _index (range (`self.NbEnnemy`))
      (bind (_returnvalue_x _returnvalue_y _returnvalue_z) (`KismetMathLibrary.BreakVector` (`self.K2_GetActorLocation` (`|GetArrayItem` (`self.Spawners`) _index))))
      (`|SpawnActorFromClass` (`|GetArrayItem` (`self.EnnemiesToSpawn`) (`self.EnemyChoice`)) (`KismetMathLibrary.MakeTransform` (`KismetMathLibrary.MakeVector` _returnvalue_x _returnvalue_y (- _returnvalue_z 10.0))) "Undefined" "MultiplyWithRoot" null null))
    (`KismetSystemLibrary.PrintString` "Ennemy Spawned")))

(fn `UserConstructionScript`)
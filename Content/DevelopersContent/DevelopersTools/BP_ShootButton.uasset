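; BP_ShootButton is a one-shot button in the developer tools folder that lowers a linked Door when its trigger box is overlapped.
; While Activated is true, an overlap swaps the Cube material and plays a Timeline that lerps the Door down by Offset, then clears Activated.
; The start position is cached in world space but applied as relative location.
; The Vajra and Chakram projectile check is disconnected, so overlaps are not filtered.
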(event `self.ReceiveBeginPlay`
  (set `self.Origin` (`SceneComponent.K2_GetComponentLocation` (`StaticMeshActor.StaticMeshComponent` (`self.Door`)))))

(event `self.Box.OnComponentBeginOverlap`
  (params (OverlappedComponent :type "PrimitiveComponent Object Reference") (OtherActor :type "Actor Object Reference") (OtherComp :type "PrimitiveComponent Object Reference") (OtherBodyIndex :type Integer) (bFromSweep :type Boolean) (SweepResult :type "HitResult Structure (by ref)"))
  (bind (_origin_x _origin_y _origin_z) (`KismetMathLibrary.BreakVector` (`self.Origin`)))
  (if (`self.Activated`)
    (`PrimitiveComponent.SetMaterial` (`self.Cube`) 0 "/Game/DevelopersContent/_GENERATED/Lucaslebeauf/LevelPrototyping/Textures/M_PrototypeGrid_Wall1.M_PrototypeGrid_Wall1")
    (bind (_direction _newtrack_0) (`Timeline|Timeline` :!via `PlayFromStart`)
      (:`Update`
        (`SceneComponent.K2_SetRelativeLocation` (`StaticMeshActor.StaticMeshComponent` (`self.Door`)) (`KismetMathLibrary.VLerp` (`self.Origin`) (`KismetMathLibrary.MakeVector` _origin_x _origin_y (- _origin_z (`self.Offset`))) _newtrack_0) false false)
        (set `self.Activated` false)))))

(fn `UserConstructionScript`)
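; BP_Water_Down is an actor that lowers itself, apparently as arena water, and presents a cinematic when an arena is cleared.
; OnArenaCleaned hides the player's HUD, disables input, blends to another camera and plays a level sequence, then restores all three after the sequence's duration.
; A separate WaterDown event, not called within this graph, uses a Timeline-driven Lerp to sink the actor a fixed distance from its current location.
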(event `self.ReceiveBeginPlay`
  (bind _asbp_first_person_character (cast `/Game/NIRVANA/Core/Characters/FirstPerson/BP_FirstPersonCharacter` (`GameplayStatics.GetPlayerCharacter` 0)))
  (set `self.PlayerRef` _asbp_first_person_character))

(event `/Game/NIRVANA/Core/Placeables/Management/BPI_ArenaManager.OnArenaCleaned`
  (params (ArenaManager :type "/Game/NIRVANA/Core/Placeables/Management/BP_ArenaManager Object Reference"))
  (bind _returnvalue (`GameplayStatics.GetPlayerController` 0))
  (bind _returnvalue_2 (`GameplayStatics.GetPlayerController` 0))
  (bind _playerref (`self.PlayerRef`))
  (bind _playerref_2 (`self.PlayerRef`))
  (bind _sequenceplayer (`LevelSequenceActor.SequencePlayer` (`self.SequencerToPlay`)))
  (`Widget.SetVisibility` (`/Game/NIRVANA/Core/Characters/FirstPerson/BP_FirstPersonCharacter.WB_Base_Ref` _playerref) "Hidden")
  (`self.DisableInput` _playerref _returnvalue_2)
  (set `self.CamToReturn` (`Controller.GetViewTarget` _returnvalue_2))
  (`PlayerController.SetViewTargetWithBlend` _returnvalue_2 (`self.CamToBlend`) 0.0 "VTBlend_Linear" 0.0 false)
  (`MovieSceneSequencePlayer.Play` _sequenceplayer)
  (`KismetSystemLibrary.Delay` (`TimeManagementBlueprintLibrary.Conv_QualifiedFrameTimeToSeconds` (`MovieSceneSequencePlayer.GetDuration` _sequenceplayer)))
  (`PlayerController.SetViewTargetWithBlend` _returnvalue (`self.CamToReturn`) 0.0 "VTBlend_Linear" 0.0 false)
  (`self.EnableInput` _playerref_2 _returnvalue)
  (`Widget.SetVisibility` (`/Game/NIRVANA/Core/Characters/FirstPerson/BP_FirstPersonCharacter.WB_Base_Ref` _playerref_2) "Visible"))

(event `WaterDown`
  (bind (_initlocation_x _initlocation_y _initlocation_z) (`KismetMathLibrary.BreakVector` (`self.InitLocation`)))
  (set `self.InitLocation` (`self.K2_GetActorLocation`))
  (bind (_direction _newtrack_0) (`Timeline|Timeline`)
    (:`Update`
      (`self.K2_SetActorTransform` (`ActorComponent.GetOwner` (`self.StaticMesh`)) (`KismetMathLibrary.MakeTransform` (`KismetMathLibrary.MakeVector` _initlocation_x _initlocation_y (`KismetMathLibrary.Lerp` _initlocation_z (+ _initlocation_z -2300.0) _newtrack_0))) false false))))

(fn `UserConstructionScript`)
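; Tutorial door trigger that shifts a referenced static mesh actor, apparently a door, when the player enters or an arena is cleared.
; An overlap by the cached first-person character fires Actionnate only while Activated is set; OnArenaCleaned calls it without that check.
; Actionnate snaps the mesh's relative location by optional X and Z offsets, without interpolation, then clears Activated.
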(event `self.ReceiveBeginPlay`
  (bind _asbp_first_person_character (cast `/Game/NIRVANA/Core/Characters/FirstPerson/BP_FirstPersonCharacter` (`GameplayStatics.GetPlayerCharacter` 0)))
  (set `self.PlayerRef` _asbp_first_person_character))

(event `self.Box.OnComponentBeginOverlap`
  (params (OverlappedComponent :type "PrimitiveComponent Object Reference") (OtherActor :type "Actor Object Reference") (OtherComp :type "PrimitiveComponent Object Reference") (OtherBodyIndex :type Integer) (bFromSweep :type Boolean) (SweepResult :type "HitResult Structure (by ref)"))
  (if (`self.Activated`)
    (if (== OtherActor (`self.PlayerRef`))
      (`self.Actionnate`))))

(event `/Game/NIRVANA/Core/Placeables/Management/BPI_ArenaManager.OnArenaCleaned`
  (params (ArenaManager :type "/Game/NIRVANA/Core/Placeables/Management/BP_ArenaManager Object Reference"))
  (`self.Actionnate`))

(event `Actionnate`
  (bind _meshtomove (`self.MeshToMove`))
  (bind _returnvalue (`SceneComponent.GetRelativeTransform` (`StaticMeshActor.StaticMeshComponent` _meshtomove)))
  (`SceneComponent.K2_SetRelativeLocation` (`StaticMeshActor.StaticMeshComponent` _meshtomove) (`KismetMathLibrary.MakeVector` (`KismetMathLibrary.SelectFloat` (+ (.x (.location _returnvalue)) (`self.OffsetX`)) (.x (.location _returnvalue)) (`self.MoveX`)) (.y (.location _returnvalue)) (`KismetMathLibrary.SelectFloat` (+ (.z (.location _returnvalue)) (`self.OffsetZ`)) (.z (.location _returnvalue)) (`self.MoveZ`))) false false)
  (set `self.Activated` false))

(fn `UserConstructionScript`)
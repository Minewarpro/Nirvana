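; Water actor Blueprint that sinks out of its starting position when the arena is cleaned.
; The construction script fits the static mesh to the Box component, placing it at the box's Z extent and scaling it in X and Y.
; OnArenaCleaned stores the actor's location, then a Timeline lerps it straight down by a fixed distance.
; BeginPlay only calls the parent and prints a debug string.
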(event `self.ReceiveBeginPlay`
  (`parent.ReceiveBeginPlay`)
  (`KismetSystemLibrary.PrintString` "Hello"))

(event `/Game/NIRVANA/Core/Placeables/Management/BPI_ArenaManager.OnArenaCleaned`
  (params (ArenaManager :type "/Game/NIRVANA/Core/Placeables/Management/BP_ArenaManager Object Reference"))
  (bind (_initlocation_x _initlocation_y _initlocation_z) (`KismetMathLibrary.BreakVector` (`self.InitLocation`)))
  (set `self.InitLocation` (`self.K2_GetActorLocation`))
  (bind (_direction _newtrack_0) (`Timeline|Timeline`)
    (:`Update`
      (`self.K2_SetActorTransform` (`KismetMathLibrary.MakeTransform` (`KismetMathLibrary.MakeVector` _initlocation_x _initlocation_y (`KismetMathLibrary.Lerp` _initlocation_z (+ _initlocation_z -2000.0) _newtrack_0)))))))

(fn `UserConstructionScript`
  (bind _staticmesh (`self.StaticMesh`))
  (bind (_boxextent_x _boxextent_y _boxextent_z) (`KismetMathLibrary.BreakVector` (`BoxComponent.BoxExtent` (`self.Box`))))
  (`parent.UserConstructionScript`)
  (`SceneComponent.K2_SetRelativeLocation` _staticmesh (`KismetMathLibrary.MakeVector` 0.0 0.0 _boxextent_z) false false)
  (`SceneComponent.SetRelativeScale3D` _staticmesh (`KismetMathLibrary.MakeVector` (/ _boxextent_x 48.0) (/ _boxextent_y 48.0) 1.0)))
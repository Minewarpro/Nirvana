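; Developer playtest actor that times how long the first-person player takes to reach its trigger.
; Counting starts on BeginPlay once the player character casts successfully.
; Tick adds a fixed step after each short Delay rather than using delta time, so the count depends on frame rate.
; When the player overlaps the trigger while Activated, it stops, deactivates and prints the elapsed count in minutes.
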(event `self.ReceiveBeginPlay`
  (bind _asbp_first_person_character (cast `/Game/NIRVANA/Core/Characters/FirstPerson/BP_FirstPersonCharacter` (`GameplayStatics.GetPlayerCharacter` 0)))
  (set `self.PlayerRef` _asbp_first_person_character)
  (set `self.IsRunning` true))

(event `self.trigger.OnComponentBeginOverlap`
  (params (OverlappedComponent :type "PrimitiveComponent Object Reference") (OtherActor :type "Actor Object Reference") (OtherComp :type "PrimitiveComponent Object Reference") (OtherBodyIndex :type Integer) (bFromSweep :type Boolean) (SweepResult :type "HitResult Structure (by ref)"))
  (if (and (== OtherActor (`self.PlayerRef`)) (`self.Activated`))
    (set `self.IsRunning` false)
    (set `self.Activated` false)
    (`KismetSystemLibrary.PrintString` (`KismetStringLibrary.Conv_DoubleToString` (/ (`self.Seconds`) 60.0)))))

(event `self.ReceiveTick`
  (params (DeltaSeconds :type "Float (single-precision)"))
  (if (`self.IsRunning`)
    (`KismetSystemLibrary.Delay` 0.01)
    (set `self.Seconds` (+ (`self.Seconds`) 0.01))))

(fn `UserConstructionScript`)
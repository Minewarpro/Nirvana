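; Developer timing tool that measures how long the first-person player takes to travel from a Start trigger to an End trigger.
; The player overlapping Start begins timing, and overlapping End prints the elapsed seconds and resets it.
; Tick accumulates time in fixed increments behind a short Delay, so the reading depends on frame rate rather than true elapsed time.
; The construction script positions End from exposed location variables.
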(event `self.ReceiveBeginPlay`
  (bind _asbp_first_person_character (cast `/Game/NIRVANA/Core/Characters/FirstPerson/BP_FirstPersonCharacter` (`GameplayStatics.GetPlayerCharacter` 0)))
  (set `self.PlayerRef` _asbp_first_person_character))

(event `self.Start.OnComponentBeginOverlap`
  (params (OverlappedComponent :type "PrimitiveComponent Object Reference") (OtherActor :type "Actor Object Reference") (OtherComp :type "PrimitiveComponent Object Reference") (OtherBodyIndex :type Integer) (bFromSweep :type Boolean) (SweepResult :type "HitResult Structure (by ref)"))
  (if (== OtherActor (`self.PlayerRef`))
    (if (not (`self.IsRunning`))
      (set `self.IsRunning` true))))

(event `self.End.OnComponentBeginOverlap`
  (params (OverlappedComponent :type "PrimitiveComponent Object Reference") (OtherActor :type "Actor Object Reference") (OtherComp :type "PrimitiveComponent Object Reference") (OtherBodyIndex :type Integer) (bFromSweep :type Boolean) (SweepResult :type "HitResult Structure (by ref)"))
  (if (== OtherActor (`self.PlayerRef`))
    (if (`self.IsRunning`)
      (set `self.IsRunning` false)
      (`KismetSystemLibrary.PrintString` (`KismetStringLibrary.Conv_DoubleToString` (`self.Seconds`)))
      (set `self.Seconds` 0.0))))

(event `self.ReceiveTick`
  (params (DeltaSeconds :type "Float (single-precision)"))
  (if (`self.IsRunning`)
    (`KismetSystemLibrary.Delay` 0.01)
    (set `self.Seconds` (+ (`self.Seconds`) 0.01))))

(fn `UserConstructionScript`
  (`SceneComponent.K2_SetRelativeLocation` (`self.End`) (`KismetMathLibrary.MakeVector` (`self.EndLocX`) (`self.EndLocY`) (`self.EndLocZ`)) false false))
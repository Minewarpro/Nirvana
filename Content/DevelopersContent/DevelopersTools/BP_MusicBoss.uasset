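; Boss music actor that switches 2D tracks through the phases of a boss encounter via custom events.
; Intro, DropEvent and Ending start the intro, fight and ending tracks, the latter two deactivating the previous one.
; KillMusic starts the chill track without stopping the ending track, as that deactivation node is disconnected.
; End deactivates the chill track and destroys the actor.
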(event `self.ReceiveBeginPlay`)

(event `Intro`
  (bind _returnvalue (`GameplayStatics.SpawnSound2D` "/Game/NIRVANA/Sound/IntroBoss.IntroBoss" 1.0 1.0 0.0 null))
  (set `self.IntroSound` _returnvalue))

(event `KillMusic`
  (bind _returnvalue (`GameplayStatics.SpawnSound2D` (`self.MusicChill`) 1.0 1.0 0.0 null))
  (set `self.Sound2dEnd` _returnvalue))

(event `End`
  (`ActorComponent.SetActive` (`self.Sound2dEnd`) false false)
  (`self.K2_DestroyActor`))

(event `DropEvent`
  (`ActorComponent.SetActive` (`self.IntroSound`) false false)
  (bind _returnvalue (`GameplayStatics.SpawnSound2D` (`self.Music`) 1.0 1.0 0.0 null))
  (set `self.Sound2DFight` _returnvalue))

(event `Ending`
  (`ActorComponent.SetActive` (`self.Sound2DFight`) false false)
  (bind _returnvalue (`GameplayStatics.SpawnSound2D` "/Game/NIRVANA/Sound/BossEnding.BossEnding" 1.0 1.0 0.0 null))
  (set `self.EndingSound` _returnvalue))

(fn `UserConstructionScript`)
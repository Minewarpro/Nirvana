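; BP_MovingWall is an actor that slides a referenced static mesh wall along its relative X axis.
; On BeginPlay it caches the first-person player character, stores the wall's starting relative location, then calls StartMove, which only runs if that cast succeeds.
; StartMove waits a configurable delay, then plays a timeline that lerps the wall from its origin to the X offset without sweeping.
; The cached player reference is not used afterward.
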(event `self.ReceiveBeginPlay`
  (bind _returnvalue_location (`KismetMathLibrary.BreakTransform` (`SceneComponent.GetRelativeTransform` (`StaticMeshActor.StaticMeshComponent` (`self.WallToMove`)))))
  (bind _asbp_first_person_character (cast `/Game/NIRVANA/Core/Characters/FirstPerson/BP_FirstPersonCharacter` (`GameplayStatics.GetPlayerCharacter` 0)))
  (set `self.PlayerRef` _asbp_first_person_character)
  (set `self.Origin` _returnvalue_location)
  (`self.StartMove`))

(event `StartMove`
  (bind (_origin_x _origin_y _origin_z) (`KismetMathLibrary.BreakVector` (`self.Origin`)))
  (`KismetSystemLibrary.Delay` (`self.Delay`))
  (bind (_direction _newtrack_0) (`Timeline|Timeline` :!via `PlayFromStart`)
    (:`Update`
      (`SceneComponent.K2_SetRelativeLocation` (`StaticMeshActor.StaticMeshComponent` (`self.WallToMove`)) (`KismetMathLibrary.VLerp` (`self.Origin`) (`KismetMathLibrary.MakeVector` (+ _origin_x (`self.Offset`)) _origin_y _origin_z) _newtrack_0) false false))))

(fn `UserConstructionScript`)
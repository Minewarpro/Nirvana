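; BP_MusicPlayerAutel is a music trigger actor that fades an audio component in and out as the first-person character crosses its boxes.
; Overlapping Box fades Audio in over three seconds, then destroys Box so the fade-in cannot repeat.
; Overlapping Box1 fades Audio out logarithmically and also destroys Box rather than itself, leaving Box1 active.
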(event `self.Box.OnComponentBeginOverlap`
  (params (OverlappedComponent :type "PrimitiveComponent Object Reference") (OtherActor :type "Actor Object Reference") (OtherComp :type "PrimitiveComponent Object Reference") (OtherBodyIndex :type Integer) (bFromSweep :type Boolean) (SweepResult :type "HitResult Structure (by ref)"))
  (cast `/Game/NIRVANA/Core/Characters/FirstPerson/BP_FirstPersonCharacter` OtherActor)
  (`AudioComponent.FadeIn` (`self.Audio`) 3.0 1.0 0.0 "Logarithmic")
  (`ActorComponent.K2_DestroyComponent` (`self.Box`)))

(event `self.Box1.OnComponentBeginOverlap`
  (params (OverlappedComponent :type "PrimitiveComponent Object Reference") (OtherActor :type "Actor Object Reference") (OtherComp :type "PrimitiveComponent Object Reference") (OtherBodyIndex :type Integer) (bFromSweep :type Boolean) (SweepResult :type "HitResult Structure (by ref)"))
  (cast `/Game/NIRVANA/Core/Characters/FirstPerson/BP_FirstPersonCharacter` OtherActor)
  (`AudioComponent.FadeOut` (`self.Audio`) 3.0 0.0 "Logarithmic")
  (`ActorComponent.K2_DestroyComponent` (`self.Box`)))

(fn `UserConstructionScript`)
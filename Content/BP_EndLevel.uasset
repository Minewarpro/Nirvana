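; BP_EndLevel is a trigger volume that ends the current level and loads the next one when the first-person player character enters its box.
; On overlap it disables player input and fades the camera and audio to black over two seconds.
; It then resets the saved spawn location in Game_Instance to an identity transform and opens the level set in LevelToLoad.
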(event `self.Box.OnComponentBeginOverlap`
  (params (OverlappedComponent :type "PrimitiveComponent Object Reference") (OtherActor :type "Actor Object Reference") (OtherComp :type "PrimitiveComponent Object Reference") (OtherBodyIndex :type Integer) (bFromSweep :type Boolean) (SweepResult :type "HitResult Structure (by ref)"))
  (bind _asbp_first_person_character (cast `/Game/NIRVANA/Core/Characters/FirstPerson/BP_FirstPersonCharacter` OtherActor))
  (`self.DisableInput` _asbp_first_person_character (`GameplayStatics.GetPlayerController` 0))
  (`PlayerCameraManager.StartCameraFade` (`GameplayStatics.GetPlayerCameraManager` 0) 0.0 1.0 2.0 (struct :`A` 1.0) true true)
  (`KismetSystemLibrary.Delay` 2.0)
  (set `/Game/NIRVANA/Core/GameModes/Game_Instance.Spawn Location` (`KismetMathLibrary.MakeTransform` (0.0 0.0 0.0)) (cast `/Game/NIRVANA/Core/GameModes/Game_Instance` (`GameplayStatics.GetGameInstance`) :!pure true))
  (`GameplayStatics.OpenLevelBySoftObjectPtr` (`self.LevelToLoad`)))

(fn `UserConstructionScript`)